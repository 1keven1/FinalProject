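; BP_Lantern_Box is a placeable box lantern prop from the Stylized Village assets, with a mesh and a point light.
; Its construction script applies the Color, Intensity and IsOn variables to the light and swaps the mesh between on and off lantern materials.
; Mesh shadow casting is disabled in both states, and the event graph holds only empty stub events, so nothing is scripted at runtime.
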(fn `UserConstructionScript`
  (bind _ison (`self.IsOn`))
  (bind _pointlight (`self.PointLight`))
  (bind _sm_lantern_box (`self.SM_Lantern_Box`))
  (`LightComponent.SetLightColor` _pointlight (`self.Color`) true)
  (`LightComponent.SetIntensity` _pointlight (`self.Intensity`))
  (`SceneComponent.SetVisibility` _pointlight _ison false)
  (if _ison
    (`PrimitiveComponent.SetCastShadow` _sm_lantern_box false)
    (`PrimitiveComponent.SetMaterial` _sm_lantern_box 0 "/Game/outsideArts/Stylized_Village/Assets/Props/Lanterns/Materials/MI_Lanterns_On.MI_Lanterns_On")
    (else
      (`PrimitiveComponent.SetCastShadow` _sm_lantern_box false)
      (`PrimitiveComponent.SetMaterial` _sm_lantern_box 0 "/Game/outsideArts/Stylized_Village/Assets/Props/Lanterns/Materials/MI_Lanterns_Off.MI_Lanterns_Off"))))