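; BP_Dials is a steampunk workshop dial prop that comes in eight selectable types.
; The Construction Script uses DialType to index arrays of hierarchical instanced mesh components, adding a body, hand and cover instance.
; Per-type Y offsets seat the hand and cover, DialHandRotation sets the hand's pitch, and some types share hand or cover meshes.
; The event graph is unused, so the dial has no runtime behavior.
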(fn `UserConstructionScript`
  (bind _hismc_dialcover05 (`self.HISMC_DialCover05`))
  (bind _hismc_dialhand07 (`self.HISMC_DialHand07`))
  (bind _dial_type (`self.Dial Type`))
  (bind _hismc_dialcover07 (`self.HISMC_DialCover07`))
  (bind _output (`|GetArrayItem` (`self.Mesh Type`) (`KismetMathLibrary.Conv_ByteToInt` _dial_type)))
  ;[1 1 1] Instanced Dial Parts
  (set `self.Mesh Type` (`|MakeArray` (`self.HISMC_Dial01`) (`self.HISMC_Dial02`) (`self.HISMC_Dial03`) (`self.HISMC_Dial04`) (`self.HISMC_Dial05`) (`self.HISMC_Dial06`) (`self.HISMC_Dial07`) (`self.HISMC_Dial08`) :!type "InstancedStaticMeshComponent Object Reference"))
  (`InstancedStaticMeshComponent.AddInstance` _output (`KismetMathLibrary.MakeTransform` (0.0 0.0 0.0)) false)
  (set `self.Mesh Type` (`|MakeArray` (`self.HISMC_DialHand01`) (`self.HISMC_DialHand02`) (`self.HISMC_DialHand03`) (`self.HISMC_DialHand04`) (`self.HISMC_DialHand05`) (`self.HISMC_DialHand06`) _hismc_dialhand07 _hismc_dialhand07 :!type "InstancedStaticMeshComponent Object Reference"))
  (switch `/Game/outsideArts/SteampunkWorkshop/Blueprints/Enumerators/Dials/EDialType` _dial_type
    (:`NewEnumerator0`
      (set `self.Dial Hand Position` 30.0))
    (:`NewEnumerator1`
      (set `self.Dial Hand Position` 16.0))
    (:`NewEnumerator4`
      (set `self.Dial Hand Position` 17.5))
    (:`NewEnumerator5`
      (set `self.Dial Hand Position` 17.0))
    (:`NewEnumerator6`
      (set `self.Dial Hand Position` 18.5 :!label _label))
    (:`NewEnumerator7`
      (goto _label))
    (:`NewEnumerator8`
      (set `self.Dial Hand Position` 18.0))
    (:`NewEnumerator9`
      (set `self.Dial Hand Position` 7.0)))
  (`InstancedStaticMeshComponent.AddInstance` _output (`KismetMathLibrary.MakeTransform` (`KismetMathLibrary.MakeVector` 0.0 (`self.Dial Hand Position`)) (`KismetMathLibrary.MakeRotator` 0.0 (`self.Dial Hand Rotation`))) false)
  (set `self.Mesh Type` (`|MakeArray` (`self.HISMC_DialCover01`) (`self.HISMC_DialCover02`) (`self.HISMC_DialCover03`) (`self.HISMC_DialCover04`) _hismc_dialcover05 _hismc_dialcover05 _hismc_dialcover07 _hismc_dialcover07 :!type "InstancedStaticMeshComponent Object Reference"))
  (switch `/Game/outsideArts/SteampunkWorkshop/Blueprints/Enumerators/Dials/EDialType` _dial_type
    (:`NewEnumerator0`
      (set `self.Dial Cover Position` 31.0))
    (:`NewEnumerator1`
      (set `self.Dial Cover Position` 18.0))
    (:`NewEnumerator4`
      (set `self.Dial Cover Position` 17.5))
    (:`NewEnumerator5`
      (set `self.Dial Cover Position` 18.5))
    (:`NewEnumerator6`
      (set `self.Dial Cover Position` 18.700001))
    (:`NewEnumerator7`
      (set `self.Dial Cover Position` 18.5))
    (:`NewEnumerator8`
      (set `self.Dial Cover Position` 18.9))
    (:`NewEnumerator9`
      (set `self.Dial Cover Position` 8.0)))
  (`InstancedStaticMeshComponent.AddInstance` _output (`KismetMathLibrary.MakeTransform` (`KismetMathLibrary.MakeVector` 0.0 (`self.Dial Cover Position`))) false))