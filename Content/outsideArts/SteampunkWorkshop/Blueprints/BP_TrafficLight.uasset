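; Procedural steampunk traffic light prop, assembled in the Construction Script from hierarchical instanced static meshes with no active runtime logic.
; Stacks a base, a selectable generator and a barrel, where all but the first barrel type add eight cannisters in a circle.
; Adds shrinking rings of a chosen style and count, one style twisting per step.
; Green, yellow and red lamps use dynamic materials, with on/off toggles setting intensity and saturation.
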(fn `UserConstructionScript`
  (bind _radius_test (`self.Radius Test`))
  (bind _hismc_tl_redlight (`self.HISMC_TL_RedLight`))
  (bind _hismc_tl_yellowlight (`self.HISMC_TL_YellowLight`))
  (bind _y_translate_test (`self.Y Translate Test`))
  (bind _hismc_tl_greenlight (`self.HISMC_TL_GreenLight`))
  (bind _light_intensity (`self.Light Intensity`))
  (bind _light_saturation (`self.Light Saturation`))
  (bind _returnvalue (`KismetMathLibrary.Conv_ByteToInt` (`self.Ring Type`)))
  (bind _returnvalue_2 (* _radius_test -1.0))
  (bind _output (`|GetArrayItem` (`self.Cannister Mesh Type`) (`KismetMathLibrary.Conv_ByteToInt` (`self.Barrel Type`))))
  (bind _returnvalue_3 (`KismetMathLibrary.Sqrt` (/ (`KismetMathLibrary.Square` _radius_test) 2.0)))
  (bind _returnvalue_4 (* _returnvalue_3 -1.0))
  (`|ExecutionSequence`
    (:`then_0`
      ;[1 1 1] Base
      (`InstancedStaticMeshComponent.AddInstance` (`self.HISMC_TL_Base`) (`KismetMathLibrary.MakeTransform` (0.0 0.0 0.0)) false)
      ;[1 1 1] Traffic Light Generator
      (set `self.Generator Mesh Type` (`|MakeArray` (`self.HISMC_TL_Generator01`) (`self.HISMC_TL_Generator02`) (`self.HISMC_TL_Generator03`) (`self.HISMC_TL_Generator04`) (`self.HISMC_TL_Generator05`) (`self.HISMC_TL_Generator06`)))
      (`InstancedStaticMeshComponent.AddInstance` (`|GetArrayItem` (`self.Generator Mesh Type`) (`KismetMathLibrary.Conv_ByteToInt` (`self.Generator Type`))) (`KismetMathLibrary.MakeTransform` (0.0 30.0 0.0)) false))
    (:`then_1`
      ;[1 1 1] Barrel
      (switch `/Game/outsideArts/SteampunkWorkshop/Blueprints/Enumerators/TrafficLight/ETLBarrelType` (`self.Barrel Type`)
        (:`NewEnumerator0`
          (`InstancedStaticMeshComponent.AddInstance` (`self.HISMC_TL_Barrel01`) (`KismetMathLibrary.MakeTransform` (0.0 30.0 132.0)) false))
        (:`NewEnumerator1`
          (`InstancedStaticMeshComponent.AddInstance` (`self.HISMC_TL_BarrelTemplate`) (`KismetMathLibrary.MakeTransform` (0.0 30.0 132.0)) false :!label _label)
          (set `self.Cannister Mesh Type` (`|MakeArray` null (`self.HISMC_TL_Cannister01`) (`self.HISMC_TL_Cannister02`) (`self.HISMC_TL_Cannister03`) (`self.HISMC_TL_Cannister04`) :!type "InstancedStaticMeshComponent Object Reference"))
          (`InstancedStaticMeshComponent.AddInstance` _output (`KismetMathLibrary.MakeTransform` (`KismetMathLibrary.MakeVector` 0.0 (+ _radius_test _y_translate_test) 166.0)) false)
          (`InstancedStaticMeshComponent.AddInstance` _output (`KismetMathLibrary.MakeTransform` (`KismetMathLibrary.MakeVector` 0.0 (+ _returnvalue_2 _y_translate_test) 166.0)) false)
          (`InstancedStaticMeshComponent.AddInstance` _output (`KismetMathLibrary.MakeTransform` (`KismetMathLibrary.MakeVector` _radius_test _y_translate_test 166.0)) false)
          (`InstancedStaticMeshComponent.AddInstance` _output (`KismetMathLibrary.MakeTransform` (`KismetMathLibrary.MakeVector` _returnvalue_2 _y_translate_test 166.0)) false)
          (`InstancedStaticMeshComponent.AddInstance` _output (`KismetMathLibrary.MakeTransform` (`KismetMathLibrary.MakeVector` _returnvalue_3 (+ _returnvalue_3 _y_translate_test) 166.0)) false)
          (`InstancedStaticMeshComponent.AddInstance` _output (`KismetMathLibrary.MakeTransform` (`KismetMathLibrary.MakeVector` _returnvalue_4 (+ _returnvalue_4 _y_translate_test) 166.0)) false)
          (`InstancedStaticMeshComponent.AddInstance` _output (`KismetMathLibrary.MakeTransform` (`KismetMathLibrary.MakeVector` _returnvalue_3 (+ _returnvalue_4 _y_translate_test) 166.0)) false)
          (`InstancedStaticMeshComponent.AddInstance` _output (`KismetMathLibrary.MakeTransform` (`KismetMathLibrary.MakeVector` _returnvalue_4 (+ _y_translate_test _returnvalue_3) 166.0)) false))
        (:`NewEnumerator2`
          (goto _label))
        (:`NewEnumerator5`
          (goto _label))
        (:`NewEnumerator6`
          (goto _label))))
    (:`then_2`
      ;[1 1 1] Light System
      (`InstancedStaticMeshComponent.AddInstance` _hismc_tl_greenlight (`KismetMathLibrary.MakeTransform` (0.0 18.0 400.0) (struct :`Yaw` 90.0)) false)
      (`InstancedStaticMeshComponent.AddInstance` _hismc_tl_greenlight (`KismetMathLibrary.MakeTransform` (0.0 18.0 410.0)) false)
      (`InstancedStaticMeshComponent.AddInstance` _hismc_tl_greenlight (`KismetMathLibrary.MakeTransform` (0.0 18.0 420.0) (struct :`Yaw` -90.0)) false)
      (bind _returnvalue_5 (`PrimitiveComponent.CreateDynamicMaterialInstance` _hismc_tl_greenlight 0 "/Game/outsideArts/SteampunkWorkshop/Materials/TrafficLights/MI_TL_GreenLight.MI_TL_GreenLight" "None"))
      (if (`self.GreenLightON`)
        (`MaterialInstanceDynamic.SetScalarParameterValue` _returnvalue_5 _light_intensity 0.25)
        (`MaterialInstanceDynamic.SetScalarParameterValue` _returnvalue_5 _light_saturation 0.2)
        (else
          (`MaterialInstanceDynamic.SetScalarParameterValue` _returnvalue_5 _light_intensity 0.01)
          (`MaterialInstanceDynamic.SetScalarParameterValue` _returnvalue_5 _light_saturation 0.7))))
    (:`then_3`
      (`InstancedStaticMeshComponent.AddInstance` _hismc_tl_yellowlight (`KismetMathLibrary.MakeTransform` (0.0 18.0 430.0) (struct :`Yaw` 90.0)) false)
      (`InstancedStaticMeshComponent.AddInstance` _hismc_tl_yellowlight (`KismetMathLibrary.MakeTransform` (0.0 18.0 440.0)) false)
      (`InstancedStaticMeshComponent.AddInstance` _hismc_tl_yellowlight (`KismetMathLibrary.MakeTransform` (0.0 18.0 450.0) (struct :`Yaw` -90.0)) false)
      (bind _returnvalue_6 (`PrimitiveComponent.CreateDynamicMaterialInstance` _hismc_tl_yellowlight 0 "/Game/outsideArts/SteampunkWorkshop/Materials/TrafficLights/MI_TL_YellowLight.MI_TL_YellowLight" "None"))
      (if (`self.YellowLightON`)
        (`MaterialInstanceDynamic.SetScalarParameterValue` _returnvalue_6 _light_intensity 0.25)
        (`MaterialInstanceDynamic.SetScalarParameterValue` _returnvalue_6 _light_saturation 0.0)
        (else
          (`MaterialInstanceDynamic.SetScalarParameterValue` _returnvalue_6 _light_intensity 0.01)
          (`MaterialInstanceDynamic.SetScalarParameterValue` _returnvalue_6 _light_saturation 0.5))))
    (:`then_4`
      ;[1 1 1] Rings
      (for _index (range (+ (`KismetMathLibrary.Clamp` (`self.AdditionalRing(0-7)`) 0 7) 1))
        (set `self.Ring Mesh Type` (`|MakeArray` (`self.HISMC_TL_Ring01`) (`self.HISMC_TL_Ring02`) (`self.HISMC_TL_Ring03`) (`self.HISMC_TL_Ring04`) :!type "InstancedStaticMeshComponent Object Reference"))
        (bind _returnvalue_7 (`KismetMathLibrary.Conv_IntToDouble` _index))
        (bind _returnvalue_8 (* _returnvalue_7 0.0))
        (set `self.Ring Rotation` (`|MakeArray` _returnvalue_8 _returnvalue_8 _returnvalue_8 (* _returnvalue_7 45.0)))
        (`InstancedStaticMeshComponent.AddInstance` (`|GetArrayItem` (`self.Ring Mesh Type`) _returnvalue) (`KismetMathLibrary.MakeTransform` (`KismetMathLibrary.MakeVector` 0.0 18.9 (+ (* _returnvalue_7 17.0) 250.0)) (`KismetMathLibrary.MakeRotator` 0.0 0.0 (`|GetArrayItem` (`self.Ring Rotation`) _returnvalue)) (`KismetMathLibrary.Conv_DoubleToVector` (+ (* _returnvalue_7 -0.04) 1.0))) false)))
    (:`then_5`
      (`InstancedStaticMeshComponent.AddInstance` _hismc_tl_redlight (`KismetMathLibrary.MakeTransform` (0.0 18.0 460.0) (struct :`Yaw` 90.0)) false)
      (`InstancedStaticMeshComponent.AddInstance` _hismc_tl_redlight (`KismetMathLibrary.MakeTransform` (0.0 18.0 470.0)) false)
      (`InstancedStaticMeshComponent.AddInstance` _hismc_tl_redlight (`KismetMathLibrary.MakeTransform` (0.0 18.0 480.0) (struct :`Yaw` -90.0)) false)
      (bind _returnvalue_9 (`PrimitiveComponent.CreateDynamicMaterialInstance` _hismc_tl_redlight 0 "/Game/outsideArts/SteampunkWorkshop/Materials/TrafficLights/MI_TL_RedLight.MI_TL_RedLight" "None"))
      (if (`self.RedLightON`)
        (`MaterialInstanceDynamic.SetScalarParameterValue` _returnvalue_9 _light_intensity 0.7)
        (`MaterialInstanceDynamic.SetScalarParameterValue` _returnvalue_9 _light_saturation 0.2)
        (else
          (`MaterialInstanceDynamic.SetScalarParameterValue` _returnvalue_9 _light_intensity 0.01)
          (`MaterialInstanceDynamic.SetScalarParameterValue` _returnvalue_9 _light_saturation 0.7))))))