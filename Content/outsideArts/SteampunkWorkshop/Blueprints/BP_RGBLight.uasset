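; BP_RGBLight is a workshop light fixture whose color is selected by the LightColor variable.
; The Construction Script adds one instance each to the light and grill HISM components, then creates dynamic materials for the filament and glass.
; LightColor indexes separate hue arrays to tint both materials and an added point light, keeping them in step.
; The event graph holds no runtime logic.
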(fn `UserConstructionScript`
  (bind _hismc_rgblight (`self.HISMC_RGBLight`))
  (bind _filament_hue (`self.Filament Hue`))
  (bind _glass_hue (`self.Glass Hue`))
  (bind _light_hue (`self.Light Hue`))
  (bind _returnvalue (`KismetMathLibrary.Conv_ByteToInt` (`self.Light Color`)))
  ;[1 1 1] RGBLight
  (`InstancedStaticMeshComponent.AddInstance` _hismc_rgblight (`KismetMathLibrary.MakeTransform` (0.0 0.0 0.0)) false)
  (`InstancedStaticMeshComponent.AddInstance` (`self.HISMC_RGBLightGrill`) (`KismetMathLibrary.MakeTransform` (0.0 0.0 0.0)) false)
  ;[1 1 1] Light Color
  (bind _returnvalue_2 (`PrimitiveComponent.CreateDynamicMaterialInstance` _hismc_rgblight 0 "/Game/outsideArts/SteampunkWorkshop/Materials/Misc/MI_RGBLight01.MI_RGBLight01" "None"))
  (bind _returnvalue_3 (`PrimitiveComponent.CreateDynamicMaterialInstance` _hismc_rgblight 1 "/Game/outsideArts/SteampunkWorkshop/Materials/Misc/MI_RGBLight01Glass.MI_RGBLight01Glass" "None"))
  (set `self.Filament Hue` _filament_hue)
  (`MaterialInstanceDynamic.SetVectorParameterValue` _returnvalue_2 "Filament Hue" (`|GetArrayItem` _filament_hue _returnvalue))
  (set `self.Glass Hue` _glass_hue)
  (`MaterialInstanceDynamic.SetVectorParameterValue` _returnvalue_3 "Glass Hue" (`|GetArrayItem` _glass_hue _returnvalue))
  (bind _returnvalue_4 (`AddComponent|NODE_AddPointLightComponent-1` :`RelativeTransform` (`KismetMathLibrary.MakeTransform` (0.0 12.5 0.0))))
  (set `self.Light Hue` _light_hue)
  (`LightComponent.SetLightColor` _returnvalue_4 (`|GetArrayItem` _light_hue _returnvalue) true))