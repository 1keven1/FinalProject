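; Steampunk hydraulic forge press prop, assembled procedurally as a static set piece with no runtime logic.
; The construction script places each part (base, feeds, pillars, mount, top, cylinder, exhausts, pipes and mount pins) as hierarchical instanced static mesh instances at hardcoded transforms.
; Two upper pillar pieces are mirrored with negative X scale as separately added static mesh components rather than instances.
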(fn `UserConstructionScript`
  (bind _hismc_forgepressfeed (`self.HISMC_ForgePressFeed`))
  (bind _hismc_forgepresspillar03 (`self.HISMC_ForgePressPillar03`))
  (bind _hismc_forgepresspiller01 (`self.HISMC_ForgePressPiller01`))
  (bind _hismc_forgepresspin (`self.HISMC_ForgePressPin`))
  (bind _hismc_forgepresspiller02 (`self.HISMC_ForgePressPiller02`))
  (bind _hismc_forgepressexhaust (`self.HISMC_ForgePressExhaust`))
  (bind _hismc_forgepresspipe (`self.HISMC_ForgePressPipe`))
  (`|ExecutionSequence`
    (:`then_0`
      ;[1 1 1] ForgePress Base
      (`InstancedStaticMeshComponent.AddInstance` (`self.HISMC_ForgePressBase`) (`KismetMathLibrary.MakeTransform` (0.0 0.0 0.0)) false)
      ;[1 1 1] ForgePress Feed
      (`InstancedStaticMeshComponent.AddInstance` _hismc_forgepressfeed (`KismetMathLibrary.MakeTransform` (0.0 0.0 30.0)) false)
      (`InstancedStaticMeshComponent.AddInstance` _hismc_forgepressfeed (`KismetMathLibrary.MakeTransform` (0.0 0.0 330.0) (struct :`Pitch` -180.0)) false)
      ;[1 1 1] ForgePress Pillar01
      (`InstancedStaticMeshComponent.AddInstance` _hismc_forgepresspiller01 (`KismetMathLibrary.MakeTransform` (400.0 300.0 30.0)) false)
      (`InstancedStaticMeshComponent.AddInstance` _hismc_forgepresspiller01 (`KismetMathLibrary.MakeTransform` (400.0 -300.0 30.0)) false)
      (`InstancedStaticMeshComponent.AddInstance` _hismc_forgepresspiller01 (`KismetMathLibrary.MakeTransform` (-400.0 300.0 30.0)) false)
      (`InstancedStaticMeshComponent.AddInstance` _hismc_forgepresspiller01 (`KismetMathLibrary.MakeTransform` (-400.0 -300.0 30.0)) false)
      ;[1 1 1] ForgePress Pillar01
      (`InstancedStaticMeshComponent.AddInstance` _hismc_forgepresspiller02 (`KismetMathLibrary.MakeTransform` (400.0 300.0 30.0)) false)
      (`InstancedStaticMeshComponent.AddInstance` _hismc_forgepresspiller02 (`KismetMathLibrary.MakeTransform` (400.0 -300.0 30.0)) false)
      (`InstancedStaticMeshComponent.AddInstance` _hismc_forgepresspiller02 (`KismetMathLibrary.MakeTransform` (-400.0 300.0 30.0)) false)
      (`InstancedStaticMeshComponent.AddInstance` _hismc_forgepresspiller02 (`KismetMathLibrary.MakeTransform` (-400.0 -300.0 30.0)) false)
      ;[1 1 1] ForgePress FeedTop
      (`InstancedStaticMeshComponent.AddInstance` (`self.HISMC_ForgePressFeedTop`) (`KismetMathLibrary.MakeTransform` (0.0 0.0 325.0) (struct) (1.0 1.0 0.5)) false)
      ;[1 1 1] ForgePress Mount
      (`InstancedStaticMeshComponent.AddInstance` (`self.HISMC_ForgePressMount`) (`KismetMathLibrary.MakeTransform` (0.0 0.0 475.0)) false)
      ;[1 1 1] ForgePress Top
      (`InstancedStaticMeshComponent.AddInstance` (`self.HISMC_ForgePressTop`) (`KismetMathLibrary.MakeTransform` (0.0 0.0 900.0)) false)
      ;[1 1 1] ForgePress Exhuast
      (`InstancedStaticMeshComponent.AddInstance` _hismc_forgepressexhaust (`KismetMathLibrary.MakeTransform` (-280.0 0.0 1125.0) (struct :`Yaw` 90.0)) false)
      (`InstancedStaticMeshComponent.AddInstance` _hismc_forgepressexhaust (`KismetMathLibrary.MakeTransform` (280.0 0.0 1125.0) (struct :`Yaw` -90.0)) false)
      ;[1 1 1] ForgePress Cylinder
      (`InstancedStaticMeshComponent.AddInstance` (`self.HISMC_ForgePressCylinder`) (`KismetMathLibrary.MakeTransform` (0.0 0.0 720.0)) false))
    (:`then_1`
      ;[1 1 1] ForgePress Pipe
      (`InstancedStaticMeshComponent.AddInstance` _hismc_forgepresspipe (`KismetMathLibrary.MakeTransform` (-83.0 160.0 1195.0)) false)
      (`InstancedStaticMeshComponent.AddInstance` _hismc_forgepresspipe (`KismetMathLibrary.MakeTransform` (83.0 160.0 1195.0)) false)
      (`InstancedStaticMeshComponent.AddInstance` _hismc_forgepresspipe (`KismetMathLibrary.MakeTransform` (-83.0 -160.0 1195.0) (struct :`Yaw` 180.0)) false)
      (`InstancedStaticMeshComponent.AddInstance` _hismc_forgepresspipe (`KismetMathLibrary.MakeTransform` (83.0 -160.0 1195.0) (struct :`Yaw` 180.0)) false))
    (:`then_2`
      ;[1 1 1] ForgePress Top
      (`InstancedStaticMeshComponent.AddInstance` _hismc_forgepresspillar03 (`KismetMathLibrary.MakeTransform` (0.0 0.0 910.0)) false)
      (`AddComponent|NODE_AddStaticMeshComponent-0` :`RelativeTransform` (`KismetMathLibrary.MakeTransform` (0.0 0.0 910.0) (struct) (-1.0 1.0 1.0)))
      (`InstancedStaticMeshComponent.AddInstance` _hismc_forgepresspillar03 (`KismetMathLibrary.MakeTransform` (0.0 0.0 910.0) (struct :`Yaw` 180.0)) false)
      (`AddComponent|NODE_AddStaticMeshComponent-1` :`RelativeTransform` (`KismetMathLibrary.MakeTransform` (0.0 0.0 910.0) (struct :`Yaw` 180.0) (-1.0 1.0 1.0))))
    (:`then_3`
      ;[1 1 1] Instanced ForgeMount Pins
      (`InstancedStaticMeshComponent.AddInstance` _hismc_forgepresspin (`KismetMathLibrary.MakeTransform` (-55.0 231.0 658.0) (struct) (1.5 1.5 1.5)) false)
      (`InstancedStaticMeshComponent.AddInstance` _hismc_forgepresspin (`KismetMathLibrary.MakeTransform` (-55.0 231.0 600.0) (struct) (1.5 1.5 1.5)) false)
      (`InstancedStaticMeshComponent.AddInstance` _hismc_forgepresspin (`KismetMathLibrary.MakeTransform` (-55.0 231.0 543.0) (struct) (1.5 1.5 1.5)) false)
      (`InstancedStaticMeshComponent.AddInstance` _hismc_forgepresspin (`KismetMathLibrary.MakeTransform` (55.0 231.0 658.0) (struct) (1.5 1.5 1.5)) false)
      (`InstancedStaticMeshComponent.AddInstance` _hismc_forgepresspin (`KismetMathLibrary.MakeTransform` (55.0 231.0 600.0) (struct) (1.5 1.5 1.5)) false)
      (`InstancedStaticMeshComponent.AddInstance` _hismc_forgepresspin (`KismetMathLibrary.MakeTransform` (55.0 231.0 543.0) (struct) (1.5 1.5 1.5)) false)
      (`InstancedStaticMeshComponent.AddInstance` _hismc_forgepresspin (`KismetMathLibrary.MakeTransform` (-60.0 -231.0 658.0) (struct :`Roll` 180.0) (1.5 1.5 1.5)) false)
      (`InstancedStaticMeshComponent.AddInstance` _hismc_forgepresspin (`KismetMathLibrary.MakeTransform` (-60.0 -231.0 600.0) (struct :`Roll` 180.0) (1.5 1.5 1.5)) false)
      (`InstancedStaticMeshComponent.AddInstance` _hismc_forgepresspin (`KismetMathLibrary.MakeTransform` (-60.0 -231.0 543.0) (struct :`Roll` 180.0) (1.5 1.5 1.5)) false)
      (`InstancedStaticMeshComponent.AddInstance` _hismc_forgepresspin (`KismetMathLibrary.MakeTransform` (60.0 -231.0 658.0) (struct :`Roll` 180.0) (1.5 1.5 1.5)) false)
      (`InstancedStaticMeshComponent.AddInstance` _hismc_forgepresspin (`KismetMathLibrary.MakeTransform` (60.0 -231.0 600.0) (struct :`Roll` 180.0) (1.5 1.5 1.5)) false)
      (`InstancedStaticMeshComponent.AddInstance` _hismc_forgepresspin (`KismetMathLibrary.MakeTransform` (60.0 -231.0 543.0) (struct :`Roll` 180.0) (1.5 1.5 1.5)) false)
      (`InstancedStaticMeshComponent.AddInstance` _hismc_forgepresspin (`KismetMathLibrary.MakeTransform` (-284.0 276.0 543.0) (struct :`Yaw` -25.0) (1.5 2.0 1.5)) false)
      (`InstancedStaticMeshComponent.AddInstance` _hismc_forgepresspin (`KismetMathLibrary.MakeTransform` (-284.0 276.0 600.0) (struct :`Yaw` -25.0) (1.5 2.0 1.5)) false)
      (`InstancedStaticMeshComponent.AddInstance` _hismc_forgepresspin (`KismetMathLibrary.MakeTransform` (-284.0 276.0 658.0) (struct :`Yaw` -25.0) (1.5 2.0 1.5)) false)
      (`InstancedStaticMeshComponent.AddInstance` _hismc_forgepresspin (`KismetMathLibrary.MakeTransform` (284.0 276.0 543.0) (struct :`Yaw` 25.0) (1.5 2.0 1.5)) false)
      (`InstancedStaticMeshComponent.AddInstance` _hismc_forgepresspin (`KismetMathLibrary.MakeTransform` (284.0 276.0 600.0) (struct :`Yaw` 25.0) (1.5 2.0 1.5)) false)
      (`InstancedStaticMeshComponent.AddInstance` _hismc_forgepresspin (`KismetMathLibrary.MakeTransform` (284.0 276.0 658.0) (struct :`Yaw` 25.0) (1.5 2.0 1.5)) false)
      (`InstancedStaticMeshComponent.AddInstance` _hismc_forgepresspin (`KismetMathLibrary.MakeTransform` (-284.0 -276.0 543.0) (struct :`Yaw` 25.0 :`Roll` 180.0) (1.5 2.0 1.5)) false)
      (`InstancedStaticMeshComponent.AddInstance` _hismc_forgepresspin (`KismetMathLibrary.MakeTransform` (-284.0 -276.0 600.0) (struct :`Yaw` 25.0 :`Roll` 180.0) (1.5 2.0 1.5)) false)
      (`InstancedStaticMeshComponent.AddInstance` _hismc_forgepresspin (`KismetMathLibrary.MakeTransform` (-284.0 -276.0 658.0) (struct :`Yaw` 25.0 :`Roll` 180.0) (1.5 2.0 1.5)) false)
      (`InstancedStaticMeshComponent.AddInstance` _hismc_forgepresspin (`KismetMathLibrary.MakeTransform` (284.0 -276.0 543.0) (struct :`Yaw` -25.0 :`Roll` 180.0) (1.5 2.0 1.5)) false)
      (`InstancedStaticMeshComponent.AddInstance` _hismc_forgepresspin (`KismetMathLibrary.MakeTransform` (284.0 -276.0 600.0) (struct :`Yaw` -25.0 :`Roll` 180.0) (1.5 2.0 1.5)) false)
      (`InstancedStaticMeshComponent.AddInstance` _hismc_forgepresspin (`KismetMathLibrary.MakeTransform` (284.0 -276.0 658.0) (struct :`Yaw` -25.0 :`Roll` 180.0) (1.5 2.0 1.5)) false)
      (`InstancedStaticMeshComponent.AddInstance` _hismc_forgepresspin (`KismetMathLibrary.MakeTransform` (-338.0 217.0 658.0) (struct :`Yaw` 140.0) (1.5 2.0 1.5)) false)
      (`InstancedStaticMeshComponent.AddInstance` _hismc_forgepresspin (`KismetMathLibrary.MakeTransform` (-338.0 217.0 600.0) (struct :`Yaw` 140.0) (1.5 2.0 1.5)) false)
      (`InstancedStaticMeshComponent.AddInstance` _hismc_forgepresspin (`KismetMathLibrary.MakeTransform` (-338.0 217.0 543.0) (struct :`Yaw` 140.0) (1.5 2.0 1.5)) false)
      (`InstancedStaticMeshComponent.AddInstance` _hismc_forgepresspin (`KismetMathLibrary.MakeTransform` (-338.0 -217.0 543.0) (struct :`Yaw` 40.0) (1.5 2.0 1.5)) false)
      (`InstancedStaticMeshComponent.AddInstance` _hismc_forgepresspin (`KismetMathLibrary.MakeTransform` (-338.0 -217.0 600.0) (struct :`Yaw` 40.0) (1.5 2.0 1.5)) false)
      (`InstancedStaticMeshComponent.AddInstance` _hismc_forgepresspin (`KismetMathLibrary.MakeTransform` (-338.0 -217.0 658.0) (struct :`Yaw` 40.0) (1.5 2.0 1.5)) false)
      (`InstancedStaticMeshComponent.AddInstance` _hismc_forgepresspin (`KismetMathLibrary.MakeTransform` (-270.0 46.0 543.0) (struct :`Yaw` 90.0) (1.5 2.0 1.5)) false)
      (`InstancedStaticMeshComponent.AddInstance` _hismc_forgepresspin (`KismetMathLibrary.MakeTransform` (-270.0 46.0 600.0) (struct :`Yaw` 90.0) (1.5 2.0 1.5)) false)
      (`InstancedStaticMeshComponent.AddInstance` _hismc_forgepresspin (`KismetMathLibrary.MakeTransform` (-270.0 46.0 658.0) (struct :`Yaw` 90.0) (1.5 2.0 1.5)) false)
      (`InstancedStaticMeshComponent.AddInstance` _hismc_forgepresspin (`KismetMathLibrary.MakeTransform` (-270.0 -47.0 543.0) (struct :`Yaw` 90.0) (1.5 2.0 1.5)) false)
      (`InstancedStaticMeshComponent.AddInstance` _hismc_forgepresspin (`KismetMathLibrary.MakeTransform` (-270.0 -49.0 600.0) (struct :`Yaw` 90.0) (1.5 2.0 1.5)) false)
      (`InstancedStaticMeshComponent.AddInstance` _hismc_forgepresspin (`KismetMathLibrary.MakeTransform` (-270.0 -47.0 658.0) (struct :`Yaw` 90.0) (1.5 2.0 1.5)) false)
      (`InstancedStaticMeshComponent.AddInstance` _hismc_forgepresspin (`KismetMathLibrary.MakeTransform` (338.0 217.0 658.0) (struct :`Yaw` -140.0) (1.5 2.0 1.5)) false)
      (`InstancedStaticMeshComponent.AddInstance` _hismc_forgepresspin (`KismetMathLibrary.MakeTransform` (338.0 217.0 600.0) (struct :`Yaw` -140.0) (1.5 2.0 1.5)) false)
      (`InstancedStaticMeshComponent.AddInstance` _hismc_forgepresspin (`KismetMathLibrary.MakeTransform` (338.0 217.0 543.0) (struct :`Yaw` -140.0) (1.5 2.0 1.5)) false)
      (`InstancedStaticMeshComponent.AddInstance` _hismc_forgepresspin (`KismetMathLibrary.MakeTransform` (338.0 -217.0 543.0) (struct :`Yaw` -40.0) (1.5 2.0 1.5)) false)
      (`InstancedStaticMeshComponent.AddInstance` _hismc_forgepresspin (`KismetMathLibrary.MakeTransform` (338.0 -217.0 600.0) (struct :`Yaw` -40.0) (1.5 2.0 1.5)) false)
      (`InstancedStaticMeshComponent.AddInstance` _hismc_forgepresspin (`KismetMathLibrary.MakeTransform` (338.0 -217.0 658.0) (struct :`Yaw` -40.0) (1.5 2.0 1.5)) false)
      (`InstancedStaticMeshComponent.AddInstance` _hismc_forgepresspin (`KismetMathLibrary.MakeTransform` (270.0 46.0 543.0) (struct :`Yaw` 90.0 :`Roll` 180.0) (1.5 2.0 1.5)) false)
      (`InstancedStaticMeshComponent.AddInstance` _hismc_forgepresspin (`KismetMathLibrary.MakeTransform` (270.0 46.0 600.0) (struct :`Yaw` 90.0 :`Roll` 180.0) (1.5 2.0 1.5)) false)
      (`InstancedStaticMeshComponent.AddInstance` _hismc_forgepresspin (`KismetMathLibrary.MakeTransform` (270.0 46.0 658.0) (struct :`Yaw` 90.0 :`Roll` 180.0) (1.5 2.0 1.5)) false)
      (`InstancedStaticMeshComponent.AddInstance` _hismc_forgepresspin (`KismetMathLibrary.MakeTransform` (270.0 -43.0 543.0) (struct :`Yaw` 90.0 :`Roll` 180.0) (1.5 2.0 1.5)) false)
      (`InstancedStaticMeshComponent.AddInstance` _hismc_forgepresspin (`KismetMathLibrary.MakeTransform` (270.0 -43.0 600.0) (struct :`Yaw` 90.0 :`Roll` 180.0) (1.5 2.0 1.5)) false)
      (`InstancedStaticMeshComponent.AddInstance` _hismc_forgepresspin (`KismetMathLibrary.MakeTransform` (270.0 -43.0 658.0) (struct :`Yaw` 90.0 :`Roll` 180.0) (1.5 2.0 1.5)) false))))