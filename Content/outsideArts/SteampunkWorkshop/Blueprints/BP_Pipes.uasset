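; BP_Pipes is a configurable steampunk workshop prop that builds one pipe, machine or valve piece in the Construction Script.
; PipeType picks an array of hierarchical instanced mesh components, and PipeSectionType indexes it to add a single instance.
; Nested switches then choose a material pair, indexed by PipeMaterial and applied to slot 0.
; Machines and valves are shared by both pipe types; Valves 05 to 07 get no material override.
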(fn `UserConstructionScript`
  (bind _hismc_pipe01_machine03 (`self.HISMC_Pipe01_Machine03`))
  (bind _pipe_type (`self.Pipe Type`))
  (bind _pipe_section_type (`self.Pipe Section Type`))
  (bind _hismc_valve05 (`self.HISMC_Valve05`))
  (bind _hismc_valve06 (`self.HISMC_Valve06`))
  (bind _hismc_valve07 (`self.HISMC_Valve07`))
  (bind _hismc_pipe03_valve01 (`self.HISMC_Pipe03_Valve01`))
  (bind _hismc_pipe03_valve02 (`self.HISMC_Pipe03_Valve02`))
  (bind _hismc_pipe05_valve03 (`self.HISMC_Pipe05_Valve03`))
  (bind _hismc_pipe_machine02 (`self.HISMC_Pipe_Machine02`))
  (bind _hismc_pipe_machine01 (`self.HISMC_Pipe_Machine01`))
  (bind _hismc_pipe06_valve04 (`self.HISMC_Pipe06_Valve04`))
  (bind _hismc_pipe06_valve04_01 (`self.HISMC_Pipe06_Valve04_01`))
  (bind _output (`|GetArrayItem` (`self.Pipe Mesh Type`) (`KismetMathLibrary.Conv_ByteToInt` _pipe_section_type)))
  (bind _output_2 (`|GetArrayItem` (`self.Pipe Material Type`) (`KismetMathLibrary.Conv_ByteToInt` (`self.Pipe Material`))))
  ;[1 1 1] Pipe Type
  (switch `/Game/outsideArts/SteampunkWorkshop/Blueprints/Enumerators/Pipes/EPipeType` _pipe_type
    (:`NewEnumerator0`
      ;[1 1 1] Pipe Section Type
      (set `self.Pipe Mesh Type` (`|MakeArray` (`self.HISMC_Pipe01_01`) (`self.HISMC_Pipe01_02`) (`self.HISMC_Pipe01_03`) (`self.HISMC_Pipe01_04`) (`self.HISMC_Pipe01_05`) (`self.HISMC_Pipe01_06`) _hismc_pipe_machine01 _hismc_pipe_machine02 _hismc_pipe01_machine03 _hismc_pipe03_valve01 _hismc_pipe03_valve02 _hismc_pipe05_valve03 _hismc_pipe06_valve04 _hismc_pipe06_valve04_01 _hismc_valve05 _hismc_valve06 _hismc_valve07 :!type "InstancedStaticMeshComponent Object Reference")))
    (:`NewEnumerator1`
      (set `self.Pipe Mesh Type` (`|MakeArray` (`self.HISMC_Pipe02_01`) (`self.HISMC_Pipe02_02`) (`self.HISMC_Pipe02_03`) (`self.HISMC_Pipe02_04`) (`self.HISMC_Pipe02_05`) (`self.HISMC_Pipe02_06`) _hismc_pipe_machine01 _hismc_pipe_machine02 _hismc_pipe01_machine03 _hismc_pipe03_valve01 _hismc_pipe03_valve02 _hismc_pipe05_valve03 _hismc_pipe06_valve04 _hismc_pipe06_valve04_01 _hismc_valve05 _hismc_valve06 _hismc_valve07 :!type "InstancedStaticMeshComponent Object Reference"))))
  (`InstancedStaticMeshComponent.AddInstance` _output (`KismetMathLibrary.MakeTransform` (0.0 0.0 0.0)) false)
  ;[1 1 1] Pipe Material
  (switch `/Game/outsideArts/SteampunkWorkshop/Blueprints/Enumerators/Pipes/EPipeType` _pipe_type
    (:`NewEnumerator0`
      (switch `/Game/outsideArts/SteampunkWorkshop/Blueprints/Enumerators/Pipes/EPipeSectionType` _pipe_section_type
        (:`NewEnumerator0`
          (set `self.Pipe Material Type` (`|MakeArray` "/Game/outsideArts/SteampunkWorkshop/Materials/Pipes/MI_Pipe01_01_01.MI_Pipe01_01_01" "/Game/outsideArts/SteampunkWorkshop/Materials/Pipes/MI_Pipe01_01_02.MI_Pipe01_01_02" :!type "MaterialInterface Object Reference") :!label _label))
        (:`NewEnumerator1`
          (goto _label))
        (:`NewEnumerator2`
          (goto _label))
        (:`NewEnumerator4`
          (set `self.Pipe Material Type` (`|MakeArray` "/Game/outsideArts/SteampunkWorkshop/Materials/Pipes/MI_Pipe01_04_01.MI_Pipe01_04_01" "/Game/outsideArts/SteampunkWorkshop/Materials/Pipes/MI_Pipe01_04_02.MI_Pipe01_04_02" :!type "MaterialInterface Object Reference")))
        (:`NewEnumerator5`
          (goto _label))
        (:`NewEnumerator6`
          (goto _label))
        (:`NewEnumerator7`
          (set `self.Pipe Material Type` (`|MakeArray` "/Game/outsideArts/SteampunkWorkshop/Materials/Pipes/MI_PipeMachine01_01.MI_PipeMachine01_01" "/Game/outsideArts/SteampunkWorkshop/Materials/Pipes/MI_PipeMachine01_02.MI_PipeMachine01_02" :!type "MaterialInterface Object Reference") :!label _label_2))
        (:`NewEnumerator8`
          (set `self.Pipe Material Type` (`|MakeArray` "/Game/outsideArts/SteampunkWorkshop/Materials/Pipes/MI_PipeMachine02_01.MI_PipeMachine02_01" "/Game/outsideArts/SteampunkWorkshop/Materials/Pipes/MI_PipeMachine02_02.MI_PipeMachine02_02" :!type "MaterialInterface Object Reference") :!label _label_3))
        (:`NewEnumerator9`
          (set `self.Pipe Material Type` (`|MakeArray` "/Game/outsideArts/SteampunkWorkshop/Materials/Pipes/MI_PipeMachine03_01.MI_PipeMachine03_01" "/Game/outsideArts/SteampunkWorkshop/Materials/Pipes/MI_PipeMachine03_02.MI_PipeMachine03_02" :!type "MaterialInterface Object Reference") :!label _label_4))
        (:`NewEnumerator10`
          (set `self.Pipe Material Type` (`|MakeArray` "/Game/outsideArts/SteampunkWorkshop/Materials/Pipes/MI_Pipe03_Valve01_01.MI_Pipe03_Valve01_01" "/Game/outsideArts/SteampunkWorkshop/Materials/Pipes/MI_Pipe03_Valve01_02.MI_Pipe03_Valve01_02" :!type "MaterialInterface Object Reference") :!label _label_5))
        (:`NewEnumerator11`
          (set `self.Pipe Material Type` (`|MakeArray` "/Game/outsideArts/SteampunkWorkshop/Materials/Pipes/MI_Pipe03_Valve02_01.MI_Pipe03_Valve02_01" "/Game/outsideArts/SteampunkWorkshop/Materials/Pipes/MI_Pipe03_Valve02_02.MI_Pipe03_Valve02_02" :!type "MaterialInterface Object Reference") :!label _label_6))
        (:`NewEnumerator12`
          (set `self.Pipe Material Type` (`|MakeArray` "/Game/outsideArts/SteampunkWorkshop/Materials/Pipes/MI_Pipe05_Valve03_01.MI_Pipe05_Valve03_01" "/Game/outsideArts/SteampunkWorkshop/Materials/Pipes/MI_Pipe05_Valve03_02.MI_Pipe05_Valve03_02" :!type "MaterialInterface Object Reference") :!label _label_7))
        (:`NewEnumerator13`
          (set `self.Pipe Material Type` (`|MakeArray` "/Game/outsideArts/SteampunkWorkshop/Materials/Pipes/MI_Pipe06_Valve04_01.MI_Pipe06_Valve04_01" "/Game/outsideArts/SteampunkWorkshop/Materials/Pipes/MI_Pipe06_Valve04_02.MI_Pipe06_Valve04_02" :!type "MaterialInterface Object Reference") :!label _label_8))
        (:`NewEnumerator14`
          (goto _label_8)))
      (`PrimitiveComponent.SetMaterial` _output 0 _output_2))
    (:`NewEnumerator1`
      (switch `/Game/outsideArts/SteampunkWorkshop/Blueprints/Enumerators/Pipes/EPipeSectionType` _pipe_section_type
        (:`NewEnumerator0`
          _)
        (:`NewEnumerator1`
          _)
        (:`NewEnumerator2`
          _)
        (:`NewEnumerator4`
          _)
        (:`NewEnumerator5`
          _)
        (:`NewEnumerator6`
          _)
        (:`NewEnumerator7`
          (goto _label_2))
        (:`NewEnumerator8`
          (goto _label_3))
        (:`NewEnumerator9`
          (goto _label_4))
        (:`NewEnumerator10`
          (goto _label_5))
        (:`NewEnumerator11`
          (goto _label_6))
        (:`NewEnumerator12`
          (goto _label_7))
        (:`NewEnumerator13`
          (goto _label_8))
        (:`NewEnumerator14`
          (goto _label_8)))
      (set `self.Pipe Material Type` (`|MakeArray` "/Game/outsideArts/SteampunkWorkshop/Materials/Pipes/MI_Pipe02_01_01.MI_Pipe02_01_01" "/Game/outsideArts/SteampunkWorkshop/Materials/Pipes/MI_Pipe02_01_02.MI_Pipe02_01_02" :!type "MaterialInterface Object Reference"))
      (`PrimitiveComponent.SetMaterial` _output 0 _output_2))))