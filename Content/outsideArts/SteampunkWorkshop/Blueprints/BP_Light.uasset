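; Configurable steampunk workshop light fixture, assembled entirely in the Construction Script with no runtime logic.
; Fixture type, bulb type and bulb count choose which hierarchical instanced mesh components receive instances, with multiple bulbs fanned out by yaw.
; When the light is enabled, it adds one point light with configurable intensity and radius.
; Otherwise, dynamic materials switch off glass emissive and dim the filament.
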(fn `UserConstructionScript`
  (bind _returnvalue (`KismetMathLibrary.Conv_ByteToInt` (`self.Bulb Type`)))
  (bind _output (`|GetArrayItem` (`self.Bulb Mesh Type`) _returnvalue))
  ;[1 1 1] Light Fixture
  (switch `/Game/outsideArts/SteampunkWorkshop/Blueprints/Enumerators/Lights/ELightFixtureType` (`self.Light Fixture Type`)
    (:`NewEnumerator0`
      (`InstancedStaticMeshComponent.AddInstance` (`self.HISMC_LightFixture01`) (`KismetMathLibrary.MakeTransform` (0.0 0.0 0.0)) false))
    (:`NewEnumerator1`
      (`InstancedStaticMeshComponent.AddInstance` (`self.HISMC_LightFixture02`) (`KismetMathLibrary.MakeTransform` (0.0 25.0 0.0)) false)))
  ;[1 1 1] Instanced Bulb Type
  (set `self.Bulb Mesh Type` (`|MakeArray` (`self.HISMC_Bulb04`) (`self.HISMC_Bulb05`) (`self.HISMC_Bulb06`) :!type "InstancedStaticMeshComponent Object Reference"))
  (switch `/Game/outsideArts/SteampunkWorkshop/Blueprints/Enumerators/Lights/ENumberOfBulbs` (`self.Number Of Bulbs`)
    (:`NewEnumerator0`
      ;[1 1 1] Bulb & Point Light Instances
      (`InstancedStaticMeshComponent.AddInstance` _output (`KismetMathLibrary.MakeTransform` (0.0 25.0 0.0) (`KismetMathLibrary.MakeRotator` 0.0)) false))
    (:`NewEnumerator1`
      (`InstancedStaticMeshComponent.AddInstance` _output (`KismetMathLibrary.MakeTransform` (0.0 25.0 0.0) (`KismetMathLibrary.MakeRotator` 0.0 0.0 -45.0)) false)
      (`InstancedStaticMeshComponent.AddInstance` _output (`KismetMathLibrary.MakeTransform` (0.0 25.0 0.0) (`KismetMathLibrary.MakeRotator` 0.0 0.0 45.0)) false))
    (:`NewEnumerator2`
      (`InstancedStaticMeshComponent.AddInstance` _output (`KismetMathLibrary.MakeTransform` (0.0 25.0 0.0) (`KismetMathLibrary.MakeRotator` 0.0 0.0 -90.0)) false)
      (`InstancedStaticMeshComponent.AddInstance` _output (`KismetMathLibrary.MakeTransform` (0.0 25.0 0.0) (`KismetMathLibrary.MakeRotator` 0.0)) false)
      (`InstancedStaticMeshComponent.AddInstance` _output (`KismetMathLibrary.MakeTransform` (0.0 25.0 0.0) (`KismetMathLibrary.MakeRotator` 0.0 0.0 90.0)) false)))
  ;[1 1 1] Light Parameters
  (if (`self.Enable Light`)
    (bind _returnvalue_2 (`AddComponent|NODE_AddPointLightComponent-0` :`RelativeTransform` (`KismetMathLibrary.MakeTransform` (0.0 75.0 -55.0) (struct :`Pitch` -90.0))))
    (`SceneComponent.K2_SetRelativeRotation` _returnvalue_2 (`KismetMathLibrary.MakeRotator` -90.0 -90.0) false false)
    (`LightComponent.SetIntensity` _returnvalue_2 (`self.Light Intensity`))
    (`PointLightComponent.SetAttenuationRadius` _returnvalue_2 (`self.Light Radius`))
    (else
      ;[1 1 1] Bulb Light Parameters
      (bind _output_get (set `self.Bulb Material Type` (`|MakeArray` (`self.MI_Bulb04Glass`) (`self.MI_Bulb05Glass`) (`self.MI_Bulb06Glass`))))
      (bind _returnvalue_3 (`PrimitiveComponent.CreateDynamicMaterialInstance` _output 1 (`|GetArrayItem` _output_get _returnvalue) "None"))
      (`MaterialInstanceDynamic.SetScalarParameterValue` _returnvalue_3 (`self.Emissive Amount`) 0.0)
      (bind _output_get_2 (set `self.Bulb Material Type` (`|MakeArray` (`self.MI_Bulb04`) (`self.MI_Bulb05`) (`self.MI_Bulb06`))))
      (bind _returnvalue_4 (`PrimitiveComponent.CreateDynamicMaterialInstance` _output 0 (`|GetArrayItem` _output_get_2 _returnvalue) "None"))
      (`MaterialInstanceDynamic.SetScalarParameterValue` _returnvalue_4 (`self.Filament Intensity`) 0.1))))