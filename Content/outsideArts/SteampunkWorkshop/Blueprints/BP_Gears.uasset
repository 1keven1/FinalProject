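; Animated clockwork for a steampunk clock, with meshing gears, shafts, mounts and two opposed sets of hour, minute and second hands.
; The construction script builds HISM parts, posing "Constr" copies by ClockWindRevs and hiding their "Sim" twins in game.
; Tick rotates the Sim components from accumulated time, TimeSpeedFraction and ClockWindRevs through hard-coded chained gear ratios.
; Tick also swaps visibility to the Sim copies every frame.
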(event `self.ReceiveTick`
  (params (DeltaSeconds :type "Float (single-precision)"))
  (bind _hismc_hourhand_01_sim (`self.HISMC_HourHand_01_Sim`))
  (bind _hismc_gears10_sim (`self.HISMC_Gears10_Sim`))
  (bind _hismc_secondhand_sim (`self.HISMC_SecondHand_Sim`))
  (bind _hismc_secondhand_01_sim (`self.HISMC_SecondHand_01_Sim`))
  (bind _hismc_gear01_sim (`self.HISMC_Gear01_Sim`))
  (bind _hismc_gear06_sim (`self.HISMC_Gear06_Sim`))
  (bind _hismc_gear02_sim (`self.HISMC_Gear02_Sim`))
  (bind _hismc_gear05_sim (`self.HISMC_Gear05_Sim`))
  (bind _hismc_gear04_sim (`self.HISMC_Gear04_Sim`))
  (bind _hismc_minutehand_sim (`self.HISMC_MinuteHand_Sim`))
  (bind _hismc_gears07_sim (`self.HISMC_Gears07_Sim`))
  (bind _hismc_hourhand_sim (`self.HISMC_HourHand_Sim`))
  (bind _hismc_gears08_sim (`self.HISMC_Gears08_Sim`))
  (bind _hismc_minutehand_01_sim (`self.HISMC_MinuteHand_01_Sim`))
  (bind _hismc_gears01_01_sim (`self.HISMC_Gears01_01_Sim`))
  (bind _hismc_gears09_sim (`self.HISMC_Gears09_Sim`))
  (bind _hismc_gear03_sim (`self.HISMC_Gear03_Sim`))
  (bind _output_get (set `self.Counter` (+ DeltaSeconds (`self.Counter`))))
  (bind _returnvalue (+ (* _output_get (* (`self.Time Speed Fraction`) 0.1)) (* (`self.Clock Wind Revs`) 360.0)))
  ;[1 1 1] Gear02
  (`SceneComponent.K2_SetRelativeLocationAndRotation` _hismc_gear02_sim (0.0 0.0 0.0) (`KismetMathLibrary.MakeRotator` 0.0 _returnvalue) false false)
  (`SceneComponent.SetHiddenInGame` (`self.HISMC_Gear02_Constr`) true false)
  (`SceneComponent.SetHiddenInGame` _hismc_gear02_sim false false)
  (bind _returnvalue_2 (* _returnvalue -6.0))
  ;[1 1 1] Gears01
  (`SceneComponent.K2_SetRelativeLocationAndRotation` _hismc_gear01_sim (-58.599998 0.0 0.0) (`KismetMathLibrary.MakeRotator` 0.0 _returnvalue_2) false false)
  (`SceneComponent.SetHiddenInGame` (`self.HISMC_Gear01_Constr`) true false)
  (`SceneComponent.SetHiddenInGame` _hismc_gear01_sim false false)
  ;[1 1 1] Gears04
  (`SceneComponent.K2_SetRelativeLocationAndRotation` _hismc_gear04_sim (-58.599998 -10.0 0.0) (`KismetMathLibrary.MakeRotator` 0.0 _returnvalue_2) false false)
  (`SceneComponent.SetHiddenInGame` (`self.HISMC_Gear04_Constr`) true false)
  (`SceneComponent.SetHiddenInGame` _hismc_gear04_sim false false)
  (bind _returnvalue_3 (* _returnvalue_2 -2.0))
  ;[1 1 1] Gears03
  (`SceneComponent.K2_SetRelativeLocationAndRotation` _hismc_gear03_sim (0.0 -10.0 0.0) (`KismetMathLibrary.MakeRotator` 0.0 _returnvalue_3) false false)
  (`SceneComponent.SetHiddenInGame` (`self.HISMC_Gear03_Constr`) true false)
  (`SceneComponent.SetHiddenInGame` _hismc_gear03_sim false false)
  ;[1 1 1] Gears05
  (`SceneComponent.K2_SetRelativeLocationAndRotation` _hismc_gear05_sim (0.0 -20.0 0.0) (`KismetMathLibrary.MakeRotator` 0.0 _returnvalue_3) false false)
  (`SceneComponent.SetHiddenInGame` (`self.HISMC_Gear05_Constr`) true false)
  (`SceneComponent.SetHiddenInGame` _hismc_gear05_sim false false)
  (bind _returnvalue_4 (* _returnvalue_3 -5.0))
  ;[1 1 1] Gears01_01
  (`SceneComponent.K2_SetRelativeLocationAndRotation` _hismc_gears01_01_sim (0.0 -20.0 -50.68) (`KismetMathLibrary.MakeRotator` 0.0 _returnvalue_4) false false)
  (`SceneComponent.SetHiddenInGame` (`self.HISMC_Gears01_01_Const`) true false)
  (`SceneComponent.SetHiddenInGame` _hismc_gears01_01_sim false false)
  ;[1 1 1] Gears06
  (`SceneComponent.K2_SetRelativeLocationAndRotation` _hismc_gear06_sim (0.0 10.0 0.0) (`KismetMathLibrary.MakeRotator` 0.0 _returnvalue) false false)
  (`SceneComponent.SetHiddenInGame` (`self.HISMC_Gear06_Constr`) true false)
  (`SceneComponent.SetHiddenInGame` _hismc_gear06_sim false false)
  (bind _returnvalue_5 (/ _returnvalue -4.0))
  ;[1 1 1] Gears07
  (`SceneComponent.K2_SetRelativeLocationAndRotation` _hismc_gears07_sim (0.0 10.0 58.665001) (`KismetMathLibrary.MakeRotator` 0.0 _returnvalue_5) false false)
  (`SceneComponent.SetHiddenInGame` (`self.HISMC_Gears07_Constr`) true false)
  (`SceneComponent.SetHiddenInGame` _hismc_gears07_sim false false)
  ;[1 1 1] Gears08
  (`SceneComponent.K2_SetRelativeLocationAndRotation` _hismc_gears08_sim (0.0 20.0 58.665001) (`KismetMathLibrary.MakeRotator` 0.0 _returnvalue_5) false false)
  (`SceneComponent.SetHiddenInGame` (`self.HISMC_Gears08_Constr`) true false)
  (`SceneComponent.SetHiddenInGame` _hismc_gears08_sim false false)
  ;[1 1 1] Gears09
  (`SceneComponent.K2_SetRelativeLocationAndRotation` _hismc_gears09_sim (0.0 20.0 0.0) (`KismetMathLibrary.MakeRotator` 0.0 (/ _returnvalue_5 -3.0)) false false)
  (`SceneComponent.SetHiddenInGame` (`self.HISMC_Gears09_Constr`) true false)
  (`SceneComponent.SetHiddenInGame` _hismc_gears09_sim false false)
  ;[1 1 1] Gears10
  (`SceneComponent.K2_SetRelativeLocationAndRotation` _hismc_gears10_sim (66.800003 0.0 0.0) (`KismetMathLibrary.MakeRotator` 0.0 (* _returnvalue -3.0)) false false)
  (`SceneComponent.SetHiddenInGame` (`self.HISMC_Gears10_Constr`) true false)
  (`SceneComponent.SetHiddenInGame` _hismc_gears10_sim false false)
  (bind _returnvalue_6 (* _returnvalue_4 1.0))
  ;[1 1 1] Second Hand
  (`SceneComponent.K2_SetRelativeLocationAndRotation` _hismc_secondhand_sim (0.0 -48.0 -50.68) (`KismetMathLibrary.MakeRotator` 0.0 _returnvalue_6 180.0) false false)
  (`SceneComponent.SetHiddenInGame` (`self.HISMC_SecondHand_Constr`) true false)
  (`SceneComponent.SetHiddenInGame` _hismc_secondhand_sim false false)
  ;[1 1 1] Second Hand
  (`SceneComponent.K2_SetRelativeLocationAndRotation` _hismc_secondhand_01_sim (0.0 48.0 -50.68) (`KismetMathLibrary.MakeRotator` 0.0 (* _returnvalue_6 -1.0) 180.0) false false)
  (`SceneComponent.SetHiddenInGame` (`self.HISMC_SecondHand_01_Constr`) true false)
  (`SceneComponent.SetHiddenInGame` _hismc_secondhand_01_sim false false)
  (bind _returnvalue_7 (* _returnvalue -1.0))
  ;[1 1 1] Minute Hand
  (`SceneComponent.K2_SetRelativeLocationAndRotation` _hismc_minutehand_sim (0.0 -55.0 0.0) (`KismetMathLibrary.MakeRotator` 0.0 _returnvalue_7 180.0) false false)
  (`SceneComponent.SetHiddenInGame` (`self.HISMC_MinuteHand_Constr`) true false)
  (`SceneComponent.SetHiddenInGame` _hismc_minutehand_sim false false)
  ;[1 1 1] Minute Hand 01
  (`SceneComponent.K2_SetRelativeLocationAndRotation` _hismc_minutehand_01_sim (0.0 55.0 0.0) (`KismetMathLibrary.MakeRotator` 0.0 (* _returnvalue_7 1.0)) false false)
  (`SceneComponent.SetHiddenInGame` (`self.HISMC_MinuteHand_01_Constr`) true false)
  (`SceneComponent.SetHiddenInGame` _hismc_minutehand_01_sim false false)
  (bind _returnvalue_8 (/ _returnvalue_7 12.0))
  ;[1 1 1] Hour Hand
  (`SceneComponent.K2_SetRelativeLocationAndRotation` _hismc_hourhand_sim (0.0 -47.0 0.0) (`KismetMathLibrary.MakeRotator` 0.0 _returnvalue_8 180.0) false false)
  (`SceneComponent.SetHiddenInGame` (`self.HISMC_HourHand_Constr`) true false)
  (`SceneComponent.SetHiddenInGame` _hismc_hourhand_sim false false)
  ;[1 1 1] Hour Hand 01
  (`SceneComponent.K2_SetRelativeLocationAndRotation` _hismc_hourhand_01_sim (0.0 47.0 0.0) (`KismetMathLibrary.MakeRotator` 0.0 (* _returnvalue_8 1.0)) false false)
  (`SceneComponent.SetHiddenInGame` (`self.HISMC_HourHand_01_Constr`) true false)
  (`SceneComponent.SetHiddenInGame` _hismc_hourhand_01_sim false false))

(fn `UserConstructionScript`
  (bind _hismc_clockshaft01 (`self.HISMC_ClockShaft01`))
  (bind _hismc_clockmount01 (`self.HISMC_ClockMount01`))
  (bind _hismc_gear01_sim (`self.HISMC_Gear01_Sim`))
  (bind _hismc_secondhand_01_sim (`self.HISMC_SecondHand_01_Sim`))
  (bind _hismc_gear02_sim (`self.HISMC_Gear02_Sim`))
  (bind _hismc_clockmount02 (`self.HISMC_ClockMount02`))
  (bind _hismc_clockmount03 (`self.HISMC_ClockMount03`))
  (bind _hismc_gear03_sim (`self.HISMC_Gear03_Sim`))
  (bind _hismc_gear04_sim (`self.HISMC_Gear04_Sim`))
  (bind _hismc_gear05_sim (`self.HISMC_Gear05_Sim`))
  (bind _hismc_gears07_sim (`self.HISMC_Gears07_Sim`))
  (bind _hismc_minutehand_sim (`self.HISMC_MinuteHand_Sim`))
  (bind _hismc_gears08_sim (`self.HISMC_Gears08_Sim`))
  (bind _hismc_secondhand_sim (`self.HISMC_SecondHand_Sim`))
  (bind _hismc_hourhand_sim (`self.HISMC_HourHand_Sim`))
  (bind _hismc_minutehand_01_sim (`self.HISMC_MinuteHand_01_Sim`))
  (bind _hismc_gears01_01_sim (`self.HISMC_Gears01_01_Sim`))
  (bind _hismc_gears09_sim (`self.HISMC_Gears09_Sim`))
  (bind _hismc_gears10_sim (`self.HISMC_Gears10_Sim`))
  (bind _hismc_gear06_sim (`self.HISMC_Gear06_Sim`))
  (bind _hismc_hourhand_01_sim (`self.HISMC_HourHand_01_Sim`))
  (bind _returnvalue (* (`self.Clock Wind Revs`) 360.0))
  (bind _returnvalue_2 (/ _returnvalue -4.0))
  (bind _returnvalue_3 (* _returnvalue -6.0))
  (bind _returnvalue_4 (* _returnvalue -1.0))
  (bind _returnvalue_5 (/ _returnvalue_4 12.0))
  (bind _returnvalue_6 (* _returnvalue_3 -2.0))
  (bind _returnvalue_7 (* _returnvalue_6 -5.0))
  (bind _returnvalue_8 (* _returnvalue_7 1.0))
  ;[1 1 1] Gear02
  (`InstancedStaticMeshComponent.AddInstance` (`self.HISMC_Gear02_Constr`) (`KismetMathLibrary.MakeTransform` (0.0 0.0 0.0) (`KismetMathLibrary.MakeRotator` 0.0 _returnvalue)) false)
  (`InstancedStaticMeshComponent.AddInstance` _hismc_gear02_sim (`KismetMathLibrary.MakeTransform` (0.0 0.0 0.0)) false)
  (`SceneComponent.SetHiddenInGame` _hismc_gear02_sim true false)
  ;[1 1 1] Gears01
  (`InstancedStaticMeshComponent.AddInstance` (`self.HISMC_Gear01_Constr`) (`KismetMathLibrary.MakeTransform` (-58.599998 0.0 0.0) (`KismetMathLibrary.MakeRotator` 0.0 _returnvalue_3)) false)
  (`InstancedStaticMeshComponent.AddInstance` _hismc_gear01_sim (`KismetMathLibrary.MakeTransform` (0.0 0.0 0.0)) false)
  (`SceneComponent.SetHiddenInGame` _hismc_gear01_sim true false)
  ;[1 1 1] Gears04
  (`InstancedStaticMeshComponent.AddInstance` (`self.HISMC_Gear04_Constr`) (`KismetMathLibrary.MakeTransform` (-58.599998 -10.0 0.0) (`KismetMathLibrary.MakeRotator` 0.0 _returnvalue_3)) false)
  (`InstancedStaticMeshComponent.AddInstance` _hismc_gear04_sim (`KismetMathLibrary.MakeTransform` (0.0 0.0 0.0)) false)
  (`SceneComponent.SetHiddenInGame` _hismc_gear04_sim true false)
  ;[1 1 1] Gears03
  (`InstancedStaticMeshComponent.AddInstance` (`self.HISMC_Gear03_Constr`) (`KismetMathLibrary.MakeTransform` (0.0 -10.0 0.0) (`KismetMathLibrary.MakeRotator` 0.0 _returnvalue_6)) false)
  (`InstancedStaticMeshComponent.AddInstance` _hismc_gear03_sim (`KismetMathLibrary.MakeTransform` (0.0 0.0 0.0)) false)
  (`SceneComponent.SetHiddenInGame` _hismc_gear03_sim true false)
  ;[1 1 1] Gears05
  (`InstancedStaticMeshComponent.AddInstance` (`self.HISMC_Gear05_Constr`) (`KismetMathLibrary.MakeTransform` (0.0 -20.0 0.0) (`KismetMathLibrary.MakeRotator` 0.0 _returnvalue_6)) false)
  (`InstancedStaticMeshComponent.AddInstance` _hismc_gear05_sim (`KismetMathLibrary.MakeTransform` (0.0 0.0 0.0)) false)
  (`SceneComponent.SetHiddenInGame` _hismc_gear05_sim true false)
  ;[1 1 1] Gears01_01
  (`InstancedStaticMeshComponent.AddInstance` (`self.HISMC_Gears01_01_Const`) (`KismetMathLibrary.MakeTransform` (0.0 -20.0 -50.68) (`KismetMathLibrary.MakeRotator` 0.0 _returnvalue_7)) false)
  (`InstancedStaticMeshComponent.AddInstance` _hismc_gears01_01_sim (`KismetMathLibrary.MakeTransform` (0.0 0.0 0.0)) false)
  (`SceneComponent.SetHiddenInGame` _hismc_gears01_01_sim true false)
  ;[1 1 1] Gears06
  (`InstancedStaticMeshComponent.AddInstance` (`self.HISMC_Gear06_Constr`) (`KismetMathLibrary.MakeTransform` (0.0 10.0 0.0) (`KismetMathLibrary.MakeRotator` 0.0 _returnvalue)) false)
  (`InstancedStaticMeshComponent.AddInstance` _hismc_gear06_sim (`KismetMathLibrary.MakeTransform` (0.0 0.0 0.0)) false)
  (`SceneComponent.SetHiddenInGame` _hismc_gear06_sim true false)
  ;[1 1 1] Gears07
  (`InstancedStaticMeshComponent.AddInstance` (`self.HISMC_Gears07_Constr`) (`KismetMathLibrary.MakeTransform` (0.0 10.0 58.665001) (`KismetMathLibrary.MakeRotator` 0.0 _returnvalue_2)) false)
  (`InstancedStaticMeshComponent.AddInstance` _hismc_gears07_sim (`KismetMathLibrary.MakeTransform` (0.0 0.0 0.0)) false)
  (`SceneComponent.SetHiddenInGame` _hismc_gears07_sim true false)
  ;[1 1 1] Gears08
  (`InstancedStaticMeshComponent.AddInstance` (`self.HISMC_Gears08_Constr`) (`KismetMathLibrary.MakeTransform` (0.0 20.0 58.665001) (`KismetMathLibrary.MakeRotator` 0.0 _returnvalue_2)) false)
  (`InstancedStaticMeshComponent.AddInstance` _hismc_gears08_sim (`KismetMathLibrary.MakeTransform` (0.0 0.0 0.0)) false)
  (`SceneComponent.SetHiddenInGame` _hismc_gears08_sim true false)
  ;[1 1 1] Gears09
  (`InstancedStaticMeshComponent.AddInstance` (`self.HISMC_Gears09_Constr`) (`KismetMathLibrary.MakeTransform` (0.0 20.0 0.0) (`KismetMathLibrary.MakeRotator` 0.0 (/ _returnvalue_2 -3.0))) false)
  (`InstancedStaticMeshComponent.AddInstance` _hismc_gears09_sim (`KismetMathLibrary.MakeTransform` (0.0 0.0 0.0)) false)
  (`SceneComponent.SetHiddenInGame` _hismc_gears09_sim true false)
  ;[1 1 1] Gears10
  (`InstancedStaticMeshComponent.AddInstance` (`self.HISMC_Gears10_Constr`) (`KismetMathLibrary.MakeTransform` (66.800003 0.0 0.0) (`KismetMathLibrary.MakeRotator` 0.0 (* _returnvalue -3.0))) false)
  (`InstancedStaticMeshComponent.AddInstance` _hismc_gears10_sim (`KismetMathLibrary.MakeTransform` (0.0 0.0 0.0)) false)
  (`SceneComponent.SetHiddenInGame` _hismc_gears10_sim true false)
  ;[1 1 1] ClockShaft
  (`InstancedStaticMeshComponent.AddInstance` _hismc_clockshaft01 (`KismetMathLibrary.MakeTransform` (0.0 0.0 0.0)) false)
  (`InstancedStaticMeshComponent.AddInstance` _hismc_clockshaft01 (`KismetMathLibrary.MakeTransform` (-58.599998 -5.0 0.0) (struct) (1.0 0.25 1.0)) false)
  (`InstancedStaticMeshComponent.AddInstance` _hismc_clockshaft01 (`KismetMathLibrary.MakeTransform` (0.0 0.0 -50.68) (struct) (0.6 0.55 0.6)) false)
  (`InstancedStaticMeshComponent.AddInstance` _hismc_clockshaft01 (`KismetMathLibrary.MakeTransform` (0.0 10.0 58.665001) (struct) (1.0 0.25 1.0)) false)
  (`InstancedStaticMeshComponent.AddInstance` _hismc_clockshaft01 (`KismetMathLibrary.MakeTransform` (66.800003 0.0 0.0) (struct) (0.5 0.125 0.5)) false)
  ;[1 1 1] Clock Mount01
  (`InstancedStaticMeshComponent.AddInstance` _hismc_clockmount01 (`KismetMathLibrary.MakeTransform` (0.0 20.0 -50.68)) false)
  (`InstancedStaticMeshComponent.AddInstance` _hismc_clockmount01 (`KismetMathLibrary.MakeTransform` (0.0 -45.0 -50.68)) false)
  (`InstancedStaticMeshComponent.AddInstance` _hismc_clockmount01 (`KismetMathLibrary.MakeTransform` (66.800003 -20.0 0.0) (struct :`Pitch` 90.0)) false)
  (`InstancedStaticMeshComponent.AddInstance` _hismc_clockmount01 (`KismetMathLibrary.MakeTransform` (66.800003 -5.0 0.0) (struct :`Pitch` 90.0)) false)
  (`InstancedStaticMeshComponent.AddInstance` _hismc_clockmount02 (`KismetMathLibrary.MakeTransform` (-58.599998 20.0 0.0) (struct :`Yaw` 180.0)) false)
  (`InstancedStaticMeshComponent.AddInstance` _hismc_clockmount02 (`KismetMathLibrary.MakeTransform` (-58.599998 -30.0 0.0) (struct :`Yaw` 180.0)) false)
  (`InstancedStaticMeshComponent.AddInstance` _hismc_clockmount03 (`KismetMathLibrary.MakeTransform` (0.0 -10.0 58.665001) (struct :`Yaw` 180.0)) false)
  (`InstancedStaticMeshComponent.AddInstance` _hismc_clockmount03 (`KismetMathLibrary.MakeTransform` (0.0 30.0 58.665001) (struct :`Yaw` 180.0)) false)
  ;[1 1 1] Second Hand
  (`InstancedStaticMeshComponent.AddInstance` (`self.HISMC_SecondHand_Constr`) (`KismetMathLibrary.MakeTransform` (0.0 -48.0 -50.68) (`KismetMathLibrary.MakeRotator` 0.0 _returnvalue_8 180.0)) false)
  (`InstancedStaticMeshComponent.AddInstance` _hismc_secondhand_sim (`KismetMathLibrary.MakeTransform` (0.0 0.0 0.0)) false)
  (`SceneComponent.SetHiddenInGame` _hismc_secondhand_sim true false)
  ;[1 1 1] Second Hand 01
  (`InstancedStaticMeshComponent.AddInstance` (`self.HISMC_SecondHand_01_Constr`) (`KismetMathLibrary.MakeTransform` (0.0 48.0 -50.68) (`KismetMathLibrary.MakeRotator` 0.0 (* _returnvalue_8 -1.0))) false)
  (`InstancedStaticMeshComponent.AddInstance` _hismc_secondhand_01_sim (`KismetMathLibrary.MakeTransform` (0.0 0.0 0.0)) false)
  (`SceneComponent.SetHiddenInGame` _hismc_secondhand_01_sim true false)
  ;[1 1 1] Minute Hand
  (`InstancedStaticMeshComponent.AddInstance` (`self.HISMC_MinuteHand_Constr`) (`KismetMathLibrary.MakeTransform` (0.0 -50.0 0.0) (`KismetMathLibrary.MakeRotator` 0.0 _returnvalue_4 180.0)) false)
  (`InstancedStaticMeshComponent.AddInstance` _hismc_minutehand_sim (`KismetMathLibrary.MakeTransform` (0.0 0.0 0.0)) false)
  (`SceneComponent.SetHiddenInGame` _hismc_minutehand_sim true false)
  ;[1 1 1] Minute Hand 01
  (`InstancedStaticMeshComponent.AddInstance` (`self.HISMC_MinuteHand_01_Constr`) (`KismetMathLibrary.MakeTransform` (0.0 50.0 0.0) (`KismetMathLibrary.MakeRotator` 0.0 (* _returnvalue_4 1.0))) false)
  (`InstancedStaticMeshComponent.AddInstance` _hismc_minutehand_01_sim (`KismetMathLibrary.MakeTransform` (0.0 0.0 0.0)) false)
  (`SceneComponent.SetHiddenInGame` _hismc_minutehand_01_sim true false)
  ;[1 1 1] Hour Hand
  (`InstancedStaticMeshComponent.AddInstance` (`self.HISMC_HourHand_Constr`) (`KismetMathLibrary.MakeTransform` (0.0 -47.0 0.0) (`KismetMathLibrary.MakeRotator` 0.0 _returnvalue_5 180.0)) false)
  (`InstancedStaticMeshComponent.AddInstance` _hismc_hourhand_sim (`KismetMathLibrary.MakeTransform` (0.0 0.0 0.0)) false)
  (`SceneComponent.SetHiddenInGame` _hismc_hourhand_sim true false)
  ;[1 1 1] Hour Hand
  (`InstancedStaticMeshComponent.AddInstance` (`self.HISMC_HourHand_01_Constr`) (`KismetMathLibrary.MakeTransform` (0.0 47.0 0.0) (`KismetMathLibrary.MakeRotator` 0.0 (* _returnvalue_5 1.0))) false)
  (`InstancedStaticMeshComponent.AddInstance` _hismc_hourhand_01_sim (`KismetMathLibrary.MakeTransform` (0.0 0.0 0.0)) false)
  (`SceneComponent.SetHiddenInGame` _hismc_hourhand_01_sim true false))