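; Procedural steampunk vat prop that builds itself in the construction script, in one of two size variants chosen by VatType.
; Hierarchical instanced static mesh components supply the base, glass, liquid, coils, pins, rod and arc, plus an optional mount with its own pins.
; Liquid height, rotation and hues are adjustable through scale and a dynamic material, and a point light takes the first hue.
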(fn `UserConstructionScript`
  (bind _hismc_vatpin01 (`self.HISMC_VatPin01`))
  (bind _arcsize (`self.ArcSize`))
  (bind _liquid_hue_1 (`self.Liquid Hue 1`))
  (bind _mount_present_ (`self.Mount Present?`))
  (bind _vat_type (`self.Vat Type`))
  (bind _output (`|GetArrayItem` (`self.MeshType`) (`KismetMathLibrary.Conv_ByteToInt` _vat_type)))
  (`|ExecutionSequence`
    (:`then_0`
      ;[1 1 1] Mount Present?
      (if _mount_present_
        ;[1 1 1] VatMount
        (set `self.MeshType` (`|MakeArray` (`self.HISMC_VatMount`) (`self.HISMC_VatMount02`) :!type "InstancedStaticMeshComponent Object Reference"))
        (`InstancedStaticMeshComponent.AddInstance` _output (`KismetMathLibrary.MakeTransform` (0.0 0.0 0.0)) false))
      ;[1 1 1] VatBase
      (set `self.MeshType` (`|MakeArray` (`self.HISMC_VatBase`) (`self.HISMC_VatBase02`) :!type "InstancedStaticMeshComponent Object Reference"))
      (`InstancedStaticMeshComponent.AddInstance` _output (`KismetMathLibrary.MakeTransform` (0.0 0.0 0.0)) false)
      ;[1 1 1] VatGlass
      (set `self.MeshType` (`|MakeArray` (`self.HISMC_VatGlass`) (`self.HISMC_VatGlass02`) :!type "InstancedStaticMeshComponent Object Reference"))
      (`InstancedStaticMeshComponent.AddInstance` _output (`KismetMathLibrary.MakeTransform` (0.0 208.0 71.0)) false)
      ;[1 1 1] Vat Liquid
      (set `self.MeshType` (`|MakeArray` (`self.HISMC_VatLiquid`) (`self.HISMC_VatLiquid02`) :!type "InstancedStaticMeshComponent Object Reference"))
      (`InstancedStaticMeshComponent.AddInstance` _output (`KismetMathLibrary.MakeTransform` (0.0 208.0 71.0) (`KismetMathLibrary.MakeRotator` 0.0 0.0 (`self.Liquid Rotation`)) (`KismetMathLibrary.MakeVector` 1.0 1.0 (`self.Liquid Height Fraction`))) false)
      ;[1 1 1] Liquid Hue
      (bind _returnvalue (`PrimitiveComponent.CreateDynamicMaterialInstance` _output 0 "/Game/outsideArts/SteampunkWorkshop/Materials/Vat/MI_VatLiquid.MI_VatLiquid" "None"))
      (`MaterialInstanceDynamic.SetVectorParameterValue` _returnvalue "Liquid Hue 1" _liquid_hue_1)
      (`MaterialInstanceDynamic.SetVectorParameterValue` _returnvalue "Liquid Hue 4" (`self.Liquid Hue 4`))
      ;[1 1 1] Light
      (switch `/Game/outsideArts/SteampunkWorkshop/Blueprints/Enumerators/Vat/EVatType` _vat_type
        (:`NewEnumerator0`
          (set `self.Light Height` 225.0))
        (:`NewEnumerator1`
          (set `self.Light Height` 350.0)))
      (bind _returnvalue_2 (`AddComponent|NODE_AddPointLightComponent-0` :`RelativeTransform` (`KismetMathLibrary.MakeTransform` (`KismetMathLibrary.MakeVector` 0.0 208.0 (`self.Light Height`)))))
      (`LightComponent.SetLightColor` _returnvalue_2 _liquid_hue_1 true))
    (:`then_1`
      (if _mount_present_
        ;[1 1 1] VatPin01
        (switch `/Game/outsideArts/SteampunkWorkshop/Blueprints/Enumerators/Vat/EVatType` _vat_type
          (:`NewEnumerator0`
            (set `self.No Of VatPin01` 12))
          (:`NewEnumerator1`
            (set `self.No Of VatPin01` 24)))
        (for _index (range (+ (`self.No Of VatPin01`) 1))
          (bind _returnvalue_3 (+ (* (`KismetMathLibrary.Conv_IntToDouble` _index) 25.0) 35.0))
          (`InstancedStaticMeshComponent.AddInstance` _hismc_vatpin01 (`KismetMathLibrary.MakeTransform` (`KismetMathLibrary.MakeVector` 56.0 126.0 _returnvalue_3)) false)
          (`InstancedStaticMeshComponent.AddInstance` _hismc_vatpin01 (`KismetMathLibrary.MakeTransform` (`KismetMathLibrary.MakeVector` -56.0 126.0 _returnvalue_3)) false))))
    (:`then_2`
      ;[1 1 1] VatPin02
      (for _index_2 (range 12)
        (`InstancedStaticMeshComponent.AddInstance` (`self.HISMC_VatPin02`) (`KismetMathLibrary.MakeTransform` (0.0 208.0 0.0) (`KismetMathLibrary.MakeRotator` 0.0 0.0 (* (`KismetMathLibrary.Conv_IntToDouble` _index_2) 30.0))) false)))
    (:`then_3`
      ;[1 1 1] Vat Coil
      (switch `/Game/outsideArts/SteampunkWorkshop/Blueprints/Enumerators/Vat/EVatType` _vat_type
        (:`NewEnumerator0`
          (set `self.No Of Vat Coil` 7))
        (:`NewEnumerator1`
          (set `self.No Of Vat Coil` 19)))
      (for _index_3 (range (+ (`self.No Of Vat Coil`) 1))
        (`InstancedStaticMeshComponent.AddInstance` (`self.HISMC_VatCoil`) (`KismetMathLibrary.MakeTransform` (`KismetMathLibrary.MakeVector` 0.0 208.0 (+ (* (`KismetMathLibrary.Conv_IntToDouble` _index_3) 25.0) 80.0)) (struct) (1.25 1.25 1.0)) false)))
    (:`then_4`
      ;[1 1 1] Vat Rod
      (set `self.MeshType` (`|MakeArray` (`self.HISMC_VatRod`) (`self.HISMC_VatRod02`) :!type "InstancedStaticMeshComponent Object Reference"))
      (switch `/Game/outsideArts/SteampunkWorkshop/Blueprints/Enumerators/Vat/EVatType` _vat_type
        (:`NewEnumerator0`
          (set `self.VatRod Length Fraction` 1.05))
        (:`NewEnumerator1`
          (set `self.VatRod Length Fraction` 0.85)))
      (`InstancedStaticMeshComponent.AddInstance` _output (`KismetMathLibrary.MakeTransform` (0.0 208.0 70.0) (struct) (`KismetMathLibrary.MakeVector` 1.0 1.0 (`self.VatRod Length Fraction`))) false)
      ;[1 1 1] Vat Arc
      (set `self.MeshType` (`|MakeArray` (`self.HISMC_VatArc`) (`self.HISMC_VatArc02`) :!type "InstancedStaticMeshComponent Object Reference"))
      (switch `/Game/outsideArts/SteampunkWorkshop/Blueprints/Enumerators/Vat/EVatType` _vat_type
        (:`NewEnumerator0`
          (set `self.ArcSize` 1.0))
        (:`NewEnumerator1`
          (set `self.ArcSize` 1.1)))
      (`InstancedStaticMeshComponent.AddInstance` _output (`KismetMathLibrary.MakeTransform` (0.0 208.0 70.0) (struct) (`KismetMathLibrary.MakeVector` _arcsize _arcsize 1.05)) false))))