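; BP_Lathe is a configurable lathe prop assembled entirely in the Construction Script, with no active event logic.
; It adds light-fixture and stand instances plus two spot lights, then selects bed, treadle, headstock and tailstock variants from type variables.
; Each part is an instance on its own HISM component, and a clamped position variable slides the tailstock along the X axis.
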(fn `UserConstructionScript`
  ;[1 1 1] Lathe Light Components
  (`InstancedStaticMeshComponent.AddInstance` (`self.HISMC_LatheLight01`) (`KismetMathLibrary.MakeTransform` (0.0 0.0 0.0)) false)
  (bind _returnvalue (`AddComponent|NODE_AddSpotLightComponent-0` :`RelativeTransform` (`KismetMathLibrary.MakeTransform` (-100.0 0.0 350.0) (struct :`Pitch` -90.0))))
  (bind _returnvalue_2 (`AddComponent|NODE_AddSpotLightComponent-1` :`RelativeTransform` (`KismetMathLibrary.MakeTransform` (100.0 0.0 350.0) (struct :`Pitch` -90.0))))
  (`SpotLightComponent.SetOuterConeAngle` _returnvalue 30.0)
  (`SpotLightComponent.SetOuterConeAngle` _returnvalue_2 30.0)
  (`InstancedStaticMeshComponent.AddInstance` (`self.HISMC_LatheStand01`) (`KismetMathLibrary.MakeTransform` (0.0 0.0 0.0)) false)
  ;[1 1 1] Lathe Bed
  (switch `/Game/outsideArts/SteampunkWorkshop/Blueprints/Enumerators/Lathes/ELatheBed` (`self.Bed Type`)
    (:`NewEnumerator0`
      (`InstancedStaticMeshComponent.AddInstance` (`self.HISMC_LatheBed01`) (`KismetMathLibrary.MakeTransform` (0.0 0.0 100.0)) false))
    (:`NewEnumerator1`
      (`InstancedStaticMeshComponent.AddInstance` (`self.HISMC_LatheBed02`) (`KismetMathLibrary.MakeTransform` (0.0 0.0 100.0)) false))
    (:`NewEnumerator2`
      (`InstancedStaticMeshComponent.AddInstance` (`self.HISMC_LatheBed03`) (`KismetMathLibrary.MakeTransform` (0.0 0.0 100.0)) false)))
  ;[1 1 1] Treadle Type
  (switch `/Game/outsideArts/SteampunkWorkshop/Blueprints/Enumerators/Lathes/ELatheTradle` (`self.Treadle Type`)
    (:`NewEnumerator0`
      (`InstancedStaticMeshComponent.AddInstance` (`self.HISMC_LatheTreadle01`) (`KismetMathLibrary.MakeTransform` (0.0 0.0 0.0)) false))
    (:`NewEnumerator1`
      (`InstancedStaticMeshComponent.AddInstance` (`self.HISMC_LatheTreadle02`) (`KismetMathLibrary.MakeTransform` (0.0 0.0 0.0)) false)))
  ;[1 1 1] HeadStock Type
  (set `self.Headstock Mesh Type` (`|MakeArray` (`self.HISMC_LatheHeadstock01`) (`self.HISMC_LatheHeadstock02`) (`self.HISMC_LatheHeadstock03`) :!type "InstancedStaticMeshComponent Object Reference"))
  (`InstancedStaticMeshComponent.AddInstance` (`|GetArrayItem` (`self.Headstock Mesh Type`) (`KismetMathLibrary.Conv_ByteToInt` (`self.HeadStock Type`))) (`KismetMathLibrary.MakeTransform` (-155.0 0.0 121.0)) false)
  ;[1 1 1] Tailstock Type
  (set `self.Tailstock Mesh Type` (`|MakeArray` (`self.HISMC_LatheTailstock01`) (`self.HISMC_LatheTailstock02`) (`self.HISMC_LatheTailstock03`) :!type "InstancedStaticMeshComponent Object Reference"))
  (`InstancedStaticMeshComponent.AddInstance` (`|GetArrayItem` (`self.Tailstock Mesh Type`) (`KismetMathLibrary.Conv_ByteToInt` (`self.Tailstock Type`))) (`KismetMathLibrary.MakeTransform` (`KismetMathLibrary.MakeVector` (`KismetMathLibrary.FClamp` (`self.TailStock Position`) -30.0 170.0) 0.0 106.5)) false))