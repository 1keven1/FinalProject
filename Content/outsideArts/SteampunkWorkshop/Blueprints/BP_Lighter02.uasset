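; BP_Lighter02 is a modular steampunk workshop prop, a "lighter" machine assembled procedurally in its Construction Script.
; GeneratorType picks one of six generator meshes, and MachineType adds one of two static mesh machines above the stand.
; The stand, ring, rods, pins and arcs are hierarchical instanced mesh instances at fixed offsets, with loops placing rods and two tiers of pins radially around the generator.
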(fn `UserConstructionScript`
  (bind _hismc_lighterarc (`self.HISMC_LighterArc`))
  (bind _hismc_lighterpin (`self.HISMC_LighterPin`))
  (`|ExecutionSequence`
    (:`then_0`
      ;[1 1 1] Lighter Generators
      (set `self.Generator Mesh Type` (`|MakeArray` (`self.HISMC_Generator01`) (`self.HISMC_Generator02`) (`self.HISMC_Generator03`) (`self.HISMC_Generator04`) (`self.HISMC_Generator05`) (`self.HISMC_Generator06`)))
      (`InstancedStaticMeshComponent.AddInstance` (`|GetArrayItem` (`self.Generator Mesh Type`) (`KismetMathLibrary.Conv_ByteToInt` (`self.Generator Type`))) (`KismetMathLibrary.MakeTransform` (0.0 120.0 0.0)) false)
      ;[1 1 1] Lighter Stand
      (`InstancedStaticMeshComponent.AddInstance` (`self.HISMC_LighterStand02`) (`KismetMathLibrary.MakeTransform` (0.0 0.0 131.0)) false))
    (:`then_1`
      ;[1 1 1] Lighter Ring
      (`InstancedStaticMeshComponent.AddInstance` (`self.HISMC_LighterRing03`) (`KismetMathLibrary.MakeTransform` (0.0 120.0 185.0)) false))
    (:`then_2`
      ;[1 1 1] Lighter Rod 04
      (for _index (range 4)
        (`InstancedStaticMeshComponent.AddInstance` (`self.HISMC_LighterRod04`) (`KismetMathLibrary.MakeTransform` (0.0 120.0 0.0) (`KismetMathLibrary.MakeRotator` 0.0 0.0 (* (`KismetMathLibrary.Conv_IntToDouble` _index) 90.0))) false)))
    (:`then_3`
      ;[1 1 1] Lighter Pin
      (for _index_2 (range 12)
        (bind _returnvalue (* (`KismetMathLibrary.Conv_IntToDouble` _index_2) 30.0))
        (`InstancedStaticMeshComponent.AddInstance` _hismc_lighterpin (`KismetMathLibrary.MakeTransform` (0.0 120.0 154.0) (`KismetMathLibrary.MakeRotator` 0.0 0.0 _returnvalue) (1.0 1.0 0.6)) false)
        (`InstancedStaticMeshComponent.AddInstance` _hismc_lighterpin (`KismetMathLibrary.MakeTransform` (0.0 120.0 222.0) (`KismetMathLibrary.MakeRotator` 0.0 0.0 _returnvalue)) false)))
    (:`then_4`
      ;[1 1 1] Lighter02Machines
      (switch `/Game/outsideArts/SteampunkWorkshop/Blueprints/Enumerators/Lighter/ELighter01MachineType` (`self.MachineType`)
        (:`NewEnumerator0`
          (`AddComponent|NODE_AddStaticMeshComponent-0` :`RelativeTransform` (`KismetMathLibrary.MakeTransform` (0.0 0.0 256.0))))
        (:`NewEnumerator1`
          (`AddComponent|NODE_AddStaticMeshComponent-1` :`RelativeTransform` (`KismetMathLibrary.MakeTransform` (0.0 0.0 256.0))))))
    (:`then_5`
      ;[1 1 1] Ligher Arc
      (`InstancedStaticMeshComponent.AddInstance` _hismc_lighterarc (`KismetMathLibrary.MakeTransform` (-64.5 120.0 22.700001) (`KismetMathLibrary.MakeRotator` 0.0)) false)
      (`InstancedStaticMeshComponent.AddInstance` _hismc_lighterarc (`KismetMathLibrary.MakeTransform` (64.5 120.0 22.700001)) false)
      (`InstancedStaticMeshComponent.AddInstance` _hismc_lighterarc (`KismetMathLibrary.MakeTransform` (0.0 55.0 22.700001)) false)
      (`InstancedStaticMeshComponent.AddInstance` _hismc_lighterarc (`KismetMathLibrary.MakeTransform` (0.0 183.0 22.700001)) false))))