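; Steampunk Tesla coil prop actor assembled procedurally in the Construction Script from hierarchical instanced static mesh components, with no runtime logic.
; Fixed offsets place the base, generator, four-way mounts, charges, rods, spine, cannisters and arc meshes.
; Loops stack central and spine rings up the column, shrinking the upper ones into a taper.
; Type variables select the generator, charge, cannister and spine ring mesh variants by indexing component arrays.
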(fn `UserConstructionScript`
  (bind _hismc_tc2_mount (`self.HISMC_TC2_Mount`))
  (bind _hismc_tc2_centralring (`self.HISMC_TC2_CentralRing`))
  (bind _hismc_tc2_rod (`self.HISMC_TC2_Rod`))
  (bind _hismc_tc2_cannisterarc (`self.HISMC_TC2_CannisterArc`))
  (bind _returnvalue (`KismetMathLibrary.Sqrt` (/ (`KismetMathLibrary.Square` 120.0) 2.0)))
  (bind _output (`|GetArrayItem` (`self.Charge Mesh Type`) (`KismetMathLibrary.Conv_ByteToInt` (`self.Charge Type`))))
  (bind _output_2 (`|GetArrayItem` (`self.Cannister Mesh Type`) (`KismetMathLibrary.Conv_ByteToInt` (`self.Cannister Type`))))
  (bind _returnvalue_2 (* _returnvalue -1.0))
  (`|ExecutionSequence`
    (:`then_0`
      ;[1 1 1] Base
      (`InstancedStaticMeshComponent.AddInstance` (`self.HISMC_TC2_Base`) (`KismetMathLibrary.MakeTransform` (0.0 0.0 0.0)) false)
      ;[1 1 1] Generator Types
      (set `self.Generator Mesh Types` (`|MakeArray` (`self.HISMC_TL_Generator01`) (`self.HISMC_TL_Generator02`) (`self.HISMC_TL_Generator03`) (`self.HISMC_TL_Generator04`) (`self.HISMC_TL_Generator05`) (`self.HISMC_TL_Generator06`)))
      (`InstancedStaticMeshComponent.AddInstance` (`|GetArrayItem` (`self.Generator Mesh Types`) (`KismetMathLibrary.Conv_ByteToInt` (`self.Generator Type`))) (`KismetMathLibrary.MakeTransform` (0.0 0.0 83.0)) false)
      ;[1 1 1] Mount
      (`InstancedStaticMeshComponent.AddInstance` _hismc_tc2_mount (`KismetMathLibrary.MakeTransform` (0.0 80.0 0.0)) false)
      (`InstancedStaticMeshComponent.AddInstance` _hismc_tc2_mount (`KismetMathLibrary.MakeTransform` (0.0 -80.0 0.0) (struct :`Yaw` 180.0)) false)
      (`InstancedStaticMeshComponent.AddInstance` _hismc_tc2_mount (`KismetMathLibrary.MakeTransform` (80.0 0.0 0.0) (struct :`Yaw` -90.0)) false)
      (`InstancedStaticMeshComponent.AddInstance` _hismc_tc2_mount (`KismetMathLibrary.MakeTransform` (-80.0 0.0 0.0) (struct :`Yaw` 90.0)) false))
    (:`then_1`
      ;[1 1 1] Charge
      (set `self.Charge Mesh Type` (`|MakeArray` (`self.HISMC_TC2_Charge01`) (`self.HISMC_TC2_Charge02`) (`self.HISMC_TL_Charge03`)))
      (`InstancedStaticMeshComponent.AddInstance` _output (`KismetMathLibrary.MakeTransform` (0.0 130.0 5.9)) false)
      (`InstancedStaticMeshComponent.AddInstance` _output (`KismetMathLibrary.MakeTransform` (0.0 -130.0 5.9)) false)
      (`InstancedStaticMeshComponent.AddInstance` _output (`KismetMathLibrary.MakeTransform` (130.0 0.0 5.9)) false)
      (`InstancedStaticMeshComponent.AddInstance` _output (`KismetMathLibrary.MakeTransform` (-130.0 0.0 5.9)) false)
      ;[1 1 1] Spine
      (`InstancedStaticMeshComponent.AddInstance` (`self.HISMC_TC2_Spine`) (`KismetMathLibrary.MakeTransform` (0.0 0.0 215.0)) false)
      ;[1 1 1] Rod
      (`InstancedStaticMeshComponent.AddInstance` _hismc_tc2_rod (`KismetMathLibrary.MakeTransform` (`KismetMathLibrary.MakeVector` _returnvalue _returnvalue) (struct :`Yaw` -135.0)) false)
      (`InstancedStaticMeshComponent.AddInstance` _hismc_tc2_rod (`KismetMathLibrary.MakeTransform` (`KismetMathLibrary.MakeVector` _returnvalue_2 _returnvalue_2) (struct :`Yaw` 45.0)) false)
      (`InstancedStaticMeshComponent.AddInstance` _hismc_tc2_rod (`KismetMathLibrary.MakeTransform` (`KismetMathLibrary.MakeVector` _returnvalue _returnvalue_2) (struct :`Yaw` 135.0)) false)
      (`InstancedStaticMeshComponent.AddInstance` _hismc_tc2_rod (`KismetMathLibrary.MakeTransform` (`KismetMathLibrary.MakeVector` _returnvalue_2 _returnvalue) (struct :`Yaw` -45.0)) false)
      ;[1 1 1] Central Arc
      (`InstancedStaticMeshComponent.AddInstance` (`self.HISMC_TC2_CentralArc`) (`KismetMathLibrary.MakeTransform` (0.0 0.0 257.0)) false)
      ;[1 1 1] SpineArc
      (`InstancedStaticMeshComponent.AddInstance` (`self.HISMC_TC2_SpineArc`) (`KismetMathLibrary.MakeTransform` (0.0 0.0 407.0)) false))
    (:`then_2`
      ;[1 1 1] Central Ring
      (for _index (range 9)
        (`InstancedStaticMeshComponent.AddInstance` _hismc_tc2_centralring (`KismetMathLibrary.MakeTransform` (`KismetMathLibrary.MakeVector` 0.0 0.0 (+ (* (`KismetMathLibrary.Conv_IntToDouble` _index) 11.0) 278.0))) false)))
    (:`then_3`
      (for _index_2 (range 19)
        (bind _returnvalue_3 (`KismetMathLibrary.Conv_IntToDouble` _index_2))
        (`InstancedStaticMeshComponent.AddInstance` _hismc_tc2_centralring (`KismetMathLibrary.MakeTransform` (`KismetMathLibrary.MakeVector` 0.0 0.0 (+ (* _returnvalue_3 15.0) 420.0)) (struct) (`KismetMathLibrary.Conv_DoubleToVector` (+ (* _returnvalue_3 -0.025) 1.0))) false)))
    (:`then_4`
      ;[1 1 1] Cannisters
      (set `self.Cannister Mesh Type` (`|MakeArray` (`self.HISMC_TC2_Cannister01`) (`self.HISMC_TC2_Cannister02`)))
      (`InstancedStaticMeshComponent.AddInstance` _output_2 (`KismetMathLibrary.MakeTransform` (0.0 50.0 256.5)) false)
      (`InstancedStaticMeshComponent.AddInstance` _output_2 (`KismetMathLibrary.MakeTransform` (0.0 -50.0 256.5)) false)
      (`InstancedStaticMeshComponent.AddInstance` _output_2 (`KismetMathLibrary.MakeTransform` (50.0 0.0 256.5)) false)
      (`InstancedStaticMeshComponent.AddInstance` _output_2 (`KismetMathLibrary.MakeTransform` (-50.0 0.0 256.5)) false)
      (`InstancedStaticMeshComponent.AddInstance` _hismc_tc2_cannisterarc (`KismetMathLibrary.MakeTransform` (0.0 50.0 276.5)) false)
      (`InstancedStaticMeshComponent.AddInstance` _hismc_tc2_cannisterarc (`KismetMathLibrary.MakeTransform` (0.0 -50.0 276.5)) false)
      (`InstancedStaticMeshComponent.AddInstance` _hismc_tc2_cannisterarc (`KismetMathLibrary.MakeTransform` (50.0 0.0 276.5)) false)
      (`InstancedStaticMeshComponent.AddInstance` _hismc_tc2_cannisterarc (`KismetMathLibrary.MakeTransform` (-50.0 0.0 276.5)) false))
    (:`then_5`
      ;[1 1 1] Spine Ring 01
      (for _index_3 (range 5)
        (bind _returnvalue_4 (`KismetMathLibrary.Conv_IntToDouble` _index_3))
        (`InstancedStaticMeshComponent.AddInstance` (`self.HISMC_TC2_SpineRing04`) (`KismetMathLibrary.MakeTransform` (`KismetMathLibrary.MakeVector` 0.0 0.0 (+ (- (* _returnvalue_4 80.0) (* _returnvalue_4 20.0)) 440.0)) (struct) (`KismetMathLibrary.Conv_DoubleToVector` (+ (* _returnvalue_4 -0.12) 1.0))) false)))
    (:`then_6`
      ;[1 1 1] Spine Ring 02
      (for _index_4 (range 1 5)
        (set `self.Spine Ring Mesh Type` (`|MakeArray` (`self.HISMC_TC2_SpineRing01`) (`self.HISMC_TC2_SpineRing02`) (`self.HISMC_TC2_SpineRing03`)))
        (bind _returnvalue_5 (`KismetMathLibrary.Conv_IntToDouble` _index_4))
        (`InstancedStaticMeshComponent.AddInstance` (`|GetArrayItem` (`self.Spine Ring Mesh Type`) (`KismetMathLibrary.Conv_ByteToInt` (`self.Spine Ring Type`))) (`KismetMathLibrary.MakeTransform` (`KismetMathLibrary.MakeVector` 0.0 0.0 (+ (- (- (* _returnvalue_5 80.0) (* _returnvalue_5 20.0)) (- 40.0 10.0)) 440.0)) (struct) (`KismetMathLibrary.Conv_DoubleToVector` (+ (- (* _returnvalue_5 -0.12) -0.06) 1.0))) false)))
    (:`then_7`
      ;[1 1 1] Spine Ring Arc
      (for _index_5 (range 9)
        (bind _returnvalue_6 (`KismetMathLibrary.Conv_IntToDouble` _index_5))
        (`InstancedStaticMeshComponent.AddInstance` (`self.HISMC_TC2_SpineRingArc`) (`KismetMathLibrary.MakeTransform` (`KismetMathLibrary.MakeVector` 0.0 0.0 (+ (- (* _returnvalue_6 40.0) (* _returnvalue_6 10.0)) 440.0)) (`KismetMathLibrary.MakeRotator` 0.0 0.0 (* _returnvalue_6 60.0)) (`KismetMathLibrary.Conv_DoubleToVector` (+ (* _returnvalue_6 -0.06) 1.0))) false)))))