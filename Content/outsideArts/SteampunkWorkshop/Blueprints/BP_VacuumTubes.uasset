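; BP_VacuumTubes is a steampunk workshop prop that builds one of three vacuum tube variants, chosen by VacuumTubeType.
; The construction script adds tube, glass and current arc meshes as hierarchical instanced static mesh instances, with the first two types sharing a glass mesh.
; Type 02 stacks rotated arcs in a rising loop, while Type 03 places four pillars and arcs around the center.
; The event graph has no active logic.
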(fn `UserConstructionScript`
  (bind _vacuum_tube_type (`self.Vacuum Tube Type`))
  (bind _hismc_vacuumglass01 (`self.HISMC_VacuumGlass01`))
  (bind _hismc_vacuumpiller (`self.HISMC_VacuumPiller`))
  (bind _hismc_vacuumarc03 (`self.HISMC_VacuumArc03`))
  (bind _output (`|GetArrayItem` (`self.Mesh Type`) (`KismetMathLibrary.Conv_ByteToInt` _vacuum_tube_type)))
  ;[1 1 1] Instanced Vacuum Tube
  (set `self.Mesh Type` (`|MakeArray` (`self.HISMC_VacuumTube01`) (`self.HISMC_VacuumTube02`) (`self.HISMC_VacuumTube03`) :!type "InstancedStaticMeshComponent Object Reference"))
  (`InstancedStaticMeshComponent.AddInstance` _output (`KismetMathLibrary.MakeTransform` (0.0 0.0 0.0)) false)
  ;[1 1 1] Instanced Vacuum Glass
  (set `self.Mesh Type` (`|MakeArray` _hismc_vacuumglass01 _hismc_vacuumglass01 (`self.HISMC_VacuumGlass02`) :!type "InstancedStaticMeshComponent Object Reference"))
  (switch `/Game/outsideArts/SteampunkWorkshop/Blueprints/Enumerators/VacuumTubes/EVacuumTubeType` _vacuum_tube_type
    (:`NewEnumerator0`
      _)
    (:`NewEnumerator1`
      _)
    (:`NewEnumerator2`
      (`InstancedStaticMeshComponent.AddInstance` _hismc_vacuumpiller (`KismetMathLibrary.MakeTransform` (0.0 -42.0 21.0)) false)
      (`InstancedStaticMeshComponent.AddInstance` _hismc_vacuumpiller (`KismetMathLibrary.MakeTransform` (0.0 42.0 21.0) (struct :`Yaw` 180.0)) false)
      (`InstancedStaticMeshComponent.AddInstance` _hismc_vacuumpiller (`KismetMathLibrary.MakeTransform` (42.0 0.0 21.0) (struct :`Yaw` 90.0)) false)
      (`InstancedStaticMeshComponent.AddInstance` _hismc_vacuumpiller (`KismetMathLibrary.MakeTransform` (-42.0 0.0 21.0) (struct :`Yaw` -90.0)) false)))
  (`InstancedStaticMeshComponent.AddInstance` _output (`KismetMathLibrary.MakeTransform` (0.0 0.0 21.0)) false)
  ;[1 1 1] Instanced Vacuum Current Arc
  (switch `/Game/outsideArts/SteampunkWorkshop/Blueprints/Enumerators/VacuumTubes/EVacuumTubeType` _vacuum_tube_type
    (:`NewEnumerator0`
      (`InstancedStaticMeshComponent.AddInstance` (`self.HISMC_VacuumArc01`) (`KismetMathLibrary.MakeTransform` (0.0 0.0 20.0)) false))
    (:`NewEnumerator1`
      (for _index (range 6)
        (`InstancedStaticMeshComponent.AddInstance` (`self.HISMC_VacuumArc02`) (`KismetMathLibrary.MakeTransform` (`KismetMathLibrary.MakeVector` 0.0 0.0 (+ (* _index 10.0) 90.0)) (`KismetMathLibrary.MakeRotator` 0.0 0.0 (* _index 45.0))) false)))
    (:`NewEnumerator2`
      (`InstancedStaticMeshComponent.AddInstance` _hismc_vacuumarc03 (`KismetMathLibrary.MakeTransform` (0.0 -42.0 21.0)) false)
      (`InstancedStaticMeshComponent.AddInstance` _hismc_vacuumarc03 (`KismetMathLibrary.MakeTransform` (0.0 42.0 21.0) (struct :`Yaw` 180.0)) false)
      (`InstancedStaticMeshComponent.AddInstance` _hismc_vacuumarc03 (`KismetMathLibrary.MakeTransform` (42.0 0.0 21.0) (struct :`Yaw` 90.0)) false)
      (`InstancedStaticMeshComponent.AddInstance` _hismc_vacuumarc03 (`KismetMathLibrary.MakeTransform` (-42.0 0.0 21.0) (struct :`Yaw` -90.0)) false))))