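; BP_LatheMount is a construction-script prop that assembles a steampunk workshop lathe mount from hierarchical instanced static meshes.
; A Height enum picks the matching pillar, belt and generator mount variants and sets the vertical offset for beams, upper wheel, axle and generator.
; A separate GeneratorType enum selects the generator mesh, and the event graph holds no runtime logic.
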(fn `UserConstructionScript`
  (bind _hismc_lathebeam01 (`self.HISMC_LatheBeam01`))
  (bind _hismc_lathebeam02 (`self.HISMC_LatheBeam02`))
  (bind _height (`self.Height`))
  (bind _meshheight (`self.MeshHeight`))
  (bind _output (`|GetArrayItem` (`self.LatheMountMeshType`) (`KismetMathLibrary.Conv_ByteToInt` _height)))
  ;[1 1 1] LathePillar
  (set `self.LatheMountMeshType` (`|MakeArray` (`self.HISMC_LathePillar01`) (`self.HISMC_LathePillar02`) :!type "InstancedStaticMeshComponent Object Reference"))
  (`InstancedStaticMeshComponent.AddInstance` _output (`KismetMathLibrary.MakeTransform` (243.0 55.0 0.0)) false)
  (`InstancedStaticMeshComponent.AddInstance` _output (`KismetMathLibrary.MakeTransform` (-250.0 55.0 0.0)) false)
  (`InstancedStaticMeshComponent.AddInstance` _output (`KismetMathLibrary.MakeTransform` (-250.0 -55.0 0.0)) false)
  (`InstancedStaticMeshComponent.AddInstance` _output (`KismetMathLibrary.MakeTransform` (243.0 -55.0 0.0)) false)
  ;[1 1 1] MeshHeight
  (switch `/Game/outsideArts/SteampunkWorkshop/Blueprints/Enumerators/LatheMount/EMountHeight` _height
    (:`NewEnumerator0`
      (set `self.MeshHeight` 250.0))
    (:`NewEnumerator1`
      (set `self.MeshHeight` 325.0)))
  ;[1 1 1] LatheBeam01
  (`InstancedStaticMeshComponent.AddInstance` _hismc_lathebeam01 (`KismetMathLibrary.MakeTransform` (`KismetMathLibrary.MakeVector` 0.0 55.0 _meshheight)) false)
  (`InstancedStaticMeshComponent.AddInstance` _hismc_lathebeam01 (`KismetMathLibrary.MakeTransform` (`KismetMathLibrary.MakeVector` 0.0 -55.0 _meshheight) (struct :`Roll` 180.0)) false)
  ;[1 1 1] LatheBeam 02
  (`InstancedStaticMeshComponent.AddInstance` _hismc_lathebeam02 (`KismetMathLibrary.MakeTransform` (`KismetMathLibrary.MakeVector` 243.0 0.0 _meshheight)) false)
  (`InstancedStaticMeshComponent.AddInstance` _hismc_lathebeam02 (`KismetMathLibrary.MakeTransform` (`KismetMathLibrary.MakeVector` -250.0 0.0 _meshheight) (struct :`Pitch` 180.0)) false)
  ;[1 1 1] LatheWheels
  (`InstancedStaticMeshComponent.AddInstance` (`self.HISMC_LatheWheel01`) (`KismetMathLibrary.MakeTransform` (234.0 0.0 39.273998)) false)
  (`InstancedStaticMeshComponent.AddInstance` (`self.HISMC_LatheWheel02`) (`KismetMathLibrary.MakeTransform` (`KismetMathLibrary.MakeVector` 234.0 0.0 _meshheight)) false)
  ;[1 1 1] LatheAxle
  (`InstancedStaticMeshComponent.AddInstance` (`self.HISMC_LatheAxle`) (`KismetMathLibrary.MakeTransform` (`KismetMathLibrary.MakeVector` 0.0 0.0 _meshheight)) false)
  ;[1 1 1] LatheBelt
  (set `self.LatheMountMeshType` (`|MakeArray` (`self.HISMC_LatheBelt01`) (`self.HISMC_LatheBelt02`) :!type "InstancedStaticMeshComponent Object Reference"))
  (`InstancedStaticMeshComponent.AddInstance` _output (`KismetMathLibrary.MakeTransform` (234.0 0.0 39.273998)) false)
  ;[1 1 1] LatheGenerator
  (set `self.GeneratorMeshType` (`|MakeArray` (`self.HISMC_LatheGenerator01`) (`self.HISMC_LatheGenerator02`) :!type "InstancedStaticMeshComponent Object Reference"))
  (`InstancedStaticMeshComponent.AddInstance` (`|GetArrayItem` (`self.GeneratorMeshType`) (`KismetMathLibrary.Conv_ByteToInt` (`self.Generator Type`))) (`KismetMathLibrary.MakeTransform` (`KismetMathLibrary.MakeVector` 0.0 0.0 _meshheight)) false)
  (set `self.LatheMountMeshType` (`|MakeArray` (`self.HISMC_LatheGeneratorMount01`) (`self.HISMC_LatheGeneratorMount02`) :!type "InstancedStaticMeshComponent Object Reference"))
  (`InstancedStaticMeshComponent.AddInstance` _output (`KismetMathLibrary.MakeTransform` (0.0 0.0 0.0)) false))