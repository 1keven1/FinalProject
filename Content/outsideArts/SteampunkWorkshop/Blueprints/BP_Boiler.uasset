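; Modular steampunk boiler prop, assembled entirely in the construction script with no active event logic.
; Fixed face, exhaust and spot light surround a body of repeated side and base instances, sized by BoilerSections (clamped) and capped with a rear piece.
; Type selectors index arrays of HISMC components to choose mesh variants for the paired feeds, ash pits and gauges, plus a single safety valve, all at hardcoded offsets.
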(fn `UserConstructionScript`
  (bind _returnvalue (`KismetMathLibrary.Clamp` (`self.Boiler Sections`) 1 4))
  (bind _output (`|GetArrayItem` (`self.Mesh Type`) (`KismetMathLibrary.Conv_ByteToInt` (`self.Boiler Gauge Type`))))
  (bind _output_2 (`|GetArrayItem` (`self.Mesh Type`) (`KismetMathLibrary.Conv_ByteToInt` (`self.Boiler Feed `))))
  (bind _output_3 (`|GetArrayItem` (`self.Mesh Type`) (`KismetMathLibrary.Conv_ByteToInt` (`self.Ash Pit Type`))))
  (`|ExecutionSequence`
    (:`then_0`
      ;[1 1 1] Instanced Boiler Face
      (`InstancedStaticMeshComponent.AddInstance` (`self.HISMC_BoilerFace`) (`KismetMathLibrary.MakeTransform` (0.0 150.0 0.0)) false))
    (:`then_1`
      ;[1 1 1] Instanced Boiler Side
      (for _index (range (+ _returnvalue 1))
        (bind _returnvalue_2 (* _index -150.0))
        (`InstancedStaticMeshComponent.AddInstance` (`self.HISMC_BoilerSide`) (`KismetMathLibrary.MakeTransform` (`KismetMathLibrary.MakeVector` 0.0 _returnvalue_2)) false)
        (`InstancedStaticMeshComponent.AddInstance` (`self.HISMC_BoilerBase`) (`KismetMathLibrary.MakeTransform` (`KismetMathLibrary.MakeVector` 0.0 (+ _returnvalue_2 75.0)) (`KismetMathLibrary.MakeRotator` 0.0 0.0 180.0)) false)))
    (:`then_2`
      ;[1 1 1] Instanced Base Rear
      (`InstancedStaticMeshComponent.AddInstance` (`self.HISMC_BaseRear`) (`KismetMathLibrary.MakeTransform` (`KismetMathLibrary.MakeVector` 0.0 (* _returnvalue -150.0))) false))
    (:`then_3`
      ;[1 1 1] Instanced Boiler Feed
      (set `self.Mesh Type` (`|MakeArray` (`self.HISMC_BoilerFeed01`) (`self.HISMC_BoilerFeed02`) (`self.HISMC_BoilerFeed03`) :!type "InstancedStaticMeshComponent Object Reference"))
      (`InstancedStaticMeshComponent.AddInstance` _output_2 (`KismetMathLibrary.MakeTransform` (-67.0 207.279999 135.0)) false)
      (`InstancedStaticMeshComponent.AddInstance` _output_2 (`KismetMathLibrary.MakeTransform` (67.0 207.279999 135.0)) false))
    (:`then_4`
      ;[1 1 1] Instanced Boiler Ash Pit
      (set `self.Mesh Type` (`|MakeArray` (`self.HISMC_BoilerAshPit01`) (`self.HISMC_BoilerAshPit02`) (`self.HISMC_BoilerAshPit03`) :!type "InstancedStaticMeshComponent Object Reference"))
      (`InstancedStaticMeshComponent.AddInstance` _output_3 (`KismetMathLibrary.MakeTransform` (-8.0 187.5 98.0) (struct :`Roll` 10.0)) false)
      (`InstancedStaticMeshComponent.AddInstance` _output_3 (`KismetMathLibrary.MakeTransform` (8.0 187.5 98.0) (struct :`Roll` 10.0)) false))
    (:`then_5`
      ;[1 1 1] Instanced Boiler Gauge
      (set `self.Mesh Type` (`|MakeArray` (`self.HISMC_BoilerGauge01`) (`self.HISMC_BoilerGauge02`) (`self.HISMC_BoilerGauge03`) (`self.HISMC_BoilerGauge04`) :!type "InstancedStaticMeshComponent Object Reference"))
      (`InstancedStaticMeshComponent.AddInstance` _output (`KismetMathLibrary.MakeTransform` (-23.5 192.399994 270.0) (struct :`Pitch` 15.0)) false)
      (`InstancedStaticMeshComponent.AddInstance` _output (`KismetMathLibrary.MakeTransform` (23.5 192.399994 270.0) (struct :`Pitch` -15.0)) false))
    (:`then_6`
      ;[1 1 1] Instanced Boiler Exhaust
      (`InstancedStaticMeshComponent.AddInstance` (`self.HISMC_BoilerExhaust01`) (`KismetMathLibrary.MakeTransform` (0.0 180.0 402.0)) false))
    (:`then_7`
      ;[1 1 1] Boiler Light
      (`AddComponent|NODE_AddSpotLightComponent-0` :`RelativeTransform` (`KismetMathLibrary.MakeTransform` (0.0 350.0 350.0) (struct :`Pitch` -45.0 :`Yaw` -90.0 :`Roll` -180.0))))
    (:`then_8`
      ;[1 1 1] Instanced Boiler Valve Type
      (set `self.Mesh Type` (`|MakeArray` (`self.HISMC_BoilerValve01`) (`self.HISMC_BoilerValve02`) (`self.HISMC_BoilerValve03`) :!type "InstancedStaticMeshComponent Object Reference"))
      (`InstancedStaticMeshComponent.AddInstance` (`|GetArrayItem` (`self.Mesh Type`) (`KismetMathLibrary.Conv_ByteToInt` (`self.Safety Valve Type`))) (`KismetMathLibrary.MakeTransform` (0.0 100.0 500.0)) false))))