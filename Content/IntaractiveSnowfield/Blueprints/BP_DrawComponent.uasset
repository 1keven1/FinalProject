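; BP_DrawComponent registers itself as a drawer with the snow actors manager in the interactive snowfield.
; On BeginPlay it finds BP_SnowActorsManager, then caches its world XY position and yaw, or prints a warning if no manager exists.
; NeedDrawing adds the component to the manager's Drawers collection; the drawing itself is not done here.
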(event `self.ReceiveBeginPlay`
  (bind _returnvalue (`self.K2_GetComponentToWorld`))
  (bind _returnvalue_2 (`GameplayStatics.GetActorOfClass` "/Game/IntaractiveSnowfield/Blueprints/BP_SnowActorsManager.BP_SnowActorsManager_C"))
  (set `self.Manager` _returnvalue_2)
  (`/Engine/EditorBlueprintResources/StandardMacros.IsValid` _returnvalue_2
    (:`Is Valid`
      (set `self.Position` (`KismetMathLibrary.Conv_VectorToVector2D` (.location _returnvalue)))
      (set `self.Rotation` (.yaw (.rotation _returnvalue))))
    (:`Is Not Valid`
      (`KismetSystemLibrary.PrintString` "You need a SnowActor Manager"))))

(event `NeedDrawing`
  (`KismetArrayLibrary.Array_Add` (`/Game/IntaractiveSnowfield/Blueprints/BP_SnowActorsManager.Drawers` (`self.Manager`)) self))