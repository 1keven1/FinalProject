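; BP_DeBugReader_RT is a debug actor that displays an interactive snowfield's intermediate textures on five planes.
; One second after BeginPlay, if Target is valid, it reads that object's CurrentFrame, Save, Drawn, Edged and Blured textures.
; SetMat gives each plane a dynamic instance of M_DeBugMat with its texture bound to the Texture parameter.
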(event `self.ReceiveBeginPlay`
  (bind _target (`self.Target`))
  (`/Engine/EditorBlueprintResources/StandardMacros.IsValid` _target
    (:`Is Valid`
      (`KismetSystemLibrary.Delay` 1.0)
      (`self.SetMat` (`/Game/IntaractiveSnowfield/Blueprints/BP_SnowActor.CurrentFrame` _target) (`self.Plane`))
      (`self.SetMat` (`/Game/IntaractiveSnowfield/Blueprints/BP_SnowActor.Save` _target) (`self.Plane1`))
      (`self.SetMat` (`/Game/IntaractiveSnowfield/Blueprints/BP_SnowActor.Drawn` _target) (`self.Plane2`))
      (`self.SetMat` (`/Game/IntaractiveSnowfield/Blueprints/BP_SnowActor.Edged` _target) (`self.Plane3`))
      (`self.SetMat` (`/Game/IntaractiveSnowfield/Blueprints/BP_SnowActor.Blured` _target) (`self.Plane4`)))))

(fn `SetMat`
  (params (Texture :type "Texture Object Reference") (Plane :type "PrimitiveComponent Object Reference"))
  (bind _returnvalue (`KismetMaterialLibrary.CreateDynamicMaterialInstance` "/Game/IntaractiveSnowfield/Materials/M_DeBugMat.M_DeBugMat"))
  (`MaterialInstanceDynamic.SetTextureParameterValue` _returnvalue "Texture" Texture)
  (`PrimitiveComponent.SetMaterial` Plane 0 _returnvalue))

(fn `UserConstructionScript`)