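; BP_SnowActor builds the deformation textures for an interactive snowfield, accumulating marks from a Drawers list in a world-space area around the actor.
; Each Draw stamps the drawers additively into a current-frame render target, then merges it with saved history, offset by the actor's movement.
; The result is copied back as history, then edge and blur materials produce the final target.
; With IsLandActor, position updates snap to texel size.
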(event `self.ReceiveBeginPlay`
  (`self.CreateRTandMat`)
  ;[1 1 1] R=0
  (`KismetRenderingLibrary.ClearRenderTarget2D` (`self.CurrentFrame`))
  ;[1 1 1] R=1
  (`KismetRenderingLibrary.ClearRenderTarget2D` (`self.Drawn`) (struct :`R` 1.0 :`G` 1.0 :`B` 1.0 :`A` 1.0))
  ;[1 1 1] R=1
  (`KismetRenderingLibrary.ClearRenderTarget2D` (`self.Save`) (struct :`R` 1.0 :`G` 1.0 :`B` 1.0 :`A` 1.0))
  ;[1 1 1] R=0.5
  (`KismetRenderingLibrary.ClearRenderTarget2D` (`self.Edged`) (struct :`R` 0.5 :`G` 0.5 :`B` 0.5 :`A` 1.0))
  ;[1 1 1] R=0.5
  (`KismetRenderingLibrary.ClearRenderTarget2D` (`self.Blured`) (struct :`R` 0.5 :`G` 0.5 :`B` 0.5 :`A` 1.0))
  (`self.Draw`))

(event `Draw`
  (bind _currentframe (`self.CurrentFrame`))
  (bind _drawmat (`self.DrawMat`))
  (bind (_x _y) (`KismetMathLibrary.BreakVector2D` (/ (- (`self.Position`) (`self.LastPosition`)) (`self.RTSize（world size）`))))
  ;[1 1 1] Draw signets in this fram/绘制这一帧的图案
  (`KismetRenderingLibrary.ClearRenderTarget2D` _currentframe)
  (bind (_canvas _size _context) (`KismetRenderingLibrary.BeginDrawCanvasToRenderTarget` _currentframe))
  (for _array_element (`self.Drawers`)
    (`self.DrawToCurrentFrame` _canvas _array_element))
  ;[1 1 1] Draw current and save to drawn
  (`KismetRenderingLibrary.EndDrawCanvasToRenderTarget` _context)
  (`MaterialInstanceDynamic.SetScalarParameterValue` _drawmat "Uoffset" _x)
  (`MaterialInstanceDynamic.SetScalarParameterValue` _drawmat "Voffset" _y)
  (`KismetRenderingLibrary.DrawMaterialToRenderTarget` (`self.Drawn`) _drawmat)
  (`KismetRenderingLibrary.DrawMaterialToRenderTarget` (`self.Save`) (`self.CopyMat`))
  (`KismetRenderingLibrary.DrawMaterialToRenderTarget` (`self.Edged`) (`self.EdgeMat`))
  (`KismetRenderingLibrary.DrawMaterialToRenderTarget` (`self.Blured`) (`self.BlurMat`))
  (set `self.LastPosition` (`self.Position`))
  (`self.DrawFinished`))

(event `self.ReceiveTick`
  (params (DeltaSeconds :type "Float (single-precision)"))
  ;[1 1 1] Update position
  (if (`self.UpdatePositionEveryFrame`)
    (set `self.Position` (`self.UpDatePosition`))))

(event `DrawFinished`)

(fn `CreateRTandMat`
  (bind _edgeoffsetwidth (`self.EdgeOffsetWidth`))
  (bind _drawmat (`self.DrawMat`))
  (bind _copymat (`self.CopyMat`))
  (bind _edgemat (`self.EdgeMat`))
  (bind _blurmat (`self.BlurMat`))
  (bind _drawn (`self.Drawn`))
  (bind _blurwidth (`self.BlurWidth`))
  (bind _rtsize_world_size_ (`self.RTSize（world size）`))
  (bind (_rtsize_world_size__x _rtsize_world_size__y) (`KismetMathLibrary.BreakVector2D` (`self.RTSize（world size）`)))
  (bind (_returnvalue_x _returnvalue_y) (`KismetMathLibrary.BreakVector2D` (/ _rtsize_world_size_ (`self.PixelWidth_Blured`))))
  (bind (_returnvalue_x_2 _returnvalue_y_2) (`KismetMathLibrary.BreakVector2D` (/ _rtsize_world_size_ (`self.PixelWidth_Save`))))
  (bind _returnvalue (`KismetMathLibrary.FTrunc` _returnvalue_x_2))
  (bind _returnvalue_2 (`KismetMathLibrary.FTrunc` _returnvalue_y_2))
  (`|ExecutionSequence`
    (:`then_0`
      (bind _returnvalue_3 (`KismetRenderingLibrary.CreateRenderTarget2D` _returnvalue _returnvalue_2 "RTF_R8"))
      (set `self.CurrentFrame` _returnvalue_3))
    (:`then_1`
      (bind _returnvalue_4 (`KismetMaterialLibrary.CreateDynamicMaterialInstance` "/Game/IntaractiveSnowfield/Materials/MI_RT_Draw.MI_RT_Draw"))
      (set `self.DrawMat` _returnvalue_4)
      (bind _returnvalue_5 (`KismetRenderingLibrary.CreateRenderTarget2D` _returnvalue _returnvalue_2 "RTF_R8" (struct :`R` 1.0 :`G` 1.0 :`B` 1.0 :`A` 1.0)))
      (set `self.Drawn` _returnvalue_5))
    (:`then_2`
      (bind _returnvalue_6 (`KismetMaterialLibrary.CreateDynamicMaterialInstance` "/Game/IntaractiveSnowfield/Materials/M_RT_Copy.M_RT_Copy"))
      (set `self.CopyMat` _returnvalue_6)
      (bind _returnvalue_7 (`KismetRenderingLibrary.CreateRenderTarget2D` _returnvalue _returnvalue_2 "RTF_R8" (struct :`R` 1.0 :`G` 1.0 :`B` 1.0 :`A` 1.0)))
      (set `self.Save` _returnvalue_7))
    (:`then_3`
      (bind _returnvalue_8 (`KismetMaterialLibrary.CreateDynamicMaterialInstance` (`self.DrawEdge_Inst`)))
      (set `self.EdgeMat` _returnvalue_8)
      (bind _returnvalue_9 (`KismetRenderingLibrary.CreateRenderTarget2D` _returnvalue _returnvalue_2 "RTF_R8" (struct :`R` 1.0 :`G` 1.0 :`B` 1.0 :`A` 1.0)))
      (set `self.Edged` _returnvalue_9))
    (:`then_4`
      (bind _returnvalue_10 (`KismetMaterialLibrary.CreateDynamicMaterialInstance` (`self.Blur_Inst`)))
      (set `self.BlurMat` _returnvalue_10)
      (if (`self.SpecificBluredRT`)
        (set `self.Blured` (`self.NewBlurdRT`))
        (else
          (bind _returnvalue_11 (`KismetRenderingLibrary.CreateRenderTarget2D` (`KismetMathLibrary.FTrunc` _returnvalue_x) (`KismetMathLibrary.FTrunc` _returnvalue_y) "RTF_R8" (struct :`R` 1.0 :`G` 1.0 :`B` 1.0 :`A` 1.0) true))
          (set `self.Blured` _returnvalue_11))))
    (:`then_5`
      ;[1 1 1] Initialization/初始化
      (`MaterialInstanceDynamic.SetTextureParameterValue` _drawmat "SaveTexture" (`self.Save`))
      (`MaterialInstanceDynamic.SetTextureParameterValue` _drawmat "CurrentFrameTexture" (`self.CurrentFrame`))
      (`MaterialInstanceDynamic.SetTextureParameterValue` _copymat "Texture" _drawn)
      (`MaterialInstanceDynamic.SetTextureParameterValue` _edgemat "Texture" _drawn)
      (`MaterialInstanceDynamic.SetTextureParameterValue` _blurmat "Texture" (`self.Edged`))
      (`MaterialInstanceDynamic.SetScalarParameterValue` _edgemat "DistanceU" (/ _edgeoffsetwidth _rtsize_world_size__x))
      (`MaterialInstanceDynamic.SetScalarParameterValue` _edgemat "DistanceV" (/ _edgeoffsetwidth _rtsize_world_size__y))
      (`MaterialInstanceDynamic.SetScalarParameterValue` _blurmat "DistanceU" (/ _blurwidth _rtsize_world_size__x))
      (`MaterialInstanceDynamic.SetScalarParameterValue` _blurmat "DistanceV" (/ _blurwidth _rtsize_world_size__y))
      (`MaterialInstanceDynamic.SetScalarParameterValue` _blurmat "HeightOffset" (`self.HeightOffset`))
      (`MaterialInstanceDynamic.SetScalarParameterValue` _copymat "BoxMask" (`KismetMathLibrary.Conv_BoolToDouble` (`self.IsLandActor?`)))
      (`MaterialInstanceDynamic.SetScalarParameterValue` _drawmat "BoxMask" (`KismetMathLibrary.Conv_BoolToDouble` (`self.IsLandActor?`))))))

(fn `DrawToCurrentFrame`
  (params (Canvas :type "Canvas Object Reference") (DrawInfo :type "/Game/IntaractiveSnowfield/Structs/S_DrawInfor Structure"))
  (bind (_position _texture _size _rotation _depth) (break `/Game/IntaractiveSnowfield/Structs/S_DrawInfor` DrawInfo))
  (bind _pixelwidth_save (`self.PixelWidth_Save`))
  (bind _returnvalue (/ _size _pixelwidth_save))
  (`Canvas.K2_DrawTexture` Canvas _texture (+ (/ (+ (`KismetMathLibrary.GetRotated2D` (- _position (`self.Position`)) (`self.Rotation`)) (/ (`self.RTSize（world size）`) 2.0)) _pixelwidth_save) (- (0.0 0.0) (/ _returnvalue 2.0))) _returnvalue (0.0 0.0) (1.0 1.0) (`KismetMathLibrary.Conv_DoubleToLinearColor` _depth) "BLEND_Additive" (+ _rotation (`self.Rotation`)) (0.5 0.5)))

(fn `UpDatePosition`
  (returns (ReturnValue :type "Vector2D Structure"))
  (bind (_returnvalue_x _returnvalue_y) (`KismetMathLibrary.BreakVector2D` (/ (`KismetMathLibrary.Conv_VectorToVector2D` (`self.K2_GetActorLocation` self)) (`self.PixelWidth_Save`))))
  (return (select `bool` (`self.IsLandActor?`) :`false` (`KismetMathLibrary.Conv_VectorToVector2D` (`self.K2_GetActorLocation` self)) :`true` (* (`KismetMathLibrary.MakeVector2D` (`KismetMathLibrary.Conv_IntToDouble` (`KismetMathLibrary.FFloor` _returnvalue_x)) (`KismetMathLibrary.Conv_IntToDouble` (`KismetMathLibrary.FFloor` _returnvalue_y))) (`self.PixelWidth_Save`)))))

(fn `UserConstructionScript`
  (bind (_returnvalue_x _returnvalue_y _returnvalue_z) (`KismetMathLibrary.BreakVector` (`self.K2_GetActorLocation`)))
  (bind (_rtsize_world_size__x _rtsize_world_size__y) (`KismetMathLibrary.BreakVector2D` (`self.RTSize（world size）`)))
  (bind (_position_x _position_y) (`KismetMathLibrary.BreakVector2D` (`self.Position`)))
  (set `self.Position` (`KismetMathLibrary.Conv_VectorToVector2D` (`self.K2_GetActorLocation`)))
  (if (`self.ShowGrid`)
    (`SceneComponent.K2_SetWorldTransform` (`self.Decal`) (`KismetMathLibrary.MakeTransform` (`KismetMathLibrary.MakeVector` _position_x _position_y _returnvalue_z) (`KismetMathLibrary.MakeRotator` 0.0 -90.0) (`KismetMathLibrary.MakeVector` 1.0 _rtsize_world_size__y _rtsize_world_size__x)) false false)))