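; BP_SnowActorsManager is the single manager for interactive snowfields, routing snow deformation draw requests to each BP_SnowActor.
; Every Tick it rotates queued drawers into each field's local space, passes overlapping ones on for drawing, then clears the queue.
; At construction it gathers snow and capture actors and pushes quality-based pixel widths, edge and blur settings, and preview materials to them.
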(event `self.ReceiveBeginPlay`
  (bind _outactors (`GameplayStatics.GetAllActorsOfClass` "BP_SnowActorsManager_C"))
  (if (== (`KismetArrayLibrary.Array_Length` _outactors) 1)
    (bind _outactors_2 (`GameplayStatics.GetAllActorsOfClass` "/Game/IntaractiveSnowfield/Blueprints/BP_SnowActor.BP_SnowActor_C"))
    (set `self.Snowfields` _outactors_2)
    (else
      (`KismetSystemLibrary.PrintString` "You just need one mamager"))))

(event `self.ReceiveTick`
  (params (DeltaSeconds :type "Float (single-precision)"))
  (bind _snowfields (`self.Snowfields`))
  (bind _snowfields_needremove (`self.Snowfields_NeedRemove`))
  (for _array_element _snowfields
    (`/Engine/EditorBlueprintResources/StandardMacros.IsValid` _array_element
      (:`Is Valid`
        (set `self.Position` (`/Game/IntaractiveSnowfield/Blueprints/BP_SnowActor.Position` _array_element))
        (set `self.Rotation` (`/Game/IntaractiveSnowfield/Blueprints/BP_SnowActor.Rotation` _array_element))
        (set `self.DrawSize` (`/Game/IntaractiveSnowfield/Blueprints/BP_SnowActor.RTSize（world size）` _array_element))
        (`KismetArrayLibrary.Array_Clear` (`self.DrawInfo`))
        (set `self.ShouldDraw` false)
        (for _array_element_2 (`self.Drawers`)
          (`/Engine/EditorBlueprintResources/StandardMacros.IsValid` _array_element_2
            (:`Is Valid`
              (bind _position (`/Game/IntaractiveSnowfield/Blueprints/BP_DrawComponent.Position` _array_element_2))
              (bind (_returnvalue_x _returnvalue_y) (`KismetMathLibrary.BreakVector2D` (`KismetMathLibrary.GetRotated2D` (- _position (`self.Position`)) (* (`self.Rotation`) -1.0))))
              (bind _size (`/Game/IntaractiveSnowfield/Blueprints/BP_DrawComponent.Size` _array_element_2))
              (bind (_x _y) (`KismetMathLibrary.BreakVector2D` (+ _size (/ (`self.DrawSize`) 2.0))))
              ;[1 1 1] Add Info to arry/将绘制信息存到数组
              (if (and (<= (`KismetMathLibrary.Abs` _returnvalue_x) _x) (<= (`KismetMathLibrary.Abs` _returnvalue_y) _y))
                (`KismetArrayLibrary.Array_Add` (`self.DrawInfo`) (make `/Game/IntaractiveSnowfield/Structs/S_DrawInfor` _position (`/Game/IntaractiveSnowfield/Blueprints/BP_DrawComponent.Texture` _array_element_2) _size (`/Game/IntaractiveSnowfield/Blueprints/BP_DrawComponent.Rotation` _array_element_2) (`/Game/IntaractiveSnowfield/Blueprints/BP_DrawComponent.Depth` _array_element_2)))
                (set `self.ShouldDraw` true)))))
        ;[1 1 1] Call SnowActor draw/调用绘制事件
        (if (`self.ShouldDraw`)
          (set `/Game/IntaractiveSnowfield/Blueprints/BP_SnowActor.Drawers` (`self.DrawInfo`) _array_element)
          (`/Game/IntaractiveSnowfield/Blueprints/BP_SnowActor.Draw` _array_element)))
      (:`Is Not Valid`
        (`KismetArrayLibrary.Array_Add` (`self.Snowfields_NeedRemove`) _array_element))))
  ;[1 1 1] Remove invalid elements
  (if (> (`KismetArrayLibrary.Array_Length` _snowfields_needremove) 0)
    (for _array_element_3 _snowfields_needremove
      (`KismetArrayLibrary.Array_RemoveItem` _snowfields _array_element_3))
    (`KismetArrayLibrary.Array_Clear` (`self.Snowfields_NeedRemove`)))
  (`KismetSystemLibrary.PrintString` (`KismetTextLibrary.Conv_TextToString` (`|FormatText` "{n} pieces of draw information this frame" (`KismetArrayLibrary.Array_Length` (`self.Drawers`)))) true true (struct :`G` 0.66 :`B` 1.0 :`A` 1.0) 0.0001)
  ;[1 1 1] Draw finished/绘制结束
  (`KismetArrayLibrary.Array_Clear` (`self.Drawers`)))

(fn `UpdateQuality`
  (bind _quality (`self.Quality`))
  (if (`self.UseQuality`)
    (set `self.PixelWidth_Save` (select `/Game/IntaractiveSnowfield/Enums/E_SnowQuality` _quality :`NewEnumerator4` 32.0 :`NewEnumerator0` 16.0 :`NewEnumerator1` 8.0 :`NewEnumerator2` 4.0 :`NewEnumerator3` 2.0 :!type "Float (single-precision)"))
    (set `self.PixelWidth_Blur` (select `/Game/IntaractiveSnowfield/Enums/E_SnowQuality` _quality :`NewEnumerator4` 8.0 :`NewEnumerator0` 4.0 :`NewEnumerator1` 2.0 :`NewEnumerator2` 1.0 :`NewEnumerator3` 1.0 :!type "Float (single-precision)"))
    (set `self.PixelWidth_Capture` (select `/Game/IntaractiveSnowfield/Enums/E_SnowQuality` _quality :`NewEnumerator4` 32.0 :`NewEnumerator0` 16.0 :`NewEnumerator1` 8.0 :`NewEnumerator2` 4.0 :`NewEnumerator3` 2.0 :!type "Float (single-precision)")))
  (`self.UpdateSnowQualityInfo`))

(fn `UpdateSnowQualityInfo`
  (for _array_element (`self.Snowfields`)
    (`/Engine/EditorBlueprintResources/StandardMacros.IsValid` _array_element
      (:`Is Valid`
        (set `/Game/IntaractiveSnowfield/Blueprints/BP_SnowActor.PixelWidth_Save` (`self.PixelWidth_Save`) _array_element)
        (set `/Game/IntaractiveSnowfield/Blueprints/BP_SnowActor.PixelWidth_Blured` (`self.PixelWidth_Blur`) _array_element)
        (set `/Game/IntaractiveSnowfield/Blueprints/BP_SnowActor.EdgeOffsetWidth` (`self.EdgeWidth`) _array_element)
        (set `/Game/IntaractiveSnowfield/Blueprints/BP_SnowActor.BlurWidth` (`self.BlurWidth`) _array_element)
        (bind _asbp_snow_actor_mesh_base (cast `/Game/IntaractiveSnowfield/Blueprints/BP_SnowActor_MeshBase` _array_element))
        (`/Game/IntaractiveSnowfield/Blueprints/BP_SnowActor_MeshBase.CreatePreviewMat` _asbp_snow_actor_mesh_base (`self.PreviewTexSize`) (`self.PreviewTexture`)))))
  (if (`self.UseQualityToCaptures`)
    (for _array_element_2 (`self.Captures`)
      (set `/Game/IntaractiveSnowfield/Blueprints/BP_DrawActor_Capture.PixelWidth` (`self.PixelWidth_Capture`) _array_element_2))))

(fn `UserConstructionScript`
  (bind _outactors (`GameplayStatics.GetAllActorsOfClass` "/Game/IntaractiveSnowfield/Blueprints/BP_SnowActor.BP_SnowActor_C"))
  (set `self.Snowfields` _outactors)
  (bind _outactors_2 (`GameplayStatics.GetAllActorsOfClass` "/Game/IntaractiveSnowfield/Blueprints/BP_DrawActor_Capture.BP_DrawActor_Capture_C"))
  (set `self.Captures` _outactors_2)
  (`self.UpdateQuality`))