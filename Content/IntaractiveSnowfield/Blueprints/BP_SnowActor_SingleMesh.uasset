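; Single-mesh snow actor for an interactive snowfield, showing the snow surface on one static mesh.
; Construction runs the parent script, then applies the snow material to the mesh's first slot; BeginPlay only calls the parent.
; SetScale sets a component's world XY scale to the render-target world size times a multiplier, divided by the component's bounds extent, with Z fixed at one.
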(event `self.ReceiveBeginPlay`
  (`parent.ReceiveBeginPlay`))

(fn `SetScale`
  (params (`组件` :type "StaticMeshComponent Object Reference") (`乘数` :type "Float (double-precision)"))
  (bind (_origin _boxextent) (`KismetSystemLibrary.GetComponentBounds` `组件`))
  (bind (_returnvalue_x _returnvalue_y) (`KismetMathLibrary.BreakVector2D` (/ (* (`self.RTSize（world size）`) `乘数`) (`KismetMathLibrary.MakeVector2D` (.x _boxextent) (.y _boxextent)))))
  (`SceneComponent.SetWorldScale3D` `组件` (`KismetMathLibrary.MakeVector` _returnvalue_x _returnvalue_y 1.0)))

(fn `UserConstructionScript`
  (`parent.UserConstructionScript`)
  (`PrimitiveComponent.SetMaterial` (`self.StaticMesh`) 0 (`self.SnowMat`)))