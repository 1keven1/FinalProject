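; Child actor for the interactive snowfield that captures its parent actor from ground level, looking up, to feed a DrawComponent.
; An orthographic scene capture shows only the parent, whose child primitives are set to render custom depth.
; On movement, a line trace snaps the capture to the ground.
; The capture is then mirror-flipped by material into a second R8 render target, which the DrawComponent is told to draw at that position.
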(event `self.ReceiveBeginPlay`
  (bind _father (`self.Father`))
  (bind _returnvalue (`KismetMathLibrary.FTrunc` (/ (`self.OrthoWidth`) (`self.PixelWidth`))))
  (`parent.ReceiveBeginPlay`)
  ;[1 1 1] Create RT and material/创建render target和材质
  (bind _returnvalue_2 (`KismetRenderingLibrary.CreateRenderTarget2D` _returnvalue _returnvalue "RTF_R8" (struct :`R` 1.0 :`G` 1.0 :`B` 1.0 :`A` 1.0)))
  (bind _output_get (set `self.CaptureTexture` _returnvalue_2))
  (set `SceneCaptureComponent2D.TextureTarget` _output_get (`self.SceneCaptureComponent2D`))
  (bind _returnvalue_3 (`KismetRenderingLibrary.CreateRenderTarget2D` _returnvalue _returnvalue "RTF_R8" (struct :`R` 1.0 :`G` 1.0 :`B` 1.0 :`A` 1.0)))
  (set `/Game/IntaractiveSnowfield/Blueprints/BP_DrawComponent.Texture` _returnvalue_3 (`self.DrawComponent`))
  (`KismetRenderingLibrary.ClearRenderTarget2D` (`self.CaptureTexture`) (struct :`R` 1.0 :`G` 1.0 :`B` 1.0 :`A` 1.0))
  (bind _returnvalue_4 (`KismetMaterialLibrary.CreateDynamicMaterialInstance` "/Game/IntaractiveSnowfield/Materials/MI_RT_MirrorFlip.MI_RT_MirrorFlip"))
  (`MaterialInstanceDynamic.SetTextureParameterValue` _returnvalue_4 "Texture" (`self.CaptureTexture`))
  (set `self.MirrorMat` _returnvalue_4)
  ;[1 1 1] Use custom depth to draw/使用自定义深度绘制
  (`SceneCaptureComponent.ShowOnlyActorComponents` (`self.SceneCaptureComponent2D`) _father true)
  (for _array_element (`SceneComponent.GetChildrenComponents` (`Actor.RootComponent` _father) true)
    (bind `_as基元组件` (cast `PrimitiveComponent` _array_element))
    (`PrimitiveComponent.SetRenderCustomDepth` `_as基元组件` true)))

(event `self.ReceiveTick`
  (params (DeltaSeconds :type "Float (single-precision)"))
  (bind _lastlocation (`self.LastLocation`))
  (bind _drawcomponent (`self.DrawComponent`))
  (bind _returnvalue (select `bool` (`self.UseBoundOrigin`) :`false` (`self.K2_GetActorLocation`) :`true` (`self.GetActorBounds` (`self.Father`) false false)))
  ;[1 1 1] Don't update if not moved/仅在移动时更新
  (if (not (== _returnvalue (`self.LastLocation`) :`ErrorTolerance` 1.0))
    (set `self.LastLocation` _returnvalue)
    (if true
      ;[1 1 1] Find the height of the land/移动到地面高度
      (bind (_outhit _returnvalue_2) (`KismetSystemLibrary.LineTraceSingleForObjects` (+ _lastlocation (0.0 0.0 100.0)) (- _lastlocation (0.0 0.0 1000.0)) (`self.Object Types`)))
      (if _returnvalue_2
        (bind (_bblockinghit _binitialoverlap _time _distance _location) (`GameplayStatics.BreakHitResult` _outhit))
        (`SceneComponent.K2_SetWorldTransform` (`self.SceneCaptureComponent2D`) (`KismetMathLibrary.MakeTransform` _location (struct :`Pitch` 90.0 :`Roll` 90.0)) false false)
        (set `/Game/IntaractiveSnowfield/Blueprints/BP_DrawComponent.Position` (`KismetMathLibrary.MakeVector2D` (.x _location) (.y _location)) (`self.DrawComponent`))
        ;[1 1 1] Update
        (`SceneCaptureComponent2D.CaptureScene` (`self.SceneCaptureComponent2D`))
        (`KismetRenderingLibrary.DrawMaterialToRenderTarget` (cast `TextureRenderTarget2D` (`/Game/IntaractiveSnowfield/Blueprints/BP_DrawComponent.Texture` _drawcomponent) :!pure true) (`self.MirrorMat`))
        (`/Game/IntaractiveSnowfield/Blueprints/BP_DrawComponent.NeedDrawing` _drawcomponent)))))

(fn `UserConstructionScript`
  (bind _returnvalue (`self.GetParentActor`))
  (bind _orthowidth (`self.OrthoWidth`))
  (bind _returnvalue_2 (/ (`self.OrthoWidth`) 100.0))
  (`parent.UserConstructionScript`)
  (set `SceneCaptureComponent2D.OrthoWidth` _orthowidth (`self.SceneCaptureComponent2D`))
  (set `/Game/IntaractiveSnowfield/Blueprints/BP_DrawComponent.Size` (`KismetMathLibrary.MakeVector2D` _orthowidth _orthowidth) (`self.DrawComponent`))
  (`SceneComponent.SetRelativeScale3D` (`self.Plane`) (`KismetMathLibrary.MakeVector` _returnvalue_2 _returnvalue_2 1.0))
  (`/Engine/EditorBlueprintResources/StandardMacros.IsValid` _returnvalue
    (:`Is Valid`
      (set `self.Father` _returnvalue)
      (`self.SetActorTickEnabled` true))
    (:`Is Not Valid`
      (set `self.Father` self)
      (`KismetSystemLibrary.PrintText` (`|FormatText` "{name}Failed to get my father" (`KismetSystemLibrary.GetDisplayName` self))))))