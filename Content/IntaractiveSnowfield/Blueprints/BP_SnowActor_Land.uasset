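; BP_SnowActor_Land is an interactive snowfield actor that follows the first player's pawn and publishes its render-target mapping to materials.
; On BeginPlay it runs the parent logic, then moves to the pawn and attaches with snap-to-target rules.
; On DrawFinished it packs the render target's world size and Position XY into the UVXY vector of MPC_SnowfieldPara.
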(event `self.ReceiveBeginPlay`
  (`parent.ReceiveBeginPlay`)
  (`self.Attach to player pawn` (`GameplayStatics.GetPlayerPawn` 0)))

(event `self.DrawFinished`
  (bind (_position_x _position_y) (`KismetMathLibrary.BreakVector2D` (`self.Position`)))
  (bind (_rtsize_world_size__x _rtsize_world_size__y) (`KismetMathLibrary.BreakVector2D` (`self.RTSize（world size）`)))
  (`KismetMaterialLibrary.SetVectorParameterValue` "/Game/IntaractiveSnowfield/MaterialParameterCollection/MPC_SnowfieldPara.MPC_SnowfieldPara" (`self.UVXY`) (make `LinearColor` _rtsize_world_size__x _rtsize_world_size__y _position_x _position_y)))

(fn `Attach to player pawn`
  (params (NewPawn :type "Pawn Object Reference"))
  (`self.K2_SetActorLocation` (`self.K2_GetActorLocation` NewPawn))
  (`self.K2_AttachToActor` NewPawn "None" "SnapToTarget" "SnapToTarget" "SnapToTarget" false))

(fn `UserConstructionScript`
  (`parent.UserConstructionScript`))