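; Snowfield actor that builds a grid of snow-material plane meshes sized to the render-target world size in its construction script.
; The quality setting and shorter field side select mesh variant and plane width, which sets the grid count, capped at 32 planes.
; Planes attach with collision under one component, which is scaled from the first child's bounds to fit the field.
; The configured yaw is applied after scaling, keeping it out of the bounds measurement.
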(fn `CreatePlaneArry`
  (params (SceneComp :type "SceneComponent Object Reference") (Width :type Integer) (NewMesh :type "StaticMesh Object Reference") (NewBoundsScale :type "Float (double-precision)") (Collision :type "ECollisionEnabled Enum" :default "NoCollision") (Material :type "MaterialInterface Object Reference") (PlaneWidth :type "Float (double-precision)"))
  (returns (XNumb :type Integer) (YNumb :type Integer))
  (locals (XorY :type Boolean :default false) (Number :type Integer :default 0) (XNum :type Integer) (YNum :type Integer :default 0))
  (bind _returnvalue (`KismetMathLibrary.Conv_IntToDouble` Width))
  (bind (_rtsize_world_size__x _rtsize_world_size__y) (`KismetMathLibrary.BreakVector2D` (`self.RTSize（world size）`)))
  (bind _xnum (`local.XNum`))
  (bind _ynum (`local.YNum`))
  (if (> PlaneWidth 100.0)
    (bind _output_get (set `local.XNum` (`KismetMathLibrary.Max` (+ (`KismetMathLibrary.FFloor` (/ _rtsize_world_size__x PlaneWidth)) (select `bool` (> (mod _rtsize_world_size__x PlaneWidth) 0.5) :`true` 1)) 1)))
    (bind _output_get_2 (set `local.YNum` (`KismetMathLibrary.Max` (+ (`KismetMathLibrary.FFloor` (/ _rtsize_world_size__y PlaneWidth)) (select `bool` (> (mod _rtsize_world_size__y PlaneWidth) 0.5) :`true` 1)) 1)))
    (if (<= (* _output_get _output_get_2) 32)
      (for _index (range 1 (+ _xnum 1))
        (for _index_2 (range 1 (+ _ynum 1))
          (bind _returnvalue_2 (`AddComponent|NODE_AddStaticMeshComponent-0` :`RelativeTransform` (`KismetMathLibrary.MakeTransform` (`KismetMathLibrary.MakeVector` (* (- (`KismetMathLibrary.Conv_IntToDouble` _index) (/ (`KismetMathLibrary.Conv_IntToDouble` (+ _xnum 1)) 2.0)) _returnvalue) (* (- (`KismetMathLibrary.Conv_IntToDouble` _index_2) (/ (`KismetMathLibrary.Conv_IntToDouble` (+ _ynum 1)) 2.0)) _returnvalue)))))
          (`SceneComponent.K2_AttachToComponent` _returnvalue_2 SceneComp "None" "KeepRelative" "KeepRelative" "KeepRelative" true)
          (`PrimitiveComponent.SetMaterial` _returnvalue_2 0 Material)
          (`StaticMeshComponent.SetStaticMesh` _returnvalue_2 NewMesh)
          (`PrimitiveComponent.SetBoundsScale` _returnvalue_2 NewBoundsScale)
          (`PrimitiveComponent.SetCollisionEnabled` _returnvalue_2 Collision)))
      (return (`local.XNum`) (`local.YNum`))
      (else
        (`KismetSystemLibrary.PrintString` "Too many planes")))
    (else
      (`KismetSystemLibrary.PrintString` "Width is not enough"))))

(fn `CreateSnowfield`
  (`self.CreatSnowfieldArry` (`self.PlaneArryQulity`)))

(fn `CreatSnowfieldArry`
  (params (Qulity :type "/Game/IntaractiveSnowfield/Enums/E_SnowQuality Enum" :default "NewEnumerator4"))
  (bind (_meshrotation_roll _meshrotation_pitch _meshrotation_yaw) (`KismetMathLibrary.BreakRotator` (`self.MeshRotation`)))
  (bind _mesh (`self.mesh`))
  (bind (_mesh_2 `_plane宽度`) (`self.FindSuitableMesh` Qulity))
  (bind (_xnumb _ynumb) (`self.CreatePlaneArry` _mesh 100 _mesh_2 1.0 "QueryAndPhysics" (`self.SnowMat`) `_plane宽度`))
  (`SceneComponent.K2_SetWorldRotation` _mesh (`KismetMathLibrary.MakeRotator` _meshrotation_roll _meshrotation_pitch 1.0) false false)
  (`self.SetScales` _mesh 0.5 _xnumb _ynumb)
  (`SceneComponent.K2_AddWorldRotation` _mesh (`KismetMathLibrary.MakeRotator` 0.0 0.0 _meshrotation_yaw) false false))

(fn `FindSuitableMesh`
  (params (`雪地质量` :type "/Game/IntaractiveSnowfield/Enums/E_SnowQuality Enum" :default "NewEnumerator4"))
  (returns (mesh :type "StaticMesh Object Reference") (`plane宽度` :type "Float (double-precision)"))
  (locals (`雪地arry` :type "Array of StaticMesh Object Reference"))
  (bind (_rtsize_world_size__x _rtsize_world_size__y) (`KismetMathLibrary.BreakVector2D` (`self.RTSize（world size）`)))
  (bind _returnvalue (`KismetMathLibrary.FMin` _rtsize_world_size__x _rtsize_world_size__y))
  (bind _returnvalue_2 (`KismetMathLibrary.Max` (+ (`KismetMathLibrary.FFloor` (/ _returnvalue 256.0)) (`KismetMathLibrary.SelectInt` 1 0 (> (mod _returnvalue 256.0) 0.5))) 1))
  (return (select `int` (`KismetMathLibrary.Min` (select `/Game/IntaractiveSnowfield/Enums/E_SnowQuality` `雪地质量` :`NewEnumerator4` 1 :`NewEnumerator0` 2 :`NewEnumerator1` 3 :`NewEnumerator2` 3 :`NewEnumerator3` 4) _returnvalue_2) :`0` "/Game/IntaractiveSnowfield/Meshes/SM_Plane_B.SM_Plane_B" :`1` "/Game/IntaractiveSnowfield/Meshes/SM_Plane_C.SM_Plane_C" :`2` "/Game/IntaractiveSnowfield/Meshes/SM_Plane_D.SM_Plane_D" :`3` "/Game/IntaractiveSnowfield/Meshes/SM_Plane_E.SM_Plane_E" :`4` "/Game/IntaractiveSnowfield/Meshes/SM_Plane_F.SM_Plane_F" :!type "StaticMesh Object Reference") (`KismetMathLibrary.Conv_IntToDouble` (* (`KismetMathLibrary.Min` _returnvalue_2 4) 256))))

(fn `SetScales`
  (params (Comp :type "SceneComponent Object Reference") (Width :type "Float (double-precision)") (X :type Integer) (Y :type Integer))
  (bind (_origin _boxextent) (`KismetSystemLibrary.GetComponentBounds` (`SceneComponent.GetChildComponent` Comp 0)))
  (bind (_returnvalue_x _returnvalue_y) (`KismetMathLibrary.BreakVector2D` (/ (/ (* (`self.RTSize（world size）`) Width) (`KismetMathLibrary.MakeVector2D` (.x _boxextent) (.y _boxextent))) (`KismetMathLibrary.MakeVector2D` (`KismetMathLibrary.Conv_IntToDouble` X) (`KismetMathLibrary.Conv_IntToDouble` Y)))))
  (`SceneComponent.SetWorldScale3D` Comp (`KismetMathLibrary.MakeVector` _returnvalue_x _returnvalue_y 10.0)))

(fn `UserConstructionScript`
  (`parent.UserConstructionScript`)
  (`self.CreateSnowfield`))