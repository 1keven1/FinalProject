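; A snowfield draw component that stamps its signet texture beneath the owning actor to imprint marks in snow.
; On tick, when its tracked point (the component location or owner's bounds bottom) moves beyond a small tolerance, it line-traces downward.
; A hit converts surface distance into stamp depth relative to snow thickness, sets position and yaw, then calls NeedDrawing to request the draw.
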(event `self.ReceiveBeginPlay`
  (`parent.ReceiveBeginPlay`)
  (set `self.Texture` (`self.SignetTexture`))
  (set `self.father` (`self.GetOwner`)))

(event `self.ReceiveTick`
  (params (DeltaSeconds :type "Float (single-precision)"))
  (bind (_returnvalue_roll _returnvalue_pitch _returnvalue_yaw) (`KismetMathLibrary.BreakRotator` (`self.K2_GetComponentRotation`)))
  (bind _snowfieldthickness (`self.SnowfieldThickness`))
  (bind _lastlocation (`self.LastLocation`))
  (bind (_origin _boxextent) (`Actor.GetActorBounds` (`self.father`) true false))
  (bind _returnvalue (select `bool` (`self.UseBounds`) :`false` (`self.K2_GetComponentLocation`) :`true` (- _origin (`KismetMathLibrary.MakeVector` 0.0 0.0 (.z _boxextent)))))
  (`parent.ReceiveTick` DeltaSeconds)
  ;[1 1 1] Update when moved/仅在移动时更新
  (if (not (== (`self.LastLocation`) _returnvalue :`ErrorTolerance` 1.0))
    (set `self.LastLocation` _returnvalue)
    ;[1 1 1] Trace the height/检测高度
    (bind (_outhit _returnvalue_2) (`KismetSystemLibrary.LineTraceSingleForObjects` :`Start` (+ _lastlocation (0.0 0.0 100.0)) :`End` (+ _lastlocation (`KismetMathLibrary.MakeVector` 0.0 0.0 (- 0.0 (+ (`self.SnowfieldThickness`) 100.0)))) :`ObjectTypes` (`self.Object Types`) :`DrawDebugType` "ForOneFrame"))
    (if _returnvalue_2
      ;[1 1 1] Caculate signet/计算印记
      (set `self.Depth` (- 1.0 (/ (`KismetMathLibrary.FClamp` (- (`.Distance` (`GameplayStatics.BreakHitResult` _outhit)) 100.0) 0.0 _snowfieldthickness) _snowfieldthickness)))
      (set `self.Rotation` _returnvalue_yaw)
      (set `self.Position` (`KismetMathLibrary.Conv_VectorToVector2D` (`self.LastLocation`)))
      (`self.NeedDrawing`))))