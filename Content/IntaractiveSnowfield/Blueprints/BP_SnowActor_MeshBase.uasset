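; Mesh-based snow actor base for the interactive snowfield, feeding render target data into a dynamic snow material.
; Construction creates the material instance, stores the mesh yaw and rotates the decal by it.
; BeginPlay passes render target world size, position, normalized rotation and blurred texture to the material, recreating it with a default fallback if invalid.
; CreatePreviewMat substitutes a preview size and texture, while CreateSnowfield is an empty stub.
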(event `self.ReceiveBeginPlay`
  (`parent.ReceiveBeginPlay`)
  (`self.InitializeSnowMatInfo`))

(fn `CreatePreviewMat`
  (params (PreviewTexSize :type "Float (double-precision)") (PrevuewTexture :type "Texture Object Reference"))
  (bind _snowmat (`self.SnowMat`))
  (bind (_position_x _position_y) (`KismetMathLibrary.BreakVector2D` (`self.Position`)))
  (`MaterialInstanceDynamic.SetVectorParameterValue` _snowmat "UVXY" (make `LinearColor` PreviewTexSize PreviewTexSize _position_x _position_y))
  (`MaterialInstanceDynamic.SetScalarParameterValue` _snowmat "Rotation" (/ (`self.Rotation`) 360.0))
  (`MaterialInstanceDynamic.SetTextureParameterValue` _snowmat "Texture" PrevuewTexture)
  (`MaterialInstanceDynamic.SetTextureParameterValue` (`self.SnowMat`) "Texture" PrevuewTexture))

(fn `CreateSnowfield`)

(fn `InitializeSnowMatInfo`
  (bind _material (`self.Material`))
  (bind _snowmat (`self.SnowMat`))
  (bind (_rtsize_world_size__x _rtsize_world_size__y) (`KismetMathLibrary.BreakVector2D` (`self.RTSize（world size）`)))
  (bind (_position_x _position_y) (`KismetMathLibrary.BreakVector2D` (`self.Position`)))
  (`/Engine/EditorBlueprintResources/StandardMacros.IsValid` _snowmat
    (:`Is Valid`
      _)
    (:`Is Not Valid`
      ;[1 1 1] Creat one it is not valid
      (bind _returnvalue (`KismetMaterialLibrary.CreateDynamicMaterialInstance` (select `bool` (`KismetSystemLibrary.IsValid` _material) :`false` "/Game/IntaractiveSnowfield/Materials/MI_SnowSurface_snow.MI_SnowSurface_snow" :`true` _material)))
      (set `self.SnowMat` _returnvalue)))
  (`MaterialInstanceDynamic.SetVectorParameterValue` _snowmat "UVXY" (make `LinearColor` _rtsize_world_size__x _rtsize_world_size__y _position_x _position_y))
  (`MaterialInstanceDynamic.SetTextureParameterValue` _snowmat "Texture" (`self.Blured`))
  (`MaterialInstanceDynamic.SetScalarParameterValue` _snowmat "Rotation" (/ (`self.Rotation`) 360.0)))

(fn `UserConstructionScript`
  (bind (_meshrotation_roll _meshrotation_pitch _meshrotation_yaw) (`KismetMathLibrary.BreakRotator` (`self.MeshRotation`)))
  (`parent.UserConstructionScript`)
  (bind _returnvalue (`KismetMaterialLibrary.CreateDynamicMaterialInstance` (`self.Material`)))
  (set `self.SnowMat` _returnvalue)
  (set `self.Rotation` _meshrotation_yaw)
  (`SceneComponent.K2_AddWorldRotation` (`self.Decal`) (`KismetMathLibrary.MakeRotator` 0.0 0.0 _meshrotation_yaw) false false))