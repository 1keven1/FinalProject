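; Scene capture actor for snow deformation that follows the player and maintains a persistent render target.
; On begin play it clears both render targets, creates the draw material and publishes the capture size to Capture_MPC.
; Each tick it moves in XY toward the player in texel-snapped steps and publishes its location.
; It then draws into Persistent_RT, passing the normalized move as an offset to compensate for the scrolling.
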(event `self.ReceiveBeginPlay`
  (`KismetMaterialLibrary.SetScalarParameterValue` "/Game/SnowDeformations/Material/Capture_MPC.Capture_MPC" "CaptureSize" (`SceneCaptureComponent2D.OrthoWidth` (`self.SceneCapture`)))
  (bind _returnvalue (`KismetMaterialLibrary.CreateDynamicMaterialInstance` "/Game/SnowDeformations/Material/DrawToPersistent_M.DrawToPersistent_M"))
  (set `self.DrawMaterial` _returnvalue)
  (`KismetRenderingLibrary.ClearRenderTarget2D` "/Game/SnowDeformations/RenderTargets/Capture_RT.Capture_RT")
  (`KismetRenderingLibrary.ClearRenderTarget2D` "/Game/SnowDeformations/RenderTargets/Persistent_RT.Persistent_RT"))

(event `self.ReceiveTick`
  (params (DeltaSeconds :type "Float (single-precision)"))
  (`self.Move Capture`)
  (`self.Draw to Persistent`))

(fn `Draw to Persistent`
  (bind (_returnvalue_x _returnvalue_y) (`KismetMathLibrary.BreakVector2D` (/ (`self.MoveOffset`) (`SceneCaptureComponent2D.OrthoWidth` (`self.SceneCapture`)))))
  (`MaterialInstanceDynamic.SetVectorParameterValue` (`self.DrawMaterial`) "Offset" (make `LinearColor` _returnvalue_x _returnvalue_y 0.0 1.0))
  (`KismetRenderingLibrary.DrawMaterialToRenderTarget` "/Game/SnowDeformations/RenderTargets/Persistent_RT.Persistent_RT" (`self.DrawMaterial`)))

(fn `Move Capture`
  (bind _scenecapture (`self.SceneCapture`))
  (bind (_returnvalue_x _returnvalue_y) (`KismetMathLibrary.BreakVector` (`self.K2_GetActorLocation` (`GameplayStatics.GetPlayerCharacter` 0))))
  (bind (_returnvalue_x_2 _returnvalue_y_2) (`KismetMathLibrary.BreakVector` (- (`self.SnapToPixelWorldSize` _returnvalue_x _returnvalue_y (* (`SceneCaptureComponent2D.OrthoWidth` _scenecapture) (/ 1.0 (`KismetMathLibrary.Conv_IntToDouble` (`TextureRenderTarget2D.SizeX` (`SceneCaptureComponent2D.TextureTarget` _scenecapture)))))) (`self.K2_GetActorLocation`))))
  (bind _output_get (set `self.MoveOffset` (`KismetMathLibrary.MakeVector2D` _returnvalue_x_2 _returnvalue_y_2)))
  (`self.K2_AddActorWorldOffset` (`KismetMathLibrary.MakeVector` (`KismetMathLibrary.BreakVector2D` _output_get) (`.Y` (`KismetMathLibrary.BreakVector2D` _output_get))))
  (`KismetMaterialLibrary.SetVectorParameterValue` "/Game/SnowDeformations/Material/Capture_MPC.Capture_MPC" "CaptureLocation" (`KismetMathLibrary.Conv_VectorToLinearColor` (`self.K2_GetActorLocation`))))

(fn `UserConstructionScript`)