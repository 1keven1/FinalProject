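; Snowball actor that grows as it rolls and can be stacked onto another snowball.
; While not picked up and moving horizontally, Tick adds mass from the larger X/Y speed, WeightGain and delta time, then derives uniform scale from mass.
; Sphere overlaps track a neighboring Snowball_BP.
; The Attach event destroys the Sphere, welds this snowball to that neighbor and disables physics on both.
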(event `self.ReceiveBeginPlay`
  ;[1 1 1] Set mass
  (`PrimitiveComponent.SetMassOverrideInKg` (`self.Snowball`) "None" (`self.Mass`) true)
  ;[1 1 1] Set scale
  (`SceneComponent.SetWorldScale3D` (`self.Snowball`) (`KismetMathLibrary.Conv_DoubleToVector` (/ (`self.Mass`) 100.0)))
  (`SceneComponent.SetWorldScale3D` (`self.Sphere`) (`KismetMathLibrary.Conv_DoubleToVector` (/ (`self.Mass`) 100.0))))

(event `self.ReceiveTick`
  (params (DeltaSeconds :type "Float (single-precision)"))
  (bind _weightgain (`self.WeightGain`))
  (bind _snowball (`self.Snowball`))
  (bind (_returnvalue_x _returnvalue_y) (`KismetMathLibrary.BreakVector` (`SceneComponent.GetComponentVelocity` (`self.Snowball`))))
  (bind _returnvalue (`KismetMathLibrary.Abs` _returnvalue_x))
  (bind _returnvalue_2 (`KismetMathLibrary.Abs` _returnvalue_y))
  (bind _returnvalue_3 (+ (`PrimitiveComponent.GetMass` _snowball) (/ (* (`KismetMathLibrary.GetMaxElement` (`KismetMathLibrary.MakeVector` (* _returnvalue _weightgain) (* _returnvalue_2 _weightgain))) (* DeltaSeconds 1000.0)) 100000.0)))
  ;[1 1 1 1 25] Set mass and scale
  (if (and (not (`self.PickUp?`)) (or (> _returnvalue 1.0) (> _returnvalue_2 1.0)))
    ;;[1 1 1] Set Mass
    (bind _output_get (set `self.Mass` _returnvalue_3))
    (`PrimitiveComponent.SetMassOverrideInKg` _snowball "None" _output_get true)
    ;;[1 1 1] Set scale
    (`SceneComponent.SetWorldScale3D` (`self.Snowball`) (`KismetMathLibrary.Conv_DoubleToVector` (/ _returnvalue_3 100.0)))
    (`SceneComponent.SetWorldScale3D` (`self.Sphere`) (`KismetMathLibrary.Conv_DoubleToVector` (/ _returnvalue_3 100.0)))))

(event `self.Sphere.OnComponentBeginOverlap`
  (params (OverlappedComponent :type "PrimitiveComponent Object Reference") (OtherActor :type "Actor Object Reference") (OtherComp :type "PrimitiveComponent Object Reference") (OtherBodyIndex :type Integer) (bFromSweep :type Boolean) (SweepResult :type "HitResult Structure (by ref)"))
  ;[1 1 1] Overlap
  (bind _assnowball_bp (cast `/Game/SnowDeformations/Blueprints/Snowball_BP` OtherActor))
  (set `self.Snowball_BP` _assnowball_bp)
  (if (`KismetStringLibrary.NotEqual_StrStr` (`KismetSystemLibrary.GetObjectName` self) (`KismetSystemLibrary.GetObjectName` _assnowball_bp))
    (set `self.Overlap` true)))

(event `self.Sphere.OnComponentEndOverlap`
  (params (OverlappedComponent :type "PrimitiveComponent Object Reference") (OtherActor :type "Actor Object Reference") (OtherComp :type "PrimitiveComponent Object Reference") (OtherBodyIndex :type Integer))
  ;[1 1 1] Overlap
  (bind _assnowball_bp (cast `/Game/SnowDeformations/Blueprints/Snowball_BP` OtherActor))
  (if (`KismetStringLibrary.NotEqual_StrStr` (`KismetSystemLibrary.GetObjectName` self) (`KismetSystemLibrary.GetObjectName` _assnowball_bp))
    (set `self.Overlap` false)))

(event `Attach`
  (bind _snowball (`/Game/SnowDeformations/Blueprints/Snowball_BP.Snowball` (`self.Snowball_BP`)))
  (if (`self.Overlap`)
    (`ActorComponent.K2_DestroyComponent` (`self.Sphere`))
    (`SceneComponent.K2_AttachToComponent` (`self.Snowball`) _snowball "None" "KeepWorld" "KeepWorld" "KeepWorld" true)
    (`PrimitiveComponent.SetSimulatePhysics` _snowball false)
    (`PrimitiveComponent.SetSimulatePhysics` (`self.Snowball`) false)))

(fn `UserConstructionScript`)