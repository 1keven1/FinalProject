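; BP_Lazer is a laser beam effect actor that exposes the shape of its NSLightBeam effect through Length, Width and Tile variables.
; The construction script passes these values to the effect component as float parameters when the actor is constructed.
; Tick pushes the same values every frame, so changes to the variables at runtime show up in the beam.
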(event `self.ReceiveTick`
  (params (DeltaSeconds :type "Float (single-precision)"))
  (bind _ns_light_beam (`self.NS_Light_Beam`))
  (`NiagaraComponent.SetVariableFloat` _ns_light_beam "Length" (`self.Length`))
  (`NiagaraComponent.SetVariableFloat` _ns_light_beam "Width" (`self.Width`))
  (`NiagaraComponent.SetVariableFloat` _ns_light_beam "Tile" (`self.Tile`)))

(fn `UserConstructionScript`
  (bind _ns_light_beam (`self.NS_Light_Beam`))
  (`NiagaraComponent.SetVariableFloat` _ns_light_beam "Length" (`self.Length`))
  (`NiagaraComponent.SetVariableFloat` _ns_light_beam "Width" (`self.Width`))
  (`NiagaraComponent.SetVariableFloat` _ns_light_beam "Tile" (`self.Tile`)))