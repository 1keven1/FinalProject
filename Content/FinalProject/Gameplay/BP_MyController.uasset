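; Player controller that routes input to the game mode and spawns overlay UI widgets.
; On BeginPlay it caches the game mode and character, moving the audio listener onto the character's AudioListener.
; Pause and Enter cancel or confirm an open confirm window, otherwise reaching the game mode alongside filtered any-key presses and debug toggles.
; Helper functions manage a single confirm window and add screen tip and area name widgets.
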(event `self.ReceiveBeginPlay`
  (bind _mycharacter (`self.MyCharacter`))
  (`|ExecutionSequence`
    (:`then_0`
      (bind _asbp_my_game_mode_base (cast `/Game/FinalProject/Gameplay/BP_MyGameMode_Base` (`GameplayStatics.GetGameMode`)))
      (set `self.MyGameMode` _asbp_my_game_mode_base))
    (:`then_1`
      (bind _asbp_my_character (cast `/Game/FinalProject/Gameplay/Character/BP_MyCharacter` (`self.K2_GetPawn`)))
      (set `self.MyCharacter` _asbp_my_character))
    (:`then_2`
      (`/Engine/EditorBlueprintResources/StandardMacros.IsValid` _mycharacter
        (:`Is Valid`
          (`self.SetAudioListenerOverride` (`/Game/FinalProject/Gameplay/Character/BP_MyCharacter.AudioListener` _mycharacter)))))))

(event `InputAction|Pause` :paused true
  (params (Key :type "Key Structure"))
  (bind _wo_comfirm (`self.WO_Comfirm`))
  (:`Pressed`
    (`/Engine/EditorBlueprintResources/StandardMacros.IsValid` _wo_comfirm
      (:`Is Valid`
        (`/Game/FinalProject/Gameplay/UI/WO_ConfirmWIndow.CE_PressCancel` _wo_comfirm))
      (:`Is Not Valid`
        (`/Game/FinalProject/Gameplay/BP_MyGameMode_Base.PressPause` (`self.MyGameMode`))))))

(event `Key|Enter` :paused true
  (params (Key :type "Key Structure"))
  (bind _wo_comfirm (`self.WO_Comfirm`))
  (:`Pressed`
    (`/Engine/EditorBlueprintResources/StandardMacros.IsValid` _wo_comfirm
      (:`Is Valid`
        (`/Game/FinalProject/Gameplay/UI/WO_ConfirmWIndow.CE_PressConfirm` _wo_comfirm))
      (:`Is Not Valid`
        (`/Game/FinalProject/Gameplay/BP_MyGameMode_Base.PressEnter` (`self.MyGameMode`))))))

(event `Key|AnyKey` :consume false :paused true
  (params (Key :type "Key Structure"))
  (:`Pressed`
    (if (`self.CheckCanBeInputKey` Key)
      (`/Game/FinalProject/Gameplay/BP_MyGameMode_Base.PressAnyKey` (`self.MyGameMode`) Key))))

(event `Key|Equals`
  (params (Key :type "Key Structure"))
  (:`Pressed`
    (`/Game/FinalProject/Gameplay/BP_MyGameMode_Base.CE_Toggle_Debug` (`self.MyGameMode`) :!label _label)))

(event `Key|Add`
  (params (Key :type "Key Structure"))
  (:`Pressed`
    (goto _label)))

(fn `AddAreaName`
  (params (Name :type Text :default "NSLOCTEXT(\"[10ACA0A04D093029BC174D9DCF1D044B]\", \"1DB789D34D489D7A9951F3B88C314FA3\", \"测试Name\")"))
  (bind _returnvalue (`|CreateWidget` "/Game/FinalProject/Gameplay/UI/WO_AreaName.WO_AreaName_C" self Name))
  (`UserWidget.AddToViewport` _returnvalue 0))

(fn `AddConfirmWindow`
  (params (ConfirmText :type Text :default "NSLOCTEXT(\"[10ACA0A04D093029BC174D9DCF1D044B]\", \"C7CCD021430CBFDB3292CD8827AFE75A\", \"测试\")"))
  (returns (Return :type Boolean) (ConfirmWindow :type "/Game/FinalProject/Gameplay/UI/WO_ConfirmWIndow Object Reference"))
  (`/Engine/EditorBlueprintResources/StandardMacros.IsValid` (`self.WO_Comfirm`)
    (:`Is Valid`
      (return false null))
    (:`Is Not Valid`
      (bind _returnvalue (`|CreateWidget` "/Game/FinalProject/Gameplay/UI/WO_ConfirmWIndow.WO_ConfirmWIndow_C" null ConfirmText))
      (bind _output_get (set `self.WO_Comfirm` _returnvalue))
      (`UserWidget.AddToViewport` _output_get 0)
      (`Widget.SetFocus` _output_get)
      (add `/Game/FinalProject/Gameplay/UI/WO_ConfirmWIndow.ED_Cancel` _output_get (`|CreateDelegate` :!event `RemoveConfirmWindow`))
      (return true _output_get))))

(fn `AddScreenTip`
  (params (Tip :type Text :default "NSLOCTEXT(\"[10ACA0A04D093029BC174D9DCF1D044B]\", \"858522294F449F4890FE7BA373F379A6\", \"测试Tip\")"))
  (bind _returnvalue (`|CreateWidget` "/Game/FinalProject/Gameplay/UI/WO_ScreenTip.WO_ScreenTip_C" self Tip))
  (`UserWidget.AddToViewport` _returnvalue 0))

(fn `CheckCanBeInputKey`
  (params (Key :type "Key Structure" :default "None"))
  (returns (Return :type Boolean))
  (return (and (not (== Key "Escape")) (not (== Key "Enter")) (not (== Key "P")))))

(fn `RemoveConfirmWindow`
  (bind _wo_comfirm (`self.WO_Comfirm`))
  (clear `/Game/FinalProject/Gameplay/UI/WO_ConfirmWIndow.ED_Cancel` _wo_comfirm)
  (clear `/Game/FinalProject/Gameplay/UI/WO_ConfirmWIndow.ED_Confirm` _wo_comfirm)
  (`Widget.RemoveFromParent` _wo_comfirm)
  (set `self.WO_Comfirm` null))

(fn `UserConstructionScript`)