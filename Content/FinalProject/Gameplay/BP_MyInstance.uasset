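; Game instance that holds persistent game state: player settings, level save progress and collected treasures.
; Settings and game progress use separate save slots, with load, existence-check and delete helpers for the game slot.
; A cached level save object stores level name, character and torch data, and is exposed to other code.
; On Init, a data table seeds the treasure map as uncollected; pickups flip entries in memory only.
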(event `self.ReceiveInit`
  (`|ExecutionSequence`
    (:`then_0`
      (`self.LoadTreasureData`))))

(fn `DeleteSaveGameData`
  (returns (ReturnValue :type Boolean))
  (bind _returnvalue (`GameplayStatics.DeleteGameInSlot` (`self.SaveGameSlotName`)))
  (set `self.SaveGameLevel_Obj` null)
  (return _returnvalue))

(fn `DoseSaveGameExit`
  (returns (ReturnValue :type Boolean))
  (bind _returnvalue (`GameplayStatics.DoesSaveGameExist` (`self.SaveGameSlotName`)))
  (return _returnvalue))

(fn `GetSaveGameObj`
  (returns (Return :type Boolean) (SaveGameLevel :type "/Game/FinalProject/Gameplay/Z_SaveGame/BP_SaveGame_Level Object Reference"))
  (bind _savegamelevel_obj (`self.SaveGameLevel_Obj`))
  (`/Engine/EditorBlueprintResources/StandardMacros.IsValid` _savegamelevel_obj
    (:`Is Valid`
      (return true _savegamelevel_obj))
    (:`Is Not Valid`
      (return false null))))

(fn `GetTreasureData`
  (returns (Treasures :type "Map of /Game/FinalProject/Gameplay/Treasure/ETreasure Enum to Boolean"))
  (return (`self.Treasures`)))

(fn `LoadGame`
  (returns (ReturnValue :type Boolean) (LevelName :type String) (CharacterData :type "/Game/FinalProject/Gameplay/Z_SaveGame/SSave_Character Structure"))
  (bind _returnvalue (`self.DoseSaveGameExit`))
  (if _returnvalue
    (bind _returnvalue_2 (`GameplayStatics.LoadGameFromSlot` (`self.SaveGameSlotName`)))
    (bind _asbp_save_game_level (cast `/Game/FinalProject/Gameplay/Z_SaveGame/BP_SaveGame_Level` _returnvalue_2))
    (bind _output_get (set `self.SaveGameLevel_Obj` _asbp_save_game_level))
    (bind (_levelname _characterdata) (`/Game/FinalProject/Gameplay/Z_SaveGame/BP_SaveGame_Level.GetData` _output_get))
    (return true _levelname _characterdata)
    (else
      (return false ""))))

(fn `LoadSettings`
  (returns (Exist :type Boolean) (Settings :type "/Game/FinalProject/Gameplay/Z_SaveGame/SSettings Structure"))
  (bind _savesettingsslotname (`self.SaveSettingsSlotName`))
  (bind _returnvalue (`GameplayStatics.DoesSaveGameExist` _savesettingsslotname))
  (if _returnvalue
    (bind _returnvalue_2 (`GameplayStatics.LoadGameFromSlot` _savesettingsslotname))
    (bind _asbp_save_game_settings (cast `/Game/FinalProject/Gameplay/Z_SaveGame/BP_SaveGame_Settings` _returnvalue_2))
    (bind _output_get (set `self.Settings` (`/Game/FinalProject/Gameplay/Z_SaveGame/BP_SaveGame_Settings.Settings` _asbp_save_game_settings)))
    (return true _output_get)
    (else
      (return false (`self.Settings`)))))

(fn `LoadTreasureData`
  (bind _outrownames (`DataTableFunctionLibrary.GetDataTableRowNames` (`self.DT_TreasureData`)))
  (for _array_element _outrownames
    (bind _returnvalue (`|GetDataTableRow` (`self.DT_TreasureData`) _array_element)
      (:`then`
        (`BlueprintMapLibrary.Map_Add` (`self.Treasures`) (`.Treasure_2_09D73C894D7D1AAD965045BB81CE8C66` (break `/Game/FinalProject/Gameplay/Treasure/STreasureData` _returnvalue)))))))

(fn `PickUpTreasure`
  (params (TreasureType :type "/Game/FinalProject/Gameplay/Treasure/ETreasure Enum" :default "NewEnumerator0"))
  (bind _treasures (`self.Treasures`))
  (`BlueprintMapLibrary.Map_Remove` _treasures TreasureType)
  (`BlueprintMapLibrary.Map_Add` _treasures TreasureType true)
  (return))

(fn `SaveGame`
  (params (CharacterData :type "/Game/FinalProject/Gameplay/Z_SaveGame/SSave_Character Structure") (TorchsData :type "Map of String to /Game/FinalProject/Gameplay/Z_SaveGame/SSave_Torch Structure"))
  (returns (ReturnValue :type Boolean))
  (`|ExecutionSequence`
    (:`then_0`
      (`/Engine/EditorBlueprintResources/StandardMacros.IsValid` (`self.SaveGameLevel_Obj`)
        (:`Is Not Valid`
          (bind _returnvalue (`GameplayStatics.CreateSaveGameObject` "/Game/FinalProject/Gameplay/Z_SaveGame/BP_SaveGame_Level.BP_SaveGame_Level_C"))
          (set `self.SaveGameLevel_Obj` _returnvalue))))
    (:`then_1`
      (bind _returnvalue_2 (`GameplayStatics.GetCurrentLevelName` true))
      (`/Game/FinalProject/Gameplay/Z_SaveGame/BP_SaveGame_Level.SetData` (`self.SaveGameLevel_Obj`) _returnvalue_2 CharacterData TorchsData))
    (:`then_2`
      (bind _returnvalue_3 (`GameplayStatics.SaveGameToSlot` (`self.SaveGameLevel_Obj`) (`self.SaveGameSlotName`)))
      (return _returnvalue_3))))

(fn `SaveSettings`
  (params (Settings :type "/Game/FinalProject/Gameplay/Z_SaveGame/SSettings Structure"))
  (bind _output_get (set `self.Settings` Settings))
  (bind _returnvalue (`GameplayStatics.CreateSaveGameObject` "/Game/FinalProject/Gameplay/Z_SaveGame/BP_SaveGame_Settings.BP_SaveGame_Settings_C"))
  (set `/Game/FinalProject/Gameplay/Z_SaveGame/BP_SaveGame_Settings.Settings` _output_get _returnvalue)
  (bind _returnvalue_2 (`GameplayStatics.SaveGameToSlot` _returnvalue (`self.SaveSettingsSlotName`)))
  (if (not _returnvalue_2)
    (`KismetSystemLibrary.PrintString` "保存失败" true true (struct :`R` 1.0 :`A` 1.0) 5.0)))