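; BP_Treasure is a pickup actor that a character can interact with to collect treasure.
; Its construction script finds the DTTreasureData row matching TreasureType and applies that row's mesh.
; Interaction functions always allow pickup, show a "捡起" (pick up) tip and supply a move-to point just short of the item, facing it.
; Interacting passes TreasureType to the character's PickUpTreasure and destroys the actor.
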(event `self.ReceiveBeginPlay`)

(fn `ChechCanInteract`
  (params (InteractComponent :type "PrimitiveComponent Object Reference") (Character :type "/Game/FinalProject/Gameplay/Character/BP_MyCharacter Object Reference"))
  (returns (`Return Value` :type Boolean))
  (return true))

(fn `GetInteractState`
  (returns (bInteract :type Boolean))
  (return false))

(fn `GetInteractTipUIInfo`
  (params (InteractComponent :type "PrimitiveComponent Object Reference"))
  (returns (WorldPosition :type "Vector Structure") (TipText :type Text))
  (return (`SceneComponent.K2_GetComponentLocation` (`self.TipPos`)) "捡起"))

(fn `GetMoveToInfo`
  (params (InteractComponent :type "PrimitiveComponent Object Reference") (Character :type "/Game/FinalProject/Gameplay/Character/BP_MyCharacter Object Reference"))
  (returns (InteractType :type "/Game/FinalProject/Gameplay/Interactive/EInteractType Enum") (NeedHolster :type Boolean) (NeedHold :type Boolean) (TargetPos :type "Vector Structure") (TargetRot :type "Rotator Structure"))
  (bind (_returnvalue_x _returnvalue_y) (`KismetMathLibrary.BreakVector` (`self.K2_GetActorLocation` Character)))
  (bind (_returnvalue_x_2 _returnvalue_y_2) (`KismetMathLibrary.BreakVector` (`self.K2_GetActorLocation`)))
  (bind _returnvalue (`KismetMathLibrary.MakeVector` _returnvalue_x_2 _returnvalue_y_2))
  (bind _returnvalue_2 (`KismetMathLibrary.MakeVector` _returnvalue_x _returnvalue_y))
  (return "NewEnumerator6" false false (+ (`self.K2_GetActorLocation`) (* (`KismetMathLibrary.Normal` (- _returnvalue_2 _returnvalue)) 20.0)) (`KismetMathLibrary.FindLookAtRotation` _returnvalue_2 _returnvalue)))

(fn `Interact`
  (params (Character :type "/Game/FinalProject/Gameplay/Character/BP_MyCharacter Object Reference") (InteractComponent :type "PrimitiveComponent Object Reference"))
  (returns (InteractType :type "/Game/FinalProject/Gameplay/Interactive/EInteractType Enum") (TargetActor :type "Actor Object Reference") (InteractAction :type "/Game/FinalProject/Gameplay/Character/EInteractAction Enum"))
  (`/Game/FinalProject/Gameplay/Character/BP_MyCharacter.PickUpTreasure` Character (`self.TreasureType`))
  (`self.K2_DestroyActor`)
  (return "NewEnumerator0" null "NewEnumerator2"))

(fn `Move`
  (params (Character :type "/Game/FinalProject/Gameplay/Character/BP_MyCharacter Object Reference") (Value :type "Float (double-precision)"))
  (returns (Velocity :type "Vector Structure"))
  (return (0.0 0.0 0.0)))

(fn `StopInteract`
  (params (Character :type "/Game/FinalProject/Gameplay/Character/BP_MyCharacter Object Reference"))
  (returns (ReturnValue :type Boolean) (InteractAction :type "/Game/FinalProject/Gameplay/Character/EInteractAction Enum"))
  (return false "NewEnumerator2"))

(fn `UserConstructionScript`
  (bind (_treasuredata_treasure _treasuredata_showname _treasuredata_description _treasuredata_mesh) (break `/Game/FinalProject/Gameplay/Treasure/STreasureData` (`self.TreasureData`)))
  (`|ExecutionSequence`
    (:`then_0`
      (bind _outrownames (`DataTableFunctionLibrary.GetDataTableRowNames` (`self.DT_TreasureData`)))
      (for _array_element _outrownames
        (bind _returnvalue (`|GetDataTableRow` (`self.DT_TreasureData`) _array_element)
          (:`then`
            (if (`|EnumEquality` (`.Treasure_2_09D73C894D7D1AAD965045BB81CE8C66` (break `/Game/FinalProject/Gameplay/Treasure/STreasureData` _returnvalue)) (`self.TreasureType`))
              (set `self.TreasureData` _returnvalue))))))
    (:`then_1`
      (`StaticMeshComponent.SetStaticMesh` (`self.Mesh`) _treasuredata_mesh))))