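; Base game mode that handles master audio fade-in and provides shared hooks for input and level loading.
; BeginPlay sets the base sound mix, and a custom event plays a speed-adjustable timeline that drives the master sound class volume through a mix override.
; OpenLevel loads a level by name, while the pause, any-key and Enter functions are empty stubs.
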(event `self.ReceiveBeginPlay`
  (`|ExecutionSequence`
    (:`then_0`
      (`GameplayStatics.SetBaseSoundMix` (`self.BaseSoundMix`)))))

(event `CE_A_FadeInVolume`
  (params (Speed :type "Float (double-precision)" :default 1.0))
  (`TimelineComponent.SetPlayRate` (`self.TL_FadeInVolume`) Speed)
  (bind (_direction _volume) (`Timeline|TL_FadeInVolume` :!via `PlayFromStart`)
    (:`Update`
      (`GameplayStatics.SetSoundMixClassOverride` (`self.BaseSoundMix`) "/Game/FinalProject/Sound/_SoundClassAndMix/MySoundClass_Master.MySoundClass_Master" _volume 1.0 0.0))))

(fn `OpenLevel`
  (params (Level :type "World Soft Object Reference") (LevelName :type Name))
  (`GameplayStatics.OpenLevel` LevelName))

(fn `PressAnyKey`
  (params (Key :type "Key Structure" :default "None")))

(fn `PressEnter`)

(fn `PressPause`)

(fn `UserConstructionScript`)