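; BP_Module_DoorUp is a module actor that wraps an upward door, apparently driven by conducted energy, as a child actor.
; The construction script casts the DoorUp child to BP_Door_Up_New and copies the module's voltage limit, height limit and move speed onto it.
; Conduct forwards incoming energy to the child's ConductMessage and returns its result, leaving the event graph unused.
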(fn `Conduct`
  (params (EnergyIn :type "Float (double-precision)"))
  (returns (Consume :type "Float (double-precision)"))
  (bind _consume (message `/Game/FinalProject/Gameplay/Electronic/IElectronic.Conduct` (`ChildActorComponent.ChildActor` (`self.DoorUp`)) EnergyIn))
  (return _consume))

(fn `UserConstructionScript`
  (bind _asbp_door_up_new (cast `/Game/FinalProject/Gameplay/Electronic/BP_Door_Up_New` (`ChildActorComponent.ChildActor` (`self.DoorUp`))))
  (set `/Game/FinalProject/Gameplay/Electronic/BP_Door_Up_New.MaxVolt` (`self.MaxVolt`) _asbp_door_up_new)
  (set `/Game/FinalProject/Gameplay/Electronic/BP_Door_Up_New.MaxHeight` (`self.MaxHeight`) _asbp_door_up_new)
  (set `/Game/FinalProject/Gameplay/Electronic/BP_Door_Up_New.MoveSpeed` (`self.MoveSpeed`) _asbp_door_up_new))