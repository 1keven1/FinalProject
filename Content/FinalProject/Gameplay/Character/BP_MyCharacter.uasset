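; Player character with a grappling-hook swing and object interaction, such as picking up a torch.
; A state enum gates input and per-tick logic, which picks hook points and interactables by camera aim, distance and line-of-sight, then updates UI tips.
; Hooking makes the character follow a spawned rope actor's particle, pushed by input, keeping momentum on release.
; Interacting auto-walks and turns the character to a target before attaching the item to its hand socket.
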(event `InputAction|Hook`
  (params (Key :type "Key Structure"))
  (:`Pressed`
    (`self.SwitchCharacterState`
      (:`Stand`
        (`/Engine/EditorBlueprintResources/StandardMacros.IsValid` (`self.AimedHookPoint`) :!label _label
          (:`Is Valid`
            (`self.SetHook` true))))
      (:`Run`
        (goto _label))
      (:`Hook`
        (`self.SetHook` false)))))

(event `self.ReceiveBeginPlay`
  (`|ExecutionSequence`
    (:`then_0`
      (bind _asbp_my_game_mode (cast `/Game/FinalProject/Gameplay/BP_MyGameMode` (`GameplayStatics.GetGameMode`)))
      (set `self.MyGameMode` _asbp_my_game_mode)
      (bind _asbp_my_controller (cast `/Game/FinalProject/Gameplay/BP_MyController` (`self.GetController`)))
      (set `self.MyController` _asbp_my_controller))
    (:`then_1`
      (bind _returnvalue (`|SpawnActorFromClass` "/Game/FinalProject/Gameplay/Character/BP_HookString.BP_HookString_C" (`KismetMathLibrary.MakeTransform` (0.0 0.0 0.0)) "AlwaysSpawn" "OverrideRootScale" null null))
      (bind _output_get (set `self.HookString` _returnvalue))
      (`self.SetActorHiddenInGame` _output_get true))
    (:`then_2`
      (add `self.ED_ReachMovePoint` (delegate `ReachMovePoint_Event`)))))

(event `CE_HookBehaviorTick`
  (`self.SwitchCharacterState`
    (:`Stand`
      (`self.MoveHookString` :!label _label_2))
    (:`Run`
      (goto _label_2))
    (:`Hook`
      (`self.SwingWhenHooking`))))

(event `self.HookFinder.OnComponentBeginOverlap`
  (params (OverlappedComponent :type "PrimitiveComponent Object Reference") (OtherActor :type "Actor Object Reference") (OtherComp :type "PrimitiveComponent Object Reference") (OtherBodyIndex :type Integer) (bFromSweep :type Boolean) (SweepResult :type "HitResult Structure (by ref)"))
  (`KismetArrayLibrary.Array_Add` (`self.HookPointsInRange`) OtherActor))

(event `InputAxis|LookRight`
  (params (AxisValue :type "Float (single-precision)"))
  ;[0 0 0] Move
  (`self.AddControllerYawInput` AxisValue))

(event `InputAxis|LookUp`
  (params (AxisValue :type "Float (single-precision)"))
  ;[0 0 0] Move
  (`self.AddControllerPitchInput` AxisValue))

(event `self.HookFinder.OnComponentEndOverlap`
  (params (OverlappedComponent :type "PrimitiveComponent Object Reference") (OtherActor :type "Actor Object Reference") (OtherComp :type "PrimitiveComponent Object Reference") (OtherBodyIndex :type Integer))
  (`KismetArrayLibrary.Array_RemoveItem` (`self.HookPointsInRange`) OtherActor))

(event `CE_InteractBehavior`
  (bind _aimedinteractobj (`self.AimedInteractObj`))
  (`self.SwitchCharacterState`
    (:`Stand`
      _)
    (:`Run`
      _))
  (`/Engine/EditorBlueprintResources/StandardMacros.IsValid` _aimedinteractobj
    (:`Is Valid`
      (set `self.CharatcerState` "NewEnumerator2")
      (set `self.ProcessingObj` _aimedinteractobj)
      (`|ExecutionSequence`
        (:`then_0`
          ;[0 0 0] 若拿着东西 先收到HosterTemp
          (`/Engine/EditorBlueprintResources/StandardMacros.IsValid` (`self.InHandObj`)))
        (:`then_1`
          (bind (_interacttype _targetpos _targetrot) (message `/Game/FinalProject/Gameplay/Interactive/IInteract.GetInteractInfo` _aimedinteractobj))
          (bind _output_get (set `self.InteractingType` _interacttype))
          (switch `/Game/FinalProject/Gameplay/Interactive/EInteractType` _output_get
            (:`NewEnumerator1`
              (`self.CharacterMoveTo` _targetpos _targetrot))))))))

(event `self.InteractFinder.OnComponentBeginOverlap`
  (params (OverlappedComponent :type "PrimitiveComponent Object Reference") (OtherActor :type "Actor Object Reference") (OtherComp :type "PrimitiveComponent Object Reference") (OtherBodyIndex :type Integer) (bFromSweep :type Boolean) (SweepResult :type "HitResult Structure (by ref)"))
  (`KismetArrayLibrary.Array_Add` (`self.InteractCompInRange`) OtherComp))

(event `InputAction|Interact`
  (params (Key :type "Key Structure"))
  (:`Pressed`
    (if (`self.CheckCanInteract`)
      (`self.CE_InteractBehavior`))))

(event `InputAxis|MoveForward`
  (params (AxisValue :type "Float (single-precision)"))
  (bind (_returnvalue_roll _returnvalue_pitch _returnvalue_yaw) (`KismetMathLibrary.BreakRotator` (`self.GetControlRotation`)))
  ;[0 0 0] Move
  (`self.SwitchCharacterState`
    (:`Stand`
      _)
    (:`Run`
      _))
  (`self.AddMovementInput` (`KismetMathLibrary.GetForwardVector` (`KismetMathLibrary.MakeRotator` 0.0 0.0 _returnvalue_yaw)) AxisValue))

(event `ReachMovePoint_Event`
  (`self.ReachMovePoint`))

(event `InputAction|Reach`
  (params (Key :type "Key Structure"))
  (:`Pressed`
    (`self.SwitchCharacterState`
      (:`Stand`
        _)
      (:`Run`
        _))
    (`/Engine/EditorBlueprintResources/StandardMacros.IsValid` (`self.InHandObj`)
      (:`Is Valid`
        (set `self.bReach` true))))
  (:`Released`
    (`self.SwitchCharacterState`
      (:`Stand`
        _)
      (:`Run`
        _))
    (`/Engine/EditorBlueprintResources/StandardMacros.IsValid` (`self.InHandObj`)
      (:`Is Valid`
        (set `self.bReach` false)))))

(event `self.InteractFinder.OnComponentEndOverlap`
  (params (OverlappedComponent :type "PrimitiveComponent Object Reference") (OtherActor :type "Actor Object Reference") (OtherComp :type "PrimitiveComponent Object Reference") (OtherBodyIndex :type Integer))
  (`KismetArrayLibrary.Array_RemoveItem` (`self.InteractCompInRange`) OtherComp))

(event `InputAxis|MoveRight`
  (params (AxisValue :type "Float (single-precision)"))
  (bind (_returnvalue_roll _returnvalue_pitch _returnvalue_yaw) (`KismetMathLibrary.BreakRotator` (`self.GetControlRotation`)))
  ;[0 0 0] Move
  (`self.SwitchCharacterState`
    (:`Stand`
      _)
    (:`Run`
      _))
  (`self.AddMovementInput` (`KismetMathLibrary.GetRightVector` (`KismetMathLibrary.MakeRotator` _returnvalue_roll 0.0 _returnvalue_yaw)) AxisValue))

(event `self.ReceiveTick`
  (params (DeltaSeconds :type "Float (single-precision)"))
  (`|ExecutionSequence`
    (:`then_0`
      (`self.EvaluateStandOrRun`)
      (`self.EvaluateHookPoint`)
      (`self.EvaluateInteractObj`)
      (`self.UpdateUI_InteractTips`))
    (:`then_1`
      (`self.CE_HookBehaviorTick`)
      (`self.MoveToBehaviorTick`)
      (`self.RotateCharacterWhenReach` 10.0))
    (:`then_4`
      (if (`self.bDebug`)
        (`/Game/FinalProject/Gameplay/BP_MyController.MainUI_Debug` (`self.MyController`) (`self.CharatcerState`) (`self.InteractingType`))))))

(event `InputAction|Jump` :overrideparent false
  (params (Key :type "Key Structure"))
  ;[0 0 0] Move
  (:`Pressed`
    (`self.SwitchCharacterState`
      (:`Stand`
        (`self.Jump` :!label _label_3))
      (:`Run`
        (goto _label_3))
      (:`Hook`
        (`self.SetHook` false))))
  (:`Released`
    (`self.SwitchCharacterState`
      (:`Stand`
        _)
      (:`Run`
        _))
    (`self.StopJumping`)))

(fn `CharacterMoveTo`
  (params (TargetPos :type "Vector Structure") (TargetRot :type "Rotator Structure"))
  (set `self.MoveToTargetPos` TargetPos)
  (set `self.MoveToTargetRot` (`KismetMathLibrary.SelectRotator` (struct :`Yaw` 1.0) TargetRot (== TargetRot (struct) :`ErrorTolerance` 0.1)))
  (return))

(fn `CheckActorAimed_Dot`
  (params (Actor :type "Actor Object Reference") (ResultStep :type "Float (double-precision)" :default 0.9))
  (returns (Aimed :type Boolean))
  (bind _followcamera (`self.FollowCamera`))
  (return (> (`KismetMathLibrary.Dot_VectorVector` (`KismetMathLibrary.Normal` (- (`self.K2_GetActorLocation` Actor) (`SceneComponent.K2_GetComponentLocation` _followcamera))) (`SceneComponent.GetForwardVector` _followcamera)) ResultStep)))

(fn `CheckCanInteract`
  (returns (Return :type Boolean))
  (return (and (`KismetSystemLibrary.IsValid` (`self.AimedInteractObj`)) (not (`NavMovementComponent.IsFalling` (`self.CharacterMovement`))))))

(fn `EvaluateHookPoint`
  (locals (AimedHookPoints :type "Array of Actor Object Reference"))
  (bind _hookpointsinrange (`self.HookPointsInRange`))
  (bind _aimedhookpoints (`local.AimedHookPoints`))
  (set `self.AimedHookPoint` null)
  (`self.SwitchCharacterState`
    (:`Stand`
      _)
    (:`Run`
      _)
    (:`Process`
      (return))
    (:`Hook`
      (return))
    (:`Hold`
      (return))
    (:`Push`
      (return))
    (:`Rest`
      (return)))
  (if (`KismetArrayLibrary.Array_IsNotEmpty` _hookpointsinrange)
    (`KismetArrayLibrary.Array_Clear` (`local.AimedHookPoints`))
    (for _array_element _hookpointsinrange
      (if (`self.CheckActorAimed_Dot` _array_element 0.91)
        (`KismetArrayLibrary.Array_Add` (`local.AimedHookPoints`) _array_element)))
    (if (`KismetArrayLibrary.Array_IsNotEmpty` _aimedhookpoints)
      (bind _sortedactors (`/Game/FinalProject/Gameplay/BPFL_MyFunctionLibrary.SortActorsByDistance` _aimedhookpoints self))
      (bind (_return _visableactor) (`self.GetFirstVisableActor` _sortedactors))
      (if _return
        (bind _asbp_hook_point (cast `/Game/FinalProject/Gameplay/Interactive/BP_HookPoint` _visableactor))
        (set `self.AimedHookPoint` _asbp_hook_point)
        (return)
        (else
          (return)))
      (else
        (return)))
    (else
      (return))))

(fn `EvaluateInteractObj`
  (locals (AimedInteractComps :type "Array of PrimitiveComponent Object Reference"))
  (bind _aimedinteractcomps (`local.AimedInteractComps`))
  (set `self.AimedInteractObj` null)
  (`self.SwitchCharacterState`
    (:`Stand`
      _)
    (:`Run`
      _)
    (:`Process`
      (return))
    (:`Hook`
      (return))
    (:`Hold`
      (return))
    (:`Push`
      (return))
    (:`Rest`
      (return)))
  (if (and (not (`NavMovementComponent.IsFalling` (`self.CharacterMovement`))) (`KismetArrayLibrary.Array_IsNotEmpty` (`self.InteractCompInRange`)))
    (`KismetArrayLibrary.Array_Clear` (`local.AimedInteractComps`))
    (for _array_element (`self.InteractCompInRange`)
      (if (`self.CheckActorAimed_Dot` (`ActorComponent.GetOwner` _array_element))
        (`KismetArrayLibrary.Array_Add` (`local.AimedInteractComps`) _array_element)))
    (if (`KismetArrayLibrary.Array_IsNotEmpty` _aimedinteractcomps)
      (bind _sortedcomponents (`/Game/FinalProject/Gameplay/BPFL_MyFunctionLibrary.SortCompsByDistance` _aimedinteractcomps self))
      (bind (_return _visablecomp) (`self.GetFirstVisableComp` _sortedcomponents))
      (if _return
        (bind _output_get (set `self.AimedInteractComp` _visablecomp))
        (set `self.AimedInteractObj` (`ActorComponent.GetOwner` _output_get))
        (return)
        (else
          (return)))
      (else
        (return)))
    (else
      (return))))

(fn `EvaluateStandOrRun`
  (`self.SwitchCharacterState`
    (:`Stand`
      _)
    (:`Run`
      _))
  (if (> (`KismetMathLibrary.VSize` (`MovementComponent.Velocity` (`self.CharacterMovement`))) 0.0)
    (set `self.CharatcerState` "NewEnumerator1")
    (else
      (set `self.CharatcerState` "NewEnumerator0"))))

(fn `GetFirstVisableActor`
  (params (List :type "Array of Actor Object Reference"))
  (returns (Return :type Boolean) (VisableActor :type "Actor Object Reference"))
  (for _array_element List
    (bind (_outhit _returnvalue) (`KismetSystemLibrary.LineTraceSingle` (`self.K2_GetActorLocation` _array_element) (`SceneComponent.GetSocketLocation` (`self.Mesh`) "head") "TraceTypeQuery1" false (`|MakeArray` _array_element)))
    (if (not _returnvalue)
      (return true _array_element)))
  (return false null))

(fn `GetFirstVisableComp`
  (params (List :type "Array of PrimitiveComponent Object Reference"))
  (returns (Return :type Boolean) (VisableComp :type "PrimitiveComponent Object Reference"))
  (for _array_element List
    (bind (_outhit _returnvalue) (`KismetSystemLibrary.LineTraceSingle` (`SceneComponent.K2_GetComponentLocation` _array_element) (`SceneComponent.GetSocketLocation` (`self.Mesh`) "head") "TraceTypeQuery1" false (`|MakeArray` (`ActorComponent.GetOwner` _array_element))))
    (if (not _returnvalue)
      (return true _array_element)))
  (return false null))

(fn `MoveHookString`
  (bind _aimedhookpoint (`self.AimedHookPoint`))
  (bind _hookstring (`self.HookString`))
  (bind _returnvalue (`SceneComponent.GetSocketLocation` (`self.Mesh`) "Socket_HandL"))
  (`self.K2_SetActorLocation` (`self.HookString`) _returnvalue false false)
  (`/Engine/EditorBlueprintResources/StandardMacros.IsValid` _aimedhookpoint
    (:`Is Valid`
      (`/Game/FinalProject/Gameplay/Character/BP_HookString.SetEndAttachment` _hookstring _aimedhookpoint)
      (`/Game/FinalProject/Gameplay/Character/BP_HookString.SetStringLength` _hookstring (`KismetMathLibrary.FMax` (* (`KismetMathLibrary.Vector_Distance` (`self.K2_GetActorLocation` _aimedhookpoint) _returnvalue) 0.9) 400.0)))
    (:`Is Not Valid`
      (`/Game/FinalProject/Gameplay/Character/BP_HookString.SetEndAttachment` _hookstring null))))

(fn `MoveToBehaviorTick`
  (bind _returnvalue (`self.K2_GetActorRotation`))
  (bind _movetotargetrot (`self.MoveToTargetRot`))
  (bind _movetotargetpos (`self.MoveToTargetPos`))
  (bind _yaw (.yaw _movetotargetrot))
  (bind (_returnvalue_x _returnvalue_y) (`KismetMathLibrary.BreakVector` (- _movetotargetpos (`self.K2_GetActorLocation`))))
  (bind _returnvalue_2 (`KismetMathLibrary.VSize` (`KismetMathLibrary.MakeVector` _returnvalue_x _returnvalue_y)))
  (`|ExecutionSequence`
    (:`then_0`
      (if (!= _movetotargetpos (0.0 0.0 0.0) :`ErrorTolerance` 0.1)
        (`self.AddMovementInput` (`KismetMathLibrary.Normal` (`KismetMathLibrary.MakeVector` _returnvalue_x _returnvalue_y)) (* (`KismetMathLibrary.FClamp` (* _returnvalue_2 0.03) 0.1) 0.5))
        (if (< _returnvalue_2 1.0)
          (set `self.MoveToTargetPos` (0.0 0.0 0.0)))))
    (:`then_1`
      (if (and (== (`self.MoveToTargetPos`) (0.0 0.0 0.0) :`ErrorTolerance` 0.1) (!= _movetotargetrot (struct) :`ErrorTolerance` 0.1))
        (`self.K2_SetActorRotation` (`KismetMathLibrary.RInterpTo_Constant` _returnvalue (`KismetMathLibrary.MakeRotator` 0.0 0.0 _yaw) (`GameplayStatics.GetWorldDeltaSeconds`) 400.0))
        (if (`KismetMathLibrary.NearlyEqual_FloatFloat` (.yaw _returnvalue) _yaw 0.001)
          (set `self.MoveToTargetRot` (struct))
          (`self.ED_ReachMovePoint`))))))

(fn `ReachMovePoint`
  (if (`|EnumInequality` (`self.InteractingType`) "NewEnumerator0")
    (bind (_interacttype _targetactor) (message `/Game/FinalProject/Gameplay/Interactive/IInteract.Interact` (`self.ProcessingObj`) self (`self.AimedInteractComp`)))
    (switch `/Game/FinalProject/Gameplay/Interactive/EInteractType` _interacttype
      (:`NewEnumerator1`
        (`self.K2_AttachToComponent` _targetactor (`self.Mesh`) "Socket_TorchR" "SnapToTarget" "SnapToTarget" "KeepRelative" true)
        (set `self.InHandObj` _targetactor)
        (set `self.CharatcerState` "NewEnumerator0")
        (set `self.InteractingType` "NewEnumerator0")
        (set `self.ProcessingObj` null)))))

(fn `RotateCharacterWhenReach`
  (params (RotateSpeed :type "Float (double-precision)" :default 20.0))
  (bind (_returnvalue_roll _returnvalue_pitch _returnvalue_yaw) (`KismetMathLibrary.BreakRotator` (`self.GetControlRotation`)))
  (`self.SwitchCharacterState`
    (:`Stand`
      (if (`self.bReach`)
        (`self.K2_SetActorRotation` (`KismetMathLibrary.RInterpTo` (`self.K2_GetActorRotation`) (`KismetMathLibrary.MakeRotator` 0.0 0.0 _returnvalue_yaw) (`GameplayStatics.GetWorldDeltaSeconds`) RotateSpeed))))))

(fn `SetHook`
  (params (NewHook :type Boolean))
  (bind _hookstring (`self.HookString`))
  (bind _charactermovement (`self.CharacterMovement`))
  (if NewHook
    (`/Game/FinalProject/Gameplay/Character/BP_HookString.SetAttach` _hookstring false true)
    (`self.SetActorHiddenInGame` _hookstring false)
    (set `self.CharatcerState` "NewEnumerator3")
    (else
      (`/Game/FinalProject/Gameplay/Character/BP_HookString.SetAttach` _hookstring true true)
      (`self.SetActorHiddenInGame` _hookstring true)
      (`MovementComponent.StopMovementImmediately` _charactermovement)
      (set `MovementComponent.Velocity` (+ (* (`self.SwingVelocity`) 1.0) (0.0 0.0 100.0)) _charactermovement)
      (set `self.CharatcerState` "NewEnumerator0"))))

(fn `SwingWhenHooking`
  (bind _returnvalue (`GameplayStatics.GetTimeSeconds`))
  (bind (_returnvalue_roll _returnvalue_pitch _returnvalue_yaw) (`KismetMathLibrary.BreakRotator` (`self.GetControlRotation`)))
  (bind (_returnvalue_roll_2 _returnvalue_pitch_2 _returnvalue_yaw_2) (`KismetMathLibrary.BreakRotator` (`self.GetControlRotation`)))
  (bind _returnvalue_2 (`KismetMathLibrary.FMax` (`KismetMathLibrary.Abs` (`self.GetInputAxisValue`)) (`KismetMathLibrary.Abs` (`self.GetInputAxisValue`))))
  (bind _output (`|GetArrayItem` (`/Game/FinalProject/Gameplay/Character/BP_HookString.GetParticle` (`self.HookString`))))
  (bind _returnvalue_3 (- _output (`self.LastPos`)))
  (bind _sweephitresult (`self.K2_SetActorLocation` (- _output (- (`SceneComponent.GetSocketLocation` (`self.Mesh`) "Socket_HandL") (`self.K2_GetActorLocation`))) true))
  (bind (_bblockinghit _binitialoverlap _time _distance _location _impactpoint _normal) (`GameplayStatics.BreakHitResult` _sweephitresult))
  (if (not _bblockinghit)
    (`|ExecutionSequence`
      (:`then_0`
        ;[0 0 0] Calculate Velocity
        (if (> (`KismetMathLibrary.VSize` _returnvalue_3) 0.0)
          (set `self.SwingVelocity` (/ _returnvalue_3 (- _returnvalue (`self.LastTime`))))
          (set `self.LastPos` _output)
          (set `self.LastTime` _returnvalue)))
      (:`then_1`
        ;[0 0 0] Add Force to String
        (`/Game/FinalProject/Gameplay/Character/BP_HookString.SetForce` (`self.HookString`) (* (+ (* (`KismetMathLibrary.GetForwardVector` (`KismetMathLibrary.MakeRotator` 0.0 0.0 _returnvalue_yaw)) (`self.GetInputAxisValue`)) (* (`KismetMathLibrary.GetRightVector` (`KismetMathLibrary.MakeRotator` _returnvalue_roll 0.0 _returnvalue_yaw)) (`self.GetInputAxisValue`))) 500.0))
        (if (> _returnvalue_2 0.0)
          (`self.K2_SetActorRotation` (`KismetMathLibrary.RInterpTo` (`self.K2_GetActorRotation`) (`KismetMathLibrary.MakeRotator` 0.0 0.0 _returnvalue_yaw_2) (`GameplayStatics.GetWorldDeltaSeconds`) (* _returnvalue_2 5.0))))))
    (else
      ;[0 0 0] 碰到地面取消Hook状态
      (if (> (`KismetMathLibrary.Dot_VectorVector` _normal (0.0 0.0 1.0)) 0.9)
        (`self.SetHook` false)))))

(fn `Test`
  (locals (Test :type "Float (double-precision)"))
  (bind _output_get (set `local.Test` (+ (`local.Test`) (`GameplayStatics.GetWorldDeltaSeconds`))))
  (`KismetSystemLibrary.PrintString` (`KismetStringLibrary.Conv_DoubleToString` _output_get)))

(fn `UpdateUI_InteractTips`
  (bind _aimedhookpoint (`self.AimedHookPoint`))
  (bind _mycontroller (`self.MyController`))
  (bind _aimedinteractobj (`self.AimedInteractObj`))
  (bind (_returnvalue _viewportposition) (`/Game/FinalProject/Gameplay/BPFL_MyFunctionLibrary.WorldToViewport` _mycontroller (`self.K2_GetActorLocation` _aimedhookpoint)))
  (`|ExecutionSequence`
    (:`then_0`
      (`/Engine/EditorBlueprintResources/StandardMacros.IsValid` _aimedhookpoint
        (:`Is Valid`
          (`/Game/FinalProject/Gameplay/BP_MyController.UpdateUI_HookTip` _mycontroller _returnvalue _viewportposition))
        (:`Is Not Valid`
          (`/Game/FinalProject/Gameplay/BP_MyController.UpdateUI_HookTip` _mycontroller false (0.0 0.0)))))
    (:`then_1`
      (`/Engine/EditorBlueprintResources/StandardMacros.IsValid` _aimedinteractobj
        (:`Is Valid`
          (bind (_worldposition _tiptext) (message `/Game/FinalProject/Gameplay/Interactive/IInteract.GetInteractTipUIInfo` _aimedinteractobj (`self.AimedInteractComp`)))
          (bind (_returnvalue_2 _viewportposition_2) (`/Game/FinalProject/Gameplay/BPFL_MyFunctionLibrary.WorldToViewport` _mycontroller _worldposition))
          (`/Game/FinalProject/Gameplay/BP_MyController.UpdateUI_InteractTip` _mycontroller _returnvalue_2 _tiptext _viewportposition_2))
        (:`Is Not Valid`
          (`/Game/FinalProject/Gameplay/BP_MyController.UpdateUI_InteractTip` _mycontroller false "" (0.0 0.0)))))))

(fn `UserConstructionScript`)