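; BP_HookString is a Blueprint wrapper around a Cable component that serves as the string of a hook in the character gameplay.
; Its functions set the cable's length, force and attachment at both ends, and can retarget the end to a given actor.
; A getter exposes the cable's particle locations to callers.
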(fn `GetParticle`
  (returns (Locations :type "Array of Vector Structure"))
  (return (`CableComponent.GetCableParticleLocations` (`self.Cable`))))

(fn `SetAttach`
  (params (StartAttachment :type Boolean) (EndAttachment :type Boolean))
  (bind _cable (`self.Cable`))
  (set `CableComponent.bAttachStart` StartAttachment _cable)
  (set `CableComponent.bAttachEnd` EndAttachment _cable))

(fn `SetEndAttachment`
  (params (Target :type "Actor Object Reference"))
  (`CableComponent.SetAttachEndTo` (`self.Cable`) Target "None" "None"))

(fn `SetForce`
  (params (Force :type "Vector Structure"))
  (set `CableComponent.CableForce` Force (`self.Cable`)))

(fn `SetStringLength`
  (params (Length :type "Float (double-precision)" :default 100.0))
  (set `CableComponent.CableLength` Length (`self.Cable`)))

(fn `UserConstructionScript`)