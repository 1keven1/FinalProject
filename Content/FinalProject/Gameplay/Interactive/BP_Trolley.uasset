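; Interactive trolley that a character pushes along a spline rail from either of two ends, carrying attached actors with it.
; Construction builds spline-mesh track with end caps, places the trolley and attaches an optional actor.
; Interaction functions check clearance and standing room, then toggle pawn collision; an animation notify starts or stops pushing.
; Move eases speed, advances clamped spline position unless obstructed, wakes nearby physics bodies and returns a movement vector.
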(event `self.ReceiveBeginPlay`
  (set `self.SplineInvLength` (/ 1.0 (`SplineComponent.GetSplineLength` (`self.Spline`)))))

(event `/Game/FinalProject/Gameplay/Interactive/IInteract.ProcessAnimationNotify`
  (params (Character :type "/Game/FinalProject/Gameplay/Character/BP_MyCharacter Object Reference") (InteractComp :type "PrimitiveComponent Object Reference"))
  (if (not (`self.bPushing`))
    (`/Game/FinalProject/Gameplay/Character/BP_MyCharacter.StartPush` Character (`self.SM_Trolley`))
    (set `self.bPushing` true)
    (set `self.InteractingAt1` (== (`self.InteractCollision1`) InteractComp))
    (else
      (`/Game/FinalProject/Gameplay/Character/BP_MyCharacter.StopPush` Character)
      (`PrimitiveComponent.SetCollisionResponseToChannel` (`self.SM_Trolley`) "ECC_Pawn" "ECR_Block")
      (set `self.bPushing` false))))

(event `self.AttachCollision.OnComponentBeginOverlap`
  (params (OverlappedComponent :type "PrimitiveComponent Object Reference") (OtherActor :type "Actor Object Reference") (OtherComp :type "PrimitiveComponent Object Reference") (OtherBodyIndex :type Integer) (bFromSweep :type Boolean) (SweepResult :type "HitResult Structure (by ref)"))
  (if (!= OtherActor self)
    (if (`KismetSystemLibrary.DoesImplementInterface` OtherActor "/Game/FinalProject/Gameplay/Interactive/IInteract.IInteract_C")
      (bind _binteract (message `/Game/FinalProject/Gameplay/Interactive/IInteract.GetInteractState` OtherActor))
      (if (not _binteract)
        (`self.K2_AttachToComponent` OtherActor (`self.SM_Trolley`) "None" "KeepWorld" "KeepWorld" "KeepWorld" true :!label _label))
      (else
        (goto _label)))))

(fn `ChechCanInteract`
  (params (InteractComponent :type "PrimitiveComponent Object Reference") (Character :type "/Game/FinalProject/Gameplay/Character/BP_MyCharacter Object Reference"))
  (returns (`Return Value` :type Boolean))
  (`|ExecutionSequence`
    (:`then_0`
      (bind (_out _length) (`/Game/FinalProject/Gameplay/BPFL_MyFunctionLibrary.ArrayRemoveSelfAndCharacter` (`PrimitiveComponent.GetOverlappingActors` InteractComponent null) (`local.Character`) self))
      (if (!= _length 0)
        (return false)))
    (:`then_1`
      (bind _returnvalue (`/Game/FinalProject/Gameplay/BPFL_MyFunctionLibrary.CheckCanCharacterStand` (`SceneComponent.K2_GetComponentLocation` (select `bool` (== (`local.InteractComponent`) (`self.InteractCollision1`)) :`false` (`self.InteractPos2`) :`true` (`self.InteractPos1`)))))
      (if (not _returnvalue)
        (return false)))
    (:`then_2`
      (return true))))

(fn `GetInteractState`
  (returns (bInteract :type Boolean))
  (return (`self.bPushing`)))

(fn `GetInteractTipUIInfo`
  (params (InteractComponent :type "PrimitiveComponent Object Reference"))
  (returns (WorldPosition :type "Vector Structure") (TipText :type Text))
  (return (`SceneComponent.K2_GetComponentLocation` (select `bool` (== InteractComponent (`self.InteractCollision1`)) :`false` (`self.InteractTipPos2`) :`true` (`self.InteractTipPos1`))) (`self.InteractTip`)))

(fn `GetMoveToInfo`
  (params (InteractComponent :type "PrimitiveComponent Object Reference") (Character :type "/Game/FinalProject/Gameplay/Character/BP_MyCharacter Object Reference"))
  (returns (InteractType :type "/Game/FinalProject/Gameplay/Interactive/EInteractType Enum") (NeedHolster :type Boolean) (NeedHold :type Boolean) (TargetPos :type "Vector Structure") (TargetRot :type "Rotator Structure"))
  (bind (_returnvalue_location _returnvalue_rotation) (`KismetMathLibrary.BreakTransform` (`SceneComponent.K2_GetComponentToWorld` (select `bool` (== InteractComponent (`self.InteractCollision1`)) :`false` (`self.InteractPos2`) :`true` (`self.InteractPos1`)))))
  (return "NewEnumerator5" true false _returnvalue_location _returnvalue_rotation))

(fn `Interact`
  (params (Character :type "/Game/FinalProject/Gameplay/Character/BP_MyCharacter Object Reference") (InteractComponent :type "PrimitiveComponent Object Reference"))
  (returns (InteractType :type "/Game/FinalProject/Gameplay/Interactive/EInteractType Enum") (TargetActor :type "Actor Object Reference") (InteractAction :type "/Game/FinalProject/Gameplay/Character/EInteractAction Enum"))
  (set `self.InteractingComponent` InteractComponent)
  (`PrimitiveComponent.SetCollisionResponseToChannel` (`self.SM_Trolley`) "ECC_Pawn" "ECR_Overlap")
  (return "NewEnumerator5" self "NewEnumerator6"))

(fn `Move`
  (params (Character :type "/Game/FinalProject/Gameplay/Character/BP_MyCharacter Object Reference") (Value :type "Float (double-precision)"))
  (returns (Velocity :type "Vector Structure"))
  (locals (TargetSpeed :type "Float (double-precision)"))
  (bind _returnvalue (!= Value 0.0))
  (bind _trolleypos (`self.TrolleyPos`))
  (bind _returnvalue_2 (* (`local.Value`) (`self.Speed`)))
  (bind _returnvalue_3 (`KismetMathLibrary.FClamp` (+ (`self.TrolleyPos`) (* (`GameplayStatics.GetWorldDeltaSeconds`) (`self.SplineInvLength`) _returnvalue_2))))
  (set `local.TargetSpeed` (`KismetMathLibrary.SelectFloat` (* (`self.MaxSpeed`) (`KismetMathLibrary.SelectFloat` 1.0 -1.0 (`self.InteractingAt1`))) 0.0 _returnvalue))
  (set `self.Speed` (`KismetMathLibrary.FInterpTo` (`self.Speed`) (`local.TargetSpeed`) (`GameplayStatics.GetWorldDeltaSeconds`) (`KismetMathLibrary.SelectFloat` 1.0 10.0 _returnvalue)))
  (bind _bblockinghit (`self.SetTrolleyPos` _returnvalue_3 true (`local.Character`)))
  (if (not _bblockinghit)
    (set `self.TrolleyPos` _returnvalue_3)
    (`/Game/FinalProject/Gameplay/BPFL_MyFunctionLibrary.WakeAllRidgetBodiesInSphere` (`SceneComponent.K2_GetComponentLocation` (`self.SM_Trolley`)) 100.0 (`|MakeArray` "ObjectTypeQuery2" :!type "EObjectTypeQuery Enum"))
    (return (* (`SceneComponent.GetForwardVector` (`self.SM_Trolley`)) (* _returnvalue_2 1.0 (`KismetMathLibrary.SelectFloat` 1.0 0.0 (and (< 0.0 _trolleypos) (< _trolleypos 1.0))))))
    (else
      (return (0.0 0.0 0.0)))))

(fn `SetTrolleyPos`
  (params (TrolleyPos :type "Float (double-precision)") (bSweep :type Boolean :default true) (Character :type "/Game/FinalProject/Gameplay/Character/BP_MyCharacter Object Reference") (bConstruct :type Boolean))
  (returns (bBlockingHit :type Boolean))
  (bind _spline (`self.Spline`))
  (bind (_returnvalue_location _returnvalue_rotation) (`KismetMathLibrary.BreakTransform` (`SplineComponent.GetTransformAtDistanceAlongSpline` _spline (* (`SplineComponent.GetSplineLength` _spline) TrolleyPos) "Local" false)))
  (bind _sweephitresult (`SceneComponent.K2_SetRelativeLocationAndRotation` (`self.SM_Trolley`) (+ _returnvalue_location (0.0 0.0 -5.0)) _returnvalue_rotation bSweep false))
  (if (not (`local.bConstruct`))
    (bind (_out _length) (`/Game/FinalProject/Gameplay/BPFL_MyFunctionLibrary.ArrayRemoveSelfAndCharacter` (`PrimitiveComponent.GetOverlappingActors` (`self.InteractingComponent`) null) (`local.Character`) self))
    (bind _bblockinghit (`GameplayStatics.BreakHitResult` _sweephitresult))
    (return (or (> _length 0) _bblockinghit))
    (else
      (return _bblockinghit))))

(fn `StopInteract`
  (params (Character :type "/Game/FinalProject/Gameplay/Character/BP_MyCharacter Object Reference"))
  (returns (ReturnValue :type Boolean) (InteractAction :type "/Game/FinalProject/Gameplay/Character/EInteractAction Enum"))
  (set `self.Speed` 0.0)
  (set `self.InteractingComponent` null)
  (`PrimitiveComponent.SetCollisionResponseToChannel` (`self.SM_Trolley`) "ECC_Pawn" "ECR_Block")
  (return true "NewEnumerator7"))

(fn `UserConstructionScript`
  (bind _attachingactor (`self.AttachingActor`))
  (bind _trailendmesh (`self.TrailEndMesh`))
  (`|ExecutionSequence`
    (:`then_0`
      (`self.SetTrolleyPos` (`self.TrolleyPos`) false null true))
    (:`then_1`
      (`/Engine/EditorBlueprintResources/StandardMacros.IsValid` _attachingactor
        (:`Is Valid`
          (`self.K2_AttachToComponent` _attachingactor (`self.SM_Trolley`) "Socket_Attach" "KeepWorld" "KeepWorld" "KeepWorld" true))))
    (:`then_2`
      (bind (_startpos1 _starttangent1 _endpos1 _endtangent1 _headtrans _tailtrans) (`/Game/FinalProject/Gameplay/BPFL_MyFunctionLibrary.GenerateSplineMeshBySpline` (`self.Spline`)))
      (`|ExecutionSequence`
        (:`then_0`
          (for (_array_element _array_index) _startpos1
            (bind _returnvalue (`AddComponent|NODE_AddSplineMeshComponent-0`))
            (`SplineMeshComponent.SetStartAndEnd` _returnvalue _array_element (`|GetArrayItem` _starttangent1 _array_index) (`|GetArrayItem` _endpos1 _array_index) (`|GetArrayItem` _endtangent1 _array_index) true)
            (`StaticMeshComponent.SetStaticMesh` _returnvalue (`self.TrailMesh`))))
        (:`then_1`
          (`|ExecutionSequence`
            (:`then_0`
              (bind _returnvalue_2 (`AddComponent|NODE_AddStaticMeshComponent-0` :`RelativeTransform` (`KismetMathLibrary.MakeTransform` (.location _headtrans) (.rotation _headtrans) (* (.scale _headtrans) (-1.0 1.0 1.0)))))
              (`StaticMeshComponent.SetStaticMesh` _returnvalue_2 _trailendmesh)
              (`PrimitiveComponent.SetCollisionEnabled` _returnvalue_2 "NoCollision"))
            (:`then_1`
              (bind _returnvalue_3 (`AddComponent|NODE_AddStaticMeshComponent-1` :`RelativeTransform` (`KismetMathLibrary.MakeTransform` (.location _tailtrans) (.rotation _tailtrans) (* (.scale _tailtrans) (-1.0 1.0 1.0)))))
              (`StaticMeshComponent.SetStaticMesh` _returnvalue_3 _trailendmesh)
              (`PrimitiveComponent.SetCollisionEnabled` _returnvalue_3 "NoCollision"))))))))