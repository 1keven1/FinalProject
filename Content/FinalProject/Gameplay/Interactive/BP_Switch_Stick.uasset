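; BP_Switch_Stick is an interactable lever switch that conducts energy to its targets only while On.
; Two interaction points supply character alignment and pick the action from side and state, with pawn blocking lifted during interaction.
; An animation notify starts the stick timeline, meant to rotate the lever and flip On.
; Conducting refills its energy, which Tick consumes and displays as emissive strength on a dynamic material.
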(event `self.ReceiveTick`
  (params (DeltaSeconds :type "Float (single-precision)"))
  (`self.ConsumeEnergyPF`)
  (`self.SetVisualEffects`))

(event `/Game/FinalProject/Gameplay/Interactive/IInteract.ProcessAnimationNotify`
  (params (Character :type "/Game/FinalProject/Gameplay/Character/BP_MyCharacter Object Reference") (InteractComp :type "PrimitiveComponent Object Reference"))
  (`TimelineComponent.PlayFromStart` (`self.TL_Stick`))
  (set `self.bOpening` (not (`self.bOn`))))

(fn `ChechCanInteract`
  (params (InteractComponent :type "PrimitiveComponent Object Reference") (Character :type "/Game/FinalProject/Gameplay/Character/BP_MyCharacter Object Reference"))
  (returns (`Return Value` :type Boolean))
  (return true))

(fn `Conduct`
  (params (EnergyIn :type "Float (double-precision)"))
  (returns (Consume :type "Float (double-precision)"))
  (if (`self.bOn`)
    (set `self.Energy` (`self.EnergyMax`))
    (bind _consume (`self.ConductEnergyToTargets` (`self.Targets`) (`local.EnergyIn`)))
    (return _consume)))

(fn `GetInteractInfo`
  (params (InteractComponent :type "PrimitiveComponent Object Reference"))
  (returns (InteractType :type "/Game/FinalProject/Gameplay/Interactive/EInteractType Enum") (NeedHolster :type Boolean) (NeedHold :type Boolean) (TargetPos :type "Vector Structure") (TargetRot :type "Rotator Structure"))
  (bind (_returnvalue_location _returnvalue_rotation) (`KismetMathLibrary.BreakTransform` (`SceneComponent.K2_GetComponentToWorld` (select `bool` (== InteractComponent (`self.InteractCollision_1`)) :`false` (`self.InteractPos_2`) :`true` (`self.InteractPos_1`)))))
  (`PrimitiveComponent.SetCollisionResponseToChannel` (`self.BlockCollision`) "ECC_Pawn" "ECR_Ignore")
  (return "NewEnumerator2" true false _returnvalue_location _returnvalue_rotation))

(fn `GetInteractTipUIInfo`
  (params (InteractComponent :type "PrimitiveComponent Object Reference"))
  (returns (WorldPosition :type "Vector Structure") (TipText :type Text))
  (return (`SceneComponent.K2_GetComponentLocation` (`self.InteractTipPos`)) (`self.InteractTip`)))

(fn `Interact`
  (params (Character :type "/Game/FinalProject/Gameplay/Character/BP_MyCharacter Object Reference") (InteractComponent :type "PrimitiveComponent Object Reference"))
  (returns (InteractType :type "/Game/FinalProject/Gameplay/Interactive/EInteractType Enum") (TargetActor :type "Actor Object Reference") (InteractAction :type "/Game/FinalProject/Gameplay/Character/EInteractAction Enum"))
  (return "NewEnumerator2" self (select `bool` (== (== InteractComponent (`self.InteractCollision_1`)) (not (`self.bOn`))) :`false` "NewEnumerator9" :`true` "NewEnumerator8" :!type "/Game/FinalProject/Gameplay/Character/EInteractAction Enum")))

(fn `Move`
  (params (Value :type "Float (double-precision)"))
  (returns (Velocity :type "Vector Structure"))
  (return (0.0 0.0 0.0)))

(fn `SetVisualEffects`
  (`MaterialInstanceDynamic.SetScalarParameterValue` (`self.DynaMat_Light`) "E_Strength" (`KismetMathLibrary.SelectFloat` (/ (`self.Energy`) (`self.EnergyMax`)) 0.0 (> (`self.Energy`) 0.0))))

(fn `StopInteract`
  (params (Character :type "/Game/FinalProject/Gameplay/Character/BP_MyCharacter Object Reference"))
  (returns (ReturnValue :type Boolean) (InteractAction :type "/Game/FinalProject/Gameplay/Character/EInteractAction Enum"))
  (`PrimitiveComponent.SetCollisionResponseToChannel` (`self.BlockCollision`) "ECC_Pawn" "ECR_Block")
  (return false "NewEnumerator2"))

(fn `UserConstructionScript`
  (bind _base (`self.Base`))
  (`parent.UserConstructionScript`)
  (`|ExecutionSequence`
    (:`then_0`
      (bind _returnvalue (`PrimitiveComponent.CreateDynamicMaterialInstance` _base 1 (`PrimitiveComponent.GetMaterial` _base 1) "None"))
      (set `self.DynaMat_Light` _returnvalue))
    (:`then_1`
      (`SceneComponent.K2_SetRelativeRotation` (`self.Stick`) (`KismetMathLibrary.MakeRotator` (`KismetMathLibrary.SelectFloat` -45.0 45.0 (`self.bOn`))) false false))
    (:`then_2`
      (`self.SetVisualEffects`))))