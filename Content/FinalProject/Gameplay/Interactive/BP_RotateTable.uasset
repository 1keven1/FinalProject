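; Interactive turntable that a character pushes to rotate, carrying objects attached to it.
; Move eases rotation speed and returns the character's push movement, reverting the turn if blocked and waking nearby physics bodies otherwise.
; Overlapping actors not mid-interaction attach to the table, and Tick, enabled on demand, slides one BP_ReflectMirror to the center.
; The construction script applies the start yaw and attaches an optional preset actor.
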(event `/Game/FinalProject/Gameplay/Interactive/IInteract.ProcessAnimationNotify`
  (params (Character :type "/Game/FinalProject/Gameplay/Character/BP_MyCharacter Object Reference") (InteractComp :type "PrimitiveComponent Object Reference"))
  (if (not (`self.bPushing`))
    (`/Game/FinalProject/Gameplay/Character/BP_MyCharacter.StartPush` Character (`self.Table`))
    (set `self.bPushing` true)
    (else
      (`/Game/FinalProject/Gameplay/Character/BP_MyCharacter.StopPush` Character)
      (set `self.bPushing` false))))

(event `self.AttachCollision.OnComponentBeginOverlap`
  (params (OverlappedComponent :type "PrimitiveComponent Object Reference") (OtherActor :type "Actor Object Reference") (OtherComp :type "PrimitiveComponent Object Reference") (OtherBodyIndex :type Integer) (bFromSweep :type Boolean) (SweepResult :type "HitResult Structure (by ref)"))
  (if (!= OtherActor self)
    (if (`KismetSystemLibrary.DoesImplementInterface` OtherActor "/Game/FinalProject/Gameplay/Interactive/IInteract.IInteract_C")
      (bind _binteract (message `/Game/FinalProject/Gameplay/Interactive/IInteract.GetInteractState` OtherActor))
      (if (not _binteract)
        (`|ExecutionSequence` :!label _label
          (:`then_0`
            (`self.K2_AttachToComponent` OtherActor (`self.Table`) "None" "KeepWorld" "KeepWorld" "KeepWorld" true))
          (:`then_1`
            (if (and (not (`self.bCentered`)) (== (`GameplayStatics.GetObjectClass` OtherActor) "/Game/FinalProject/Gameplay/Light/BP_ReflectMirror.BP_ReflectMirror_C"))
              (`self.SetActorTickEnabled` true)
              (set `self.bCentered` true)
              (set `self.CenterObj` OtherActor)))))
      (else
        (goto _label)))))

(event `self.AttachCollision.OnComponentEndOverlap`
  (params (OverlappedComponent :type "PrimitiveComponent Object Reference") (OtherActor :type "Actor Object Reference") (OtherComp :type "PrimitiveComponent Object Reference") (OtherBodyIndex :type Integer))
  (if (== OtherActor (`self.CenterObj`))
    (set `self.bCentered` false)
    (set `self.CenterObj` null)))

(event `self.ReceiveTick`
  (params (DeltaSeconds :type "Float (single-precision)"))
  (bind _centerobj (`self.CenterObj`))
  (bind _returnvalue (`self.K2_GetActorLocation` _centerobj))
  (bind _returnvalue_2 (`SceneComponent.K2_GetComponentLocation` (`self.AttachCollision`)))
  (`/Engine/EditorBlueprintResources/StandardMacros.IsValid` _centerobj
    (:`Is Valid`
      (if (not (== _returnvalue _returnvalue_2 :`ErrorTolerance` 0.1))
        (`self.K2_SetActorLocation` _centerobj (`KismetMathLibrary.VInterpTo_Constant` _returnvalue _returnvalue_2 DeltaSeconds 100.0) false false)
        (else
          (`self.SetActorTickEnabled` false))))))

(fn `ChechCanInteract`
  (params (InteractComponent :type "PrimitiveComponent Object Reference") (Character :type "/Game/FinalProject/Gameplay/Character/BP_MyCharacter Object Reference"))
  (returns (`Return Value` :type Boolean))
  (bind (_out _length) (`/Game/FinalProject/Gameplay/BPFL_MyFunctionLibrary.ArrayRemoveSelfAndCharacter` (`PrimitiveComponent.GetOverlappingActors` InteractComponent null) Character self))
  (return (== _length 0)))

(fn `GetInteractState`
  (returns (bInteract :type Boolean))
  (return (`self.bPushing`)))

(fn `GetInteractTipUIInfo`
  (params (InteractComponent :type "PrimitiveComponent Object Reference"))
  (returns (WorldPosition :type "Vector Structure") (TipText :type Text))
  (return (`SceneComponent.K2_GetComponentLocation` (`self.InteractTipPos`)) (`self.InteractTip`)))

(fn `GetMoveToInfo`
  (params (InteractComponent :type "PrimitiveComponent Object Reference") (Character :type "/Game/FinalProject/Gameplay/Character/BP_MyCharacter Object Reference"))
  (returns (InteractType :type "/Game/FinalProject/Gameplay/Interactive/EInteractType Enum") (NeedHolster :type Boolean) (NeedHold :type Boolean) (TargetPos :type "Vector Structure") (TargetRot :type "Rotator Structure"))
  (bind (_returnvalue_location _returnvalue_rotation) (`KismetMathLibrary.BreakTransform` (`SceneComponent.K2_GetComponentToWorld` (`self.InteractPos`))))
  (return "NewEnumerator5" true false _returnvalue_location _returnvalue_rotation))

(fn `Interact`
  (params (Character :type "/Game/FinalProject/Gameplay/Character/BP_MyCharacter Object Reference") (InteractComponent :type "PrimitiveComponent Object Reference"))
  (returns (InteractType :type "/Game/FinalProject/Gameplay/Interactive/EInteractType Enum") (TargetActor :type "Actor Object Reference") (InteractAction :type "/Game/FinalProject/Gameplay/Character/EInteractAction Enum"))
  (set `self.InteractingComponent` InteractComponent)
  (return "NewEnumerator5" self "NewEnumerator6"))

(fn `Move`
  (params (Character :type "/Game/FinalProject/Gameplay/Character/BP_MyCharacter Object Reference") (Value :type "Float (double-precision)"))
  (returns (Velocity :type "Vector Structure"))
  (locals (TargetSpeed :type "Float (double-precision)") (LastRot :type "Rotator Structure" :default (struct)))
  (bind _returnvalue (!= Value 0.0))
  (bind _returnvalue_2 (* Value (`self.RotateSpeed`)))
  (`|ExecutionSequence`
    (:`then_0`
      (set `local.TargetSpeed` (`KismetMathLibrary.SelectFloat` (`self.MaxRotateSpeed`) 0.0 _returnvalue))
      (set `self.RotateSpeed` (`KismetMathLibrary.FInterpTo` (`self.RotateSpeed`) (`local.TargetSpeed`) (`GameplayStatics.GetWorldDeltaSeconds`) (`KismetMathLibrary.SelectFloat` 1.0 10.0 _returnvalue)))
      (set `local.LastRot` (`SceneComponent.RelativeRotation` (`self.Table`))))
    (:`then_1`
      (`SceneComponent.K2_AddRelativeRotation` (`self.Table`) (`KismetMathLibrary.MakeRotator` 0.0 0.0 (* (`GameplayStatics.GetWorldDeltaSeconds`) _returnvalue_2 -1.0)) false false))
    (:`then_2`
      (bind _returnvalue_3 (`/Game/FinalProject/Gameplay/BPFL_MyFunctionLibrary.CheckCanPushFinish` (`local.Character`) self (`self.InteractingComponent`) (`SceneComponent.K2_GetComponentLocation` (`self.InteractPos`))))
      (if _returnvalue_3
        (`/Game/FinalProject/Gameplay/BPFL_MyFunctionLibrary.WakeAllRidgetBodiesInSphere` (`self.K2_GetActorLocation`) 100.0 (`|MakeArray` "ObjectTypeQuery2" :!type "EObjectTypeQuery Enum"))
        (return (* (`SceneComponent.GetForwardVector` (`self.InteractPos`)) _returnvalue_2 2.0))
        (else
          (`SceneComponent.K2_SetRelativeRotation` (`self.Table`) (`local.LastRot`) false false)
          (return (0.0 0.0 0.0)))))))

(fn `StopInteract`
  (params (Character :type "/Game/FinalProject/Gameplay/Character/BP_MyCharacter Object Reference"))
  (returns (ReturnValue :type Boolean) (InteractAction :type "/Game/FinalProject/Gameplay/Character/EInteractAction Enum"))
  (set `self.InteractingComponent` null)
  (return true "NewEnumerator7"))

(fn `UserConstructionScript`
  (bind _attachactor (`self.AttachActor`))
  (`|ExecutionSequence`
    (:`then_0`
      (`SceneComponent.K2_SetRelativeRotation` (`self.Table`) (`KismetMathLibrary.MakeRotator` 0.0 0.0 (`self.StartRotation`)) false false))
    (:`then_1`
      (`/Engine/EditorBlueprintResources/StandardMacros.IsValid` _attachactor
        (:`Is Valid`
          (`self.K2_AttachToComponent` _attachactor (`self.Table`) "Socket_Attach" "KeepWorld" "KeepWorld" "KeepWorld" true))))))