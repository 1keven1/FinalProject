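; BP_GetUpObj is an interactive physics object that a character lifts and puts down with magic, toggling its grabbed state on an animation notify.
; Interaction functions supply the tip and a circular move-to point, allowing use only when the cube is nearly still and that point is unobstructed.
; While not grabbed, hard hits play a throttled, impulse-scaled impact sound.
; Each tick while awake, velocity drives the slide sound's volume and pitch.
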(event `/Game/FinalProject/Gameplay/Interactive/IInteract.ProcessAnimationNotify`
  (params (Character :type "/Game/FinalProject/Gameplay/Character/BP_MyCharacter Object Reference") (InteractComp :type "PrimitiveComponent Object Reference"))
  (if (not (`self.bGrabed`))
    (set `self.bGrabed` true)
    (`/Game/FinalProject/Gameplay/Character/BP_MyCharacter.GetUp_Magic` Character self (`self.Cube`))
    (else
      (set `self.bGrabed` false)
      (`/Game/FinalProject/Gameplay/Character/BP_MyCharacter.PutDown_Magic` Character)
      (`PrimitiveComponent.WakeAllRigidBodies` (`self.Cube`)))))

(event `self.Cube.OnComponentHit`
  (params (HitComponent :type "PrimitiveComponent Object Reference") (OtherActor :type "Actor Object Reference") (OtherComp :type "PrimitiveComponent Object Reference") (NormalImpulse :type "Vector Structure") (Hit :type "HitResult Structure (by ref)"))
  (bind _returnvalue (`KismetMathLibrary.VSize` NormalImpulse))
  (if (not (`self.bGrabed`))
    (if (> _returnvalue 30000.0)
      (`/Engine/EditorBlueprintResources/StandardMacros.DoOnce` false :!label _label
        (:`Completed`
          (`GameplayStatics.PlaySoundAtLocation` (`self.AW_Hit`) (`.Location` (`GameplayStatics.BreakHitResult` Hit)) (struct) (`KismetMathLibrary.FClamp` (* _returnvalue 1e-05) 0.0 2.0) 1.0 0.0 null null null null)
          (`KismetSystemLibrary.Delay` 0.1)
          (goto _label :!via `Reset`))))))

(event `self.ReceiveTick`
  (params (DeltaSeconds :type "Float (single-precision)"))
  (bind _cube (`self.Cube`))
  (if (`PrimitiveComponent.IsAnyRigidBodyAwake` _cube)
    (bind _returnvalue (`PrimitiveComponent.GetPhysicsLinearVelocity` _cube "None"))
    (`self.CE_A_UpdateSlideSound` (`KismetMathLibrary.VSize` _returnvalue))))

(event `CE_A_UpdateSlideSound`
  (params (Speed :type "Float (double-precision)"))
  (bind _returnvalue (`KismetMathLibrary.MapRangeClamped` Speed 10.0 300.0 0.0 1.0))
  (bind _as_am_stone_slide (`self.AS_AM_Stone_Slide`))
  (bind _as_am_stone_slide_2 (`self.AS_AM_Stone_Slide`))
  (if (> _returnvalue 0.0)
    (if (not (`AudioComponent.IsPlaying` _as_am_stone_slide))
      (`AudioComponent.Play` _as_am_stone_slide 0.0))
    (`AudioComponent.SetVolumeMultiplier` _as_am_stone_slide_2 _returnvalue)
    (`AudioComponent.SetPitchMultiplier` _as_am_stone_slide_2 _returnvalue)
    (else
      (`AudioComponent.Stop` _as_am_stone_slide))))

(fn `ChechCanInteract`
  (params (InteractComponent :type "PrimitiveComponent Object Reference") (Character :type "/Game/FinalProject/Gameplay/Character/BP_MyCharacter Object Reference"))
  (returns (`Return Value` :type Boolean))
  (bind _character (`local.Character`))
  (bind (_returnvalue_x _returnvalue_y _returnvalue_z) (`KismetMathLibrary.BreakVector` (`SceneComponent.K2_GetComponentLocation` (`self.Cube`))))
  (`|ExecutionSequence`
    (:`then_0`
      ;[0 0 0] 在动直接不行
      (if (not (<= (`KismetMathLibrary.VSize` (`SceneComponent.GetComponentVelocity` (`self.Cube`))) 1.0))
        (return false)))
    (:`then_1`
      ;[0 0 0] 交互点在墙里也不行
      (bind _outactors (`KismetSystemLibrary.CapsuleOverlapActors` (`KismetMathLibrary.MakeVector` (.x (`/Game/FinalProject/Gameplay/BPFL_MyFunctionLibrary.GetCircularInteractPoint` (`local.Character`) (`self.Cube`) (`self.InteractDistance`))) (.y (`/Game/FinalProject/Gameplay/BPFL_MyFunctionLibrary.GetCircularInteractPoint` (`local.Character`) (`self.Cube`) (`self.InteractDistance`))) (+ (- _returnvalue_z (.x (`.Max` (`StaticMeshComponent.GetLocalBounds` (`self.Cube`))))) (`CapsuleComponent.CapsuleHalfHeight` (`Character.CapsuleComponent` (`local.Character`))))) 30.0 60.0 (`|MakeArray` "ObjectTypeQuery1" "ObjectTypeQuery2" :!type "EObjectTypeQuery Enum") null (`|MakeArray` self _character (`/Game/FinalProject/Gameplay/Character/BP_MyCharacter.HolsterObj` _character) (`/Game/FinalProject/Gameplay/Character/BP_MyCharacter.InHandObj` _character) :!type "Actor Object Reference")))
      (if (> (`KismetArrayLibrary.Array_Length` _outactors) 0)
        (return false)))
    (:`then_2`
      (return true))))

(fn `GetInteractState`
  (returns (bInteract :type Boolean))
  (return (`self.bGrabed`)))

(fn `GetInteractTipUIInfo`
  (params (InteractComponent :type "PrimitiveComponent Object Reference"))
  (returns (WorldPosition :type "Vector Structure") (TipText :type Text))
  (return (`SceneComponent.K2_GetComponentLocation` (`self.Cube`)) (`self.InteractTip`)))

(fn `GetMoveToInfo`
  (params (InteractComponent :type "PrimitiveComponent Object Reference") (Character :type "/Game/FinalProject/Gameplay/Character/BP_MyCharacter Object Reference"))
  (returns (InteractType :type "/Game/FinalProject/Gameplay/Interactive/EInteractType Enum") (NeedHolster :type Boolean) (NeedHold :type Boolean) (TargetPos :type "Vector Structure") (TargetRot :type "Rotator Structure"))
  (bind (_pos _rot) (`/Game/FinalProject/Gameplay/BPFL_MyFunctionLibrary.GetCircularInteractPoint` Character (`self.Cube`) (`self.InteractDistance`)))
  (return "NewEnumerator4" true false _pos _rot))

(fn `Interact`
  (params (Character :type "/Game/FinalProject/Gameplay/Character/BP_MyCharacter Object Reference") (InteractComponent :type "PrimitiveComponent Object Reference"))
  (returns (InteractType :type "/Game/FinalProject/Gameplay/Interactive/EInteractType Enum") (TargetActor :type "Actor Object Reference") (InteractAction :type "/Game/FinalProject/Gameplay/Character/EInteractAction Enum"))
  (return "NewEnumerator4" self "NewEnumerator4"))

(fn `Move`
  (params (Character :type "/Game/FinalProject/Gameplay/Character/BP_MyCharacter Object Reference") (Value :type "Float (double-precision)"))
  (returns (Velocity :type "Vector Structure"))
  (return (0.0 0.0 0.0)))

(fn `StopInteract`
  (params (Character :type "/Game/FinalProject/Gameplay/Character/BP_MyCharacter Object Reference"))
  (returns (ReturnValue :type Boolean) (InteractAction :type "/Game/FinalProject/Gameplay/Character/EInteractAction Enum"))
  (return true "NewEnumerator5"))

(fn `UserConstructionScript`)