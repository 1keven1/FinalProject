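; BP_Switch_Plate is a pressure-plate switch that passes energy to its targets only while something is standing on it.
; Box overlap events set the On state from the overlapping actor count and play or reverse the button timeline.
; When on, Conduct refills the plate's energy and forwards the incoming energy.
; Tick consumes energy and scales a dynamic material's emissive strength to the remaining charge.
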(event `self.ReceiveTick`
  (params (DeltaSeconds :type "Float (single-precision)"))
  (`self.ConsumeEnergyPF`)
  (`self.SetVisualEffects`))

(event `self.Box.OnComponentBeginOverlap`
  (params (OverlappedComponent :type "PrimitiveComponent Object Reference") (OtherActor :type "Actor Object Reference") (OtherComp :type "PrimitiveComponent Object Reference") (OtherBodyIndex :type Integer) (bFromSweep :type Boolean) (SweepResult :type "HitResult Structure (by ref)"))
  (`self.SetIsOn`))

(event `self.Box.OnComponentEndOverlap`
  (params (OverlappedComponent :type "PrimitiveComponent Object Reference") (OtherActor :type "Actor Object Reference") (OtherComp :type "PrimitiveComponent Object Reference") (OtherBodyIndex :type Integer))
  (`self.SetIsOn`))

(fn `Conduct`
  (params (EnergyIn :type "Float (double-precision)"))
  (returns (Consume :type "Float (double-precision)"))
  (if (`self.bOn`)
    (set `self.Energy` (`self.EnergyMax`))
    (bind _consume (`self.ConductEnergyToTargets` (`self.Targets`) (`local.EnergyIn`)))
    (return _consume)))

(fn `SetIsOn`
  (bind _tl_button (`self.TL_Button`))
  (bind _output_get (set `self.bOn` (> (`KismetArrayLibrary.Array_Length` (`PrimitiveComponent.GetOverlappingActors` (`self.Box`) null)) 0)))
  (if _output_get
    (`TimelineComponent.Play` _tl_button)
    (else
      (`TimelineComponent.Reverse` _tl_button))))

(fn `SetVisualEffects`
  (`MaterialInstanceDynamic.SetScalarParameterValue` (`self.DynaMat_Light`) "E_Strength" (`KismetMathLibrary.SelectFloat` (/ (`self.Energy`) (`self.EnergyMax`)) 0.0 (> (`self.Energy`) 0.0))))

(fn `UserConstructionScript`
  (bind _sm_switch_plate (`self.SM_Switch_Plate`))
  (`parent.UserConstructionScript`)
  (`|ExecutionSequence`
    (:`then_0`
      (bind _returnvalue (`PrimitiveComponent.CreateDynamicMaterialInstance` _sm_switch_plate 1 (`PrimitiveComponent.GetMaterial` _sm_switch_plate 1) "None"))
      (set `self.DynaMat_Light` _returnvalue))
    (:`then_1`
      (`self.SetVisualEffects`))))