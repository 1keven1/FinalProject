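; Multi-output power switch: the player pushes a handle along a rail to choose which target receives conducted energy.
; The construction script builds the rail from edge and middle meshes to match OutputNum, with dynamic materials for each output light.
; Move slides the handle, reverting if the character's push is blocked, and Conduct forwards energy only when it sits near an output.
; Tick drains stored energy and updates the base and active-output glow.
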(event `self.ReceiveTick`
  (params (DeltaSeconds :type "Float (single-precision)"))
  (`self.ConsumeEnergyPF`)
  (`self.SetVisualEffects`))

(event `/Game/FinalProject/Gameplay/Interactive/IInteract.ProcessAnimationNotify`
  (params (Character :type "/Game/FinalProject/Gameplay/Character/BP_MyCharacter Object Reference") (InteractComp :type "PrimitiveComponent Object Reference"))
  (if (not (`self.bPushing`))
    (`/Game/FinalProject/Gameplay/Character/BP_MyCharacter.StartPush` Character (`self.Switch_Multi_Handle`))
    (set `self.bPushing` true)
    (else
      (`/Game/FinalProject/Gameplay/Character/BP_MyCharacter.StopPush` Character)
      (set `self.bPushing` false))))

(fn `ChechCanInteract`
  (params (InteractComponent :type "PrimitiveComponent Object Reference") (Character :type "/Game/FinalProject/Gameplay/Character/BP_MyCharacter Object Reference"))
  (returns (`Return Value` :type Boolean))
  (bind (_out _length) (`/Game/FinalProject/Gameplay/BPFL_MyFunctionLibrary.ArrayRemoveSelfAndCharacter` (`PrimitiveComponent.GetOverlappingActors` InteractComponent null) Character self))
  (`|ExecutionSequence`
    (:`then_1`
      (return (== _length 0)))))

(fn `Conduct`
  (params (EnergyIn :type "Float (double-precision)"))
  (returns (Consume :type "Float (double-precision)"))
  (bind (_returnvalue _outputnum) (`self.GetEnabledOutput` (`self.OutputConnectRange`)))
  (bind _output (`|GetArrayItem` (`self.Targets`) _outputnum))
  (set `self.Energy` (`self.EnergyMax`))
  (if _returnvalue
    (`/Engine/EditorBlueprintResources/StandardMacros.IsValid` _output
      (:`Is Valid`
        (bind _consume (`self.ConductEnergyToTargets` (`|MakeArray` _output) (`local.EnergyIn`)))
        (return _consume)))))

(fn `GetEnabledOutput`
  (params (Range :type "Float (double-precision)" :default 0.3))
  (returns (ReturnValue :type Boolean) (OutputNum :type Integer))
  (bind _returnvalue (* (`self.HandlePos`) (- (`self.OutputNum`) 1)))
  (bind _returnvalue_2 (`KismetMathLibrary.Round` _returnvalue))
  (return (< (`KismetMathLibrary.Abs` (- _returnvalue _returnvalue_2)) (`local.Range`)) _returnvalue_2))

(fn `GetInteractState`
  (returns (bInteract :type Boolean))
  (return (`self.bPushing`)))

(fn `GetInteractTipUIInfo`
  (params (InteractComponent :type "PrimitiveComponent Object Reference"))
  (returns (WorldPosition :type "Vector Structure") (TipText :type Text))
  (return (`SceneComponent.K2_GetComponentLocation` (`self.InteractTip_Push`)) (`self.InteractTip`)))

(fn `GetMoveToInfo`
  (params (InteractComponent :type "PrimitiveComponent Object Reference") (Character :type "/Game/FinalProject/Gameplay/Character/BP_MyCharacter Object Reference"))
  (returns (InteractType :type "/Game/FinalProject/Gameplay/Interactive/EInteractType Enum") (NeedHolster :type Boolean) (NeedHold :type Boolean) (TargetPos :type "Vector Structure") (TargetRot :type "Rotator Structure"))
  (bind (_returnvalue_location _returnvalue_rotation) (`KismetMathLibrary.BreakTransform` (`SceneComponent.K2_GetComponentToWorld` (`self.InteractPos_Push`))))
  (return "NewEnumerator5" true false _returnvalue_location _returnvalue_rotation))

(fn `InitializeStaticMesh`
  (params (MeshIn :type "PrimitiveComponent Object Reference") (Index :type Integer))
  (bind _meshin (`local.MeshIn`))
  (`PrimitiveComponent.SetMaterial` MeshIn 1 (`self.DynaMat_LightBase`))
  (bind _returnvalue (`PrimitiveComponent.CreateDynamicMaterialInstance` _meshin 2 (`PrimitiveComponent.GetMaterial` _meshin 2) "None"))
  (`KismetArrayLibrary.Array_Set` (`self.DynaMats_Output`) (- (`local.Index`) 1) _returnvalue))

(fn `Interact`
  (params (Character :type "/Game/FinalProject/Gameplay/Character/BP_MyCharacter Object Reference") (InteractComponent :type "PrimitiveComponent Object Reference"))
  (returns (InteractType :type "/Game/FinalProject/Gameplay/Interactive/EInteractType Enum") (TargetActor :type "Actor Object Reference") (InteractAction :type "/Game/FinalProject/Gameplay/Character/EInteractAction Enum"))
  (return "NewEnumerator5" self "NewEnumerator6"))

(fn `Move`
  (params (Character :type "/Game/FinalProject/Gameplay/Character/BP_MyCharacter Object Reference") (Value :type "Float (double-precision)"))
  (returns (Velocity :type "Vector Structure"))
  (locals (Speed :type "Float (double-precision)") (LastPos :type "Float (double-precision)" :default 0.0))
  (bind _returnvalue (`KismetMathLibrary.FClamp` (+ (* Value (`GameplayStatics.GetWorldDeltaSeconds`) (`self.MoveSpeed`)) (`self.HandlePos`))))
  (set `local.LastPos` (`self.HandlePos`))
  (set `local.Speed` (- _returnvalue (`self.HandlePos`)))
  (set `self.HandlePos` _returnvalue)
  (bind _returnvalue_2 (`self.RefreshHandlePos` (`local.Character`)))
  (if _returnvalue_2
    (return (* (`self.GetActorRightVector`) (/ (`local.Speed`) (`GameplayStatics.GetWorldDeltaSeconds`)) 100.0 -1))
    (else
      (set `self.HandlePos` (`local.LastPos`))
      (`self.RefreshHandlePos` (`local.Character`))
      (return (0.0 0.0 0.0)))))

(fn `RefreshHandlePos`
  (params (Character :type "/Game/FinalProject/Gameplay/Character/BP_MyCharacter Object Reference"))
  (returns (ReturnValue :type Boolean))
  (`SceneComponent.K2_SetWorldLocation` (`self.Switch_Multi_Handle`) (`KismetMathLibrary.VLerp` (`self.HandleStartPos`) (`self.HandleEndPos`) (`self.HandlePos`)) false false)
  (bind _returnvalue (`/Game/FinalProject/Gameplay/BPFL_MyFunctionLibrary.CheckCanPushFinish` (`local.Character`) self (`self.InteractCollision_Push`) (`SceneComponent.K2_GetComponentLocation` (`self.InteractPos_Push`))))
  (return _returnvalue))

(fn `SetVisualEffects`
  (bind (_returnvalue _outputnum) (`self.GetEnabledOutput` (`self.OutputConnectRange`)))
  (bind _returnvalue_2 (`KismetMathLibrary.SelectFloat` (/ (`self.Energy`) (`self.EnergyMax`)) 0.0 (> (`self.Energy`) 0.0)))
  (`|ExecutionSequence`
    (:`then_0`
      (`MaterialInstanceDynamic.SetScalarParameterValue` (`self.DynaMat_LightBase`) "E_Strength" _returnvalue_2)
      (for _array_element (`self.DynaMats_Output`)
        (`MaterialInstanceDynamic.SetScalarParameterValue` _array_element "E_Strength" 0.0)))
    (:`then_1`
      (if _returnvalue
        (`MaterialInstanceDynamic.SetScalarParameterValue` (`|GetArrayItem` (`self.DynaMats_Output`) _outputnum) "E_Strength" _returnvalue_2)))))

(fn `StopInteract`
  (params (Character :type "/Game/FinalProject/Gameplay/Character/BP_MyCharacter Object Reference"))
  (returns (ReturnValue :type Boolean) (InteractAction :type "/Game/FinalProject/Gameplay/Character/EInteractAction Enum"))
  (return true "NewEnumerator7"))

(fn `UserConstructionScript`
  (bind _outputnum (`self.OutputNum`))
  (bind _outputnum_2 (`self.OutputNum`))
  (bind (_returnvalue_min _returnvalue_max) (break `Box` (`StaticMesh.GetBoundingBox` (`self.Mesh_Middle`))))
  (bind _returnvalue_x (`KismetMathLibrary.BreakVector` (- _returnvalue_max _returnvalue_min)))
  (`parent.UserConstructionScript`)
  (`|ExecutionSequence`
    (:`then_0`
      (bind _returnvalue (`KismetMaterialLibrary.CreateDynamicMaterialInstance` "/Game/FinalProject/Art/Eletronic/MI_EletronicLight.MI_EletronicLight"))
      (set `self.DynaMat_LightBase` _returnvalue)
      (`KismetArrayLibrary.Array_Resize` (`self.DynaMats_Output`) _outputnum_2)
      (`KismetArrayLibrary.Array_Resize` (`self.Targets`) _outputnum_2))
    (:`then_1`
      (for _index (range 1 (+ _outputnum 1))
        (if (== _index 1)
          (bind _returnvalue_2 (`AddComponent|NODE_AddStaticMeshComponent-0` :`RelativeTransform` (`KismetMathLibrary.MakeTransform` (0.0 0.0 0.0) (struct :`Yaw` 90.0))))
          (`StaticMeshComponent.SetStaticMesh` _returnvalue_2 (`self.Mesh_Edge`))
          (`self.InitializeStaticMesh` _returnvalue_2 _index)
          (set `self.HandleStartPos` (`SceneComponent.GetSocketLocation` _returnvalue_2 "Socket_Handle"))
          (elif (== _index _outputnum)
            (bind _returnvalue_3 (* (- _index 2) _returnvalue_x))
            (bind _returnvalue_4 (`AddComponent|NODE_AddStaticMeshComponent-1` :`RelativeTransform` (`KismetMathLibrary.MakeTransform` (`KismetMathLibrary.MakeVector` 0.0 (* _returnvalue_3 -1.0)) (struct :`Yaw` 90.0) (-1.0 1.0 1.0))))
            (`StaticMeshComponent.SetStaticMesh` _returnvalue_4 (`self.Mesh_Edge`))
            (`self.InitializeStaticMesh` _returnvalue_4 _index)
            (set `self.HandleEndPos` (`SceneComponent.GetSocketLocation` _returnvalue_4 "Socket_Handle"))
            (else
              (bind _returnvalue_5 (`AddComponent|NODE_AddStaticMeshComponent-2` :`RelativeTransform` (`KismetMathLibrary.MakeTransform` (`KismetMathLibrary.MakeVector` 0.0 (* (+ _returnvalue_3 (* _returnvalue_x 0.5)) -1.0)) (struct :`Yaw` 90.0))))
              (`StaticMeshComponent.SetStaticMesh` _returnvalue_5 (`self.Mesh_Middle`))
              (`self.InitializeStaticMesh` _returnvalue_5 _index))))))
    (:`then_2`
      (`self.RefreshHandlePos` null)
      (`self.SetVisualEffects`))))