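; Game mode for the start screen that shows the title widgets and moves the camera to and from a sandbox level-select view.
; BeginPlay caches the sandbox, sky, weather and player objects, creates the start widgets, records the camera pose and fades in.
; A reversible timeline blends camera transform, FOV and exposure along with sandbox opacity, cloud coverage and UI white cloud.
; Key presses are forwarded to the start widget, while pause can also return from level select.
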(event `self.ReceiveBeginPlay`
  (bind _playercontroller (`self.PlayerController`))
  (`parent.ReceiveBeginPlay`)
  (`|ExecutionSequence`
    (:`then_0`
      (bind _returnvalue (`GameplayStatics.GetActorOfClass` "/Game/FinalProject/Gameplay/Z_LevelManage/BP_SandBox.BP_SandBox_C"))
      (bind _output_get (set `self.SandBox` _returnvalue))
      (bind _asbp_my_controller (cast `/Game/FinalProject/Gameplay/BP_MyController` (`GameplayStatics.GetPlayerController` 0)))
      (set `self.PlayerController` _asbp_my_controller)
      (set `self.SelectCamera` (`SceneComponent.K2_GetComponentToWorld` (`/Game/FinalProject/Gameplay/Z_LevelManage/BP_SandBox.Camera` _output_get)))
      (bind _returnvalue_2 (`GameplayStatics.GetActorOfClass` "/Game/UltraDynamicSky/Blueprints/Ultra_Dynamic_Sky.Ultra_Dynamic_Sky_C"))
      (set `self.DynamicSky` _returnvalue_2)
      (bind _returnvalue_3 (`GameplayStatics.GetActorOfClass` "/Game/UltraDynamicSky/Blueprints/Ultra_Dynamic_Weather.Ultra_Dynamic_Weather_C"))
      (set `self.DynamicWeather` _returnvalue_3)
      (bind _asbp_my_instance (cast `/Game/FinalProject/Gameplay/BP_MyInstance` (`GameplayStatics.GetGameInstance`)))
      (set `self.MyInstance` _asbp_my_instance))
    (:`then_1`
      (bind _returnvalue_4 (`|CreateWidget` "/Game/FinalProject/Gameplay/UI/Start/WBP_Start_Main.WBP_Start_Main_C"))
      (bind _output_get_2 (set `self.WBP_Start_Main` _returnvalue_4))
      (`UserWidget.AddToViewport` _output_get_2 0)
      (bind _returnvalue_5 (`|CreateWidget` "/Game/FinalProject/Gameplay/UI/Start/WBP_Start.WBP_Start_C" null self))
      (set `self.StartWidget` _returnvalue_5)
      (`UserWidget.AddToViewport` (`self.StartWidget`) 0))
    (:`then_2`
      (`WidgetBlueprintLibrary.SetInputMode_GameAndUIEx` _playercontroller (`self.StartWidget`))
      (set `PlayerController.bShowMouseCursor` true _playercontroller)
      (bind _ascamera_actor (cast `CameraActor` (`Controller.GetViewTarget` _playercontroller)))
      (bind _output_get_3 (set `self.StartViewTarget` _ascamera_actor))
      (set `self.StartCamera` (`self.GetTransform` _output_get_3)))
    (:`then_3`
      (`self.CE_FadeCamera` false 0.3))))

(event `CE_SelectLevel`
  (params (bToSelect :type Boolean) (Speed :type "Float (double-precision)" :default 1.0))
  (bind (_startcamera_location _startcamera_rotation) (`KismetMathLibrary.BreakTransform` (`self.StartCamera`)))
  (bind _sandbox (`self.SandBox`))
  (bind _sandbox_2 (`self.SandBox`))
  (bind _sandbox_3 (`self.SandBox`))
  (bind _startwidget (`self.StartWidget`))
  (bind (_selectcamera_location _selectcamera_rotation) (`KismetMathLibrary.BreakTransform` (`self.SelectCamera`)))
  (bind _startviewtarget (`self.StartViewTarget`))
  (bind _cameracomponent (`CameraActor.CameraComponent` (`self.StartViewTarget`)))
  (`TimelineComponent.SetPlayRate` (`self.TL_SelectLevel`) Speed)
  (if bToSelect
    (`Widget.RemoveFromParent` _startwidget)
    (`/Game/FinalProject/Gameplay/Z_LevelManage/BP_SandBox.SetSandBoxVis` _sandbox_2 true)
    (bind (_direction _poslerp _rotlerp _sandboxopa _uiwhite) (`Timeline|TL_SelectLevel` :!label _label)
      (:`Update`
        (`|ExecutionSequence`
          (:`then_0`
            (`self.K2_SetActorLocation` _startviewtarget (`KismetMathLibrary.VLerp` _startcamera_location _selectcamera_location _poslerp) false false)
            (`self.K2_SetActorRotation` _startviewtarget (`KismetMathLibrary.RLerp` _startcamera_rotation _selectcamera_rotation _rotlerp true) false)
            (`CameraComponent.SetFieldOfView` _cameracomponent (`KismetMathLibrary.Lerp` 100.0 60.0 _poslerp))
            (setmembers `PostProcessSettings` :`StructRef` (`CameraComponent.PostProcessSettings` _cameracomponent) :`AutoExposureBias` (`KismetMathLibrary.Lerp` 11.5 10.7 _poslerp)))
          (:`then_1`
            (`/Game/FinalProject/Gameplay/Z_LevelManage/BP_SandBox.SetSandBoxOpacity` _sandbox _sandboxopa)
            (`/Game/FinalProject/Gameplay/Z_LevelManage/BP_SandBox.SetLevelUIOpacity` _sandbox _sandboxopa))
          (:`then_2`
            (set `/Game/UltraDynamicSky/Blueprints/Ultra_Dynamic_Weather.Cloud Coverage` (`KismetMathLibrary.Lerp` 5.5 0.0 _poslerp) (`self.DynamicWeather`)))
          (:`then_3`
            (`/Game/FinalProject/Gameplay/UI/Start/WBP_Start_Main.SetWhiteCloud` (`self.WBP_Start_Main`) _uiwhite))))
      (:`Finished`
        (switch `ETimelineDirection` _direction
          (:`Forward`
            (`/Game/FinalProject/Gameplay/Z_LevelManage/BP_SandBox.SetHideActorsVis` _sandbox_3 false))
          (:`Backward`
            (`/Game/FinalProject/Gameplay/Z_LevelManage/BP_SandBox.SetSandBoxVis` _sandbox_3 false)))))
    (else
      (`UserWidget.AddToViewport` _startwidget 0)
      (`/Game/FinalProject/Gameplay/Z_LevelManage/BP_SandBox.SetHideActorsVis` _sandbox_2 true)
      (goto _label :!via `Reverse`))))

(event `self.OpenLevel`
  (params (LevelName :type Name) (CameraFadeSpeed :type "Float (double-precision)"))
  (`parent.OpenLevel` LevelName CameraFadeSpeed)
  (`/Game/FinalProject/Gameplay/Z_LevelManage/BP_SandBox.SetLevelUIOpacity` (`self.SandBox`) 0.0))

(fn `PressAnyKey`
  (params (Key :type "Key Structure"))
  (`parent.PressAnyKey` Key)
  (if true
    (`/Game/FinalProject/Gameplay/UI/Start/WBP_Start.CE_PressedAnyKey` (`self.StartWidget`))))

(fn `PressEnter`
  (`parent.PressEnter`)
  (`/Game/FinalProject/Gameplay/UI/Start/WBP_Start.CE_PressedAnyKey` (`self.StartWidget`)))

(fn `PressPause`
  (bind _startwidget (`self.StartWidget`))
  (`parent.PressPause`)
  (if (`Widget.IsInViewport` _startwidget)
    (`/Game/FinalProject/Gameplay/UI/Start/WBP_Start.CE_PressedAnyKey` _startwidget)
    (else
      (`self.CE_SelectLevel` false 0.5))))

(fn `UserConstructionScript`
  (`parent.UserConstructionScript`))