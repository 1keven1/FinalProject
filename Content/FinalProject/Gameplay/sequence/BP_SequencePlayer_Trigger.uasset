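; A trigger actor that plays a cutscene when the player character enters it, then moves the game to another level.
; On overlap by BP_MyCharacter it hides the character and auto-plays SequenceToPlay with movement and look input disabled.
; When the sequence finishes, the game mode opens LevelName with a camera fade, or a warning prints if no level is set.
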(event `self.CollisionComponent.OnComponentBeginOverlap`
  (params (OverlappedComponent :type "PrimitiveComponent Object Reference") (OtherActor :type "Actor Object Reference") (OtherComp :type "PrimitiveComponent Object Reference") (OtherBodyIndex :type Integer) (bFromSweep :type Boolean) (SweepResult :type "HitResult Structure (by ref)"))
  (if (== (`GameplayStatics.GetObjectClass` OtherActor) "/Game/FinalProject/Gameplay/Character/BP_MyCharacter.BP_MyCharacter_C")
    (`self.SetActorHiddenInGame` OtherActor true)
    (bind (_outactor _returnvalue) (`LevelSequencePlayer.CreateLevelSequencePlayer` (`self.SequenceToPlay`) (make `MovieSceneSequencePlaybackSettings` true (struct) 1.0 0.0 false false true true)))
    (add `MovieSceneSequencePlayer.OnFinished` _returnvalue (delegate `SeqFinish`))))

(event `SeqFinish`
  (bind _levelname (`self.LevelName`))
  (if (!= _levelname "None")
    (bind _asbp_my_game_mode_base (cast `/Game/FinalProject/Gameplay/BP_MyGameMode_Base` (`GameplayStatics.GetGameMode`)))
    (`/Game/FinalProject/Gameplay/BP_MyGameMode_Base.OpenLevel` _asbp_my_game_mode_base _levelname 1.0)
    (else
      (`KismetSystemLibrary.PrintString` "WARNING: 未选择要打开的关卡" true true (struct :`R` 1.0 :`G` 0.016302 :`A` 1.0) 10.0))))

(fn `UserConstructionScript`)