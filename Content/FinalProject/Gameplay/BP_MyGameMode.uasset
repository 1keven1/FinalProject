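; Game mode that manages play, pause and campfire-rest states, plus player settings and save/load.
; It creates the pause and rest widgets, switching input mode, cursor and, for resting, a blended camera view to the campfire.
; Settings persist through the game instance and are applied by rebuilding input mappings at runtime and overriding sound class volumes in a base sound mix.
; Game saves pass character data through the game instance.
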(event `self.ReceiveBeginPlay`
  (`|ExecutionSequence`
    (:`then_0`
      (bind _asbp_my_controller (cast `/Game/FinalProject/Gameplay/BP_MyController` (`GameplayStatics.GetPlayerController` 0)))
      (set `self.MyController` _asbp_my_controller)
      (bind _asbp_my_character (cast `/Game/FinalProject/Gameplay/Character/BP_MyCharacter` (`GameplayStatics.GetPlayerPawn` 0)))
      (set `self.MyCharacter` _asbp_my_character)
      (bind _asbp_my_instance (cast `/Game/FinalProject/Gameplay/BP_MyInstance` (`GameplayStatics.GetGameInstance`)))
      (set `self.MyGameInstance` _asbp_my_instance))
    (:`then_1`
      (bind _returnvalue (`|CreateWidget` "/Game/FinalProject/Gameplay/UI/WBP_Pause.WBP_Pause_C" null self))
      (set `self.WBP_Pause` _returnvalue)
      (bind _returnvalue_2 (`|CreateWidget` "/Game/FinalProject/Gameplay/UI/WBP_Rest.WBP_Rest_C" null self (`self.MyCharacter`)))
      (set `self.WBP_Rest` _returnvalue_2))
    (:`then_2`
      (`WidgetBlueprintLibrary.SetInputMode_GameOnly` (`self.MyController`))
      (set `self.MyGameState` "NewEnumerator0"))
    (:`then_3`
      (`GameplayStatics.SetBaseSoundMix` (`self.BaseSoundMix`)))
    (:`then_4`
      (bind (_exist _settings) (`/Game/FinalProject/Gameplay/BP_MyInstance.LoadSettings` (`self.MyGameInstance`)))
      (if _exist
        (bind _output_get (set `self.Settings` _settings))
        (`self.ApplyAllSettings` _output_get)))))

(fn `ApplyAllSettings`
  (params (Settings :type "/Game/FinalProject/Gameplay/Z_SaveGame/SSettings Structure"))
  (bind (_inputmap_keyboard _audiosettings) (break `/Game/FinalProject/Gameplay/Z_SaveGame/SSettings` Settings))
  (`self.ApplyInputMaps` _inputmap_keyboard)
  (`self.ApplyAudioSettings` _audiosettings))

(fn `ApplyAudioSettings`
  (params (AudioSettings :type "/Game/FinalProject/Gameplay/UI/SAudioSettings Structure"))
  (bind _basesoundmix (`self.BaseSoundMix`))
  (bind (_mainvolume _sevolume _uivolume _musicvolume) (break `/Game/FinalProject/Gameplay/UI/SAudioSettings` (`local.AudioSettings`)))
  ;[0 0 0] 应用
  (`|ExecutionSequence`
    (:`then_0`
      (`GameplayStatics.SetSoundMixClassOverride` _basesoundmix "/Game/FinalProject/Sound/_SoundClassAndMix/MySoundClass_Master.MySoundClass_Master" _mainvolume 1.0 0.1))
    (:`then_1`
      (`GameplayStatics.SetSoundMixClassOverride` _basesoundmix "/Game/FinalProject/Sound/_SoundClassAndMix/SoundEffect.SoundEffect" _sevolume 1.0 0.1))
    (:`then_2`
      (`GameplayStatics.SetSoundMixClassOverride` _basesoundmix "/Game/FinalProject/Sound/_SoundClassAndMix/UI.UI" _uivolume 1.0 0.1))
    (:`then_3`
      (`GameplayStatics.SetSoundMixClassOverride` _basesoundmix "/Game/FinalProject/Sound/_SoundClassAndMix/Music.Music" _musicvolume 1.0 0.1))))

(fn `ApplyInputMaps`
  (params (InputMaps :type "/Game/FinalProject/Gameplay/UI/SInputMap_Keyboard Structure"))
  (bind _returnvalue (`InputSettings.GetInputSettings`))
  (bind _returnvalue_2 (`InputSettings.GetInputSettings`))
  (bind _returnvalue_3 (`InputSettings.GetInputSettings`))
  (bind _returnvalue_4 (`InputSettings.GetInputSettings`))
  (bind _returnvalue_5 (`InputSettings.GetInputSettings`))
  (bind (_movefwd _movebwd _moverwd _movelwd) (break `/Game/FinalProject/Gameplay/UI/SInputMap_Keyboard` (`local.InputMaps`)))
  (bind (_movefwd_2 _movebwd_2 _moverwd_2 _movelwd_2 _jump _interact _hook _reach _pause _loopup _lookright) (break `/Game/FinalProject/Gameplay/UI/SInputMap_Keyboard` (`local.InputMaps`)))
  (bind (_movefwd_3 _movebwd_3) (break `/Game/FinalProject/Gameplay/UI/SInputMap_Keyboard` (`local.InputMaps`)))
  (bind (_movefwd_4 _movebwd_4 _moverwd_3 _movelwd_3 _jump_2 _interact_2 _hook_2 _reach_2 _pause_2) (break `/Game/FinalProject/Gameplay/UI/SInputMap_Keyboard` (`local.InputMaps`)))
  (bind (_axisname _scale _key) (break `InputAxisKeyMapping` _movelwd))
  (bind (_axisname_2 _scale_2 _key_2) (break `InputAxisKeyMapping` _moverwd))
  (bind (_axisname_3 _scale_3 _key_3) (break `InputAxisKeyMapping` _movefwd_3))
  (bind (_axisname_4 _scale_4 _key_4) (break `InputAxisKeyMapping` _movebwd_3))
  (`|ExecutionSequence`
    (:`then_0`
      ;[0 0 0] 清空
      (`|ExecutionSequence`
        (:`then_0`
          (for _array_element (`InputSettings.GetAxisNames` _returnvalue)
            (for _array_element_2 (`InputSettings.GetAxisMappingByName` _returnvalue _array_element)
              (`InputSettings.RemoveAxisMapping` _returnvalue _array_element_2 false))))
        (:`then_1`
          (for _array_element_3 (`InputSettings.GetActionNames` _returnvalue)
            (for _array_element_4 (`InputSettings.GetActionMappingByName` _returnvalue _array_element_3)
              (`InputSettings.RemoveActionMapping` _returnvalue _array_element_4 false))))))
    (:`then_1`
      ;[0 0 0] 应用
      (`|ExecutionSequence`
        (:`then_0`
          (`InputSettings.AddAxisMapping` _returnvalue_2 (make `InputAxisKeyMapping` "MoveForward" _scale_3 _key_3) false)
          (`InputSettings.AddAxisMapping` _returnvalue_2 (make `InputAxisKeyMapping` "MoveForward" _scale_4 _key_4) false)
          (`InputSettings.AddAxisMapping` _returnvalue_5 (make `InputAxisKeyMapping` "MoveRight" _scale_2 _key_2) false)
          (`InputSettings.AddAxisMapping` _returnvalue_5 (make `InputAxisKeyMapping` "MoveRight" _scale _key) false))
        (:`then_1`
          (`InputSettings.AddActionMapping` _returnvalue_3 _jump_2 false)
          (`InputSettings.AddActionMapping` _returnvalue_3 _interact_2 false)
          (`InputSettings.AddActionMapping` _returnvalue_3 _hook_2 false)
          (`InputSettings.AddActionMapping` _returnvalue_3 _reach_2 false)
          (`InputSettings.AddActionMapping` _returnvalue_3 _pause_2 false))
        (:`then_2`
          (`InputSettings.AddAxisMapping` _returnvalue_4 _loopup false)
          (`InputSettings.AddAxisMapping` _returnvalue_4 _lookright false))))
    (:`then_2`
      (`InputSettings.ForceRebuildKeymaps` (`InputSettings.GetInputSettings`)))))

(fn `GetAllSettings`
  (returns (Settings :type "/Game/FinalProject/Gameplay/Z_SaveGame/SSettings Structure"))
  (return (`self.Settings`)))

(fn `GetInputMaps`
  (returns (Return :type "/Game/FinalProject/Gameplay/UI/SInputMap_Keyboard Structure"))
  (locals (KeyMap :type "/Game/FinalProject/Gameplay/UI/SInputMap_Keyboard Structure"))
  (bind _returnvalue (`InputSettings.GetInputSettings`))
  (bind _returnvalue_2 (`InputSettings.GetInputSettings`))
  (bind _returnvalue_3 (`InputSettings.GetInputSettings`))
  (bind _keymap (`local.KeyMap`))
  (bind _keymap_2 (`local.KeyMap`))
  (`|ExecutionSequence`
    (:`then_0`
      ;[0 0 0] MoveForeard/MoveRight
      (for _array_element (`InputSettings.GetAxisMappingByName` _returnvalue "MoveForward")
        (if (> (`.Scale` (break `InputAxisKeyMapping` _array_element)) 0.0)
          (setmembers `/Game/FinalProject/Gameplay/UI/SInputMap_Keyboard` :`StructRef` _keymap_2 :`MoveFWD` _array_element)
          (else
            (setmembers `/Game/FinalProject/Gameplay/UI/SInputMap_Keyboard` :`StructRef` _keymap_2 :`MoveBWD` _array_element)))))
    (:`then_1`
      (for _array_element_2 (`InputSettings.GetAxisMappingByName` _returnvalue "MoveRight")
        (if (> (`.Scale` (break `InputAxisKeyMapping` _array_element_2)) 0.0)
          (setmembers `/Game/FinalProject/Gameplay/UI/SInputMap_Keyboard` :`StructRef` _keymap :`MoveRWD` _array_element_2)
          (else
            (setmembers `/Game/FinalProject/Gameplay/UI/SInputMap_Keyboard` :`StructRef` _keymap :`MoveLWD` _array_element_2)))))
    (:`then_2`
      ;[0 0 0] ActionMappings
      (setmembers `/Game/FinalProject/Gameplay/UI/SInputMap_Keyboard` :`StructRef` (`local.KeyMap`) :`Jump` (`|GetArrayItem` (`InputSettings.GetActionMappingByName` _returnvalue_2 "Jump")) :`Interact` (`|GetArrayItem` (`InputSettings.GetActionMappingByName` _returnvalue_2 "Interact")) :`Hook` (`|GetArrayItem` (`InputSettings.GetActionMappingByName` _returnvalue_2 "Hook")) :`Reach` (`|GetArrayItem` (`InputSettings.GetActionMappingByName` _returnvalue_2 "Reach")) :`Pause` (`|GetArrayItem` (`InputSettings.GetActionMappingByName` _returnvalue_2 "Pause"))))
    (:`then_3`
      ;[0 0 0] LookUp/LookRight
      (setmembers `/Game/FinalProject/Gameplay/UI/SInputMap_Keyboard` :`StructRef` (`local.KeyMap`) :`LoopUp` (`|GetArrayItem` (`InputSettings.GetAxisMappingByName` _returnvalue_3 "LookUp")) :`LookRight` (`|GetArrayItem` (`InputSettings.GetAxisMappingByName` _returnvalue_3 "LookRight"))))
    (:`then_4`
      (return (`local.KeyMap`)))))

(fn `InputForSetting`
  (params (NewKey :type "Key Structure" :default "None"))
  (`/Game/FinalProject/Gameplay/UI/WBP_Pause.InputForSetting` (`self.WBP_Pause`) NewKey))

(fn `LoadGame`
  (bind (_returnvalue _levelname _characterdata) (`/Game/FinalProject/Gameplay/BP_MyInstance.LoadGame` (`self.MyGameInstance`)))
  (if _returnvalue
    (`/Game/FinalProject/Gameplay/Character/BP_MyCharacter.LoadData` (`self.MyCharacter`) _characterdata)))

(fn `PressPause`
  (switch `/Game/FinalProject/Gameplay/EGameState` (`self.MyGameState`)
    (:`NewEnumerator0`
      (`self.SetPause` true))
    (:`NewEnumerator2`
      (`/Game/FinalProject/Gameplay/UI/WBP_Pause.PressPause` (`self.WBP_Pause`) :!label _label))
    (:`NewEnumerator1`
      (`/Game/FinalProject/Gameplay/Character/BP_MyCharacter.CE_SetRest` (`self.MyCharacter`) false))
    (:`NewEnumerator3`
      (goto _label))))

(fn `Quit`
  (`KismetSystemLibrary.QuitGame` null "Quit"))

(fn `Restart`
  (bind _returnvalue (`GameplayStatics.GetCurrentLevelName` true))
  (`GameplayStatics.OpenLevel` (`KismetStringLibrary.Conv_StringToName` _returnvalue)))

(fn `SaveAllSettings`
  (params (Settings :type "/Game/FinalProject/Gameplay/Z_SaveGame/SSettings Structure"))
  (set `self.Settings` Settings)
  (`|ExecutionSequence`
    (:`then_0`
      (`self.ApplyAllSettings` (`self.Settings`)))
    (:`then_1`
      (`/Game/FinalProject/Gameplay/BP_MyInstance.SaveSettings` (`self.MyGameInstance`) (`self.Settings`)))))

(fn `SaveGame`
  (bind _returnvalue (`/Game/FinalProject/Gameplay/BP_MyInstance.SaveGame` (`self.MyGameInstance`) (`/Game/FinalProject/Gameplay/Character/BP_MyCharacter.GetSaveGameData` (`self.MyCharacter`))))
  (if (not _returnvalue)
    (`KismetSystemLibrary.PrintString` "WARNING: Save Game Failed" true true (struct :`R` 1.0 :`A` 1.0) 5.0)))

(fn `SetCharacterRest`
  (params (Rest :type Boolean) (Campfire :type "/Game/FinalProject/Gameplay/Fire/BP_Campfire Object Reference") (BlendTime :type "Float (single-precision)"))
  (bind _mycontroller (`self.MyController`))
  (bind _wbp_rest (`self.WBP_Rest`))
  (if Rest
    (set `self.MyGameState` "NewEnumerator1")
    (`PlayerController.SetViewTargetWithBlend` (`self.MyController`) (`local.Campfire`) (`local.BlendTime`) "VTBlend_Cubic" 0.0 false)
    (`/Game/FinalProject/Gameplay/UI/WBP_Rest.UpdateCampfireInfo` _wbp_rest (`local.Campfire`))
    (`UserWidget.AddToViewport` _wbp_rest 0)
    (`WidgetBlueprintLibrary.SetInputMode_GameAndUIEx` _mycontroller _wbp_rest)
    (set `PlayerController.bShowMouseCursor` true _mycontroller)
    (else
      (set `self.MyGameState` "NewEnumerator0")
      (`PlayerController.SetViewTargetWithBlend` (`self.MyController`) (`self.MyCharacter`) (`local.BlendTime`) "VTBlend_Cubic" 0.0 false)
      (`Widget.RemoveFromParent` (`self.WBP_Rest`))
      (`WidgetBlueprintLibrary.SetInputMode_GameOnly` _mycontroller)
      (set `PlayerController.bShowMouseCursor` false _mycontroller))))

(fn `SetPause`
  (params (Pause :type Boolean))
  (bind _wbp_pause (`self.WBP_Pause`))
  (bind _mycontroller (`self.MyController`))
  (if Pause
    (`GameplayStatics.SetGamePaused` true)
    (set `self.MyGameState` "NewEnumerator2")
    (`UserWidget.AddToViewport` _wbp_pause 0)
    (`WidgetBlueprintLibrary.SetInputMode_GameAndUIEx` _mycontroller (`self.WBP_Pause`))
    (set `PlayerController.bShowMouseCursor` true _mycontroller)
    (else
      (`GameplayStatics.SetGamePaused` false)
      (set `self.MyGameState` "NewEnumerator0")
      (`Widget.RemoveFromParent` _wbp_pause)
      (`WidgetBlueprintLibrary.SetInputMode_GameOnly` _mycontroller)
      (set `PlayerController.bShowMouseCursor` false _mycontroller))))

(fn `UserConstructionScript`)