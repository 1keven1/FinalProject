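; Laser emitter that, while Activate is set, fires a beam along its forward vector and sends LightHitMessage to each actor it hits.
; Every Tick it chains line traces, reflecting off GameTraceChannel2 components until another hit, a miss or the bounce limit ends it.
; Each trace ignores the previous hit actor, starting with Spawner.
; A mesh pool built at BeginPlay draws the segments, hidden each frame then positioned, rotated and stretched per trace.
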(event `self.ReceiveBeginPlay`
  (`|ExecutionSequence`
    (:`then_0`
      (`KismetArrayLibrary.Array_Add` (`self.LaserMeshes`) (`self.LazerMesh`)))
    (:`then_1`
      (for _ (range 1 (+ (`self.MaxBounceNum`) 1))
        (bind _returnvalue (`AddComponent|NODE_AddStaticMeshComponent-1`))
        (`StaticMeshComponent.SetStaticMesh` _returnvalue (`StaticMeshComponent.StaticMesh` (`self.LazerMesh`)))
        (`SceneComponent.SetVisibility` _returnvalue false false)
        (`PrimitiveComponent.SetCollisionEnabled` _returnvalue "NoCollision")
        (`KismetArrayLibrary.Array_Add` (`self.LaserMeshes`) _returnvalue)))))

(event `self.ReceiveTick`
  (params (DeltaSeconds :type "Float (single-precision)"))
  (`self.HideAllLazerMeshes`)
  (if (`self.bActivate`)
    (`self.ResetPreviousVariable`)
    (for _index (range (+ (`self.MaxBounceNum`) 1)) :!label _label
      (bind _output_get (set `self.BouncingIndex` _index))
      (bind (_start _dir) (`self.EvaluateBouncingStartDir` (== _output_get 0)))
      (bind _output_get_2 (set `self.PreviousDir` _dir))
      (bind (_returnvalue _location _normal _hitactor _hitcomponent) (`self.Bounce` _start _output_get_2 (`|MakeArray` (`self.PreviousHitActor`))))
      (if _returnvalue
        (message `/Game/FinalProject/Gameplay/Light/ILight.LightHit` _hitactor)
        (if (`|EnumEquality` (`PrimitiveComponent.GetCollisionObjectType` _hitcomponent) "ECC_GameTraceChannel2")
          (set `self.PreviousHitActor` _hitactor)
          (set `self.PreviousNormal` _normal)
          (set `self.PreviousLocation` _location)
          (else
            (`self.CE_BreakBouncingLoop` :!label _label_2)))
        (else
          (goto _label_2))))))

(event `CE_BreakBouncingLoop`
  (goto _label :!via `Break`))

(fn `Bounce`
  (params (Start :type "Vector Structure") (Direction :type "Vector Structure") (ActorsToIgnore :type "Array of Actor Object Reference (by ref)"))
  (returns (ReturnValue :type Boolean) (Location :type "Vector Structure") (Normal :type "Vector Structure") (HitActor :type "Actor Object Reference") (HitComponent :type "PrimitiveComponent Object Reference"))
  (bind (_outhit _returnvalue) (`KismetSystemLibrary.LineTraceSingle` Start (+ Start (* Direction (`self.MaxTraceDistance`))) "TraceTypeQuery3" false ActorsToIgnore))
  (bind (_bblockinghit _binitialoverlap _time _distance _location _impactpoint _normal _impactnormal _physmat _hitactor _hitcomponent _hitbonename _bonename _hititem _elementindex _faceindex _tracestart _traceend) (`GameplayStatics.BreakHitResult` _outhit))
  (`self.ShowLaserMesh` _tracestart (`KismetMathLibrary.SelectVector` _location _traceend _returnvalue) (`self.BouncingIndex`))
  (return _returnvalue _location _normal _hitactor _hitcomponent))

(fn `EvaluateBouncingStartDir`
  (params (bFirst :type Boolean))
  (returns (Start :type "Vector Structure") (Dir :type "Vector Structure"))
  (return (`KismetMathLibrary.SelectVector` (`self.K2_GetActorLocation`) (`self.PreviousLocation`) bFirst) (`KismetMathLibrary.SelectVector` (`self.GetActorForwardVector`) (`KismetMathLibrary.GetReflectionVector` (`self.PreviousDir`) (`self.PreviousNormal`)) bFirst)))

(fn `HideAllLazerMeshes`
  (for _array_element (`self.LaserMeshes`)
    (`SceneComponent.SetVisibility` _array_element false false)))

(fn `ResetPreviousVariable`
  (set `self.PreviousDir` (0.0 0.0 0.0))
  (set `self.PreviousLocation` (0.0 0.0 0.0))
  (set `self.PreviousNormal` (0.0 0.0 0.0))
  (set `self.PreviousHitActor` (`self.Spawner`)))

(fn `ShowLaserMesh`
  (params (Start :type "Vector Structure") (End :type "Vector Structure") (Index :type Integer))
  (bind _output (`|GetArrayItem` (`self.LaserMeshes`) Index))
  (`SceneComponent.K2_SetWorldLocationAndRotation` _output Start (`KismetMathLibrary.FindLookAtRotation` Start End) false false)
  (`SceneComponent.SetRelativeScale3D` _output (`KismetMathLibrary.MakeVector` (* (`KismetMathLibrary.Vector_Distance` Start End) 0.1) 1.0 1.0))
  (`SceneComponent.SetVisibility` _output true false))

(fn `UserConstructionScript`)