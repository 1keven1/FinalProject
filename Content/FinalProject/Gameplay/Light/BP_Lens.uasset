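; BP_Lens is an interactable lens that holds a torch and powers a BP_Lazer beam it spawns and attaches on BeginPlay.
; The player inserts or removes the torch via an animation notify, or it starts preloaded with a burning one.
; The torch's burn and stop-burn dispatchers toggle the laser, which switches off when the torch is taken.
; Interaction from left or right points checks for overlapping actors, standing room and the character's held or holstered item.
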(event `self.ReceiveBeginPlay`
  (`|ExecutionSequence`
    (:`then_0`
      (bind _returnvalue (`|SpawnActorFromClass` "/Game/FinalProject/Gameplay/Light/BP_Lazer.BP_Lazer_C" (`KismetMathLibrary.MakeTransform` (0.0 0.0 0.0)) "AlwaysSpawn" "OverrideRootScale" null 5 10000.0 false self 10.0 null))
      (bind _output_get (set `self.Lazer` _returnvalue))
      (`self.K2_AttachToComponent` _output_get (`self.LazerDir`) "None" "SnapToTarget" "SnapToTarget" "KeepRelative" true))
    (:`then_1`
      (if (`self.bLoaded`)
        (bind _returnvalue_2 (`|SpawnActorFromClass` "/Game/FinalProject/Gameplay/Fire/BP_Torch.BP_Torch_C" (`KismetMathLibrary.MakeTransform` (0.0 0.0 0.0)) "AlwaysSpawn" "OverrideRootScale" null null))
        (`self.K2_AttachToComponent` _returnvalue_2 (`self.SM_Lens`) "Socket_Torch" "SnapToTarget" "SnapToTarget" "KeepRelative" true)
        (bind _output_get_2 (set `self.Torch` _returnvalue_2))
        (`/Game/FinalProject/Gameplay/Fire/BP_Flammable_Base.StartBurn` _output_get_2)
        (`|ExecutionSequence` :!label _label
          (:`then_0`
            (`self.SetLazerActivate` (`/Game/FinalProject/Gameplay/Fire/BP_Flammable_Base.bBurn` (stale `/Game/FinalProject/Gameplay/Interactive/IInteract.ProcessAnimationNotify` _output_get))))
          (:`then_1`
            (add `/Game/FinalProject/Gameplay/Fire/BP_Flammable_Base.ED_OnBurn` (stale `/Game/FinalProject/Gameplay/Interactive/IInteract.ProcessAnimationNotify` _output_get) (delegate `ED_OnBurn`))
            (add `/Game/FinalProject/Gameplay/Fire/BP_Flammable_Base.ED_OnStopBurn` (stale `/Game/FinalProject/Gameplay/Interactive/IInteract.ProcessAnimationNotify` _output_get) (delegate `ED_OnStopBurn`))))))))

(event `/Game/FinalProject/Gameplay/Interactive/IInteract.ProcessAnimationNotify`
  (params (Character :type "/Game/FinalProject/Gameplay/Character/BP_MyCharacter Object Reference") (InteractComp :type "PrimitiveComponent Object Reference"))
  (bind _torch (`self.Torch`))
  (if (not (`self.bLoaded`))
    (bind _torch_2 (`/Game/FinalProject/Gameplay/Character/BP_MyCharacter.RemoveTorch` Character))
    (`self.K2_AttachToComponent` _torch_2 (`self.SM_Lens`) "Socket_Torch" "SnapToTarget" "SnapToTarget" "KeepRelative" true)
    (set `self.bLoaded` true)
    (bind _asbp_flammable_base (cast `/Game/FinalProject/Gameplay/Fire/BP_Flammable_Base` _torch_2))
    (bind _output_get (set `self.Torch` _asbp_flammable_base))
    (goto _label)
    (else
      (bind (_interacttype _targetactor) (message `/Game/FinalProject/Gameplay/Interactive/IInteract.Interact` (`self.Torch`) Character InteractComp))
      (bind _return_value (`/Game/FinalProject/Gameplay/Character/BP_MyCharacter.AddTorch` Character _targetactor))
      (if _return_value
        (remove `/Game/FinalProject/Gameplay/Fire/BP_Flammable_Base.ED_OnBurn` _torch (delegate `ED_OnBurn`))
        (remove `/Game/FinalProject/Gameplay/Fire/BP_Flammable_Base.ED_OnStopBurn` _torch (delegate `ED_OnStopBurn`))
        (`self.SetLazerActivate` false)
        (set `self.Torch` null)
        (set `self.bLoaded` false)))))

(event `ED_OnBurn`
  (`self.SetLazerActivate` true))

(event `ED_OnStopBurn`
  (`self.SetLazerActivate` false))

(fn `ChechCanInteract`
  (params (InteractComponent :type "PrimitiveComponent Object Reference") (Character :type "/Game/FinalProject/Gameplay/Character/BP_MyCharacter Object Reference"))
  (returns (`Return Value` :type Boolean))
  (bind _returnvalue (`KismetSystemLibrary.IsValid` (`/Game/FinalProject/Gameplay/Character/BP_MyCharacter.InHandObj` Character)))
  (bind _returnvalue_2 (`KismetSystemLibrary.IsValid` (`/Game/FinalProject/Gameplay/Character/BP_MyCharacter.HolsterObj` Character)))
  (`|ExecutionSequence`
    (:`then_0`
      (bind (_out _length) (`/Game/FinalProject/Gameplay/BPFL_MyFunctionLibrary.ArrayRemoveSelfAndCharacter` (`PrimitiveComponent.GetOverlappingActors` InteractComponent null) Character self))
      (if (!= _length 0)
        (return false)))
    (:`then_1`
      (bind _returnvalue_3 (`/Game/FinalProject/Gameplay/BPFL_MyFunctionLibrary.CheckCanCharacterStand` (`SceneComponent.K2_GetComponentLocation` (select `bool` (== (`local.InteractComponent`) (`self.InteractCollisionL`)) :`false` (`self.InteractPointR`) :`true` (`self.InteractPointL`)))))
      (if (not _returnvalue_3)
        (return false)))
    (:`then_2`
      (if (`self.bLoaded`)
        (return (and (not _returnvalue) (not _returnvalue_2)))
        (else
          (return (or _returnvalue _returnvalue_2)))))))

(fn `GetInteractTipUIInfo`
  (params (InteractComponent :type "PrimitiveComponent Object Reference"))
  (returns (WorldPosition :type "Vector Structure") (TipText :type Text))
  (return (`SceneComponent.K2_GetComponentLocation` (`self.InteractTipPos`)) (select `bool` (`self.bLoaded`) :`false` (`self.InteractTip1`) :`true` (`self.InteractTip2`))))

(fn `GetMoveToInfo`
  (params (InteractComponent :type "PrimitiveComponent Object Reference") (Character :type "/Game/FinalProject/Gameplay/Character/BP_MyCharacter Object Reference"))
  (returns (InteractType :type "/Game/FinalProject/Gameplay/Interactive/EInteractType Enum") (NeedHolster :type Boolean) (NeedHold :type Boolean) (TargetPos :type "Vector Structure") (TargetRot :type "Rotator Structure"))
  (bind _interactpointl (`self.InteractPointL`))
  (bind _interactpointr (`self.InteractPointR`))
  (bind _returnvalue (== InteractComponent (`self.InteractCollisionL`)))
  (return "NewEnumerator2" false true (`SceneComponent.K2_GetComponentLocation` (select `bool` _returnvalue :`false` _interactpointr :`true` _interactpointl)) (`SceneComponent.K2_GetComponentRotation` (select `bool` _returnvalue :`false` _interactpointr :`true` _interactpointl))))

(fn `Interact`
  (params (Character :type "/Game/FinalProject/Gameplay/Character/BP_MyCharacter Object Reference") (InteractComponent :type "PrimitiveComponent Object Reference"))
  (returns (InteractType :type "/Game/FinalProject/Gameplay/Interactive/EInteractType Enum") (TargetActor :type "Actor Object Reference") (InteractAction :type "/Game/FinalProject/Gameplay/Character/EInteractAction Enum"))
  (return "NewEnumerator2" self (select `bool` (`self.bLoaded`) :`false` "NewEnumerator0" :`true` "NewEnumerator1" :!type "/Game/FinalProject/Gameplay/Character/EInteractAction Enum")))

(fn `Move`
  (params (Value :type "Float (double-precision)"))
  (returns (Velocity :type "Vector Structure"))
  (return (0.0 0.0 0.0)))

(fn `SetLazerActivate`
  (params (Activate :type Boolean))
  (set `/Game/FinalProject/Gameplay/Light/BP_Lazer.bActivate` Activate (`self.Lazer`)))

(fn `StopInteract`
  (params (Character :type "/Game/FinalProject/Gameplay/Character/BP_MyCharacter Object Reference"))
  (returns (ReturnValue :type Boolean) (InteractAction :type "/Game/FinalProject/Gameplay/Character/EInteractAction Enum"))
  (return false "NewEnumerator2"))

(fn `UserConstructionScript`
  (if (`self.bLoaded`)
    _))