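; Interactable reflect mirror that the character can pick up and carry, or push to rotate, as enabled per instance.
; Construction script sets frame shape, handles and starting yaw.
; Interaction checks test overlaps and standing room, animation notifies switch Norm, Held and Pushed states, and Move eases rotation speed.
; Put-down aligns to the traced ground normal and delays restoring pawn collision until the character stops overlapping.
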(event `self.ReceiveBeginPlay`
  (bind _returnvalue (select `bool` (`self.bCanRotate`) :`false` "NoCollision" :`true` "QueryOnly" :!type "ECollisionEnabled Enum"))
  (bind _returnvalue_2 (select `bool` (`self.bCanHold`) :`false` "NoCollision" :`true` "QueryOnly" :!type "ECollisionEnabled Enum"))
  (`|ExecutionSequence`
    (:`then_1`
      (`PrimitiveComponent.SetCollisionEnabled` (`self.HoldHandle`) _returnvalue_2)
      (`PrimitiveComponent.SetCollisionEnabled` (`self.InteractCollision_Hold2`) _returnvalue_2)
      (`PrimitiveComponent.SetCollisionEnabled` (`self.InteractCollision_Hold1`) _returnvalue_2))
    (:`then_2`
      (`PrimitiveComponent.SetCollisionEnabled` (`self.RotateHandle`) _returnvalue)
      (`PrimitiveComponent.SetCollisionEnabled` (`self.InteractCollision_Push`) _returnvalue))))

(event `/Game/FinalProject/Gameplay/Interactive/IInteract.ProcessAnimationNotify`
  (params (Character :type "/Game/FinalProject/Gameplay/Character/BP_MyCharacter Object Reference") (InteractComp :type "PrimitiveComponent Object Reference"))
  (bind (_bblockinghit _binitialoverlap _time _distance _location _impactpoint _normal) (`GameplayStatics.BreakHitResult` (`self.PutDownHit`)))
  (bind _returnvalue (`KismetMathLibrary.Cross_VectorVector` _normal (`self.GetActorForwardVector`)))
  (switch `/Game/FinalProject/Gameplay/Light/EMirrorState` (`self.State`)
    (:`NewEnumerator0`
      (switch `/Game/FinalProject/Gameplay/Light/EMirrorState` (`self.CheckHoldOrPush` InteractComp)
        (:`NewEnumerator1`
          (`/Game/FinalProject/Gameplay/Character/BP_MyCharacter.GetUp` Character self "Socket_Hold" (`KismetMathLibrary.SelectFloat` 180.0 0.0 (== InteractComp (`self.InteractCollision_Hold1`))))
          (set `self.State` "NewEnumerator1"))
        (:`NewEnumerator2`
          (`/Game/FinalProject/Gameplay/Character/BP_MyCharacter.StartPush` Character (`self.Body_Base`))
          (set `self.State` "NewEnumerator2"))))
    (:`NewEnumerator1`
      (`/Game/FinalProject/Gameplay/Character/BP_MyCharacter.PutDown` Character self)
      (`self.K2_SetActorLocationAndRotation` _location (`KismetMathLibrary.MakeRotationFromAxes` (`KismetMathLibrary.Cross_VectorVector` _returnvalue _normal) _returnvalue _normal) true)
      (set `self.State` "NewEnumerator0")
      ;[0 0 0] 如果与角色有重叠 则等角色出去后再设置回碰撞
      (if (`self.CheckOverlapWithPawn`)
        (add `self.ED_OnCharacterEndOverlap` (delegate `ED_OnCharacterEndOverlap_Event`))
        (else
          (`self.SetColliisonResponceToPawn` true))))
    (:`NewEnumerator2`
      (`/Game/FinalProject/Gameplay/Character/BP_MyCharacter.StopPush` Character)
      (`self.SetColliisonResponceToPawn` true)
      (set `self.State` "NewEnumerator0"))))

(event `ED_OnCharacterEndOverlap_Event`
  ;[0 0 0] 如果与角色有重叠 则等角色出去后再设置回碰撞
  (`self.SetColliisonResponceToPawn` true)
  (remove `self.ED_OnCharacterEndOverlap` (delegate `ED_OnCharacterEndOverlap_Event`)))

(event `self.PawnDetectColliison.OnComponentEndOverlap`
  (params (OverlappedComponent :type "PrimitiveComponent Object Reference") (OtherActor :type "Actor Object Reference") (OtherComp :type "PrimitiveComponent Object Reference") (OtherBodyIndex :type Integer))
  (switch `/Game/FinalProject/Gameplay/Light/EMirrorState` (`self.State`)
    (:`NewEnumerator0`
      (if (== (`GameplayStatics.GetObjectClass` OtherActor) "/Game/FinalProject/Gameplay/Character/BP_MyCharacter.BP_MyCharacter_C")
        (`self.ED_OnCharacterEndOverlap`)))))

(event `/Game/FinalProject/Gameplay/Interactive/IInteract.MoveToInterrupted`
  (params (Character :type "/Game/FinalProject/Gameplay/Character/BP_MyCharacter Object Reference"))
  (`self.SetColliisonResponceToPawn` true))

(fn `ChechCanInteract`
  (params (InteractComponent :type "PrimitiveComponent Object Reference") (Character :type "/Game/FinalProject/Gameplay/Character/BP_MyCharacter Object Reference"))
  (returns (`Return Value` :type Boolean))
  (locals (OverlappingActors :type "Array of Actor Object Reference") (TopActors :type "Array of Actor Object Reference"))
  (`|ExecutionSequence`
    (:`then_0`
      ;[0 0 0] 啥都不行
      (if (and (not (`self.bCanHold`)) (not (`self.bCanRotate`)))
        (return false)))
    (:`then_1`
      ;[0 0 0] 与其它东西有重叠也不行 不然玩家走不过去
      (bind (_out _length) (`/Game/FinalProject/Gameplay/BPFL_MyFunctionLibrary.ArrayRemoveSelfAndCharacter` (`PrimitiveComponent.GetOverlappingActors` InteractComponent null) (`local.Character`) self))
      (if (> _length 0)
        (return false)))
    (:`then_2`
      (switch `/Game/FinalProject/Gameplay/Light/EMirrorState` (`self.CheckHoldOrPush` InteractComponent)
        (:`NewEnumerator0`
          (return false))
        (:`NewEnumerator1`
          ;[0 0 0] 下面没地也不得行
          (bind _returnvalue (`/Game/FinalProject/Gameplay/BPFL_MyFunctionLibrary.CheckCanCharacterStand` (`SceneComponent.K2_GetComponentLocation` (select `bool` (== (`local.InteractComponent`) (`self.InteractCollision_Hold1`)) :`false` (`self.InteractPos_Hold2`) :`true` (`self.InteractPos_Hold1`)))))
          (if _returnvalue
            _
            (else
              (return false))))
        (:`NewEnumerator2`
          (bind _returnvalue_2 (`/Game/FinalProject/Gameplay/BPFL_MyFunctionLibrary.CheckCanCharacterStand` (`SceneComponent.K2_GetComponentLocation` (`self.InteractPos_Push`))))
          (if _returnvalue_2
            _
            (else
              (return false)))))
      ;[0 0 0] 顶上有东西压着也不行
      (bind (_out_2 _length_2) (`/Game/FinalProject/Gameplay/BPFL_MyFunctionLibrary.ArrayRemoveSelfAndCharacter` (`PrimitiveComponent.GetOverlappingActors` (`self.TopDetectCollision`) null) (`local.Character`) self))
      (if (> _length_2 0)
        (return false)
        (else
          (return true))))))

(fn `CheckHoldOrPush`
  (params (InteractComp :type "Object Object Reference"))
  (returns (State :type "/Game/FinalProject/Gameplay/Light/EMirrorState Enum"))
  (`|ExecutionSequence`
    (:`then_0`
      (if (and (`self.bCanHold`) (or (== InteractComp (`self.InteractCollision_Hold1`)) (== InteractComp (`self.InteractCollision_Hold2`))))
        (return "NewEnumerator1")))
    (:`then_1`
      (if (and (`self.bCanRotate`) (== InteractComp (`self.InteractCollision_Push`)))
        (return "NewEnumerator2")))
    (:`then_2`
      (return "NewEnumerator0"))))

(fn `CheckOverlapWithPawn`
  (returns (ReturnValue :type Boolean))
  (return (`KismetArrayLibrary.Array_IsNotEmpty` (`PrimitiveComponent.GetOverlappingActors` (`self.PawnDetectColliison`) "/Game/FinalProject/Gameplay/Character/BP_MyCharacter.BP_MyCharacter_C"))))

(fn `GetInteractTipUIInfo`
  (params (InteractComponent :type "PrimitiveComponent Object Reference"))
  (returns (WorldPosition :type "Vector Structure") (TipText :type Text))
  (switch `/Game/FinalProject/Gameplay/Light/EMirrorState` (`self.CheckHoldOrPush` InteractComponent)
    (:`NewEnumerator1`
      (return (`SceneComponent.K2_GetComponentLocation` (`self.InteractTip_Hold`)) (`self.Tip_Hold`)))
    (:`NewEnumerator2`
      (return (`SceneComponent.K2_GetComponentLocation` (`self.InteractTip_Push`)) (`self.Tip_Push`)))))

(fn `GetMoveToInfo`
  (params (InteractComponent :type "PrimitiveComponent Object Reference") (Character :type "/Game/FinalProject/Gameplay/Character/BP_MyCharacter Object Reference"))
  (returns (InteractType :type "/Game/FinalProject/Gameplay/Interactive/EInteractType Enum") (NeedHolster :type Boolean) (NeedHold :type Boolean) (TargetPos :type "Vector Structure") (TargetRot :type "Rotator Structure"))
  (bind (_returnvalue_location _returnvalue_rotation) (`KismetMathLibrary.BreakTransform` (`SceneComponent.K2_GetComponentToWorld` (`self.InteractPos_Push`))))
  (bind (_returnvalue_location_2 _returnvalue_rotation_2) (`KismetMathLibrary.BreakTransform` (`SceneComponent.K2_GetComponentToWorld` (select `bool` (== InteractComponent (`self.InteractCollision_Hold1`)) :`false` (`self.InteractPos_Hold2`) :`true` (`self.InteractPos_Hold1`)))))
  (`self.SetColliisonResponceToPawn` false)
  (switch `/Game/FinalProject/Gameplay/Light/EMirrorState` (`self.CheckHoldOrPush` InteractComponent)
    (:`NewEnumerator1`
      (return "NewEnumerator4" true false _returnvalue_location_2 _returnvalue_rotation_2))
    (:`NewEnumerator2`
      (return "NewEnumerator5" true false _returnvalue_location _returnvalue_rotation))))

(fn `Interact`
  (params (Character :type "/Game/FinalProject/Gameplay/Character/BP_MyCharacter Object Reference") (InteractComponent :type "PrimitiveComponent Object Reference"))
  (returns (InteractType :type "/Game/FinalProject/Gameplay/Interactive/EInteractType Enum") (TargetActor :type "Actor Object Reference") (InteractAction :type "/Game/FinalProject/Gameplay/Character/EInteractAction Enum"))
  (switch `/Game/FinalProject/Gameplay/Light/EMirrorState` (`self.CheckHoldOrPush` InteractComponent)
    (:`NewEnumerator1`
      (return "NewEnumerator4" self "NewEnumerator4"))
    (:`NewEnumerator2`
      (return "NewEnumerator5" self "NewEnumerator6"))))

(fn `Move`
  (params (Value :type "Float (double-precision)"))
  (returns (Velocity :type "Vector Structure"))
  (locals (TargetSpeed :type "Float (double-precision)"))
  (bind _returnvalue (!= Value 0.0))
  (bind _returnvalue_2 (* Value (`self.RotateSpeed`)))
  (set `local.TargetSpeed` (`KismetMathLibrary.SelectFloat` (`self.MaxRotateSpeed`) 0.0 _returnvalue))
  (set `self.RotateSpeed` (`KismetMathLibrary.FInterpTo` (`self.RotateSpeed`) (`local.TargetSpeed`) (`GameplayStatics.GetWorldDeltaSeconds`) (`KismetMathLibrary.SelectFloat` 1.0 10.0 _returnvalue)))
  (`SceneComponent.K2_AddRelativeRotation` (`self.Body_Base`) (`KismetMathLibrary.MakeRotator` 0.0 0.0 (* (`GameplayStatics.GetWorldDeltaSeconds`) _returnvalue_2 -1.0)) false false)
  (return (* (`SceneComponent.GetForwardVector` (`self.InteractPos_Push`)) _returnvalue_2 2.0)))

(fn `SetColliisonResponceToPawn`
  (params (Collision :type Boolean))
  (`PrimitiveComponent.SetCollisionResponseToChannel` (`self.Base`) "ECC_Pawn" (select `bool` Collision :`false` "ECR_Ignore" :`true` "ECR_Block" :!type "ECollisionResponse Enum"))
  (`PrimitiveComponent.SetCollisionResponseToChannel` (`self.Body_Base`) "ECC_Pawn" (select `bool` Collision :`false` "ECR_Ignore" :`true` "ECR_Block" :!type "ECollisionResponse Enum"))
  (`PrimitiveComponent.SetCollisionResponseToChannel` (`self.MirrorFrame`) "ECC_Pawn" (select `bool` Collision :`false` "ECR_Ignore" :`true` "ECR_Block" :!type "ECollisionResponse Enum"))
  (`PrimitiveComponent.SetCollisionResponseToChannel` (`self.Mirror`) "ECC_Pawn" (select `bool` Collision :`false` "ECR_Ignore" :`true` "ECR_Block" :!type "ECollisionResponse Enum")))

(fn `StopInteract`
  (params (Character :type "/Game/FinalProject/Gameplay/Character/BP_MyCharacter Object Reference"))
  (returns (ReturnValue :type Boolean) (InteractAction :type "/Game/FinalProject/Gameplay/Character/EInteractAction Enum"))
  (locals (OverlapedActors :type "Array of Actor Object Reference"))
  (bind _returnvalue (`self.K2_GetActorLocation`))
  (switch `/Game/FinalProject/Gameplay/Light/EMirrorState` (`self.State`)
    (:`NewEnumerator1`
      (`|ExecutionSequence`
        (:`then_0`
          (bind (_out _length) (`/Game/FinalProject/Gameplay/BPFL_MyFunctionLibrary.ArrayRemoveSelfAndCharacter` (`PrimitiveComponent.GetOverlappingActors` (`self.PawnDetectColliison`) null) (`local.Character`) self))
          (if (!= _length 0)
            (return false "NewEnumerator5")))
        (:`then_1`
          (bind (_outhit _returnvalue_2) (`KismetSystemLibrary.LineTraceSingle` _returnvalue (+ _returnvalue (0.0 0.0 -100.0)) "TraceTypeQuery1"))
          (if (not _returnvalue_2)
            (return false "NewEnumerator5")
            (else
              (set `self.PutDownHit` _outhit))))
        (:`then_2`
          (return true "NewEnumerator5"))))
    (:`NewEnumerator2`
      (return true "NewEnumerator7"))))

(fn `UserConstructionScript`
  (bind _bcanrotate (`self.bCanRotate`))
  (bind _rotatehandle (`self.RotateHandle`))
  (bind _bcanhold (`self.bCanHold`))
  (bind _holdhandle (`self.HoldHandle`))
  (bind _interactcollision_push (`self.InteractCollision_Push`))
  (bind _mirrorframe (`self.MirrorFrame`))
  (bind _mirror (`self.Mirror`))
  (bind _returnvalue (select `bool` _bcanrotate :`false` "NoCollision" :`true` "QueryOnly" :!type "ECollisionEnabled Enum"))
  (bind _returnvalue_2 (select `bool` _bcanhold :`false` "NoCollision" :`true` "QueryOnly" :!type "ECollisionEnabled Enum"))
  (`|ExecutionSequence`
    (:`then_0`
      (switch `/Game/FinalProject/Gameplay/Light/EMirrorShape` (`self.MirrorShape`)
        (:`NewEnumerator0`
          (`StaticMeshComponent.SetStaticMesh` _mirrorframe "/Game/FinalProject/TestAsset/Light/SM_Mirror_Body_TrangleFrame.SM_Mirror_Body_TrangleFrame")
          (`StaticMeshComponent.SetStaticMesh` _mirror "/Game/FinalProject/TestAsset/Light/SM_Mirror_Body_Trangle.SM_Mirror_Body_Trangle"))
        (:`NewEnumerator1`
          (`StaticMeshComponent.SetStaticMesh` _mirrorframe "/Game/FinalProject/TestAsset/Light/SM_Mirror_Body_SquareFrame.SM_Mirror_Body_SquareFrame")
          (`StaticMeshComponent.SetStaticMesh` _mirror "/Game/FinalProject/TestAsset/Light/SM_Mirror_Body_Square.SM_Mirror_Body_Square"))))
    (:`then_1`
      (`SceneComponent.SetVisibility` _holdhandle _bcanhold true)
      (`PrimitiveComponent.SetCollisionEnabled` _holdhandle _returnvalue_2)
      (`PrimitiveComponent.SetCollisionEnabled` (`self.InteractCollision_Hold2`) _returnvalue_2)
      (`PrimitiveComponent.SetCollisionEnabled` (`self.InteractCollision_Hold1`) _returnvalue_2)
      (`SceneComponent.SetVisibility` (`self.InteractCollision_Hold1`) _bcanhold true)
      (`SceneComponent.SetVisibility` (`self.InteractCollision_Hold2`) _bcanhold true))
    (:`then_2`
      (`SceneComponent.SetVisibility` _rotatehandle _bcanrotate true)
      (`PrimitiveComponent.SetCollisionEnabled` _rotatehandle _returnvalue)
      (`PrimitiveComponent.SetCollisionEnabled` _interactcollision_push _returnvalue)
      (`SceneComponent.SetVisibility` _interactcollision_push _bcanrotate true))
    (:`then_3`
      (`SceneComponent.K2_SetRelativeRotation` (`self.Body_Base`) (`KismetMathLibrary.MakeRotator` 0.0 0.0 (`self.StartRotation`)) false false))))