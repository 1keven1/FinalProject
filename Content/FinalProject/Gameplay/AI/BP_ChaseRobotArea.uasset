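; BP_ChaseRobotArea is a trigger area that tells a chase robot when the player is in range.
; On BeginPlay it casts its child actor to BP_ChaseRobot and caches the reference.
; Box overlap events filter for the exact BP_MyCharacter class, passing that character to the robot's SetPlayerInRange on entry and calling it with no target on exit.
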(event `self.ReceiveBeginPlay`
  (`|ExecutionSequence`
    (:`then_0`
      (bind _asbp_chase_robot (cast `/Game/FinalProject/Gameplay/AI/BP_ChaseRobot` (`ChildActorComponent.ChildActor` (`self.ChildActor`))))
      (set `self.ChaseRobot` _asbp_chase_robot))))

(event `self.Box.OnComponentBeginOverlap`
  (params (OverlappedComponent :type "PrimitiveComponent Object Reference") (OtherActor :type "Actor Object Reference") (OtherComp :type "PrimitiveComponent Object Reference") (OtherBodyIndex :type Integer) (bFromSweep :type Boolean) (SweepResult :type "HitResult Structure (by ref)"))
  (if (== (`GameplayStatics.GetObjectClass` OtherActor) "/Game/FinalProject/Gameplay/Character/BP_MyCharacter.BP_MyCharacter_C")
    (`/Game/FinalProject/Gameplay/AI/BP_ChaseRobot.SetPlayerInRange` (`self.ChaseRobot`) OtherActor)))

(event `self.Box.OnComponentEndOverlap`
  (params (OverlappedComponent :type "PrimitiveComponent Object Reference") (OtherActor :type "Actor Object Reference") (OtherComp :type "PrimitiveComponent Object Reference") (OtherBodyIndex :type Integer))
  (if (== (`GameplayStatics.GetObjectClass` OtherActor) "/Game/FinalProject/Gameplay/Character/BP_MyCharacter.BP_MyCharacter_C")
    (`/Game/FinalProject/Gameplay/AI/BP_ChaseRobot.SetPlayerInRange` (`self.ChaseRobot`) null)))

(fn `UserConstructionScript`)