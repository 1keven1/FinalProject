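; Electrically powered vertical door that rises in proportion to the voltage it receives.
; Each tick turns conducted Energy into Volt and a target height, then clears it; Volt also drives an eased progress-bar material.
; The door mesh moves kinematically at constant speed when rising, but drops under physics when above target, with upward velocity capped and re-locking once settled.
; Movement and hard hits trigger looping and impact sounds.
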(event `self.ReceiveBeginPlay`
  (set `self.StartPos` (`self.K2_GetActorLocation`)))

(event `self.ReceiveTick`
  (params (DeltaSeconds :type "Float (single-precision)"))
  (bind (_returnvalue_x _returnvalue_y _returnvalue_z) (`KismetMathLibrary.BreakVector` (`self.K2_GetActorLocation`)))
  (bind (_returnvalue_x_2 _returnvalue_y_2 _returnvalue_z_2) (`KismetMathLibrary.BreakVector` (`self.K2_GetActorLocation`)))
  (bind (_returnvalue_x_3 _returnvalue_y_3) (`KismetMathLibrary.BreakVector` (`self.K2_GetActorLocation`)))
  (bind _sm_door_up (`self.SM_Door_Up`))
  (bind _sm_door_up_2 (`self.SM_Door_Up`))
  (bind (_returnvalue_x_4 _returnvalue_y_4 _returnvalue_z_3) (`KismetMathLibrary.BreakVector` (`SceneComponent.K2_GetComponentLocation` (`self.SM_Door_Up`))))
  (bind (_returnvalue_x_5 _returnvalue_y_5 _returnvalue_z_4) (`KismetMathLibrary.BreakVector` (`SceneComponent.K2_GetComponentLocation` (`self.SM_Door_Up`))))
  (bind _returnvalue (+ (`self.TargetHeight`) _returnvalue_z_2))
  (`|ExecutionSequence`
    (:`then_0`
      ;[0 0 0] 计算出电压 目标高度
      (bind _output_get (set `self.Volt` (`KismetMathLibrary.Conv_IntToDouble` (`KismetMathLibrary.Round` (/ (`self.Energy`) (`GameplayStatics.GetWorldDeltaSeconds`))))))
      (set `self.TargetHeight` (* (`KismetMathLibrary.FClamp` (/ _output_get (`self.MaxVolt`))) (`self.MaxHeight`)))
      (set `self.Energy` 0.0))
    (:`then_1`
      (if (>= _returnvalue _returnvalue_z_4)
        (`PrimitiveComponent.SetSimulatePhysics` (`self.SM_Door_Up`) false)
        (`SceneComponent.K2_SetWorldLocation` (`self.SM_Door_Up`) (`KismetMathLibrary.MakeVector` _returnvalue_x_3 _returnvalue_y_3 (`KismetMathLibrary.FInterpTo_Constant` _returnvalue_z_4 _returnvalue (`GameplayStatics.GetWorldDeltaSeconds`) (`self.MoveSpeed`))) true false)
        (set `self.bSpeedUp` false)
        (`self.K2_SetActorLocation` (+ (`self.StartPos`) (`KismetMathLibrary.MakeVector` (`KismetMathLibrary.RandomFloatInRange` -0.01 0.01))))
        (else
          (set `self.bMovingUp` false)
          (`PrimitiveComponent.SetSimulatePhysics` (`self.SM_Door_Up`) true)
          (`PrimitiveComponent.WakeAllRigidBodies` _sm_door_up_2)
          (bind _returnvalue_2 (`PrimitiveComponent.GetPhysicsLinearVelocity` _sm_door_up_2 "None"))
          (`|ExecutionSequence`
            (:`then_0`
              (bind _returnvalue_3 (`KismetMathLibrary.VSize` _returnvalue_2))
              (if (> _returnvalue_3 10.0)
                (set `self.bSpeedUp` true)))
            (:`then_1`
              (if (and (`self.bSpeedUp`) (< _returnvalue_3 0.1))
                (`PrimitiveComponent.SetSimulatePhysics` (`self.SM_Door_Up`) false)
                (`SceneComponent.K2_SetWorldLocation` (`self.SM_Door_Up`) (+ (`self.K2_GetActorLocation`) (`KismetMathLibrary.MakeVector` 0.0 0.0 (`self.TargetHeight`))) true false)
                (set `self.bSpeedUp` false)))))))
    (:`then_2`
      (`self.SetVisualEffects`))
    (:`then_3`
      (bind _returnvalue_4 (`PrimitiveComponent.GetPhysicsLinearVelocity` _sm_door_up "None"))
      (`PrimitiveComponent.SetPhysicsLinearVelocity` _sm_door_up (`KismetMathLibrary.MakeVector` 0.0 0.0 (`KismetMathLibrary.FMin` (.z _returnvalue_4) 100.0)) false "None"))
    (:`then_4`
      (bind _returnvalue_5 (`PrimitiveComponent.GetPhysicsLinearVelocity` (`self.SM_Door_Up`) "None"))
      (if (or (> (`KismetMathLibrary.Abs` (.z _returnvalue_5)) 1.0) (> (+ (`self.TargetHeight`) _returnvalue_z) _returnvalue_z_3))
        (`/Engine/EditorBlueprintResources/StandardMacros.DoOnce` false :!label _label
          (:`Completed`
            (`self.CE_A_PlayDoorSound` false)
            (goto _label_2 :!via `Reset`)))
        (else
          (`/Engine/EditorBlueprintResources/StandardMacros.DoOnce` true :!label _label_2
            (:`Completed`
              (`self.CE_A_PlayDoorSound` true (`KismetMathLibrary.SelectFloat` 0.5 0.0 (> (`self.TargetHeight`) 0.0)))
              (goto _label :!via `Reset`))))))))

(event `self.SM_Door_Up.OnComponentHit`
  (params (HitComponent :type "PrimitiveComponent Object Reference") (OtherActor :type "Actor Object Reference") (OtherComp :type "PrimitiveComponent Object Reference") (NormalImpulse :type "Vector Structure") (Hit :type "HitResult Structure (by ref)"))
  (bind _returnvalue (`KismetMathLibrary.Abs` (.z NormalImpulse)))
  (if (> _returnvalue 10000.0)
    (`self.CE_A_PlayImpauseSound` (`KismetMathLibrary.MultiplyMultiply_FloatFloat` (`KismetMathLibrary.FMin` (* _returnvalue 5e-06) 1.0) 2.0))))

(event `CE_A_PlayDoorSound`
  (params (Stop :type Boolean) (ImpauseVolume :type "Float (double-precision)" :default 1.0))
  (bind _audio (`self.Audio`))
  (if (not Stop)
    (`AudioComponent.FadeIn` _audio 0.1 1.0 0.0 "Linear")
    (else
      (`AudioComponent.FadeOut` _audio 0.5 0.0 "Linear")
      (`self.CE_A_PlayImpauseSound` ImpauseVolume))))

(event `CE_A_PlayImpauseSound`
  (params (Volume :type "Float (double-precision)" :default 1.0))
  (if (> Volume 0.0)
    (`GameplayStatics.PlaySoundAtLocation` (`self.DoorImpauseSound`) (`SceneComponent.K2_GetComponentLocation` (`self.SM_Door_Up`)) (struct) Volume 1.0 0.0 null null null null)))

(fn `Conduct`
  (params (EnergyIn :type "Float (double-precision)"))
  (returns (Consume :type "Float (double-precision)"))
  (bind _deltaenergy (`self.ChargeEnergy` EnergyIn))
  (return _deltaenergy))

(fn `SetVisualEffects`
  (bind _dynamat_progressbar (`self.Dynamat_ProgressBar`))
  (bind _returnvalue (`MaterialInstanceDynamic.K2_GetScalarParameterValue` _dynamat_progressbar "Value"))
  (`MaterialInstanceDynamic.SetScalarParameterValue` _dynamat_progressbar "Value" (`KismetMathLibrary.FInterpTo` _returnvalue (/ (`self.Volt`) (`self.MaxVolt`)) (`GameplayStatics.GetWorldDeltaSeconds`) 5.0)))

(fn `UserConstructionScript`
  (bind _sm_door_up (`self.SM_Door_Up`))
  (`parent.UserConstructionScript`)
  (`|ExecutionSequence`
    (:`then_0`
      (bind _returnvalue (`PrimitiveComponent.CreateDynamicMaterialInstance` _sm_door_up 1 (`PrimitiveComponent.GetMaterial` _sm_door_up 1) "None"))
      (set `self.Dynamat_ProgressBar` _returnvalue)
      (`MaterialInstanceDynamic.SetScalarParameterValue` (`self.Dynamat_ProgressBar`) "Value" (/ (`self.Volt`) (`self.MaxVolt`))))))