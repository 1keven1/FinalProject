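; Electronic converter that turns light hits into stored energy and electric power for its linked targets.
; Each hit charges it and conducts that energy to the targets at a fixed voltage, while incoming conduction is overridden to return zero.
; Tick consumes energy, drives emissive strength on a dynamic material from the charge ratio, and plays pitch-scaled audio while energy remains.
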(event `self.ReceiveTick`
  (params (DeltaSeconds :type "Float (single-precision)"))
  (`self.SetVisualEffects`)
  (`self.ConsumeEnergyPF`)
  (`self.CE_A_UpdateAudio`))

(event `/Game/FinalProject/Gameplay/Light/ILight.LightHit`
  (params (HitComponent :type "PrimitiveComponent Object Reference") (Energy :type "Float (double-precision)"))
  (`|ExecutionSequence`
    (:`then_0`
      (`self.ChargeEnergy` Energy)
      (`self.ConductEnergyToTargets` (`self.Targets`) Energy 10))))

(event `CE_A_UpdateAudio`
  (bind _audio (`self.Audio`))
  (if (> (`self.Energy`) 0.0)
    (if (`AudioComponent.IsPlaying` _audio)
      (`AudioComponent.SetPitchMultiplier` _audio (`self.GetEnergyPercentage`))
      (`AudioComponent.SetPitchMultiplier` _audio (`self.GetEnergyPercentage`))
      (else
        (`AudioComponent.Play` _audio 0.0)))
    (else
      (`AudioComponent.Stop` _audio))))

(fn `Conduct`
  (params (EnergyIn :type "Float (double-precision)") (Volt :type Integer))
  (returns (Consume :type "Float (double-precision)"))
  (return 0.0))

(fn `SetVisualEffects`
  (`MaterialInstanceDynamic.SetScalarParameterValue` (`self.DynaMat_Light`) "E_Strength" (`KismetMathLibrary.SelectFloat` (/ (`self.Energy`) (`self.EnergyMax`)) 0.0 (> (`self.Energy`) 0.0))))

(fn `UserConstructionScript`
  (bind _sm_lighttoelectric (`self.SM_LightToElectric`))
  (`parent.UserConstructionScript`)
  (`|ExecutionSequence`
    (:`then_0`
      (bind _returnvalue (`PrimitiveComponent.CreateDynamicMaterialInstance` _sm_lighttoelectric 0 (`PrimitiveComponent.GetMaterial` _sm_lighttoelectric 0) "None"))
      (set `self.DynaMat_Light` _returnvalue))
    (:`then_1`
      (`self.SetVisualEffects`))))