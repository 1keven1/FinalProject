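; BP_Debug_Light is a debug light for the electronic gameplay system that glows according to its stored energy.
; Construction runs the parent script, then creates a dynamic material on the Sphere and applies the initial glow.
; Each Tick sets emissive strength from the Energy to EnergyMax ratio, zero when empty, then calls ConsumeEnergyPF.
; Conduct passes incoming energy to ChargeEnergy and returns its result.
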(event `self.ReceiveTick`
  (params (DeltaSeconds :type "Float (single-precision)"))
  (`self.SetVisualEffects`)
  (`self.ConsumeEnergyPF`))

(fn `Conduct`
  (params (EnergyIn :type "Float (double-precision)"))
  (returns (Consume :type "Float (double-precision)"))
  (bind _deltaenergy (`self.ChargeEnergy` EnergyIn))
  (return _deltaenergy))

(fn `SetVisualEffects`
  (`MaterialInstanceDynamic.SetScalarParameterValue` (`self.DynaMat_Light`) "E_Strength" (* (`KismetMathLibrary.SelectFloat` (/ (`self.Energy`) (`self.EnergyMax`)) 0.0 (> (`self.Energy`) 0.0)) 5.0)))

(fn `UserConstructionScript`
  (bind _sphere (`self.Sphere`))
  (`parent.UserConstructionScript`)
  (`|ExecutionSequence`
    (:`then_0`
      (bind _returnvalue (`PrimitiveComponent.CreateDynamicMaterialInstance` _sphere 0 (`PrimitiveComponent.GetMaterial` _sphere 0) "None"))
      (set `self.DynaMat_Light` _returnvalue))
    (:`then_1`
      (`self.SetVisualEffects`))))