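; Base Blueprint for electronic gameplay objects that store, drain and pass on energy.
; ChargeEnergy fills up to a maximum and returns the amount accepted, while ConsumeEnergyPF drains at a per-second rate scaled by delta time.
; ConductEnergyToTargets sends energy and voltage to each target through a Conduct message and totals what they consume.
; Its own Conduct is a zero-returning stub; helpers report charge ratio and branch on remaining energy.
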(fn `ChargeEnergy`
  (params (EnergyIn :type "Float (double-precision)"))
  (returns (DeltaEnergy :type "Float (double-precision)"))
  (locals (Delta :type "Float (double-precision)"))
  (bind _energy (`self.Energy`))
  (bind _energymax (`self.EnergyMax`))
  (bind _returnvalue (- _energymax _energy))
  (if (< _energy _energymax)
    (set `local.Delta` (`KismetMathLibrary.SelectFloat` (`local.EnergyIn`) _returnvalue (> _returnvalue (`local.EnergyIn`))))
    (set `self.Energy` (`KismetMathLibrary.FMin` (+ (`local.EnergyIn`) (`self.Energy`)) (`self.EnergyMax`)))
    (return (`local.Delta`))
    (else
      (return 0.0))))

(fn `Conduct`
  (params (EnergyIn :type "Float (double-precision)") (Volt :type Integer))
  (returns (Consume :type "Float (double-precision)"))
  (return 0.0))

(fn `ConductEnergyToTargets`
  (params (Targets :type "Array of /Game/FinalProject/Gameplay/Electronic/BP_Electronic_Base Object Reference") (Energy :type "Float (double-precision)") (Volt :type Integer))
  (returns (Consume :type "Float (double-precision)"))
  (locals (TotalConsume :type "Float (double-precision)"))
  (if (`KismetArrayLibrary.Array_IsNotEmpty` Targets)
    (set `local.TotalConsume` 0.0)
    (for _array_element Targets
      (bind _consume (message `/Game/FinalProject/Gameplay/Electronic/IElectronic.Conduct` _array_element Energy Volt))
      (set `local.TotalConsume` (+ _consume (`local.TotalConsume`))))
    (return (`local.TotalConsume`))
    (else
      (return 0.0))))

(fn `ConsumeEnergyPF`
  (bind _energy (`self.Energy`))
  (if (> _energy 0.0)
    (set `self.Energy` (`KismetMathLibrary.FMax` (- _energy (* (`self.EnergyConsumePS`) (`GameplayStatics.GetWorldDeltaSeconds`)))))
    (return)
    (else
      (return))))

(fn `GetEnergyPercentage`
  (returns (ReturnValue :type "Float (double-precision)"))
  (return (`KismetMathLibrary.SelectFloat` (/ (`self.Energy`) (`self.EnergyMax`)) 0.0 (> (`self.Energy`) 0.0))))

(fn `UserConstructionScript`)