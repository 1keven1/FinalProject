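; BP_Electric_Light is an electrical device whose brightness follows its stored energy percentage.
; Construction creates a dynamic material on the Cube's second slot to drive emissive strength.
; Each tick scales point light intensity and the material's E_Strength by that percentage, then calls ConsumeEnergyPF to use energy.
; Conduct passes incoming energy to ChargeEnergy and returns its result.
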(event `self.ReceiveTick`
  (params (DeltaSeconds :type "Float (single-precision)"))
  (`|ExecutionSequence`
    (:`then_0`
      (`LightComponent.SetIntensity` (`self.PointLight`) (* (`self.GetEnergyPercentage`) (`self.LightIntensity`))))
    (:`then_1`
      (`self.SetVisualEffects`)
      (`self.ConsumeEnergyPF`))))

(fn `Conduct`
  (params (EnergyIn :type "Float (double-precision)"))
  (returns (Consume :type "Float (double-precision)"))
  (bind _deltaenergy (`self.ChargeEnergy` EnergyIn))
  (return _deltaenergy))

(fn `SetVisualEffects`
  (`MaterialInstanceDynamic.SetScalarParameterValue` (`self.DynaMat_Light`) "E_Strength" (* (`self.GetEnergyPercentage`) 3.0)))

(fn `UserConstructionScript`
  (bind _cube (`self.Cube`))
  (`parent.UserConstructionScript`)
  (`|ExecutionSequence`
    (:`then_0`
      (bind _returnvalue (`PrimitiveComponent.CreateDynamicMaterialInstance` _cube 1 (`PrimitiveComponent.GetMaterial` _cube 1) "None"))
      (set `self.DynaMat_Light` _returnvalue))
    (:`then_1`
      (`self.SetVisualEffects`))))