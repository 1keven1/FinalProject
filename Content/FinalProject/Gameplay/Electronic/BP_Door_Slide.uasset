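; Electrically powered sliding door that opens while its stored Energy is above a threshold and closes otherwise.
; Conduct charges it, while Tick consumes energy, drives the emissive material strength from the charge ratio and slides the mesh at constant speed with sweep.
; DoOnce gates switch between fading movement audio and open or close end sounds.
; An older timeline-driven movement remains as deprecated, unreachable logic.
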(event `self.ReceiveTick`
  (params (DeltaSeconds :type "Float (single-precision)"))
  (bind _sm_door_slide (`self.SM_Door_Slide`))
  (bind _returnvalue (> (`self.Energy`) 1.0))
  (bind _relativelocation (`SceneComponent.RelativeLocation` _sm_door_slide))
  (bind _returnvalue_2 (`KismetMathLibrary.SelectVector` (`self.OpenPos`) (`self.ClosePos`) (> (`self.Energy`) 1.0)))
  (`|ExecutionSequence`
    (:`then_0`
      (if (!= _relativelocation _returnvalue_2 :`ErrorTolerance` 0.001)
        (`|ExecutionSequence`
          (:`then_0`
            (`SceneComponent.K2_SetRelativeLocation` _sm_door_slide (`KismetMathLibrary.VInterpTo_Constant` _relativelocation _returnvalue_2 (`GameplayStatics.GetWorldDeltaSeconds`) 100.0) true false))
          (:`then_1`
            (`/Engine/EditorBlueprintResources/StandardMacros.DoOnce` false :!label _label
              (:`Completed`
                (`self.CE_A_PlayDoorSound` _returnvalue)
                (goto _label_2 :!via `Reset`)))))
        (else
          (`/Engine/EditorBlueprintResources/StandardMacros.DoOnce` true :!label _label_2
            (:`Completed`
              (`self.CE_A_PlayDoorSound` _returnvalue true)
              (goto _label :!via `Reset`))))))
    (:`then_1`
      (`self.ConsumeEnergyPF`)
      (`self.SetVisualEffects`))))

(event `CE_A_PlayDoorSound`
  (params (Open :type Boolean) (Stop :type Boolean))
  (bind _audio (`self.Audio`))
  (if (not Stop)
    (`AudioComponent.SetSound` _audio (select `bool` Open :`false` (`self.DoorCloseSound`) :`true` (`self.DoorOpenSound`)))
    (`AudioComponent.FadeIn` _audio 0.2 1.0 0.0 "Linear")
    (else
      (`GameplayStatics.PlaySoundAtLocation` (select `bool` Open :`false` (`self.DoorCloseEndSound`) :`true` (`self.DoorOpenEndSound`)) (`SceneComponent.K2_GetComponentLocation` (`self.SM_Door_Slide`)) (struct) 1.0 1.0 0.0 null null null null)
      (`AudioComponent.FadeOut` (`self.Audio`) 0.5 0.0 "Linear"))))

(fn `Conduct`
  (params (EnergyIn :type "Float (double-precision)"))
  (returns (Consume :type "Float (double-precision)"))
  (bind _deltaenergy (`self.ChargeEnergy` EnergyIn))
  (return _deltaenergy))

(fn `SetVisualEffects`
  (`MaterialInstanceDynamic.SetScalarParameterValue` (`self.DynaMat_Light`) "E_Strength" (/ (`self.Energy`) (`self.EnergyMax`))))

(fn `UserConstructionScript`
  (bind _sm_door_slide (`self.SM_Door_Slide`))
  (bind (_closepos_x _closepos_y _closepos_z) (`KismetMathLibrary.BreakVector` (`self.ClosePos`)))
  (bind _openpos_x (`KismetMathLibrary.BreakVector` (`self.OpenPos`)))
  (`parent.UserConstructionScript`)
  (`|ExecutionSequence`
    (:`then_0`
      (bind _returnvalue (`PrimitiveComponent.CreateDynamicMaterialInstance` _sm_door_slide 1 (`PrimitiveComponent.GetMaterial` _sm_door_slide 1) "None"))
      (set `self.DynaMat_Light` _returnvalue)
      (`self.SetVisualEffects`))
    (:`then_1`
      (set `self.OpenPos` (`KismetMathLibrary.MakeVector` _openpos_x _closepos_y _closepos_z)))
    (:`then_2`
      (`SceneComponent.K2_SetRelativeLocation` (`self.SM_Door_Slide`) (`self.ClosePos`) true false))))