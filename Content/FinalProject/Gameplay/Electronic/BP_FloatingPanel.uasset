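; An electrically powered floating panel that shuttles back and forth along a spline, pausing at each end.
; Conduct charges its energy and Tick consumes it, with energy percentage scaling movement, material glow and audio.
; Overlapping actors attach to the panel unless their interact state is active, and nearby physics bodies are woken as it moves.
; The construction script builds the spline-mesh trail with end caps and attaches an optional actor.
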(event `self.ReceiveBeginPlay`)

(event `self.ReceiveTick`
  (params (DeltaSeconds :type "Float (single-precision)"))
  (`|ExecutionSequence`
    (:`then_0`
      (`self.SetVisualEffects`)
      (`self.ConsumeEnergyPF`)
      (`self.CE_A_UpdateElectric` (`self.GetEnergyPercentage`)))
    (:`then_1`
      (if (> (`self.Energy`) 0.0)
        (set `self.TargetSpeed` (`self.MaxSpeed`))
        (if (> (`self.RemainWaitTime`) 0.0)
          (set `self.RemainWaitTime` (- (`self.RemainWaitTime`) (`GameplayStatics.GetWorldDeltaSeconds`)))
          (`self.CE_A_UpdateStone` false)
          (else
            (bind _output_get (set `self.Speed` (`KismetMathLibrary.FInterpTo_Constant` (`self.Speed`) (`self.TargetSpeed`) (`GameplayStatics.GetWorldDeltaSeconds`) 1.0)))
            (set `self.PanelPos` (`KismetMathLibrary.FInterpTo_Constant` (`self.PanelPos`) (`self.Target`) (`GameplayStatics.GetWorldDeltaSeconds`) (* (`self.GetEnergyPercentage`) _output_get 0.1)))
            (`|ExecutionSequence`
              (:`then_0`
                (if (>= (`self.PanelPos`) 1.0)
                  (set `self.PanelPos` 1.0)
                  (set `self.Target` 0.0)
                  (set `self.RemainWaitTime` (`self.WaitSecond`) :!label _label)
                  (`self.CE_A_UpdateStone` false)
                  (`self.CE_A_Hit` 2.0)))
              (:`then_1`
                (if (<= (`self.PanelPos`) 0.0)
                  (set `self.PanelPos` 0.0)
                  (set `self.Target` 1.0)
                  (goto _label)))
              (:`then_2`
                (`self.SetPanelPos`)
                (`/Game/FinalProject/Gameplay/BPFL_MyFunctionLibrary.WakeAllRidgetBodiesInSphere` (`SceneComponent.K2_GetComponentLocation` (`self.SM_FloatingPanel`)) (* 140.0 (`self.PanelSize`)) (`|MakeArray` "ObjectTypeQuery2" :!type "EObjectTypeQuery Enum"))
                (`self.CE_A_UpdateStone` true (`self.GetEnergyPercentage`))))))
        (else
          (`self.CE_A_UpdateStone` false)
          (set `self.TargetSpeed` 0.0))))))

(event `self.AttachCollision.OnComponentBeginOverlap`
  (params (OverlappedComponent :type "PrimitiveComponent Object Reference") (OtherActor :type "Actor Object Reference") (OtherComp :type "PrimitiveComponent Object Reference") (OtherBodyIndex :type Integer) (bFromSweep :type Boolean) (SweepResult :type "HitResult Structure (by ref)"))
  (if (!= OtherActor self)
    (if (`KismetSystemLibrary.DoesImplementInterface` OtherActor "/Game/FinalProject/Gameplay/Interactive/IInteract.IInteract_C")
      (bind _binteract (message `/Game/FinalProject/Gameplay/Interactive/IInteract.GetInteractState` OtherActor))
      (if (not _binteract)
        (`self.K2_AttachToComponent` OtherActor (`self.SM_FloatingPanel`) "None" "KeepWorld" "KeepWorld" "KeepWorld" true :!label _label_2))
      (else
        (goto _label_2)))))

(event `CE_A_UpdateStone`
  (params (bOn :type Boolean) (Volume :type "Float (double-precision)"))
  (bind _audio_stone (`self.Audio_Stone`))
  (bind _audio_stone_2 (`self.Audio_Stone`))
  (if bOn
    (if (not (`AudioComponent.IsPlaying` _audio_stone))
      (`AudioComponent.FadeIn` _audio_stone_2 0.3 1.0 0.0 "Linear"))
    (`AudioComponent.SetVolumeMultiplier` _audio_stone_2 Volume)
    (else
      (`AudioComponent.FadeOut` _audio_stone 0.3 0.0 "Linear"))))

(event `CE_A_UpdateElectric`
  (params (Multipler :type "Float (double-precision)"))
  (bind _audio_ele (`self.Audio_Ele`))
  (bind _audio_ele_2 (`self.Audio_Ele`))
  (if (> Multipler 0.0)
    (if (not (`AudioComponent.IsPlaying` _audio_ele))
      (`AudioComponent.Play` _audio_ele_2 0.0))
    (`AudioComponent.SetVolumeMultiplier` _audio_ele_2 Multipler)
    (`AudioComponent.SetPitchMultiplier` _audio_ele_2 Multipler)
    (else
      (`AudioComponent.Stop` _audio_ele))))

(event `CE_A_Hit`
  (params (VolumeMultiplier :type "Float (single-precision)" :default 1.0))
  (`GameplayStatics.PlaySoundAtLocation` (`self.AW_Hit`) (`SceneComponent.K2_GetComponentLocation` (`self.Audio_Stone`)) (struct) VolumeMultiplier 1.0 0.0 null null null null))

(fn `Conduct`
  (params (EnergyIn :type "Float (double-precision)") (Volt :type Integer))
  (returns (Consume :type "Float (double-precision)"))
  (bind _deltaenergy (`self.ChargeEnergy` EnergyIn))
  (return _deltaenergy))

(fn `SetPanelPos`
  (bind _spline (`self.Spline`))
  (bind _returnvalue (* (`SplineComponent.GetSplineLength` _spline) (`self.PanelPos`)))
  (`SceneComponent.K2_SetRelativeLocationAndRotation` (`self.SM_FloatingPanel`) (`SplineComponent.GetLocationAtDistanceAlongSpline` _spline _returnvalue "Local") (`SplineComponent.GetRotationAtDistanceAlongSpline` _spline _returnvalue "Local") false false))

(fn `SetVisualEffects`
  (`MaterialInstanceDynamic.SetScalarParameterValue` (`self.DynaMat_Light`) "E_Strength" (`self.GetEnergyPercentage`)))

(fn `UserConstructionScript`
  (bind _sm_floatingpanel (`self.SM_FloatingPanel`))
  (bind _panelsize (`self.PanelSize`))
  (bind _trailendmesh (`self.TrailEndMesh`))
  (bind _dynamat_light (`self.DynaMat_Light`))
  (`parent.UserConstructionScript`)
  (`|ExecutionSequence`
    (:`then_0`
      (bind _returnvalue (`PrimitiveComponent.CreateDynamicMaterialInstance` _sm_floatingpanel 0 (`PrimitiveComponent.GetMaterial` _sm_floatingpanel 0) "None"))
      (set `self.DynaMat_Light` _returnvalue)
      (`self.SetVisualEffects`))
    (:`then_1`
      (`SceneComponent.SetRelativeScale3D` (`self.SM_FloatingPanel`) (`KismetMathLibrary.Conv_DoubleToVector` _panelsize))
      (`SceneComponent.SetRelativeScale3D` (`self.Scene`) (`KismetMathLibrary.Conv_DoubleToVector` (/ 1.0 _panelsize))))
    (:`then_2`
      (`self.SetPanelPos`)
      (`/Engine/EditorBlueprintResources/StandardMacros.IsValid` (`self.AttachingActor`)
        (:`Is Valid`
          (`self.K2_AttachToComponent` (`self.AttachingActor`) (`self.Scene`) "None" "KeepWorld" "KeepWorld" "KeepWorld" true))))
    (:`then_3`
      (bind (_startpos1 _starttangent1 _endpos1 _endtangent1 _headtrans _tailtrans) (`/Game/FinalProject/Gameplay/BPFL_MyFunctionLibrary.GenerateSplineMeshBySpline` (`self.Spline`)))
      (`|ExecutionSequence`
        (:`then_0`
          (for (_array_element _array_index) _startpos1
            (bind _returnvalue_2 (`AddComponent|NODE_AddSplineMeshComponent-0`))
            (`SplineMeshComponent.SetStartAndEnd` _returnvalue_2 _array_element (`|GetArrayItem` _starttangent1 _array_index) (`|GetArrayItem` _endpos1 _array_index) (`|GetArrayItem` _endtangent1 _array_index) true)
            (`StaticMeshComponent.SetStaticMesh` _returnvalue_2 (`self.TrailMesh`))
            (`PrimitiveComponent.SetMaterial` _returnvalue_2 1 (`self.DynaMat_Light`))
            (`PrimitiveComponent.SetCollisionEnabled` _returnvalue_2 "NoCollision")))
        (:`then_1`
          (`|ExecutionSequence`
            (:`then_0`
              (bind _returnvalue_3 (`AddComponent|NODE_AddStaticMeshComponent-0` :`RelativeTransform` (`KismetMathLibrary.MakeTransform` (.location _headtrans) (.rotation _headtrans) (* (.scale _headtrans) (-1.0 1.0 1.0)))))
              (`StaticMeshComponent.SetStaticMesh` _returnvalue_3 _trailendmesh)
              (`PrimitiveComponent.SetCollisionEnabled` _returnvalue_3 "NoCollision")
              (`PrimitiveComponent.SetMaterial` _returnvalue_3 1 _dynamat_light))
            (:`then_1`
              (bind _returnvalue_4 (`AddComponent|NODE_AddStaticMeshComponent-1` :`RelativeTransform` (`KismetMathLibrary.MakeTransform` (.location _tailtrans) (.rotation _tailtrans) (* (.scale _tailtrans) (-1.0 1.0 1.0)))))
              (`StaticMeshComponent.SetStaticMesh` _returnvalue_4 _trailendmesh)
              (`PrimitiveComponent.SetCollisionEnabled` _returnvalue_4 "NoCollision")
              (`PrimitiveComponent.SetMaterial` _returnvalue_4 1 _dynamat_light))))))))