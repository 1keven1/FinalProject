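; BP_Battery is an electronic gameplay actor that acts as an energy source for its target list.
; Every tick it passes its per-second output, scaled by delta time, to ConductEnergyToTargets.
; The construction script runs the parent's, then creates a dynamic material on the battery mesh and switches its emissive strength on or off from Enable.
; Tick itself does not check Enable.
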(event `self.ReceiveTick`
  (params (DeltaSeconds :type "Float (single-precision)"))
  (`self.ConductEnergyToTargets` (`self.Targets`) (* DeltaSeconds (`self.EnergyOutputPS`))))

(fn `UserConstructionScript`
  (bind _sm_battery (`self.SM_Battery`))
  (`parent.UserConstructionScript`)
  (`|ExecutionSequence`
    (:`then_0`
      (bind _returnvalue (`PrimitiveComponent.CreateDynamicMaterialInstance` _sm_battery 2 (`PrimitiveComponent.GetMaterial` _sm_battery 2) "None"))
      (set `self.Dynamic_Light` _returnvalue))
    (:`then_1`
      (`MaterialInstanceDynamic.SetScalarParameterValue` (`self.Dynamic_Light`) "E_Strength" (`KismetMathLibrary.SelectFloat` 1.0 0.0 (`self.bEnable`))))))