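; Electrically powered vertical door that rises in proportion to the voltage it receives through Conduct.
; Each tick converts that frame's charged energy into voltage and a clamped target height, then resets the energy.
; The door rises kinematically with a sweep; when the target drops, it falls under physics, with Box moved to the target, and snaps there after settling.
; A dynamic material progress bar smoothly tracks the voltage ratio.
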(event `self.ReceiveTick`
  (params (DeltaSeconds :type "Float (single-precision)"))
  (bind _sm_door_up (`self.SM_Door_Up`))
  (bind (_relativelocation_x _relativelocation_y _relativelocation_z) (`KismetMathLibrary.BreakVector` (`SceneComponent.RelativeLocation` (`self.SM_Door_Up`))))
  (`|ExecutionSequence`
    (:`then_0`
      ;[0 0 0] 计算出电压 目标高度
      (bind _output_get (set `self.DeltaEnergy` (- (`self.Energy`) (`self.LastEnergy`))))
      (bind _output_get_2 (set `self.Volt` (/ _output_get (`GameplayStatics.GetWorldDeltaSeconds`))))
      (set `self.TargetHeight` (* (`KismetMathLibrary.FClamp` (/ _output_get_2 (`self.MaxVolt`))) (`self.MaxHeight`))))
    (:`then_1`
      (if (>= (`self.TargetHeight`) _relativelocation_z)
        (`PrimitiveComponent.SetSimulatePhysics` (`self.SM_Door_Up`) false)
        (`SceneComponent.K2_SetWorldLocation` (`self.SM_Door_Up`) (+ (`self.K2_GetActorLocation`) (`KismetMathLibrary.MakeVector` 0.0 0.0 (`KismetMathLibrary.FInterpTo_Constant` _relativelocation_z (`self.TargetHeight`) (`GameplayStatics.GetWorldDeltaSeconds`) 100.0))) true false)
        (set `self.bSpeedUp` false)
        (else
          (`PrimitiveComponent.SetSimulatePhysics` (`self.SM_Door_Up`) true)
          (`SceneComponent.K2_SetRelativeLocation` (`self.Box`) (`KismetMathLibrary.MakeVector` 0.0 0.0 (`self.TargetHeight`)) false false)
          (`PrimitiveComponent.WakeAllRigidBodies` _sm_door_up)
          (bind _returnvalue (`PrimitiveComponent.GetPhysicsLinearVelocity` _sm_door_up "None"))
          (`|ExecutionSequence`
            (:`then_0`
              (bind _returnvalue_2 (`KismetMathLibrary.VSize` _returnvalue))
              (if (> _returnvalue_2 10.0)
                (set `self.bSpeedUp` true)))
            (:`then_1`
              (if (and (`self.bSpeedUp`) (< _returnvalue_2 0.1))
                (`PrimitiveComponent.SetSimulatePhysics` (`self.SM_Door_Up`) false)
                (`SceneComponent.K2_SetWorldLocation` (`self.SM_Door_Up`) (+ (`self.K2_GetActorLocation`) (`KismetMathLibrary.MakeVector` 0.0 0.0 (`self.TargetHeight`))) true false)
                (set `self.bSpeedUp` false)))))))
    (:`then_2`
      (set `self.Energy` 0.0)
      (set `self.LastEnergy` (`self.Energy`)))
    (:`then_3`
      (`self.SetVisualEffects`))))

(fn `Conduct`
  (params (EnergyIn :type "Float (double-precision)"))
  (returns (Consume :type "Float (double-precision)"))
  (bind _deltaenergy (`self.ChargeEnergy` EnergyIn))
  (return _deltaenergy))

(fn `SetVisualEffects`
  (bind _dynamat_progressbar (`self.Dynamat_ProgressBar`))
  (bind _returnvalue (`MaterialInstanceDynamic.K2_GetScalarParameterValue` _dynamat_progressbar "Value"))
  (`MaterialInstanceDynamic.SetScalarParameterValue` _dynamat_progressbar "Value" (`KismetMathLibrary.FInterpTo` _returnvalue (/ (`self.Volt`) (`self.MaxVolt`)) (`GameplayStatics.GetWorldDeltaSeconds`) 5.0)))

(fn `UserConstructionScript`
  (bind _sm_door_up (`self.SM_Door_Up`))
  (`parent.UserConstructionScript`)
  (`|ExecutionSequence`
    (:`then_0`
      (bind _returnvalue (`PrimitiveComponent.CreateDynamicMaterialInstance` _sm_door_up 0 (`PrimitiveComponent.GetMaterial` _sm_door_up 0) "None"))
      (set `self.Dynamat_ProgressBar` _returnvalue)
      (`self.SetVisualEffects`))))