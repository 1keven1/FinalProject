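; Electronic capacitor that stores charge received through Conduct and passes it on to its connected targets.
; Each tick it runs ConsumeEnergyPF, then conducts energy at its per-second output rate, scaled by delta time, and subtracts what ConductEnergyToTargets returns.
; A dynamic material bar shows the fill ratio, set at construction and every tick.
; A looping-style audio update plays while charged, with pitch following energy percentage.
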(event `self.ReceiveTick`
  (params (DeltaSeconds :type "Float (single-precision)"))
  (bind _energyoutputps (`self.EnergyOutputPS`))
  (`|ExecutionSequence`
    (:`then_0`
      (`self.SetVisualEffect`)
      (`self.ConsumeEnergyPF`)
      (`self.CE_A_UpdateSound`))
    (:`then_1`
      (if (> (`self.Energy`) 0.0)
        (bind _consume (`self.ConductEnergyToTargets` (`self.Targets`) (* _energyoutputps (`GameplayStatics.GetWorldDeltaSeconds`)) (`KismetMathLibrary.FTrunc` _energyoutputps)))
        (set `self.Energy` (`KismetMathLibrary.FMax` (- (`self.Energy`) _consume)))))))

(event `CE_A_UpdateSound`
  (bind _audio (`self.Audio`))
  (bind _audio_2 (`self.Audio`))
  (if (> (`self.Energy`) 0.0)
    (if (not (`AudioComponent.IsPlaying` _audio))
      (`AudioComponent.Play` _audio_2 0.0))
    (`AudioComponent.SetPitchMultiplier` _audio_2 (* (`self.GetEnergyPercentage`) 1.5))
    (else
      (`AudioComponent.Stop` _audio))))

(fn `Conduct`
  (params (EnergyIn :type "Float (double-precision)") (Volt :type Integer))
  (returns (Consume :type "Float (double-precision)"))
  (bind _deltaenergy (`self.ChargeEnergy` EnergyIn))
  (return _deltaenergy))

(fn `SetVisualEffect`
  (`|ExecutionSequence`
    (:`then_0`
      (`MaterialInstanceDynamic.SetScalarParameterValue` (`self.Dynamat_ProcessBar`) "Value" (/ (`self.Energy`) (`self.EnergyMax`))))))

(fn `UserConstructionScript`
  (bind _sm_capacitor (`self.SM_Capacitor`))
  (`parent.UserConstructionScript`)
  (`|ExecutionSequence`
    (:`then_0`
      (bind _returnvalue (`PrimitiveComponent.CreateDynamicMaterialInstance` _sm_capacitor 2 (`PrimitiveComponent.GetMaterial` _sm_capacitor 2) "None"))
      (set `self.Dynamat_ProcessBar` _returnvalue))
    (:`then_1`
      (set `self.Energy` (`KismetMathLibrary.FClamp` (`self.Energy`) 0.0 (`self.EnergyMax`))))
    (:`then_2`
      (`self.SetVisualEffect`))))