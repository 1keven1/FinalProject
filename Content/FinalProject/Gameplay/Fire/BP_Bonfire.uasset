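; BP_Bonfire is a bonfire actor whose Burn flag sets whether it starts lit.
; The construction script uses Burn to toggle the fire particle and point light, and creates a dynamic coal material on the bonfire mesh.
; When burning, it sets Heat to BurningPoint and drives the coal's emissive intensity from their ratio.
; Its interaction functions are stubs returning default values, and the event graph holds no active logic.
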(fn `ChechCanInteract`
  (params (InteractComponent :type "PrimitiveComponent Object Reference") (Character :type "/Game/FinalProject/Gameplay/Character/BP_MyCharacter Object Reference"))
  (returns (`Return Value` :type Boolean))
  (return false))

(fn `GetInteractInfo`
  (params (InteractComponent :type "PrimitiveComponent Object Reference"))
  (returns (InteractType :type "/Game/FinalProject/Gameplay/Interactive/EInteractType Enum") (NeedHolster :type Boolean) (NeedHold :type Boolean) (TargetPos :type "Vector Structure") (TargetRot :type "Rotator Structure"))
  (return "NewEnumerator0" false false (0.0 0.0 0.0)))

(fn `GetInteractTipUIInfo`
  (params (InteractComponent :type "PrimitiveComponent Object Reference"))
  (returns (WorldPosition :type "Vector Structure") (TipText :type Text))
  (return (0.0 0.0 0.0) ""))

(fn `Interact`
  (params (Character :type "/Game/FinalProject/Gameplay/Character/BP_MyCharacter Object Reference") (InteractComponent :type "PrimitiveComponent Object Reference"))
  (returns (InteractType :type "/Game/FinalProject/Gameplay/Interactive/EInteractType Enum") (TargetActor :type "Actor Object Reference") (InteractAction :type "/Game/FinalProject/Gameplay/Character/EInteractAction Enum"))
  (return "NewEnumerator0" null "NewEnumerator2"))

(fn `Move`
  (params (Value :type "Float (double-precision)"))
  (returns (Velocity :type "Vector Structure"))
  (return (0.0 0.0 0.0)))

(fn `StopInteract`
  (params (Character :type "/Game/FinalProject/Gameplay/Character/BP_MyCharacter Object Reference"))
  (returns (ReturnValue :type Boolean) (InteractAction :type "/Game/FinalProject/Gameplay/Character/EInteractAction Enum"))
  (return false "NewEnumerator2"))

(fn `UserConstructionScript`
  (bind _bburn (`self.bBurn`))
  (bind _p_fire (`self.P_Fire`))
  (bind _sm_bonfire (`self.SM_Bonfire`))
  (`parent.UserConstructionScript`)
  (`|ExecutionSequence`
    (:`then_0`
      (`SceneComponent.SetVisibility` _p_fire _bburn false)
      (`ActorComponent.SetAutoActivate` _p_fire _bburn)
      (`SceneComponent.SetVisibility` (`self.PointLight`) _bburn false))
    (:`then_1`
      (bind _returnvalue (`PrimitiveComponent.CreateDynamicMaterialInstance` _sm_bonfire 1 (`PrimitiveComponent.GetMaterial` _sm_bonfire 1) "None"))
      (set `self.DynaMat_Coal` _returnvalue))
    (:`then_2`
      (if (`self.bBurn`)
        (set `self.Heat` (`self.BurningPoint`))
        (`MaterialInstanceDynamic.SetScalarParameterValue` (`self.DynaMat_Coal`) "E_Intensity" (/ (`self.Heat`) (`self.BurningPoint`)))))))