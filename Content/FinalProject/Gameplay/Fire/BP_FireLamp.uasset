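; A fire lamp that can be lit or extinguished and optionally covered, built on a parent class that supplies heat and burning behavior.
; Construction applies the Covered and Burn options: a covered lamp shows its cover, disables fire collision and cannot conduct heat.
; An uncovered lamp's collision tracks actors in fire range.
; Burn start and stop toggle particles and light, intensity interpolates on Tick, and a dynamic coal material glows with heat percentage.
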(event `self.ReceiveBeginPlay`
  (`parent.ReceiveBeginPlay`)
  (`|ExecutionSequence`
    (:`then_0`
      (`PrimitiveComponent.SetCollisionEnabled` (`self.FireCollision`) (select `bool` (`self.bCovered`) :`false` "QueryOnly" :`true` "NoCollision" :!type "ECollisionEnabled Enum")))))

(event `self.ReceiveTick`
  (params (DeltaSeconds :type "Float (single-precision)"))
  (`parent.ReceiveTick` DeltaSeconds)
  (`self.InterpLightIntensityWhenBurnPF` (`self.PointLight`)))

(event `self.FireCollision.OnComponentBeginOverlap`
  (params (OverlappedComponent :type "PrimitiveComponent Object Reference") (OtherActor :type "Actor Object Reference") (OtherComp :type "PrimitiveComponent Object Reference") (OtherBodyIndex :type Integer) (bFromSweep :type Boolean) (SweepResult :type "HitResult Structure (by ref)"))
  (`KismetArrayLibrary.Array_Add` (`self.ObjInFireRange`) OtherActor))

(event `self.FireCollision.OnComponentEndOverlap`
  (params (OverlappedComponent :type "PrimitiveComponent Object Reference") (OtherActor :type "Actor Object Reference") (OtherComp :type "PrimitiveComponent Object Reference") (OtherBodyIndex :type Integer))
  (`KismetArrayLibrary.Array_RemoveItem` (`self.ObjInFireRange`) OtherActor))

(fn `SetVisualEffects`
  (`MaterialInstanceDynamic.SetScalarParameterValue` (`self.DynaMat_Coal`) "E_Intensity" (`self.GetHeatPercentage`)))

(fn `StartBurn`
  (bind _p_fire (`self.P_Fire`))
  (bind _pointlight (`self.PointLight`))
  (`parent.StartBurn`)
  (`SceneComponent.SetVisibility` _p_fire true false)
  (`ActorComponent.Activate` _p_fire true)
  (`SceneComponent.SetVisibility` _pointlight true false)
  (`LightComponent.SetIntensity` _pointlight 0.0))

(fn `StopBurn`
  (bind _pointlight (`self.PointLight`))
  (`parent.StopBurn`)
  (`ActorComponent.Deactivate` (`self.P_Fire`))
  (`SceneComponent.SetVisibility` _pointlight false false)
  (`LightComponent.SetIntensity` _pointlight 0.0))

(fn `UserConstructionScript`
  (bind _bburn (`self.bBurn`))
  (bind _p_fire (`self.P_Fire`))
  (bind _bcovered (`self.bCovered`))
  (bind _sm_firelamp (`self.SM_FireLamp`))
  (bind _firecollision (`self.FireCollision`))
  (bind _pointlight (`self.PointLight`))
  (`parent.UserConstructionScript`)
  (`|ExecutionSequence`
    (:`then_0`
      (`SceneComponent.SetVisibility` (`self.SM_FireLamp_Cover`) _bcovered true)
      (`PrimitiveComponent.SetCollisionEnabled` _firecollision (select `bool` _bcovered :`false` "QueryOnly" :`true` "NoCollision" :!type "ECollisionEnabled Enum"))
      (`SceneComponent.SetVisibility` _firecollision (not (`self.bCovered`)) false)
      (set `self.bCanConductHeat` (not (`self.bCovered`))))
    (:`then_1`
      (bind _returnvalue (`PrimitiveComponent.CreateDynamicMaterialInstance` _sm_firelamp 1 (`PrimitiveComponent.GetMaterial` _sm_firelamp 1) "None"))
      (set `self.DynaMat_Coal` _returnvalue))
    (:`then_2`
      (`SceneComponent.SetVisibility` _p_fire _bburn false)
      (`ActorComponent.SetAutoActivate` _p_fire _bburn)
      (`SceneComponent.SetVisibility` _pointlight _bburn false)
      (`LightComponent.SetIntensity` _pointlight (`self.LightIntensity`)))
    (:`then_3`
      (if (`self.bBurn`)
        (set `self.Heat` (`self.BurningPoint`))
        (`MaterialInstanceDynamic.SetScalarParameterValue` (`self.DynaMat_Coal`) "E_Intensity" (/ (`self.Heat`) (`self.BurningPoint`)))))))