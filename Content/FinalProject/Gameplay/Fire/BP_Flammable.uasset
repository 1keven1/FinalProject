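; BP_Flammable is a flammable actor that catches fire, burns for a set time, then dissolves away.
; StartBurn activates a fire particle and fires an event that starts the burn timer, while heat conduction defers to the parent class.
; When the timer ends, a timeline drives the dynamic material's Dissolve parameter, then disables collision without destroying the actor.
; FireCollision overlaps maintain the list of actors in fire range.
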(event `self.ReceiveBeginPlay`
  (add `self.OnStartBurn` (delegate `OnStartBurn_Event`))
  (`TimelineComponent.SetPlayRate` (`self.TL_Destroy`) (/ 1.0 (`self.DestroyTime`)))
  (`MaterialInstanceDynamic.SetScalarParameterValue` (`self.Dynamat`) "Dissolve" 0.0))

(event `OnStartBurn_Event`
  (`KismetSystemLibrary.K2_SetTimerDelegate` (delegate `OnBurnOver`) (`self.BurnTime`)))

(event `OnBurnOver`
  (if (`self.bBurn`)
    (`ActorComponent.Deactivate` (`self.FireParticle`))
    (set `self.bBurn` false)
    (bind (_direction _destroy) (`Timeline|TL_Destroy`)
      (:`Update`
        (`MaterialInstanceDynamic.SetScalarParameterValue` (`self.Dynamat`) "Dissolve" _destroy))
      (:`Finished`
        (`self.SetActorEnableCollision` false)))))

(event `/Game/FinalProject/Gameplay/Fire/IFlammable.HeatConduct`
  (params (Heat :type "Float (double-precision)"))
  (`parent.HeatConduct` Heat))

(event `self.FireCollision.OnComponentBeginOverlap`
  (params (OverlappedComponent :type "PrimitiveComponent Object Reference") (OtherActor :type "Actor Object Reference") (OtherComp :type "PrimitiveComponent Object Reference") (OtherBodyIndex :type Integer) (bFromSweep :type Boolean) (SweepResult :type "HitResult Structure (by ref)"))
  (`KismetArrayLibrary.Array_Add` (`self.ObjInFireRange`) OtherActor))

(event `self.FireCollision.OnComponentEndOverlap`
  (params (OverlappedComponent :type "PrimitiveComponent Object Reference") (OtherActor :type "Actor Object Reference") (OtherComp :type "PrimitiveComponent Object Reference") (OtherBodyIndex :type Integer))
  (`KismetArrayLibrary.Array_RemoveItem` (`self.ObjInFireRange`) OtherActor))

(fn `StartBurn`
  (bind _fireparticle (`self.FireParticle`))
  (`parent.StartBurn`)
  (`ActorComponent.Activate` _fireparticle false)
  (`SceneComponent.SetVisibility` _fireparticle true false)
  (`self.OnStartBurn`))

(fn `UserConstructionScript`
  (bind _sm_flammable (`self.SM_Flammable`))
  (bind _bburn (`self.bBurn`))
  (`parent.UserConstructionScript`)
  (`|ExecutionSequence`
    (:`then_0`
      (bind _returnvalue (`PrimitiveComponent.CreateDynamicMaterialInstance` _sm_flammable 0 (`PrimitiveComponent.GetMaterial` _sm_flammable 0) "None"))
      (set `self.Dynamat` _returnvalue))
    (:`then_1`
      (bind _returnvalue_2 (`AddComponent|NODE_AddParticleSystemComponent-0`))
      (`ParticleSystemComponent.SetTemplate` _returnvalue_2 "/Game/FinalProject/TestAsset/P_Fire.P_Fire")
      (bind _output_get (set `self.FireParticle` _returnvalue_2))
      (`ActorComponent.SetAutoActivate` _output_get _bburn)
      (`SceneComponent.SetVisibility` _output_get _bburn false))))