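; BP_Torch is a burnable torch that sits on an optional Shelf and can be picked up by an empty-handed character.
; It snaps to the shelf's attach point, enables interaction only with a valid shelf, and hands itself to the character on an animation notify.
; Burn start and stop toggle fire particles and light, while Heat drives coal glow through a dynamic material.
; A fire collision tracks actors in range.
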(event `self.FireCollision.OnComponentBeginOverlap`
  (params (OverlappedComponent :type "PrimitiveComponent Object Reference") (OtherActor :type "Actor Object Reference") (OtherComp :type "PrimitiveComponent Object Reference") (OtherBodyIndex :type Integer) (bFromSweep :type Boolean) (SweepResult :type "HitResult Structure (by ref)"))
  (`KismetArrayLibrary.Array_Add` (`self.ObjInFireRange`) OtherActor))

(event `self.ReceiveBeginPlay`
  (bind _shelf (`self.Shelf`))
  (bind _interactcolliison (`self.InteractColliison`))
  (`/Engine/EditorBlueprintResources/StandardMacros.IsValid` _shelf
    (:`Is Valid`
      (`PrimitiveComponent.SetCollisionEnabled` _interactcolliison "QueryOnly")
      (`self.K2_AttachToComponent` (`/Game/FinalProject/Gameplay/Fire/BP_TorchShelf.AttachPoint` _shelf) "None" "SnapToTarget" "SnapToTarget" "KeepRelative"))
    (:`Is Not Valid`
      (`PrimitiveComponent.SetCollisionEnabled` _interactcolliison "NoCollision"))))

(event `self.FireCollision.OnComponentEndOverlap`
  (params (OverlappedComponent :type "PrimitiveComponent Object Reference") (OtherActor :type "Actor Object Reference") (OtherComp :type "PrimitiveComponent Object Reference") (OtherBodyIndex :type Integer))
  (`KismetArrayLibrary.Array_RemoveItem` (`self.ObjInFireRange`) OtherActor))

(event `self.ReceiveTick`
  (params (DeltaSeconds :type "Float (single-precision)"))
  (`parent.ReceiveTick` DeltaSeconds)
  (`|ExecutionSequence`
    (:`then_0`
      (`MaterialInstanceDynamic.SetScalarParameterValue` (`self.Dynamat_Coal`) "E_Intensity" (/ (`self.Heat`) (`self.BurningPoint`))))
    (:`then_1`
      (`self.InterpLightIntensityWhenBurnPF` (`self.PointLight`)))))

(event `/Game/FinalProject/Gameplay/Fire/IFlammable.HeatConduct`
  (params (Heat :type "Float (double-precision)"))
  (`parent.HeatConduct` Heat))

(event `/Game/FinalProject/Gameplay/Interactive/IInteract.ProcessAnimationNotify`
  (params (Character :type "/Game/FinalProject/Gameplay/Character/BP_MyCharacter Object Reference") (InteractComp :type "PrimitiveComponent Object Reference"))
  (`/Game/FinalProject/Gameplay/Character/BP_MyCharacter.AddTorch` Character self))

(fn `ChechCanInteract`
  (params (InteractComponent :type "PrimitiveComponent Object Reference") (Character :type "/Game/FinalProject/Gameplay/Character/BP_MyCharacter Object Reference"))
  (returns (`Return Value` :type Boolean))
  (return (not (`KismetSystemLibrary.IsValid` (`/Game/FinalProject/Gameplay/Character/BP_MyCharacter.InHandObj` Character)))))

(fn `GetInteractTipUIInfo`
  (params (InteractComponent :type "PrimitiveComponent Object Reference"))
  (returns (WorldPosition :type "Vector Structure") (TipText :type Text))
  (return (`self.K2_GetActorLocation`) (`self.InteractTip`)))

(fn `GetMoveToInfo`
  (params (InteractComponent :type "PrimitiveComponent Object Reference") (Character :type "/Game/FinalProject/Gameplay/Character/BP_MyCharacter Object Reference"))
  (returns (InteractType :type "/Game/FinalProject/Gameplay/Interactive/EInteractType Enum") (NeedHolster :type Boolean) (NeedHold :type Boolean) (TargetPos :type "Vector Structure") (TargetRot :type "Rotator Structure"))
  (bind (_pos _rot) (`/Game/FinalProject/Gameplay/Fire/BP_TorchShelf.GetInteractPosRot` (`self.Shelf`)))
  (return "NewEnumerator1" false false _pos _rot))

(fn `Interact`
  (params (Character :type "/Game/FinalProject/Gameplay/Character/BP_MyCharacter Object Reference") (InteractComponent :type "PrimitiveComponent Object Reference"))
  (returns (InteractType :type "/Game/FinalProject/Gameplay/Interactive/EInteractType Enum") (TargetActor :type "Actor Object Reference") (InteractAction :type "/Game/FinalProject/Gameplay/Character/EInteractAction Enum"))
  (set `self.OwnCharacter` Character)
  (`PrimitiveComponent.SetCollisionResponseToChannel` (`self.InteractColliison`) "ECC_Pawn" "ECR_Ignore")
  (`PrimitiveComponent.SetCollisionResponseToChannel` (`self.SM_Torch`) "ECC_Pawn" "ECR_Ignore")
  (return "NewEnumerator1" self "NewEnumerator3"))

(fn `Move`
  (params (Character :type "/Game/FinalProject/Gameplay/Character/BP_MyCharacter Object Reference") (Value :type "Float (double-precision)"))
  (returns (Velocity :type "Vector Structure"))
  (return (0.0 0.0 0.0)))

(fn `StartBurn`
  (bind _p_fire (`self.P_Fire`))
  (bind _pointlight (`self.PointLight`))
  (`parent.StartBurn`)
  (`SceneComponent.SetVisibility` _p_fire true false)
  (`ActorComponent.Activate` _p_fire true)
  (`SceneComponent.SetVisibility` _pointlight true false)
  (`LightComponent.SetIntensity` _pointlight 0.0))

(fn `StopBurn`
  (bind _pointlight (`self.PointLight`))
  (`parent.StopBurn`)
  (`ActorComponent.Deactivate` (`self.P_Fire`))
  (`SceneComponent.SetVisibility` _pointlight false false)
  (`LightComponent.SetIntensity` _pointlight 0.0))

(fn `StopInteract`
  (params (Character :type "/Game/FinalProject/Gameplay/Character/BP_MyCharacter Object Reference"))
  (returns (ReturnValue :type Boolean) (InteractAction :type "/Game/FinalProject/Gameplay/Character/EInteractAction Enum"))
  (return false "NewEnumerator2"))

(fn `UserConstructionScript`
  (bind _shelf (`self.Shelf`))
  (bind _p_fire (`self.P_Fire`))
  (bind _bburn (`self.bBurn`))
  (bind _pointlight (`self.PointLight`))
  (bind _coal (`self.Coal`))
  (bind _interactcolliison (`self.InteractColliison`))
  (`parent.UserConstructionScript`)
  (`|ExecutionSequence`
    (:`then_0`
      (`SceneComponent.SetVisibility` _p_fire _bburn false)
      (`ActorComponent.SetAutoActivate` _p_fire _bburn)
      (`SceneComponent.SetVisibility` _pointlight _bburn false)
      (`LightComponent.SetIntensity` _pointlight (`self.LightIntensity`)))
    (:`then_1`
      (bind _returnvalue (`PrimitiveComponent.CreateDynamicMaterialInstance` _coal 0 (`PrimitiveComponent.GetMaterial` _coal 0) "None"))
      (set `self.Dynamat_Coal` _returnvalue))
    (:`then_2`
      (if (`self.bBurn`)
        (set `self.Heat` (`self.BurningPoint`))
        (`MaterialInstanceDynamic.SetScalarParameterValue` (`self.Dynamat_Coal`) "E_Intensity" (/ (`self.Heat`) (`self.BurningPoint`)))))
    (:`then_3`
      (`/Engine/EditorBlueprintResources/StandardMacros.IsValid` _shelf
        (:`Is Valid`
          (`PrimitiveComponent.SetCollisionEnabled` _interactcolliison "QueryOnly")
          (`self.K2_AttachToComponent` (`/Game/FinalProject/Gameplay/Fire/BP_TorchShelf.AttachPoint` _shelf) "None" "SnapToTarget" "SnapToTarget" "KeepRelative"))
        (:`Is Not Valid`
          (`PrimitiveComponent.SetCollisionEnabled` _interactcolliison "NoCollision"))))))