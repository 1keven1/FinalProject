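; Campfire actor built on a heat and burn parent class, which the player can interact with, apparently to sit by, only while it burns.
; While burning it gathers overlapping flammable actors each tick; heat drives coal emissive, and burn start/stop toggles particles and an interpolated light.
; Interaction computes a spot at sit distance facing the fire, rotates the spring arm, and lets pawns through the mesh until stopped or interrupted.
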(event `self.FireColliison.OnComponentBeginOverlap`
  (params (OverlappedComponent :type "PrimitiveComponent Object Reference") (OtherActor :type "Actor Object Reference") (OtherComp :type "PrimitiveComponent Object Reference") (OtherBodyIndex :type Integer) (bFromSweep :type Boolean) (SweepResult :type "HitResult Structure (by ref)")))

(event `self.ReceiveBeginPlay`
  (`parent.ReceiveBeginPlay`))

(event `self.FireColliison.OnComponentEndOverlap`
  (params (OverlappedComponent :type "PrimitiveComponent Object Reference") (OtherActor :type "Actor Object Reference") (OtherComp :type "PrimitiveComponent Object Reference") (OtherBodyIndex :type Integer)))

(event `self.ReceiveTick`
  (params (DeltaSeconds :type "Float (single-precision)"))
  (`|ExecutionSequence`
    (:`then_0`
      (if (`self.bBurn`)
        (set `self.ObjInFireRange` (`PrimitiveComponent.GetOverlappingActors` (`self.FireColliison`) "/Game/FinalProject/Gameplay/Fire/BP_Flammable_Base.BP_Flammable_Base_C"))))
    (:`then_1`
      (`parent.ReceiveTick` DeltaSeconds)
      (`self.SetVisualEffects`)
      (`self.InterpLightIntensityWhenBurnPF` (`self.PointLight`)))))

(event `/Game/FinalProject/Gameplay/Fire/IFlammable.HeatConduct`
  (params (Heat :type "Float (double-precision)"))
  (`parent.HeatConduct` Heat))

(event `/Game/FinalProject/Gameplay/Interactive/IInteract.MoveToInterrupted`
  (params (Character :type "/Game/FinalProject/Gameplay/Character/BP_MyCharacter Object Reference"))
  (`PrimitiveComponent.SetCollisionResponseToChannel` (`self.SM_Bonfire`) "ECC_Pawn" "ECR_Block"))

(fn `ChechCanInteract`
  (params (InteractComponent :type "PrimitiveComponent Object Reference") (Character :type "/Game/FinalProject/Gameplay/Character/BP_MyCharacter Object Reference"))
  (returns (`Return Value` :type Boolean))
  (return (`self.bBurn`)))

(fn `GetInteractState`
  (returns (bInteract :type Boolean))
  (return false))

(fn `GetInteractTipUIInfo`
  (params (InteractComponent :type "PrimitiveComponent Object Reference"))
  (returns (WorldPosition :type "Vector Structure") (TipText :type Text))
  (return (`SceneComponent.K2_GetComponentLocation` (`self.IneractTipPos`)) (`self.InteractTipText`)))

(fn `GetMoveToInfo`
  (params (InteractComponent :type "PrimitiveComponent Object Reference") (Character :type "/Game/FinalProject/Gameplay/Character/BP_MyCharacter Object Reference"))
  (returns (InteractType :type "/Game/FinalProject/Gameplay/Interactive/EInteractType Enum") (NeedHolster :type Boolean) (NeedHold :type Boolean) (TargetPos :type "Vector Structure") (TargetRot :type "Rotator Structure"))
  (bind (_returnvalue_x _returnvalue_y) (`KismetMathLibrary.BreakVector` (`self.K2_GetActorLocation` Character)))
  (bind (_returnvalue_x_2 _returnvalue_y_2) (`KismetMathLibrary.BreakVector` (`self.K2_GetActorLocation`)))
  (bind _returnvalue (`KismetMathLibrary.MakeVector` _returnvalue_x_2 _returnvalue_y_2))
  (bind _returnvalue_2 (`KismetMathLibrary.MakeVector` _returnvalue_x _returnvalue_y))
  (bind _returnvalue_3 (`KismetMathLibrary.FindLookAtRotation` _returnvalue_2 _returnvalue))
  (`PrimitiveComponent.SetCollisionResponseToChannel` (`self.SM_Bonfire`) "ECC_Pawn" "ECR_Ignore")
  (`SceneComponent.K2_SetRelativeRotation` (`self.SpringArm`) _returnvalue_3 false false)
  (return "NewEnumerator3" true false (+ (`self.K2_GetActorLocation`) (* (`KismetMathLibrary.Normal` (- _returnvalue_2 _returnvalue)) (`self.SitDistance`))) _returnvalue_3))

(fn `Interact`
  (params (Character :type "/Game/FinalProject/Gameplay/Character/BP_MyCharacter Object Reference") (InteractComponent :type "PrimitiveComponent Object Reference"))
  (returns (InteractType :type "/Game/FinalProject/Gameplay/Interactive/EInteractType Enum") (TargetActor :type "Actor Object Reference") (InteractAction :type "/Game/FinalProject/Gameplay/Character/EInteractAction Enum"))
  (return "NewEnumerator3" self "NewEnumerator10"))

(fn `Move`
  (params (Character :type "/Game/FinalProject/Gameplay/Character/BP_MyCharacter Object Reference") (Value :type "Float (double-precision)"))
  (returns (Velocity :type "Vector Structure"))
  (return (0.0 0.0 0.0)))

(fn `SetVisualEffects`
  (`MaterialInstanceDynamic.SetScalarParameterValue` (`self.DynaMat_Coal`) "E_Intensity" (`self.GetHeatPercentage`)))

(fn `StartBurn`
  (bind _p_fire (`self.P_Fire`))
  (bind _pointlight (`self.PointLight`))
  (`parent.StartBurn`)
  (`SceneComponent.SetVisibility` _p_fire true false)
  (`ActorComponent.Activate` _p_fire true)
  (`SceneComponent.SetVisibility` _pointlight true false)
  (`LightComponent.SetIntensity` _pointlight 0.0))

(fn `StopBurn`
  (bind _pointlight (`self.PointLight`))
  (`parent.StopBurn`)
  (`ActorComponent.Deactivate` (`self.P_Fire`))
  (`SceneComponent.SetVisibility` _pointlight false false)
  (`LightComponent.SetIntensity` _pointlight 0.0))

(fn `StopInteract`
  (params (Character :type "/Game/FinalProject/Gameplay/Character/BP_MyCharacter Object Reference"))
  (returns (ReturnValue :type Boolean) (InteractAction :type "/Game/FinalProject/Gameplay/Character/EInteractAction Enum"))
  (`PrimitiveComponent.SetCollisionResponseToChannel` (`self.SM_Bonfire`) "ECC_Pawn" "ECR_Block")
  (return true "NewEnumerator11"))

(fn `UserConstructionScript`
  (bind _bburn (`self.bBurn`))
  (bind _p_fire (`self.P_Fire`))
  (bind _sm_bonfire (`self.SM_Bonfire`))
  (bind _pointlight (`self.PointLight`))
  (`parent.UserConstructionScript`)
  (`|ExecutionSequence`
    (:`then_0`
      (`SceneComponent.SetVisibility` _p_fire _bburn false)
      (`ActorComponent.SetAutoActivate` _p_fire _bburn)
      (`SceneComponent.SetVisibility` _pointlight _bburn false)
      (`LightComponent.SetIntensity` _pointlight (`self.LightIntensity`)))
    (:`then_1`
      (bind _returnvalue (`PrimitiveComponent.CreateDynamicMaterialInstance` _sm_bonfire 1 (`PrimitiveComponent.GetMaterial` _sm_bonfire 1) "None"))
      (set `self.DynaMat_Coal` _returnvalue))
    (:`then_2`
      (if (`self.bBurn`)
        (set `self.Heat` (`self.BurningPoint`))
        (`MaterialInstanceDynamic.SetScalarParameterValue` (`self.DynaMat_Coal`) "E_Intensity" (/ (`self.Heat`) (`self.BurningPoint`)))))))