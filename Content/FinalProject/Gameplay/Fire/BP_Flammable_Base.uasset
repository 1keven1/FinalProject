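; Base flammable Blueprint that models fire spreading between objects through accumulated heat.
; While burning, it sends frame-time-scaled heat each tick to objects in its fire range through HeatConduct messages.
; When not burning, it gains received heat, loses it gradually, and ignites at its burning point.
; Start and stop burn functions set the state and call dispatchers; the range list is not populated here.
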(event `self.ReceiveTick`
  (params (DeltaSeconds :type "Float (single-precision)"))
  (`self.ConductHeat`)
  (`self.DissipationHeatPF`))

(event `/Game/FinalProject/Gameplay/Fire/IFlammable.HeatConduct`
  (params (Heat :type "Float (double-precision)"))
  (`self.ReceiveHeat` Heat))

(fn `ConductHeat`
  (if (and (`self.bBurn`) (`KismetArrayLibrary.Array_IsNotEmpty` (`self.ObjInFireRange`)))
    (for _array_element (`self.ObjInFireRange`)
      (message `/Game/FinalProject/Gameplay/Fire/IFlammable.HeatConduct` _array_element (* (`self.HeatOutputPS`) (`GameplayStatics.GetWorldDeltaSeconds`))))
    (else
      (return))))

(fn `DissipationHeatPF`
  (if (and (> (`self.Heat`) 0.0) (not (`self.bBurn`)))
    (set `self.Heat` (`KismetMathLibrary.FMax` (- (`self.Heat`) (* (`self.HeatDissipationPS`) (`GameplayStatics.GetWorldDeltaSeconds`)))))))

(fn `GetBurn`
  (returns (bBurn :type Boolean))
  (return (`self.bBurn`)))

(fn `ReceiveHeat`
  (params (Heat :type "Float (double-precision)"))
  (if (not (`self.bBurn`))
    (bind _output_get (set `self.Heat` (+ Heat (`self.Heat`))))
    (if (>= _output_get (`self.BurningPoint`))
      (`self.StartBurn`)
      (return)
      (else
        (return)))
    (else
      (return))))

(fn `StartBurn`
  (set `self.bBurn` true)
  (set `self.Heat` (`self.BurningPoint`))
  (`self.ED_OnBurn`))

(fn `StopBurn`
  (set `self.bBurn` false)
  (`self.ED_OnStopBurn`))

(fn `UserConstructionScript`)