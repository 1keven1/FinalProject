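; Level-select sandbox actor that displays level widgets on a fadeable sandbox model.
; BeginPlay fills five level widgets from a data table, adds two simple open-level widgets for levels 5 and 6, then starts hidden.
; A timeline fades a shared dynamic material, hiding listed actors after fade-in and restoring them when fade-out begins.
; The saved level number locks later level widgets, and functions expose sandbox and UI opacity.
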(event `self.ReceiveBeginPlay`
  (bind _levelcomponents (`self.LevelComponents`))
  (`|ExecutionSequence`
    (:`then_0`
      (`KismetArrayLibrary.Array_Add` _levelcomponents (`self.Widget_01`))
      (`KismetArrayLibrary.Array_Add` _levelcomponents (`self.Widget_02`))
      (`KismetArrayLibrary.Array_Add` _levelcomponents (`self.Widget_03`))
      (`KismetArrayLibrary.Array_Add` _levelcomponents (`self.Widget_04`))
      (`KismetArrayLibrary.Array_Add` _levelcomponents (`self.Widget_05`))
      (bind _asbp_my_game_mode_base (cast `/Game/FinalProject/Gameplay/BP_MyGameMode_Base` (`GameplayStatics.GetGameMode`)))
      (set `self.MyGameMode` _asbp_my_game_mode_base))
    (:`then_1`
      (for (_array_element _array_index) (`self.LevelComponents`)
        (bind _returnvalue (`|GetDataTableRow` (`self.DT_Level`) (`KismetStringLibrary.Conv_StringToName` (`KismetStringLibrary.Conv_IntToString` _array_index)))
          (:`then`
            (bind (_showname _levelname) (break `/Game/FinalProject/Gameplay/Z_LevelManage/SLevelData` _returnvalue))
            (bind _returnvalue_2 (`|CreateWidget` "/Game/FinalProject/Gameplay/UI/Start/WBP_Level.WBP_Level_C" null (`self.MyGameMode`) _showname _levelname false _array_index))
            (`WidgetComponent.SetWidget` _array_element _returnvalue_2)
            (`KismetArrayLibrary.Array_Add` (`self.WBPLevels`) _returnvalue_2)
            (`/Game/FinalProject/Gameplay/UI/Start/WBP_Level.CE_Refresh` _returnvalue_2)))))
    (:`then_2`
      (bind _returnvalue_3 (`|CreateWidget` "/Game/FinalProject/Gameplay/UI/Start/WBP_OpenLevelSimple.WBP_OpenLevelSimple_C" null 5))
      (`WidgetComponent.SetWidget` (`self.Widget_yincang1`) _returnvalue_3)
      (bind _returnvalue_4 (`|CreateWidget` "/Game/FinalProject/Gameplay/UI/Start/WBP_OpenLevelSimple.WBP_OpenLevelSimple_C" null 6))
      (`WidgetComponent.SetWidget` (`self.Widget_yincang2`) _returnvalue_4))
    (:`then_3`
      (`self.SetSandBoxVis` false)
      (`self.SetLevelUIOpacity` 0.0))))

(event `CE_LoadLevel`
  (params (GameModeStart :type "/Game/FinalProject/Gameplay/BP_MyGameMode_Start Object Reference"))
  (bind _levelnum (`/Game/FinalProject/Gameplay/BP_MyGameMode_Start.GetLoadLevelNum` GameModeStart))
  (`self.SetLoadLevelNum` _levelnum))

(event `CE_SetVis`
  (params (bVis :type Boolean) (Speed :type "Float (double-precision)" :default 1.0))
  (`TimelineComponent.SetPlayRate` (`self.TL_Vis`) Speed)
  (if bVis
    (`SceneComponent.SetVisibility` (`self.SM_Sandbox`) true false)
    (bind (_direction _opacity) (`Timeline|TL_Vis` :!label _label)
      (:`Update`
        (`MaterialInstanceDynamic.SetScalarParameterValue` (`self.DynaMat`) "Opacity" _opacity))
      (:`Finished`
        (switch `ETimelineDirection` _direction
          (:`Forward`
            (`self.SetHideActorsVis` false))
          (:`Backward`
            (`SceneComponent.SetVisibility` (`self.SM_Sandbox`) false false)))))
    (else
      (`self.SetHideActorsVis` true)
      (goto _label :!via `Reverse`))))

(fn `SetHideActorsVis`
  (params (bVis :type Boolean))
  (for _array_element (`self.HideActors`)
    (`/Engine/EditorBlueprintResources/StandardMacros.IsValid` _array_element
      (:`Is Valid`
        (`self.SetActorHiddenInGame` _array_element (not bVis))))))

(fn `SetLevelUIOpacity`
  (params (Opacity :type "Float (double-precision)"))
  (for _array_element (`self.WBPLevels`)
    (`Widget.SetRenderOpacity` _array_element Opacity)))

(fn `SetLoadLevelNum`
  (params (LevelNum :type Integer))
  (for (_array_element _array_index) (`self.WBPLevels`)
    (`/Game/FinalProject/Gameplay/UI/Start/WBP_Level.SetLocked` _array_element (> _array_index LevelNum))))

(fn `SetSandBoxOpacity`
  (params (Value :type "Float (single-precision)"))
  (`MaterialInstanceDynamic.SetScalarParameterValue` (`self.DynaMat`) "Opacity" Value))

(fn `SetSandBoxVis`
  (params (bVis :type Boolean))
  (`SceneComponent.SetVisibility` (`self.SM_Sandbox`) bVis true))

(fn `UserConstructionScript`
  (bind _sm_sandbox (`self.SM_Sandbox`))
  (`|ExecutionSequence`
    (:`then_0`
      (bind _returnvalue (`PrimitiveComponent.CreateDynamicMaterialInstance` _sm_sandbox 0 (`PrimitiveComponent.GetMaterial` _sm_sandbox 0) "None"))
      (bind _output_get (set `self.DynaMat` _returnvalue))
      (`PrimitiveComponent.SetMaterial` (`self.SM_Temple`) 0 _output_get)
      (`PrimitiveComponent.SetMaterial` (`self.SM_IN`) 0 _output_get))
    (:`then_1`
      (`TimelineComponent.SetPlayRate` (`self.TL_Vis`) (`self.ShowSpeed`)))))