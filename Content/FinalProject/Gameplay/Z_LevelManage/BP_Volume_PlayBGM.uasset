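; BP_Volume_PlayBGM is a level trigger volume that switches the background music when the player character enters it.
; It caches BP_MyGameMode on BeginPlay, then on Box overlap by a BP_MyCharacter calls its PlayBGM with the Music track and a one-second fade-in.
; A PlayOnce flag routes the call through a DoOnce so the track triggers only on the first entry.
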(event `self.ReceiveBeginPlay`
  (bind _asbp_my_game_mode (cast `/Game/FinalProject/Gameplay/BP_MyGameMode` (`GameplayStatics.GetGameMode`)))
  (set `self.MyGameMode` _asbp_my_game_mode))

(event `self.Box.OnComponentBeginOverlap`
  (params (OverlappedComponent :type "PrimitiveComponent Object Reference") (OtherActor :type "Actor Object Reference") (OtherComp :type "PrimitiveComponent Object Reference") (OtherBodyIndex :type Integer) (bFromSweep :type Boolean) (SweepResult :type "HitResult Structure (by ref)"))
  (bind _mygamemode (`self.MyGameMode`))
  (bind _music (`self.Music`))
  (if (== (`GameplayStatics.GetObjectClass` OtherActor) "/Game/FinalProject/Gameplay/Character/BP_MyCharacter.BP_MyCharacter_C")
    (if (`self.bPlayOnce`)
      (`/Engine/EditorBlueprintResources/StandardMacros.DoOnce` false
        (:`Completed`
          (`/Game/FinalProject/Gameplay/BP_MyGameMode.PlayBGM` _mygamemode _music 1.0)))
      (else
        (`/Game/FinalProject/Gameplay/BP_MyGameMode.PlayBGM` _mygamemode _music 1.0)))))

(fn `UserConstructionScript`)