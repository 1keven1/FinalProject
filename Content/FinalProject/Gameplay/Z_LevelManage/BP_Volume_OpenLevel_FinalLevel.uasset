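; BP_Volume_OpenLevel_FinalLevel is a trigger volume that branches to one of two levels depending on whether all treasure is collected.
; When BP_MyCharacter overlaps the box, it asks the game mode's IsFullTreasure and plays the matching level sequence with input disabled and the player hidden.
; When the sequence finishes, the game mode opens the matching level with a camera fade, or a warning prints if the name is None.
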(event `self.ReceiveBeginPlay`
  (bind _asbp_my_game_mode (cast `/Game/FinalProject/Gameplay/BP_MyGameMode` (`GameplayStatics.GetGameMode`)))
  (set `self.MyGameMode` _asbp_my_game_mode))

(event `self.Box.OnComponentBeginOverlap`
  (params (OverlappedComponent :type "PrimitiveComponent Object Reference") (OtherActor :type "Actor Object Reference") (OtherComp :type "PrimitiveComponent Object Reference") (OtherBodyIndex :type Integer) (bFromSweep :type Boolean) (SweepResult :type "HitResult Structure (by ref)"))
  (if (== (`GameplayStatics.GetObjectClass` OtherActor) "/Game/FinalProject/Gameplay/Character/BP_MyCharacter.BP_MyCharacter_C")
    (bind _return (`/Game/FinalProject/Gameplay/BP_MyGameMode.IsFullTreasure` (`self.MyGameMode`)))
    (bind (_outactor _returnvalue) (`LevelSequencePlayer.CreateLevelSequencePlayer` (select `bool` _return :`false` (`self.Seq_NoFullTreasure`) :`true` (`self.Seq_FullTreasure`)) (make `MovieSceneSequencePlaybackSettings` true (struct) 1.0 0.0 false false true true true)))
    (add `MovieSceneSequencePlayer.OnFinished` _returnvalue (delegate `Finish`))))

(event `Finish`
  (bind _returnvalue (select `bool` (stale `self.Box.OnComponentBeginOverlap` _return) :`false` (`self.Level_NoFullTreasure`) :`true` (`self.Level_FullTreasure`)))
  (if (and (!= _returnvalue "None") (!= _returnvalue "None"))
    (`/Game/FinalProject/Gameplay/BP_MyGameMode_Base.OpenLevel` (`self.MyGameMode`) _returnvalue 1.0)
    (else
      (`KismetSystemLibrary.PrintString` "WARNING: 关卡名为空" true true (struct :`R` 1.0 :`G` 0.059893 :`A` 1.0) 5.0))))

(fn `UserConstructionScript`)